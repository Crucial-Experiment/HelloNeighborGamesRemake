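; Atmosphere manager that switches the level between Morning, Day, Evening and Night looks and ambience.
; The construction script finds the scene's sky, light, weather, fog and atmosphere actors; NextStage cycles the time and triggers a refresh.
; Refresh routes through a server event to an all-refresh, applying the current stage's struct to lights, sky, audio and post process.
; Weather toggles by coin flip inside that all-refresh when allowed; fog is never updated.
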(event `Refresh (Server)`
  (`self.Refresh (All)`))

(event `Refresh`
  (`self.Refresh (Server)`))

(event `Refresh (All)`
  (bind _audio (`self.Audio`))
  (`|ExecutionSequence`
    (:`then_0`
      (`self.Update Directional Light`)
      (`self.Update Sky Sphere`))
    (:`then_1`
      (`self.Update Sky Light`))
    (:`then_2`
      (`self.Update Weather`))
    (:`then_3`
      (`AudioComponent.SetSound` _audio (`.Ambience Cue` (`self.Get Structure`)))
      (`AudioComponent.Play` _audio 0.0))
    (:`then_4`
      (`self.Update Sky Atmosphere`))
    (:`then_5`
      (`self.Update Post Process`))))

(event `self.ReceiveBeginPlay`
  (`self.Refresh`))

(fn `Next Stage`
  (returns (`Current Time` :type "/Game/Function/Time_Enum Enum"))
  (bind _result (`/Engine/EditorBlueprintResources/StandardMacros.IncrementInt` (`KismetMathLibrary.Conv_ByteToInt` (`self.Current Time`)))
    (:`  `
      (set `self.Current Time` (cast `/Game/Function/Time_Enum` (`KismetMathLibrary.Conv_IntToByte` (mod _result 4))))
      (`self.Refresh`)
      (return (`self.Current Time`)))))

(fn `UserConstructionScript`
  (`|ExecutionSequence`
    (:`then_0`
      (bind _returnvalue (`GameplayStatics.GetActorOfClass` "/Engine/EngineSky/BP_Sky_Sphere.BP_Sky_Sphere_C"))
      (set `self.Sky Sphere` _returnvalue))
    (:`then_1`
      (bind _returnvalue_2 (`GameplayStatics.GetActorOfClass` "/Script/Engine.DirectionalLight"))
      (set `self.Directional Light` _returnvalue_2))
    (:`then_2`
      (bind _returnvalue_3 (`GameplayStatics.GetActorOfClass` "/Script/Engine.SkyLight"))
      (set `self.Sky Light` _returnvalue_3))
    (:`then_3`
      (bind _returnvalue_4 (`GameplayStatics.GetActorOfClass` "/Game/Objects/BP_Objects/BP_Weather.BP_Weather_C"))
      (set `self.Weather` _returnvalue_4))
    (:`then_4`
      (bind _returnvalue_5 (`GameplayStatics.GetActorOfClass` "/Script/Engine.ExponentialHeightFog"))
      (set `self.Exponential Height Fog` _returnvalue_5))
    (:`then_5`
      (bind _returnvalue_6 (`GameplayStatics.GetActorOfClass` "/Script/Engine.SkyAtmosphere"))
      (set `self.Sky Atmosphere` _returnvalue_6))))
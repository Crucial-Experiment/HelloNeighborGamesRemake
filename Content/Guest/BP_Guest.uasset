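; BP_Guest is a guest actor that tracks whether it is on screen and can end the game with a catch sequence.
; Tick sets IsVisible only if the actor is still recently rendered after a short delay, and clears it as soon as it is not.
; The Restart event plays the visitor catch sound, waits, hides the PointLight, then restarts the game through the game mode.
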(event `self.ReceiveTick`
  (params (DeltaSeconds :type "Float (single-precision)"))
  (bind _returnvalue (`self.WasRecentlyRendered` 0.2))
  (if _returnvalue
    (`KismetSystemLibrary.Delay` 0.15)
    (if _returnvalue
      (set `self.Is Visible` _returnvalue))
    (else
      (set `self.Is Visible` false))))

(event `Restart`
  (`GameplayStatics.PlaySound2D` "/Game/Sounds/Guest/S_Visitor_Catch.S_Visitor_Catch" 1.0 1.0 0.0 null null)
  (`KismetSystemLibrary.Delay` 1.0)
  (`SceneComponent.SetVisibility` (`self.PointLight`) false false)
  (`GameMode.RestartGame` (`/Game/Function/BP_FunctionLibrary.Get Game Mode`)))

(fn `UserConstructionScript`)
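; Behavior tree task in which the Neighbor checks under a bed for the player while hunting.
; An EQS query picks from the best 25% of bed candidates, then the Neighbor moves to a random result's check arrow and aligns to it.
; Chained animations play a look under the bed, then a found or not-found reaction based on PlayerIsHere.
; A find triggers the AI controller's catch animation and clears that flag.
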(event `self.ReceiveExecuteAI`
  (params (OwnerController :type "AIController Object Reference") (ControlledPawn :type "Pawn Object Reference"))
  (bind _neighbor (`self.Neighbor`))
  (`parent.ReceiveExecuteAI` OwnerController ControlledPawn)
  (`/Engine/EditorBlueprintResources/StandardMacros.IsValid` _neighbor
    (:`Is Valid`
      (bind _returnvalue (`EnvQueryManager.RunEQSQuery` "/Game/Sosed/Ai/Task/EQuery/EQ_Find_Bed.EQ_Find_Bed" _neighbor "RandomBest25Pct"))
      (add `EnvQueryInstanceBlueprintWrapper.OnQueryFinishedEvent` _returnvalue (delegate `On Finished`)))
    (:`Is Not Valid`
      (`self.Finish`))))

(event `On Finished`
  (params (QueryInstance :type "EnvQueryInstanceBlueprintWrapper Object Reference") (QueryStatus :type "EEnvQueryStatus Enum" :default "Processing"))
  (bind _neighbor (`self.Neighbor`))
  (bind _neighbor_2 (`self.Neighbor`))
  (switch `EEnvQueryStatus` QueryStatus
    (:`Success`
      (bind _resultactors (`EnvQueryInstanceBlueprintWrapper.GetQueryResultsAsActors` QueryInstance))
      (bind _asbp_bed (cast `/Game/Objects/BP_Objects/BP_Bed` (`KismetArrayLibrary.Array_Random` _resultactors)))
      (bind _check_arrow (`/Game/Objects/BP_Objects/BP_Bed.Check Arrow` _asbp_bed))
      (bind _returnvalue (`SceneComponent.K2_GetComponentLocation` _check_arrow))
      (`|AIMoveTo` (`self.Neighbor`) _returnvalue null 2.0
        (:`then`
          (`/Game/Sosed/BP_Sosed.Draw Debug Path` (`self.Neighbor`) _returnvalue))
        (:`OnSuccess`
          (`Actor.K2_SetActorRotation` _neighbor (`SceneComponent.K2_GetComponentRotation` _check_arrow) false)
          (bind _play_length (`/Game/Sosed/BP_Sosed.Play Animation` _neighbor (`/Game/Objects/BP_Objects/BP_Bed.Under Start` _asbp_bed) false))
          (`KismetSystemLibrary.Delay` _play_length)
          (if (`/Game/Objects/BP_Objects/BP_Bed.Player Is Here?` _asbp_bed)
            (bind _play_length_2 (`/Game/Sosed/BP_Sosed.Play Animation` _neighbor_2 (`/Game/Objects/BP_Objects/BP_Bed.Under Found` _asbp_bed) false))
            (`KismetSystemLibrary.Delay` _play_length_2)
            (bind _asai_sosed_controller (cast `/Game/Sosed/Ai/AI_Sosed_Controller` (`AIBlueprintHelperLibrary.GetAIController` (`self.Neighbor`))))
            (bind _asbp_player (cast `/Game/Player/BP_Player` (`GameplayStatics.GetPlayerCharacter` 0)))
            (`/Game/Sosed/Ai/AI_Sosed_Controller.Catch Animation` _asai_sosed_controller (make `/Game/Sosed/Ai/Sosed_Ai_Catch_Struct` _asbp_player (`self.Neighbor`) "/Game/Sounds/Music/catch_Cue.catch_Cue"))
            (set `/Game/Objects/BP_Objects/BP_Bed.Player Is Here?` false _asbp_bed)
            (`self.Finish`)
            (else
              (bind _play_length_3 (`/Game/Sosed/BP_Sosed.Play Animation` _neighbor_2 (`/Game/Objects/BP_Objects/BP_Bed.Under Not Found` _asbp_bed) false))
              (`KismetSystemLibrary.Delay` _play_length_3)
              (`self.Finish`))))
        (:`OnFail`
          (`self.Finish`))))
    (:`Failed`
      (`self.Finish`))))
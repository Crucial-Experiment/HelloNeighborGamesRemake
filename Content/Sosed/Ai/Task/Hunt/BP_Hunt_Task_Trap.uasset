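; Behavior tree task for the Neighbor's hunt AI that sends him to a nearby spot to set a trap.
; It picks a random navigable point around him, moves there with a debug path drawn, then plays the trap reload animation and spawns the trap at his trap point.
; Timed delays step the trap through states with collision off, then restore walking and trap collision before finishing.
; A failed move or invalid Neighbor finishes immediately.
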(event `self.ReceiveExecuteAI`
  (params (OwnerController :type "AIController Object Reference") (ControlledPawn :type "Pawn Object Reference"))
  (bind _neighbor (`self.Neighbor`))
  (bind _neighbor_2 (`self.Neighbor`))
  (bind _neighbor_3 (`self.Neighbor`))
  (`parent.ReceiveExecuteAI` OwnerController ControlledPawn)
  (`/Engine/EditorBlueprintResources/StandardMacros.IsValid` _neighbor_3
    (:`Is Valid`
      (`/Game/Sosed/BP_Sosed.Set Task State` _neighbor_3 "NewEnumerator1")
      (bind _randomlocation (`NavigationSystemV1.K2_GetRandomLocationInNavigableRadius` (`Actor.K2_GetActorLocation` _neighbor_3) 450.0 null "/Script/NavigationSystem.RecastFilter_UseDefaultArea"))
      (`|AIMoveTo` _neighbor _randomlocation null 2.0
        (:`then`
          (`/Game/Sosed/BP_Sosed.Draw Debug Path` (`self.Neighbor`) _randomlocation))
        (:`OnSuccess`
          (`/Game/Sosed/BP_Sosed.Play Animation` _neighbor (`/Game/Sosed/BP_Sosed.Trap Reload` _neighbor) false)
          (bind _returnvalue (`|SpawnActorFromClass` (`/Game/Sosed/BP_Sosed.Trap Class` _neighbor_2) (`SceneComponent.K2_GetComponentToWorld` (`/Game/Sosed/BP_Sosed.Trap Point` _neighbor_2)) "Undefined" "MultiplyWithRoot" null null))
          (`/Game/Objects/BP_Objects/BP_Trap.Set State` _returnvalue "NewEnumerator1")
          (`Actor.SetActorEnableCollision` _returnvalue false)
          (`KismetSystemLibrary.Delay` 1.8)
          (`/Game/Objects/BP_Objects/BP_Trap.Set State` _returnvalue "NewEnumerator2")
          (`KismetSystemLibrary.Delay` 2.6)
          (`CharacterMovementComponent.SetMovementMode` (`Character.CharacterMovement` (`self.Neighbor`)) "MOVE_Walking" 0)
          (`Actor.SetActorEnableCollision` _returnvalue true)
          (`self.Finish`))
        (:`OnFail`
          (`self.Finish`))))
    (:`Is Not Valid`
      (`self.Finish`))))
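; Behavior tree hunt task in which the Neighbor sets a water bucket trap on a door.
; An EQS door query picks randomly from the best 5% of results, then filters for bucket-capable doors without locks, chair, StartLook or existing bucket.
; An eligible door gets a spawned bucket, a bucket check, a new rotate state and a full water fill.
; Invalid Neighbor, failed queries and ineligible results just finish the task.
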(event `self.ReceiveExecuteAI`
  (params (OwnerController :type "AIController Object Reference") (ControlledPawn :type "Pawn Object Reference"))
  (bind _neighbor (`self.Neighbor`))
  (`parent.ReceiveExecuteAI` OwnerController ControlledPawn)
  (`/Engine/EditorBlueprintResources/StandardMacros.IsValid` _neighbor
    (:`Is Valid`
      (bind _returnvalue (`EnvQueryManager.RunEQSQuery` "/Game/Sosed/Ai/Task/EQuery/EQ_Find_Door.EQ_Find_Door" _neighbor "RandomBest5Pct"))
      (add `EnvQueryInstanceBlueprintWrapper.OnQueryFinishedEvent` _returnvalue (delegate `On Finished`)))
    (:`Is Not Valid`
      (`self.Finish`))))

(event `On Finished`
  (params (QueryInstance :type "EnvQueryInstanceBlueprintWrapper Object Reference") (QueryStatus :type "EEnvQueryStatus Enum" :default "Processing"))
  (switch `EEnvQueryStatus` QueryStatus
    (:`Success`
      (bind _resultactors (`EnvQueryInstanceBlueprintWrapper.GetQueryResultsAsActors` QueryInstance))
      (for _array_element _resultactors
        (bind _asbp_rotate (cast `/Game/Objects/Structurs/BP_Rotate` _array_element)
          (:`then`
            (if (`/Game/Objects/Structurs/BP_Rotate.Can Place Bucket` _asbp_rotate)
              (if (and (== (`KismetArrayLibrary.Array_Length` (`/Game/Objects/Structurs/BP_Rotate.Locks` _asbp_rotate)) 0) (not (`/Game/Objects/Structurs/BP_Rotate.Auto Lock` _asbp_rotate)) (not (`KismetSystemLibrary.IsValid` (`/Game/Objects/Structurs/BP_Rotate.Chair` _asbp_rotate))) (not (`/Game/Objects/Structurs/BP_Rotate.Start Look` _asbp_rotate)))
                (`/Game/Objects/Structurs/BP_Rotate.Bucket` _asbp_rotate
                  (:`then`
                    (`self.Finish` :!label _label))
                  (:`else`
                    (`KismetSystemLibrary.PrintString` (`KismetSystemLibrary.GetDisplayName` _array_element) true false)
                    (bind (_returnvalue_location _returnvalue_rotation) (`KismetMathLibrary.BreakTransform` (`Actor.GetTransform` _asbp_rotate)))
                    (bind _returnvalue (`|SpawnActorFromClass` (`/Game/Sosed/BP_Sosed.Bucket Class` (`self.Neighbor`)) (`KismetMathLibrary.MakeTransform` _returnvalue_location _returnvalue_rotation) "Undefined" "MultiplyWithRoot" null null))
                    (set `/Game/Objects/Structurs/BP_Rotate.Bucket` _returnvalue _asbp_rotate)
                    (`/Game/Objects/Structurs/BP_Rotate.Check Bucket` _asbp_rotate)
                    (set `/Game/Objects/Structurs/BP_Rotate.Rotate State` "NewEnumerator1" _asbp_rotate)
                    (bind _watercomponent (`/Game/Objects/BP_Objects/BP_Bucket_2.WaterComponent` _returnvalue))
                    (set `/Game/Objects/Structurs/WaterComponent.Fill` 1.0 _watercomponent)
                    (`/Game/Objects/Structurs/WaterComponent.Update Water Box` _watercomponent)
                    (`self.Finish`)))
                (else
                  (goto _label)))
              (else
                (`self.Finish`))))
          (:`CastFailed`
            (goto _label)))))
    (:`Failed`
      (`self.Finish`))))
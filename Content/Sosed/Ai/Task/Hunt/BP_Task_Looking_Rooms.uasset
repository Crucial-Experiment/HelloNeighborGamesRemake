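; Neighbor AI hunt task that searches rooms, favoring the one with the highest PlayerCount.
; An EQS query supplies candidate rooms; the Neighbor walks to the winner, plays a look-around animation, decrements its count and randomly repeats while the count remains nonzero.
; When that peak count is high, a second EQS query picks a nearby door and, if eligible, attaches a spawned chair and switches its nav modifier to low-height.
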(event `self.ReceiveExecuteAI`
  (params (OwnerController :type "AIController Object Reference") (ControlledPawn :type "Pawn Object Reference"))
  (bind _neighbor (`self.Neighbor`))
  (`parent.ReceiveExecuteAI` OwnerController ControlledPawn)
  (`/Engine/EditorBlueprintResources/StandardMacros.IsValid` _neighbor
    (:`Is Valid`
      (bind _returnvalue (`EnvQueryManager.RunEQSQuery` "/Game/Sosed/Ai/Task/EQuery/EQ_Find_Search_Room.EQ_Find_Search_Room" _neighbor "RandomBest25Pct"))
      (add `EnvQueryInstanceBlueprintWrapper.OnQueryFinishedEvent` _returnvalue (delegate `On Finished`)))
    (:`Is Not Valid`
      (`self.Finish`))))

(event `On Finished`
  (params (QueryInstance :type "EnvQueryInstanceBlueprintWrapper Object Reference") (QueryStatus :type "EEnvQueryStatus Enum" :default "Processing"))
  (bind _neighbor (`self.Neighbor`))
  (bind _neighbor_2 (`self.Neighbor`))
  (switch `EEnvQueryStatus` QueryStatus
    (:`Success`
      (bind _resultactors (`EnvQueryInstanceBlueprintWrapper.GetQueryResultsAsActors` QueryInstance))
      (if (!= (`KismetArrayLibrary.Array_Length` _resultactors) 0)
        (for _array_element _resultactors
          (bind _asbp_room (cast `/Game/Sosed/BP_Room` _array_element))
          (bind _playercount (`/Game/Sosed/BP_Room.PlayerCount` _asbp_room))
          (if (> _playercount (`self.Current Room Count`))
            (set `self.Current Room Count` _playercount)))
        (for _array_element_2 _resultactors
          (bind _asbp_room_2 (cast `/Game/Sosed/BP_Room` _array_element_2))
          (if (== (`/Game/Sosed/BP_Room.PlayerCount` _asbp_room_2) (`self.Current Room Count`))
            (`|ExecutionSequence`
              (:`then_0`
                (bind _returnvalue (`Actor.K2_GetActorLocation` _asbp_room_2))
                (`|AIMoveTo` _neighbor_2 _returnvalue null :!label _label
                  (:`then`
                    (`/Game/Sosed/BP_Sosed.Draw Debug Path` _neighbor_2 _returnvalue))
                  (:`OnSuccess`
                    (bind _play_length (`/Game/Sosed/BP_Sosed.Play Animation` _neighbor (`/Game/Sosed/BP_Sosed.Look Around` _neighbor) false :!label _label_2))
                    (`KismetSystemLibrary.Delay` _play_length)
                    (bind _playercount_2 (`/Game/Sosed/BP_Room.PlayerCount` _asbp_room_2))
                    (`/Engine/EditorBlueprintResources/StandardMacros.DecrementInt` _playercount_2
                      (:`  `
                        (if (and (!= _playercount_2 0) (`KismetMathLibrary.RandomBool`))
                          (goto _label)
                          (elif (>= (`self.Current Room Count`) 10)
                            (bind _returnvalue_2 (`EnvQueryManager.RunEQSQuery` "/Game/Sosed/Ai/Task/EQuery/EQ_Find_Near_Door.EQ_Find_Near_Door" (`self.Neighbor`) "RandomBest5Pct"))
                            (add `EnvQueryInstanceBlueprintWrapper.OnQueryFinishedEvent` _returnvalue_2 (delegate `On Finished 2`))
                            (else
                              (`self.Finish`)))))))
                  (:`OnFail`
                    (goto _label_2))))
              (:`then_1`
                (break)))))
        (else
          (`self.Finish`))))
    (:`Failed`
      (`self.Finish`))))

(event `On Finished 2`
  (params (QueryInstance :type "EnvQueryInstanceBlueprintWrapper Object Reference") (QueryStatus :type "EEnvQueryStatus Enum" :default "Processing"))
  (switch `EEnvQueryStatus` QueryStatus
    (:`Success`
      (bind _resultactors (`EnvQueryInstanceBlueprintWrapper.GetQueryResultsAsActors` QueryInstance))
      (bind _asbp_rotate (cast `/Game/Objects/Structurs/BP_Rotate` (`KismetArrayLibrary.Array_Random` _resultactors)))
      (if (and (== (`KismetArrayLibrary.Array_Length` (`/Game/Objects/Structurs/BP_Rotate.Locks` _asbp_rotate)) 0) (not (`/Game/Objects/Structurs/BP_Rotate.Auto Lock` _asbp_rotate)) (not (`KismetSystemLibrary.IsValid` (`/Game/Objects/Structurs/BP_Rotate.Chair` _asbp_rotate))) (not (`/Game/Objects/Structurs/BP_Rotate.Start Look` _asbp_rotate)) (`/Game/Objects/Structurs/BP_Rotate.Can Place Chair` _asbp_rotate))
        (bind _returnvalue_location (`KismetMathLibrary.BreakTransform` (`Actor.GetTransform` _asbp_rotate)))
        (bind _returnvalue (`|SpawnActorFromClass` "/Game/Objects/BP_Objects/BP_Chair.BP_Chair_C" (`KismetMathLibrary.MakeTransform` _returnvalue_location) "Undefined" "MultiplyWithRoot" null null))
        (set `/Game/Objects/Structurs/BP_Rotate.Chair` _returnvalue _asbp_rotate)
        (set `/Game/Objects/BP_Objects/BP_Chair.Rotate` _asbp_rotate _returnvalue)
        (`/Game/Objects/Structurs/BP_Object.Set Flat Mode` _returnvalue "NewEnumerator1")
        (`Actor.K2_AttachToComponent` _returnvalue (`/Game/Objects/Structurs/BP_Rotate.Scene` _asbp_rotate) "None" "SnapToTarget" "SnapToTarget" "SnapToTarget" true)
        (`NavModifierComponent.SetAreaClass` (`/Game/Objects/Structurs/BP_Rotate.NavModifier` _asbp_rotate) "/Script/NavigationSystem.NavArea_LowHeight")
        (`self.Finish`)
        (else
          (`self.Finish`))))
    (:`Failed`
      (`self.Finish`))))
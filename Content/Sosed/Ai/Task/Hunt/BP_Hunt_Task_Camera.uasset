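; AI hunt task that has the Neighbor set up a camera at a position found by an EQS query.
; The Neighbor moves to a random query result and plays a look-around animation; a failed move skips straight to placement.
; It then spawns a camera holder oriented toward the Neighbor, attaches a new camera to its arrow and plays a metal crunch sound.
; Each placement step draws its own random result location.
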(event `self.ReceiveExecuteAI`
  (params (OwnerController :type "AIController Object Reference") (ControlledPawn :type "Pawn Object Reference"))
  (bind _neighbor (`self.Neighbor`))
  (`parent.ReceiveExecuteAI` OwnerController ControlledPawn)
  (`/Engine/EditorBlueprintResources/StandardMacros.IsValid` _neighbor
    (:`Is Valid`
      (bind _returnvalue (`EnvQueryManager.RunEQSQuery` "/Game/Sosed/Ai/Task/EQuery/EQ_Find_Camera_Position.EQ_Find_Camera_Position" _neighbor "RandomBest25Pct"))
      (add `EnvQueryInstanceBlueprintWrapper.OnQueryFinishedEvent` _returnvalue (delegate `On Finished`)))
    (:`Is Not Valid`
      (`self.Finish`))))

(event `On Finished`
  (params (QueryInstance :type "EnvQueryInstanceBlueprintWrapper Object Reference") (QueryStatus :type "EEnvQueryStatus Enum" :default "Processing"))
  (bind _neighbor (`self.Neighbor`))
  (bind _neighbor_2 (`self.Neighbor`))
  (switch `EEnvQueryStatus` QueryStatus
    (:`Success`
      (bind (_resultlocations _returnvalue) (`EnvQueryInstanceBlueprintWrapper.GetQueryResultsAsLocations` QueryInstance))
      (if _returnvalue
        (bind _returnvalue_2 (- (`KismetArrayLibrary.Array_Random` _resultlocations) (0.0 0.0 20.0)))
        (`|AIMoveTo` _neighbor_2 _returnvalue_2 null 2.0
          (:`OnSuccess`
            (bind _play_length (`/Game/Sosed/BP_Sosed.Play Animation` _neighbor (`/Game/Sosed/BP_Sosed.Look Around` _neighbor) false))
            (`KismetSystemLibrary.Delay` _play_length)
            (`SkeletalMeshComponent.SetAnimationMode` (`Character.Mesh` _neighbor) "AnimationBlueprint" true))
          (:`OnFail`
            _))
        (bind _returnvalue_3 (`KismetMathLibrary.FindLookAtRotation` _returnvalue_2 (`Actor.K2_GetActorLocation` _neighbor_2)))
        (bind _returnvalue_4 (`|SpawnActorFromClass` (`/Game/Sosed/BP_Sosed.Camera Hold Class` (`self.Neighbor`)) (`KismetMathLibrary.MakeTransform` _returnvalue_2 (`KismetMathLibrary.MakeRotator` 0.0 0.0 (- (.yaw _returnvalue_3) 90.0))) "Undefined" "MultiplyWithRoot" null null))
        (bind _arrow (`/Game/Objects/BP_Objects/BP_Camera_Hold.Arrow` _returnvalue_4))
        (`SceneComponent.K2_SetWorldRotation` _arrow _returnvalue_3 false false)
        (bind _returnvalue_5 (`|SpawnActorFromClass` (`/Game/Sosed/BP_Sosed.Camera Class` (`self.Neighbor`)) (`KismetMathLibrary.MakeTransform` _returnvalue_2) "Undefined" "MultiplyWithRoot" null null))
        (`/Game/Objects/Structurs/BP_Object.Set Flat Mode` _returnvalue_5 "NewEnumerator1")
        (`Actor.K2_AttachToComponent` _returnvalue_5 _arrow "None" "SnapToTarget" "SnapToTarget" "SnapToTarget" true)
        (`GameplayStatics.PlaySoundAtLocation` "/Game/Sounds/Objects/Noise/camera_metal_crunch_Cue.camera_metal_crunch_Cue" _returnvalue_2 (struct) 1.0 1.0 0.0 null null null null)
        (set `/Game/Objects/BP_Objects/BP_Camera_Hold.Camera` _returnvalue_5 _returnvalue_4)
        (`self.Finish`)
        (else
          (`self.Finish`))))
    (:`Failed`
      (`self.Finish`))))
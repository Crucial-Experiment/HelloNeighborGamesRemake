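; Neighbor AI task that has the Neighbor fetch a watering can and water a flower pot.
; An EQS query picks a can to walk to and take, and the hand-taken event launches a second query for a pot.
; At the pot it plays the can's watering animation with water active, then returns to the saved pickup location to drop it.
; Failures finish the task, and some drop the can first.
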(event `self.ReceiveExecuteAI`
  (params (OwnerController :type "AIController Object Reference") (ControlledPawn :type "Pawn Object Reference"))
  (`parent.ReceiveExecuteAI` OwnerController ControlledPawn)
  (bind _returnvalue (`EnvQueryManager.RunEQSQuery` "/Game/Sosed/Ai/Task/EQuery/EQ_Find_Watering_Can.EQ_Find_Watering_Can" (`self.Neighbor`) "RandomBest5Pct"))
  (add `EnvQueryInstanceBlueprintWrapper.OnQueryFinishedEvent` _returnvalue (delegate `On Query Finished`)))

(event `self.Neighbor Hand Actor Already Have`
  (params (Actor :type "/Game/Objects/Structurs/BP_Object Object Reference"))
  (`self.Finish`))

(event `On Query Finished`
  (params (QueryInstance :type "EnvQueryInstanceBlueprintWrapper Object Reference") (QueryStatus :type "EEnvQueryStatus Enum" :default "Processing"))
  (bind _neighbor (`self.Neighbor`))
  (switch `EEnvQueryStatus` QueryStatus
    (:`Success`
      (bind _resultactors (`EnvQueryInstanceBlueprintWrapper.GetQueryResultsAsActors` QueryInstance))
      (bind _asbp_watering_can (cast `/Game/Objects/BP_Objects/BP_Watering_Can` (`KismetArrayLibrary.Array_Random` _resultactors))
        (:`then`
          (bind _returnvalue (`SceneComponent.K2_GetComponentLocation` (`/Game/Objects/Structurs/BP_Object.Root` _asbp_watering_can)))
          (set `self.Can Temp Loc` _returnvalue)
          (`|AIMoveTo` (`self.Neighbor`) _returnvalue null 45.0
            (:`then`
              (`/Game/Sosed/BP_Sosed.Draw Debug Path` _neighbor (`SceneComponent.K2_GetComponentLocation` (`/Game/Objects/Structurs/BP_Object.Root` _asbp_watering_can))))
            (:`OnSuccess`
              (`/Game/Sosed/BP_Sosed.Try Take` _neighbor _asbp_watering_can "NewEnumerator1" "wateringCan"))
            (:`OnFail`
              (`self.Finish`))))
        (:`CastFailed`
          (`self.Finish`))))
    (:`Failed`
      (`self.Finish`))))

(event `On Query Finished 2`
  (params (QueryInstance :type "EnvQueryInstanceBlueprintWrapper Object Reference") (QueryStatus :type "EEnvQueryStatus Enum" :default "Processing"))
  (bind _neighbor (`self.Neighbor`))
  (switch `EEnvQueryStatus` QueryStatus
    (:`Success`
      (bind _resultactors (`EnvQueryInstanceBlueprintWrapper.GetQueryResultsAsActors` QueryInstance))
      (bind _asbp_pot (cast `/Game/Objects/BP_Objects/BP_Pot` (`KismetArrayLibrary.Array_Random` _resultactors))
        (:`then`
          (bind _arrow (`/Game/Objects/BP_Objects/BP_Pot.Arrow` _asbp_pot))
          (bind _returnvalue (`SceneComponent.K2_GetComponentLocation` _arrow))
          (`|AIMoveTo` _neighbor _returnvalue null
            (:`then`
              (`/Game/Sosed/BP_Sosed.Draw Debug Path` _neighbor _returnvalue))
            (:`OnSuccess`
              (bind (_returnvalue_roll _returnvalue_pitch _returnvalue_yaw) (`KismetMathLibrary.BreakRotator` (`SceneComponent.K2_GetComponentRotation` _arrow)))
              (`Actor.K2_SetActorRotation` _neighbor (`KismetMathLibrary.MakeRotator` 0.0 0.0 _returnvalue_yaw) false)
              (bind _play_length (`/Game/Sosed/BP_Sosed.Play Animation` _neighbor (`/Game/Objects/BP_Objects/BP_Watering_Can.Watering Flowers` (stale `self.Neighbor Hand Actor Taken` _asbp_watering_can)) true))
              (bind _water (`/Game/Objects/BP_Objects/BP_Watering_Can.Water` (stale `self.Neighbor Hand Actor Taken` _asbp_watering_can)))
              (`ActorComponent.Activate` _water false)
              (`KismetSystemLibrary.Delay` _play_length)
              (`ActorComponent.Deactivate` _water)
              (`SkeletalMeshComponent.SetAnimationMode` (`Character.Mesh` _neighbor) "AnimationBlueprint" true)
              (`|AIMoveTo` (`self.Neighbor`) (`self.Can Temp Loc`) null 35.0
                (:`then`
                  (`/Game/Sosed/BP_Sosed.Draw Debug Path` (`self.Neighbor`) (`self.Can Temp Loc`)))
                (:`OnSuccess`
                  (`/Game/Sosed/BP_Sosed.Try Drop` (`self.Neighbor`) (stale `self.Neighbor Hand Actor Taken` _asbp_watering_can) "NewEnumerator1" null :!label _label)
                  (`self.Finish`))
                (:`OnFail`
                  (goto _label))))
            (:`OnFail`
              (goto _label))))
        (:`CastFailed`
          (goto _label))))
    (:`Failed`
      (`self.Finish`))))

(event `self.Neighbor Hand Actor Taken`
  (params (Actor :type "/Game/Objects/Structurs/BP_Object Object Reference"))
  (bind _asbp_watering_can (cast `/Game/Objects/BP_Objects/BP_Watering_Can` Actor))
  (`Actor.SetActorEnableCollision` _asbp_watering_can false)
  (bind _root (`/Game/Objects/Structurs/BP_Object.Root` _asbp_watering_can))
  (`PrimitiveComponent.SetSimulatePhysics` _root false)
  (`|ExecutionSequence`
    (:`then_0`
      (bind _returnvalue (`EnvQueryManager.RunEQSQuery` "/Game/Sosed/Ai/Task/EQuery/EQ_Find_Pot.EQ_Find_Pot" (`self.Neighbor`) "RandomBest5Pct"))
      (add `EnvQueryInstanceBlueprintWrapper.OnQueryFinishedEvent` _returnvalue (delegate `On Query Finished 2`)))
    (:`then_1`
      (if (== (`GameplayStatics.GetObjectClass` (`KismetArrayLibrary.Array_Random` (stale `On Query Finished` _resultactors))) "/Game/Objects/BP_Objects/BP_Kettle.BP_Kettle_C")
        (`SceneComponent.K2_SetRelativeLocationAndRotation` _root (-8.83281 -3.29493 -12.270365) (struct :`Pitch` 4.261438 :`Yaw` -93.421073 :`Roll` 9.790963) false true)))))
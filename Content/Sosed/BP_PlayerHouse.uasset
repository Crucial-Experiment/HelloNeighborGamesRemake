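; BP_PlayerHouse is a box trigger volume for the player's house that shakes off an attacking Sosed when the player enters.
; Overlap begin and end events toggle PlayerIsHere.
; On entry, if the found Sosed is in Attack, it sets the AI controller's CanSeePlayer to false and empties the blackboard Player key.
; It then switches Sosed to Hunt and randomizes the controller's hunt task.
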(event `self.Box.OnComponentBeginOverlap`
  (params (OverlappedComponent :type "PrimitiveComponent Object Reference") (OtherActor :type "Actor Object Reference") (OtherComp :type "PrimitiveComponent Object Reference") (OtherBodyIndex :type Integer) (bFromSweep :type Boolean) (SweepResult :type "HitResult Structure (by ref)"))
  (cast `/Game/Player/BP_Player` OtherActor)
  (set `self.Player is here?` true)
  (bind _sosed (`/Game/Function/BP_MacroLibrary.Find Sosed`)
    (:`Is Valid`
      (switch `/Game/Sosed/Ai/Struct/Sosed_Stage_Enum` (`/Game/Sosed/BP_Sosed.Current State` _sosed)
        (:`NewEnumerator2`
          (bind _asai_sosed_controller (cast `/Game/Sosed/Ai/AI_Sosed_Controller` (`AIBlueprintHelperLibrary.GetAIController` _sosed)))
          (set `/Game/Sosed/Ai/AI_Sosed_Controller.Can See Player?` false _asai_sosed_controller)
          (`BlackboardComponent.SetValueAsObject` (`AIBlueprintHelperLibrary.GetBlackboard` _asai_sosed_controller) "Player" null)
          (`/Game/Sosed/BP_Sosed.Set State` _sosed "NewEnumerator1")
          (`/Game/Sosed/Ai/AI_Sosed_Controller.Randomize Hunt Task` _asai_sosed_controller))))))

(event `self.Box.OnComponentEndOverlap`
  (params (OverlappedComponent :type "PrimitiveComponent Object Reference") (OtherActor :type "Actor Object Reference") (OtherComp :type "PrimitiveComponent Object Reference") (OtherBodyIndex :type Integer))
  (cast `/Game/Player/BP_Player` OtherActor)
  (set `self.Player is here?` false))

(fn `UserConstructionScript`)
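; BP_Sosed is the AI Neighbor character that hunts, attacks and catches the player.
; SetState syncs Idle/Hunt/Attack/Check to the Blackboard, speed and music; hiding during Attack disables perception and starts bed or cupboard hunt tasks.
; It handles networked catches, thrown tomato/glue/traps, hit reactions and two-handed item pickup.
; Time of day drives the flashlight, holidays swap mesh and props, and mobile lowers run speed.
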(event `On Player Hid (Attack Only)`
  (params (`Call Actor` :type "Actor Object Reference") (`Player Is Here?` :type Boolean))
  (bind _returnvalue (`GameplayStatics.GetObjectClass` `Call Actor`))
  (bind _returnvalue_2 (`AIBlueprintHelperLibrary.GetBlackboard` null))
  ;[1 1 1] On Player Hid
  (if `Player Is Here?`
    (switch `/Game/Sosed/Ai/Struct/Sosed_Stage_Enum` (`self.Current State`)
      (:`NewEnumerator2`
        (bind _asai_sosed_controller (cast `/Game/Sosed/Ai/AI_Sosed_Controller` (`AIBlueprintHelperLibrary.GetAIController` self))
          (:`then`
            (`AIPerceptionComponent.SetSenseEnabled` (`/Game/Sosed/Ai/AI_Sosed_Controller.AIPerception Sight` _asai_sosed_controller) "/Script/AIModule.AISense_Sight" false)
            (`AIPerceptionComponent.SetSenseEnabled` (`/Game/Sosed/Ai/AI_Sosed_Controller.AIPerception Hearing` _asai_sosed_controller) "/Script/AIModule.AISense_Hearing" false))
          (:`CastFailed`
            _))
        (`self.Set State` "NewEnumerator1")
        (`|ExecutionSequence`
          (:`then_0`
            (if (== _returnvalue "/Game/Objects/BP_Objects/BP_Bed.BP_Bed_C")
              (`BlackboardComponent.SetValueAsInt` _returnvalue_2 "HuntTask" 3)))
          (:`then_1`
            (if (== _returnvalue "/Game/Objects/BP_Objects/BP_Cupboard.BP_Cupboard_C")
              (`BlackboardComponent.SetValueAsInt` _returnvalue_2 "HuntTask" 4))))))
    (else
      (`self.Set State` "NewEnumerator2"))))

(event `On Player Catch_Event`
  ;[1 1 1] On Player Hid
  (bind _asai_sosed_controller (cast `/Game/Sosed/Ai/AI_Sosed_Controller` (`AIBlueprintHelperLibrary.GetAIController` self)))
  (`AIPerceptionComponent.SetSenseEnabled` (`/Game/Sosed/Ai/AI_Sosed_Controller.AIPerception Sight` _asai_sosed_controller) "/Script/AIModule.AISense_Sight" true)
  (`AIPerceptionComponent.SetSenseEnabled` (`/Game/Sosed/Ai/AI_Sosed_Controller.AIPerception Hearing` _asai_sosed_controller) "/Script/AIModule.AISense_Hearing" true)
  (`BlackboardComponent.SetValueAsInt` (`AIBlueprintHelperLibrary.GetBlackboard` null) "HuntTask" 0))

(event `self.ReceiveBeginPlay`
  ;[1 1 1] Begin Play
  (bind _returnvalue (`GameplayStatics.GetActorOfClass` "/Game/BP_Atmosphere_And_Time_Manager.BP_Atmosphere_And_Time_Manager_C"))
  (`/Engine/EditorBlueprintResources/StandardMacros.IsValid` _returnvalue
    (:`Is Valid`
      (`self.Check Flashlight` (`/Game/BP_Atmosphere_And_Time_Manager.Current Time` _returnvalue)))
    (:`Is Not Valid`
      _))
  (add `self.On Player Hid` (delegate `On Player Hid (Attack Only)`))
  (add `self.On Player Catch` (delegate `On Player Catch_Event`))
  (`self.Mobile Game`)
  (`self.Check Holiday`))

(event `self.Near Sphere.OnComponentBeginOverlap`
  (params (OverlappedComponent :type "PrimitiveComponent Object Reference") (OtherActor :type "Actor Object Reference") (OtherComp :type "PrimitiveComponent Object Reference") (OtherBodyIndex :type Integer) (bFromSweep :type Boolean) (SweepResult :type "HitResult Structure (by ref)"))
  ;[1 1 1] Player hit the trigger
  (cast `/Game/Player/BP_Player` OtherActor)
  (switch `/Game/Sosed/Ai/Struct/Sosed_Stage_Enum` (`self.Current State`)
    (:`NewEnumerator0`
      (`AudioComponent.Play` (`self.Near Idle`) 0.0 :!label _label))
    (:`NewEnumerator1`
      (`AudioComponent.Play` (`self.Near Hunt`) 0.0))
    (:`NewEnumerator2`
      (`AudioComponent.Stop` (`self.Near Idle`) :!label _label_2)
      (`AudioComponent.Stop` (`self.Near Hunt`)))
    (:`NewEnumerator3`
      (goto _label))))

(event `Catch Player (All)`
  (params (Player :type "/Game/Player/BP_Player Object Reference"))
  ;[1 1 1] Player got caught
  (if (`self.Caught`)
    (bind _asai_sosed_controller (cast `/Game/Sosed/Ai/AI_Sosed_Controller` (`AIBlueprintHelperLibrary.GetAIController` self)))
    (set `self.Caught` false)
    (`/Game/Sosed/Ai/AI_Sosed_Controller.Catch Animation` _asai_sosed_controller (make `/Game/Sosed/Ai/Sosed_Ai_Catch_Struct` Player self "/Game/Sounds/Music/catch_Cue.catch_Cue" true null))
    (`self.Set Task State` "NewEnumerator4")
    (`ForceFeedbackComponent.Play` (`self.ForceFeedback`) 0.0)))

(event `self.Player Catch.OnComponentBeginOverlap`
  (params (OverlappedComponent :type "PrimitiveComponent Object Reference") (OtherActor :type "Actor Object Reference") (OtherComp :type "PrimitiveComponent Object Reference") (OtherBodyIndex :type Integer) (bFromSweep :type Boolean) (SweepResult :type "HitResult Structure (by ref)"))
  ;[1 1 1] Player got caught
  (switch `/Game/Sosed/Ai/Struct/Sosed_State_Enum` (`self.Current Task State`)
    (:`NewEnumerator4`
      _)
    (:`NewEnumerator1`
      _)
    (:`NewEnumerator5`
      _)
    (:`NewEnumerator6`
      _))
  (bind _asbp_player (cast `/Game/Player/BP_Player` OtherActor))
  (`self.Catch Player (Server)` _asbp_player))

(event `self.Near Sphere.OnComponentEndOverlap`
  (params (OverlappedComponent :type "PrimitiveComponent Object Reference") (OtherActor :type "Actor Object Reference") (OtherComp :type "PrimitiveComponent Object Reference") (OtherBodyIndex :type Integer))
  ;[1 1 1] Player hit the trigger
  (cast `/Game/Player/BP_Player` OtherActor)
  (goto _label_2))

(event `Catch Player (Server)`
  (params (Player :type "/Game/Player/BP_Player Object Reference"))
  ;[1 1 1] Player got caught
  (`self.Catch Player (All)` Player))

(event `self.CapsuleComponent.OnComponentHit`
  (params (HitComponent :type "PrimitiveComponent Object Reference") (OtherActor :type "Actor Object Reference") (OtherComp :type "PrimitiveComponent Object Reference") (NormalImpulse :type "Vector Structure") (Hit :type "HitResult Structure (by ref)"))
  (bind _charactermovement (`self.CharacterMovement`))
  ;[1 1 1] Hit
  (if (`|EnumInequality` (`self.Current Task State`) "NewEnumerator0")
    (bind _asbp_object (cast `/Game/Objects/Structurs/BP_Object` OtherActor))
    (if (>= (`KismetMathLibrary.VSize` (`self.GetVelocity` _asbp_object)) 600.0)
      (`CharacterMovementComponent.SetMovementMode` _charactermovement "MOVE_None" 0)
      (bind _play_length (`self.Play Animation` (`self.Hitted`)))
      (`KismetSystemLibrary.Delay` _play_length)
      (`SkeletalMeshComponent.SetAnimationMode` (`self.Mesh`) "AnimationBlueprint" true)
      (if (`|EnumEquality` (`self.Current State`) "NewEnumerator0")
        (bind _play_length_2 (`self.Play Animation` (`self.Look Around`)))
        (`KismetSystemLibrary.Delay` _play_length_2))
      (`CharacterMovementComponent.SetMovementMode` _charactermovement "MOVE_Walking" 0))))

(event `Try Take`
  (params (Actor :type "/Game/Objects/Structurs/BP_Object Object Reference") (Hand :type "/Game/Objects/Enum/HandEnum Enum" :default "NewEnumerator0") (Socket :type Name) (`Custom Take Anim` :type "AnimSequence Object Reference"))
  (bind _returnvalue (`SkeletalMeshComponent.GetAnimInstance` (`self.Mesh`)))
  ;[1 1 1] Try Take and Try Drop
  (`/Engine/EditorBlueprintResources/StandardMacros.IsValid` Actor
    (:`Is Valid`
      (switch `/Game/Objects/Enum/HandEnum` Hand
        (:`NewEnumerator0`
          (bind _holding_left_actor (`self.Holding Left Actor`)
            (:`then`
              (`self.Hand Actor Already Have` _holding_left_actor))
            (:`else`
              (bind _play_length (`self.Play Animation` (select `bool` (`KismetSystemLibrary.IsValid` `Custom Take Anim`) :`false` (`self.Take`) :`true` `Custom Take Anim`) :!label _label_3))
              (`KismetSystemLibrary.Delay` _play_length)
              (`SkeletalMeshComponent.SetAnimationMode` (`self.Mesh`) "AnimationBlueprint" true)
              (`/Game/Objects/Structurs/BP_Object.Set Flat Mode` Actor "NewEnumerator1")
              (`self.SetActorEnableCollision` Actor false)
              (`PrimitiveComponent.SetSimulatePhysics` (`/Game/Objects/Structurs/BP_Object.Root` Actor) false)
              (`self.K2_AttachToComponent` Actor (`self.Mesh`) Socket "SnapToTarget" "SnapToTarget" "SnapToTarget" true)
              (switch `/Game/Objects/Enum/HandEnum` Hand
                (:`NewEnumerator0`
                  (bind _output_get (set `self.Holding Left Actor` Actor))
                  (bind _asbp_anim_sosed (cast `/Game/Sosed/BP_AnimSosed` _returnvalue)
                    (:`then`
                      (set `/Game/Sosed/BP_AnimSosed.LeftHandWeight` 1.0 _asbp_anim_sosed))
                    (:`CastFailed`
                      _))
                  (`self.Hand Actor Taken` _output_get))
                (:`NewEnumerator1`
                  (bind _output_get_2 (set `self.Holding Right Actor` Actor))
                  (bind _asbp_anim_sosed_2 (cast `/Game/Sosed/BP_AnimSosed` _returnvalue)
                    (:`then`
                      (set `/Game/Sosed/BP_AnimSosed.RightHandWeight` 1.0 _asbp_anim_sosed_2))
                    (:`CastFailed`
                      _))
                  (`self.Hand Actor Taken` _output_get_2))))))
        (:`NewEnumerator1`
          (bind _holding_right_actor (`self.Holding Right Actor`)
            (:`then`
              (`self.Hand Actor Already Have` _holding_right_actor))
            (:`else`
              (goto _label_3))))))
    (:`Is Not Valid`
      (`self.Hand Actor Already Have` Actor))))

(event `Try Drop`
  (params (Actor :type "/Game/Objects/Structurs/BP_Object Object Reference") (Hand :type "/Game/Objects/Enum/HandEnum Enum" :default "NewEnumerator0") (Anim :type "AnimSequence Object Reference"))
  (bind _returnvalue (`SkeletalMeshComponent.GetAnimInstance` (`self.Mesh`)))
  ;[1 1 1] Try Take and Try Drop
  (`/Engine/EditorBlueprintResources/StandardMacros.IsValid` Actor
    (:`Is Valid`
      (switch `/Game/Objects/Enum/HandEnum` Hand
        (:`NewEnumerator0`
          (bind _holding_left_actor (`self.Holding Left Actor`)
            (:`then`
              (if (== _holding_left_actor Actor)
                (`/Engine/EditorBlueprintResources/StandardMacros.IsValid` Anim :!label _label_4
                  (:`Is Valid`
                    (bind _play_length (`self.Play Animation` Anim))
                    (`KismetSystemLibrary.Delay` _play_length)
                    (`SkeletalMeshComponent.SetAnimationMode` (`self.Mesh`) "AnimationBlueprint" true))
                  (:`Is Not Valid`
                    _))
                (`self.K2_DetachFromActor` Actor "KeepWorld" "KeepWorld" "KeepWorld")
                (`/Game/Objects/Structurs/BP_Object.Set Flat Mode` Actor "NewEnumerator0")
                (`self.SetActorEnableCollision` Actor true)
                (`PrimitiveComponent.SetSimulatePhysics` (`/Game/Objects/Structurs/BP_Object.Root` Actor) true)
                (switch `/Game/Objects/Enum/HandEnum` Hand
                  (:`NewEnumerator0`
                    (set `self.Holding Left Actor` null)
                    (bind _asbp_anim_sosed (cast `/Game/Sosed/BP_AnimSosed` _returnvalue)
                      (:`then`
                        (set `/Game/Sosed/BP_AnimSosed.LeftHandWeight` 0.0 _asbp_anim_sosed))
                      (:`CastFailed`
                        _)))
                  (:`NewEnumerator1`
                    (set `self.Holding Right Actor` null)
                    (bind _asbp_anim_sosed_2 (cast `/Game/Sosed/BP_AnimSosed` _returnvalue)
                      (:`then`
                        (set `/Game/Sosed/BP_AnimSosed.RightHandWeight` 0.0 _asbp_anim_sosed_2))
                      (:`CastFailed`
                        _))))
                (`self.Hand Actor Dropped` Actor)))
            (:`else`
              (`self.Hand Actor Already Have` _holding_left_actor))))
        (:`NewEnumerator1`
          (bind _holding_right_actor (`self.Holding Right Actor`)
            (:`then`
              (if (== _holding_right_actor Actor)
                (goto _label_4)))
            (:`else`
              (`self.Hand Actor Already Have` _holding_right_actor))))))
    (:`Is Not Valid`
      (`self.Hand Actor Already Have` Actor))))

(event `On Throw Tomato`
  (params (Player :type "/Game/Player/BP_Player Object Reference"))
  ;[1 1 1] On Throw Tomato
  (bind _returnvalue (`|SpawnActorFromClass` (`self.Tomato Class`) (`KismetMathLibrary.MakeTransform` (+ (`self.K2_GetActorLocation`) (* (`self.GetActorForwardVector`) 150.0) (0.0 0.0 50.0))) "Undefined" "MultiplyWithRoot" null null))
  (`KismetSystemLibrary.Delay` 0.02)
  (`/Game/Objects/BP_Objects/BP_Tomato.Throw` _returnvalue Player))

(event `On Throw Glue`
  (params (Player :type "/Game/Player/BP_Player Object Reference"))
  ;[1 1 1] On Throw Glue
  (bind _returnvalue (`|SpawnActorFromClass` (`self.Glue Class`) (`KismetMathLibrary.MakeTransform` (+ (`self.K2_GetActorLocation`) (* (`self.GetActorForwardVector`) 100.0) (0.0 0.0 50.0))) "Undefined" "SelectDefaultAtRuntime" null null))
  (`/Game/Objects/BP_Objects/BP_Glue.Throw` _returnvalue Player))

(event `On Throw Trap`
  (params (Player :type "/Game/Player/BP_Player Object Reference"))
  ;[1 1 1] On Throw Trap
  (bind _returnvalue (`|SpawnActorFromClass` (`self.Trap Class`) (`KismetMathLibrary.MakeTransform` (+ (`self.K2_GetActorLocation`) (* (`self.GetActorForwardVector`) 150.0) (0.0 0.0 50.0))) "Undefined" "MultiplyWithRoot" null null))
  (`KismetSystemLibrary.Delay` 0.02)
  (`/Game/Objects/BP_Objects/BP_Trap.Throw` _returnvalue Player))

(fn `Check Flashlight`
  (params (Time :type "/Game/Function/Time_Enum Enum" :default "NewEnumerator0"))
  (bind _holding_left_actor (`self.Holding Left Actor`))
  (switch `/Game/Function/Time_Enum` Time
    (:`NewEnumerator0`
      (bind _flashlight (`self.Flashlight` :!label _label)
        (:`then`
          (`|ExecutionSequence`
            (:`then_0`
              (`self.K2_AttachToComponent` _flashlight (`self.Mesh`) "Skt_Flashlight" "SnapToTarget" "SnapToTarget" "SnapToTarget" true)
              (`/Game/Objects/Structurs/BP_Object.Set Flat Mode` _flashlight "NewEnumerator1")
              (`self.SetActorEnableCollision` _flashlight false)
              (`/Engine/EditorBlueprintResources/StandardMacros.IsValid` _holding_left_actor
                (:`Is Valid`
                  (if (== _flashlight _holding_left_actor)
                    (set `self.Holding Left Actor` _flashlight :!label _label_2)))
                (:`Is Not Valid`
                  (goto _label_2))))
            (:`then_1`
              (`/Game/Objects/BP_Objects/BP_Flashlight.Neighbor Use` _flashlight "NewEnumerator0"))))
        (:`else`)))
    (:`NewEnumerator1`
      (bind _flashlight_2 (`self.Flashlight` :!label _label_3)
        (:`then`
          (`/Game/Objects/Structurs/BP_Object.Set Flat Mode` _flashlight_2 "NewEnumerator3")
          (if (== (`self.Holding Left Actor`) _flashlight_2)
            (set `self.Holding Left Actor` null)))
        (:`else`)))
    (:`NewEnumerator2`
      (goto _label_3))
    (:`NewEnumerator3`
      (goto _label))))

(fn `Draw Debug Path`
  (params (End :type "Vector Structure"))
  (locals (`End Move` :type "Vector Structure") (`Previous Point` :type "Vector Structure") (PathLength :type "Float (double-precision)"))
  (bind _returnvalue (`KismetMathLibrary.NotEqualExactly_VectorVector` End))
  (bind _previous_point (`local.Previous Point`))
  (bind _returnvalue_2 (`SceneComponent.K2_GetComponentLocation` (`self.Mesh`)))
  (bind _returnvalue_3 (select `bool` _returnvalue :`false` (`local.End Move`) :`true` End))
  (bind _travel_time (`/Game/Function/BP_FunctionLibrary.Calculate Travel Time` _returnvalue_2 _returnvalue_3 self))
  (if (`self.Debug Path`)
    (if _returnvalue
      (set `local.End Move` End))
    (bind _returnvalue_4 (`NavigationSystemV1.FindPathToLocationSynchronously` _returnvalue_2 _returnvalue_3 null "/Script/NavigationSystem.RecastFilter_UseDefaultArea"))
    (for _array_element (`NavigationPath.PathPoints` _returnvalue_4)
      (`KismetSystemLibrary.DrawDebugSphere` _array_element 24.0 12 (struct :`R` 1.0 :`G` 1.0 :`B` 1.0 :`A` 1.0) _travel_time)
      (`KismetSystemLibrary.DrawDebugLine` (select `bool` (`KismetMathLibrary.NotEqualExactly_VectorVector` _previous_point) :`false` (`SceneComponent.K2_GetComponentLocation` (`self.Mesh`)) :`true` _previous_point) _array_element (struct :`R` 1.0 :`G` 1.0 :`B` 1.0 :`A` 1.0) _travel_time)
      (set `local.Previous Point` _array_element))))

(fn `Look To Object`
  (params (Object :type "Actor Object Reference"))
  (`/Engine/EditorBlueprintResources/StandardMacros.IsValid` Object
    (:`Is Valid`
      (bind _output_get (set `self.Head See Object` Object))
      (set `self.Head See Rotation` (`KismetMathLibrary.FindLookAtRotation` (`SceneComponent.GetSocketLocation` (`self.Mesh`) "DEF-head") (`self.K2_GetActorLocation` _output_get))))
    (:`Is Not Valid`
      (set `self.Head See Object` null)
      (set `self.Head See Rotation` (struct)))))

(fn `New Transform`
  (params (Location :type "Vector Structure") (Rotation :type "Rotator Structure"))
  (bind (_returnvalue_x _returnvalue_y _returnvalue_z) (`KismetMathLibrary.BreakVector` (`self.K2_GetActorLocation`)))
  (`self.K2_SetActorLocation` (`KismetMathLibrary.MakeVector` Location_X Location_Y _returnvalue_z))
  (`self.K2_SetActorRotation` (`KismetMathLibrary.MakeRotator` 0.0 0.0 Rotation_Yaw)))

(fn `Play Animation`
  (params (Anim :type "AnimSequence Object Reference") (Loop :type Boolean))
  (returns (`Play Length` :type "Float (double-precision)"))
  (bind _returnvalue (`AnimSequenceBase.GetPlayLength` Anim))
  (for _array_element (`self.Sight Anims`)
    (if (== Anim _array_element)
      (bind _asbp_anim_sosed (cast `/Game/Sosed/BP_AnimSosed` (`SkeletalMeshComponent.GetAnimInstance` (`self.Mesh`)))
        (:`then`
          (set `/Game/Sosed/BP_AnimSosed.Custom Anim` Anim _asbp_anim_sosed)
          (set `/Game/Sosed/BP_AnimSosed.Is Custom Anim` true _asbp_anim_sosed)
          (`/Game/Sosed/BP_AnimSosed.Set Custom Anim Timer` _asbp_anim_sosed _returnvalue))
        (:`CastFailed`
          _))
      (return _returnvalue)))
  (switch `/Game/Sosed/Ai/Struct/Sosed_Stage_Enum` (`self.Current State`)
    (:`NewEnumerator0`
      (`SkeletalMeshComponent.PlayAnimation` (`self.Mesh`) Anim Loop :!label _label)
      (return (`AnimSequenceBase.GetPlayLength` Anim)))
    (:`NewEnumerator1`
      (goto _label))
    (:`NewEnumerator2`
      (for _array_element_2 (`self.Attack Anims`)
        (if (== Anim _array_element_2)
          (`SkeletalMeshComponent.PlayAnimation` (`self.Mesh`) Anim Loop)
          (return (`AnimSequenceBase.GetPlayLength` Anim)))))
    (:`NewEnumerator3`
      (goto _label))))

(fn `Set Game Time`
  (if (`self.Changing Time of Day`)
    (bind _current_time (`/Game/BP_Atmosphere_And_Time_Manager.Next Stage` (`/Game/Function/BP_FunctionLibrary.Get Atmosphere And Time Manager`)))
    (`self.Check Flashlight` _current_time)))

(fn `Set State`
  (params (`New State` :type "/Game/Sosed/Ai/Struct/Sosed_Stage_Enum Enum" :default "NewEnumerator0"))
  (bind _holding_left_actor (`self.Holding Left Actor`))
  (bind _mesh (`self.Mesh`))
  (bind _holding_right_actor (`self.Holding Right Actor`))
  (bind _charactermovement (`self.CharacterMovement`))
  (bind _run_speed (`self.Run Speed`))
  (bind _attack (`self.Attack`))
  (bind _output_get (set `self.Current State` `New State`))
  (`BlackboardComponent.SetValueAsEnum` (`AIBlueprintHelperLibrary.GetBlackboard` self) "State" _output_get)
  (`self.State Mode Change` _output_get)
  (`BlackboardComponent.SetValueAsInt` (`AIBlueprintHelperLibrary.GetBlackboard` null) "AttackTask" 0)
  (`CharacterMovementComponent.SetMovementMode` (`self.CharacterMovement`) "MOVE_Walking" 0)
  (`self.Set Task State` "NewEnumerator4")
  (switch `/Game/Sosed/Ai/Struct/Sosed_Stage_Enum` _output_get
    (:`NewEnumerator0`
      (set `CharacterMovementComponent.MaxWalkSpeed` (`self.Walk Speed`) _charactermovement)
      (`AudioComponent.Stop` _attack)
      (`SkeletalMeshComponent.SetAnimationMode` _mesh "AnimationBlueprint" true :!label _label)
      (bind _asbp_anim_sosed (cast `/Game/Sosed/BP_AnimSosed` (`SkeletalMeshComponent.GetAnimInstance` _mesh)))
      (set `/Game/Sosed/BP_AnimSosed.Is Custom Anim` false _asbp_anim_sosed)
      (set `/Game/Sosed/BP_AnimSosed.Custom Anim` null _asbp_anim_sosed))
    (:`NewEnumerator1`
      (set `CharacterMovementComponent.MaxWalkSpeed` _run_speed _charactermovement)
      (`AudioComponent.Stop` _attack)
      (goto _label))
    (:`NewEnumerator2`
      (set `CharacterMovementComponent.MaxWalkSpeed` _run_speed _charactermovement)
      (`|ExecutionSequence`
        (:`then_0`
          (if (`self.Sound Attack`)
            (`AudioComponent.Play` _attack 0.0)
            (goto _label)
            (else
              (goto _label))))
        (:`then_1`
          ;[0 1 0.8321] Drop All Items (except for flashlight)
          (`|ExecutionSequence`
            (:`then_0`
              (if (!= _holding_right_actor (`self.Flashlight`))
                (`self.Try Drop` _holding_right_actor "NewEnumerator1")))
            (:`then_1`
              (if (!= _holding_left_actor (`self.Flashlight`))
                (`self.Try Drop` _holding_left_actor)))))))
    (:`NewEnumerator3`
      (set `CharacterMovementComponent.MaxWalkSpeed` (`self.Run Speed`) (`self.CharacterMovement`))
      (`AudioComponent.Stop` (`self.Attack`))
      (goto _label))))

(fn `Set Task State`
  (params (`New State` :type "/Game/Sosed/Ai/Struct/Sosed_State_Enum Enum" :default "NewEnumerator4"))
  (set `self.Current Task State` `New State`))

(fn `UserConstructionScript`
  (`self.Set State` (`self.Current State`))
  (`AudioComponent.SetSound` (`self.Attack`) (`self.Sound Attack Music`)))
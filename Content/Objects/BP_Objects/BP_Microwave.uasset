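; BP_Microwave is a microwave object whose door, the Part component, swings open and shut when interacted with.
; A RotateState of Open, Closing, Close or Opening gates Interact, so input during movement is ignored.
; One timeline plays or reverses to lerp the door's relative rotation, then settles the state on finish.
; The open sound plays as movement starts, while the close sound waits until the door has shut.
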(event `/Game/Function/BP_Interface.Interact`
  (params (Component :type "PrimitiveComponent Object Reference") (Location :type "Vector Structure"))
  (if (== Component (`self.Part`))
    (switch `/Game/Objects/Enum/RotateStateEnum` (`self.Rotate State`)
      (:`NewEnumerator0`
        (set `self.Rotate State` "NewEnumerator3")
        (`|ExecutionSequence`
          (:`then_0`
            (bind (_direction _alpha) (`Timeline|Rotate Timeline` :!via `Reverse` :!label _label)
              (:`Update`
                (`SceneComponent.K2_SetRelativeRotation` (`self.Part`) (`KismetMathLibrary.RLerp` (struct) (struct :`Yaw` 100.0) _alpha) false false))
              (:`Finished`
                (switch `/Game/Objects/Enum/RotateStateEnum` (`self.Rotate State`)
                  (:`NewEnumerator2`
                    (set `self.Rotate State` "NewEnumerator0"))
                  (:`NewEnumerator3`
                    (set `self.Rotate State` "NewEnumerator1")
                    (`GameplayStatics.PlaySoundAtLocation` "/Game/Sounds/Objects/OpenClosed/microwave_door_close_Cue.microwave_door_close_Cue" (`self.K2_GetActorLocation`) (struct) 1.0 1.0 0.0 null null null null))))))))
      (:`NewEnumerator1`
        (set `self.Rotate State` "NewEnumerator2")
        (`|ExecutionSequence`
          (:`then_0`
            (goto _label))
          (:`then_1`
            (`GameplayStatics.PlaySoundAtLocation` "/Game/Sounds/Objects/OpenClosed/microwave_open_door_Cue.microwave_open_door_Cue" (`self.K2_GetActorLocation`) (struct) 1.0 1.0 0.0 null null null null)))))))

(fn `UserConstructionScript`)
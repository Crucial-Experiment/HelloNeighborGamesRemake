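; Tube tap object that switches a water stream on or off, gated by a generator or available water, with state sent through server and multicast events.
; A timeline scales the linked Water actor and its boxes to fill or drain depending on Pour, starting or stopping any shark in it.
; While on, Tick fills overlapping WaterComponents and speeds cooling of one captured actor until the tap turns off.
; State changes also report to tutorial and GameJolt components.
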(event `self.ReceiveBeginPlay`
  ;[1 1 1] Tube Tap
  (`parent.ReceiveBeginPlay`)
  (bind _water (`self.Water`)
    (:`then`
      (set `self.Water Scale` (`self.GetActorScale3D` _water)))
    (:`else`)))

(event `Set State (Server)`
  (params (`New State` :type "/Game/Objects/Enum/TumblerStateEnum Enum" :default "NewEnumerator0"))
  ;[1 1 1] Tube Tap
  (`self.Set State (All)` `New State`))

(event `self.Stop Child`
  (bind _pour_ (`self.Pour?`))
  (bind _water_scale (`self.Water Scale`))
  (bind (_water_scale_x _water_scale_y) (`KismetMathLibrary.BreakVector` (`self.Water Scale`)))
  (bind _water (`self.Water`))
  (bind _returnvalue (`KismetMathLibrary.MakeVector` _water_scale_x _water_scale_y))
  (bind _water_box (`/Game/Objects/BP_Objects/BP_Water.Water Box` _water))
  ;[1 1 1] Tube Tap
  (`parent.Stop Child`)
  (`|ExecutionSequence`
    (:`then_0`
      (bind (_direction _alpha) (`Timeline|Шкала времени` :!via `Stop` :!label _label)
        (:`Update`
          (`self.SetActorScale3D` _water (`KismetMathLibrary.VLerp` (select `bool` _pour_ :`false` _water_scale :`true` _returnvalue) (select `bool` _pour_ :`false` _returnvalue :`true` _water_scale) _alpha))
          (`BoxComponent.SetBoxExtent` _water_box (`KismetMathLibrary.VLerp` (select `bool` _pour_ :`false` (32.0 32.0 32.0) :!type "Vector Structure") (select `bool` _pour_ :`true` (32.0 32.0 32.0) :!type "Vector Structure") _alpha) true)
          (`BoxComponent.SetBoxExtent` (`/Game/Objects/BP_Objects/BP_Water.Evaporation Box` _water) (`KismetMathLibrary.VLerp` (select `bool` _pour_ :`false` (32.0 32.0 32.0) :!type "Vector Structure") (select `bool` _pour_ :`true` (32.0 32.0 32.0) :!type "Vector Structure") _alpha) true))
        (:`Finished`
          (`ActorComponent.Deactivate` (`self.Water Drop`) :!label _label_2)
          (`AudioComponent.Stop` (`self.water_move`))
          (if (not (`self.Pour?`))
            (set `PrimitiveComponent.bGenerateOverlapEvents` false (`/Game/Objects/BP_Objects/BP_Water.Evaporation Box` _water))
            (set `PrimitiveComponent.bGenerateOverlapEvents` false _water_box)
            (bind _shark (`/Game/Objects/BP_Objects/BP_Water.Shark` _water)
              (:`then`
                (`/Game/Objects/BP_Objects/BP_Shark.Stop Shark` _shark))
              (:`else`))))))
    (:`then_1`
      (set `PrimitiveComponent.bGenerateOverlapEvents` false (`self.Water Zone`))
      (goto _label_2))))

(event `Set State (All)`
  (params (`New State` :type "/Game/Objects/Enum/TumblerStateEnum Enum" :default "NewEnumerator0"))
  (bind _gamejoltcomponent (`self.GameJoltComponent`))
  (bind _water (`self.Water`))
  (bind _tutorialcomponent (`self.TutorialComponent`))
  (bind _water_zone (`self.Water Zone`))
  (bind _water_drop (`self.Water Drop`))
  (bind _water_2 (`self.Water`))
  ;[1 1 1] Tube Tap
  (switch `/Game/Objects/Enum/TumblerStateEnum` `New State`
    (:`NewEnumerator0`
      (`ActorComponent.Activate` _water_drop false)
      (`/Game/Objects/Tutorial/TutorialComponent.Check Use Type` _tutorialcomponent "NewEnumerator3")
      (`/Game/Objects/GameJolt/GameJoltComponent.Check Use Type` _gamejoltcomponent "NewEnumerator3")
      (set `PrimitiveComponent.bGenerateOverlapEvents` true _water_zone))
    (:`NewEnumerator1`
      (`ActorComponent.Deactivate` _water_drop)
      (`/Game/Objects/Tutorial/TutorialComponent.Check Use Type` _tutorialcomponent "NewEnumerator4")
      (`/Game/Objects/GameJolt/GameJoltComponent.Check Use Type` _gamejoltcomponent "NewEnumerator4")
      (set `PrimitiveComponent.bGenerateOverlapEvents` false _water_zone)))
  (if (`self.Pour?`)
    (set `PrimitiveComponent.bGenerateOverlapEvents` true (`/Game/Objects/BP_Objects/BP_Water.Evaporation Box` _water_2))
    (set `PrimitiveComponent.bGenerateOverlapEvents` true (`/Game/Objects/BP_Objects/BP_Water.Water Box` _water_2))
    (bind _shark (`/Game/Objects/BP_Objects/BP_Water.Shark` _water)
      (:`then`
        (`/Game/Objects/BP_Objects/BP_Shark.Start Shark` _shark _water)
        (goto _label))
      (:`else`
        (goto _label)))
    (else
      (goto _label))))

(event `self.Set State`
  ;[1 1 1] Tube Tap
  (`parent.Set State`)
  (if (and (or (`self.Generator`) (`self.Has Water`)) (`KismetSystemLibrary.IsValid` (`self.Water`)))
    (`self.Set State (Server)` (`self.State`))))

(event `self.Start Child`
  ;[1 1 1] Tube Tap
  (`parent.Start Child`)
  (if (and (or (`self.Generator`) (`self.Has Water`)) (`|EnumEquality` (`self.State`) "NewEnumerator0"))
    (`self.Set State (Server)` "NewEnumerator0")))

(event `self.ReceiveTick`
  (params (DeltaSeconds :type "Float (single-precision)"))
  ;[1 1 1] Water Zone
  (if (`|EnumEquality` (`self.State`) "NewEnumerator0")
    (for _array_element (`PrimitiveComponent.GetOverlappingActors` (`self.Water Zone`) "/Game/Objects/Structurs/BP_Object.BP_Object_C")
      (`|ExecutionSequence`
        (:`then_0`
          (bind _returnvalue (`self.GetComponentByClass` _array_element "/Game/Objects/Structurs/WaterComponent.WaterComponent_C"))
          (`/Engine/EditorBlueprintResources/StandardMacros.IsValid` _returnvalue
            (:`Is Valid`
              (`/Game/Objects/Structurs/WaterComponent.Filling` _returnvalue))))
        (:`then_1`
          (`/Engine/EditorBlueprintResources/StandardMacros.DoOnce` false :!label _label_3
            (:`Completed`
              (`|ExecutionSequence`
                (:`then_0`
                  (bind _output_get (set `self.Actor Temperature` _array_element))
                  (`/Game/Objects/Structurs/WaterComponent.Update Temperature` (`self.WaterComponent`) _output_get true))
                (:`then_1`
                  (goto _label_4 :!via `Reset`))))))))
    (else
      (`|ExecutionSequence`
        (:`then_0`
          (goto _label_3 :!via `Reset`))
        (:`then_1`
          (`/Engine/EditorBlueprintResources/StandardMacros.DoOnce` false :!label _label_4
            (:`Completed`
              (bind _actor_temperature (`self.Actor Temperature`)
                (:`then`
                  (`/Game/Objects/Structurs/WaterComponent.Update Temperature` (`self.WaterComponent`) _actor_temperature false)
                  (set `self.Actor Temperature` null))
                (:`else`)))))))))

(fn `UserConstructionScript`
  (`parent.UserConstructionScript`))
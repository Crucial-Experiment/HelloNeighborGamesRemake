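; BP_Flour_Package is a holdable flour package that scatters flour actors where the player aims, up to a maximum count.
; On left mouse press it checks that the player holds this package, scattering is allowed and the count is below the limit, then runs a short line trace.
; The trace location goes through a server event to a multicast, so each machine spawns BP_Flour, plays a sound and increments its count.
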(event `Spawn Flour (All)`
  (params (Location :type "Vector Structure"))
  (`|SpawnActorFromClass` "/Game/Objects/BP_Objects/BP_Flour.BP_Flour_C" (`KismetMathLibrary.MakeTransform` (+ Location (0.0 0.0 1.0))) "Undefined" "MultiplyWithRoot" null null)
  (`GameplayStatics.PlaySoundAtLocation` "/Game/Sounds/Objects/Noise/insert_glob_Cue.insert_glob_Cue" Location (struct) 1.0 1.0 0.0 null null null null)
  (`/Engine/EditorBlueprintResources/StandardMacros.IncrementInt` (`self.Flour Count`)))

(event `self.On Press LMB`
  (bind _player (`/Game/Function/BP_MacroLibrary.Find Player`)
    (:`Is Valid`
      (bind _item (`/Game/Player/BP_Player.Get Item` _player))
      (if (and (== _item self) (!= (`self.Flour Count`) (`self.Flour Count Max`)) (`self.Can Scatter?`))
        (bind (_actor _component _location) (`self.Line Trace` 250.0))
        (`self.Spawn Flour (Server)` _location)))))

(event `Spawn Flour (Server)`
  (params (Location :type "Vector Structure"))
  (`self.Spawn Flour (All)` Location))

(fn `UserConstructionScript`
  (`parent.UserConstructionScript`))
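; BP_Plate is a breakable plate object that shatters when struck by a fast-moving actor.
; When its root registers a hit, it checks whether the other actor's speed is at least a fixed threshold.
; If so, it spawns DestroyClass at its own transform, passes CrashPlate into that actor's GlassBreak variable, then destroys itself.
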(event `self.Root.OnComponentHit`
  (params (HitComponent :type "PrimitiveComponent Object Reference") (OtherActor :type "Actor Object Reference") (OtherComp :type "PrimitiveComponent Object Reference") (NormalImpulse :type "Vector Structure") (Hit :type "HitResult Structure (by ref)"))
  (`/Engine/EditorBlueprintResources/StandardMacros.IsValid` OtherActor
    (:`Is Valid`
      (if (>= (`KismetMathLibrary.VSize` (`self.GetVelocity` OtherActor)) 200.0)
        (bind _returnvalue (`|SpawnActorFromClass` (`self.Destroy Class`) (`self.GetTransform`) "Undefined" "MultiplyWithRoot" null null))
        (set `/Game/Objects/Destroy/BP_GC_Plate.Glass Break` (`self.Crash Plate`) _returnvalue)
        (`self.K2_DestroyActor`)))))

(fn `UserConstructionScript`
  (`parent.UserConstructionScript`))
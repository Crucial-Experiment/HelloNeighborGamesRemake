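; Switchable generator that players toggle by VR hand overlap or interaction, playing sound and smoke and powering or cutting its linked Electricity objects.
; Any change away from its starting state sends the neighbor AI (Sosed) to check it through blackboard values.
; Toggles report to tutorial and GameJolt components, with visuals multicast in online mode.
; State saves to JSON, and loading replays the interaction when it differs.
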(event `self.Button.OnComponentBeginOverlap`
  (params (OverlappedComponent :type "PrimitiveComponent Object Reference") (OtherActor :type "Actor Object Reference") (OtherComp :type "PrimitiveComponent Object Reference") (OtherBodyIndex :type Integer) (bFromSweep :type Boolean) (SweepResult :type "HitResult Structure (by ref)"))
  (bind _tutorialcomponent (`self.TutorialComponent`))
  (bind _gamejoltcomponent (`self.GameJoltComponent`))
  (bind _state (`self.State`))
  (bind _p_smoke (`self.P_Smoke`))
  (bind _working (`self.working`))
  ;[1 1 1] Interact
  (if (`self.Overlap VR Hands` OtherActor OtherComp)
    (`|ExecutionSequence` :!label _label
      (:`then_0`
        (switch `/Game/Objects/Enum/TumblerStateEnum` _state
          (:`NewEnumerator0`
            (set `self.State` "NewEnumerator1")
            (`AudioComponent.Stop` _working)
            (`ActorComponent.Deactivate` _p_smoke)
            (`/Game/Objects/Tutorial/TutorialComponent.Check Use Type` _tutorialcomponent "NewEnumerator4")
            (`/Game/Objects/GameJolt/GameJoltComponent.Check Use Type` _gamejoltcomponent "NewEnumerator4"))
          (:`NewEnumerator1`
            (set `self.State` "NewEnumerator0")
            (`AudioComponent.Play` _working 0.0)
            (`ActorComponent.Activate` _p_smoke false)
            (`/Game/Objects/Tutorial/TutorialComponent.Check Use Type` _tutorialcomponent "NewEnumerator3")
            (`/Game/Objects/GameJolt/GameJoltComponent.Check Use Type` _gamejoltcomponent "NewEnumerator3")))
        (`self.Tumbler` _state))
      (:`then_1`
        (if (`|EnumInequality` (`self.State`) (`self.Def State`))
          (bind _sosed (`/Game/Function/BP_MacroLibrary.Find Sosed`)
            (:`Is Valid`
              (if (`|EnumInequality` (`/Game/Sosed/BP_Sosed.Current State` _sosed) "NewEnumerator2")
                (bind _returnvalue (`AIBlueprintHelperLibrary.GetBlackboard` _sosed))
                (`BlackboardComponent.SetValueAsInt` _returnvalue "CheckTask" 6)
                (`BlackboardComponent.SetValueAsVector` _returnvalue "Check Location" (`SceneComponent.K2_GetComponentLocation` (`self.Arrow`)))
                (`BlackboardComponent.SetValueAsObject` _returnvalue "Generator" self)
                (`/Game/Sosed/BP_Sosed.Set State` _sosed "NewEnumerator3"))))))
      (:`then_2`
        (if (`/Game/Function/BP_GameInstance.Online Mode` (`/Game/Function/BP_FunctionLibrary.Get Game Instance`))
          (`self.Interact (All)`))))))

(event `Interact (Server)`
  (params (Component :type "PrimitiveComponent Object Reference"))
  ;[1 1 1] Interact
  (if (== Component (`self.Button`))
    (goto _label)))

(event `self.ReceiveBeginPlay`
  (bind _state (`self.State`))
  ;[1 1 1] Begin Play
  (`parent.ReceiveBeginPlay`)
  (`self.Set Flat Mode` "NewEnumerator1")
  (`self.Tumbler` _state)
  (set `self.Def State` _state)
  (switch `/Game/Objects/Enum/TumblerStateEnum` _state
    (:`NewEnumerator0`
      (`AudioComponent.Play` (`self.working`) 0.0)
      (`ActorComponent.Activate` (`self.P_Smoke`) false))))

(event `/Game/Function/BP_Interface.Interact`
  (params (Component :type "PrimitiveComponent Object Reference") (Location :type "Vector Structure"))
  ;[1 1 1] Interact
  (`self.Interact (Server)` Component))

(event `Interact (All)`
  (bind _working (`self.working`))
  (bind _p_smoke (`self.P_Smoke`))
  ;[1 1 1] Server Visual
  (switch `/Game/Objects/Enum/TumblerStateEnum` (`self.State`)
    (:`NewEnumerator0`
      (`AudioComponent.Play` _working 0.0)
      (`ActorComponent.Activate` _p_smoke false))
    (:`NewEnumerator1`
      (`AudioComponent.Stop` _working)
      (`ActorComponent.Deactivate` _p_smoke))))

(event `self.Enable`
  ;[1 1 1] Tumbler
  (`parent.Enable`)
  (switch `/Game/Objects/Enum/TumblerStateEnum` (`self.State`) :!label _label_2
    (:`NewEnumerator0`
      (for _array_element (`self.Electricity`)
        (`/Engine/EditorBlueprintResources/StandardMacros.IsValid` _array_element
          (:`Is Valid`
            (`self.Enable` _array_element)))))))

(event `Tumbler`
  (params (State :type "/Game/Objects/Enum/TumblerStateEnum Enum" :default "NewEnumerator0"))
  (bind _generator (`self.Generator`))
  ;[1 1 1] Tumbler
  (if (or (`self.Has Electricity`) _generator)
    (switch `/Game/Objects/Enum/TumblerStateEnum` State
      (:`NewEnumerator0`
        (goto _label_2))
      (:`NewEnumerator1`
        (for _array_element (`self.Electricity`) :!label _label_3
          (`/Engine/EditorBlueprintResources/StandardMacros.IsValid` _array_element
            (:`Is Valid`
              (`self.Disable` _array_element))))))
    (elif (not _generator)
      (goto _label_3))))

(event `self.Disable`
  ;[1 1 1] Tumbler
  (`parent.Disable`)
  (goto _label_3))

(fn `Load Data`
  (params (JSON :type String))
  (returns (Object :type "VaRestJsonObject Object Reference"))
  (bind _object (`parent.Load Data` JSON))
  (`|ExecutionSequence`
    (:`then_0`
      (bind (_has_field_ _return_value) (`/Game/Function/BP_JSON_FunctionLibrary.Get Value As Int` _object "State"))
      (if (and _has_field_ (!= _return_value (`KismetMathLibrary.Conv_ByteToInt` (`self.State`))))
        (`self.Interact` (`self.Button`))))
    (:`then_1`
      (return _object))))

(fn `Save Data`
  (returns (JSON :type "VaRestJsonObject Object Reference"))
  (bind _json (`parent.Save Data`))
  (`VaRestJsonObject.SetIntegerField` _json "State" (`KismetMathLibrary.Conv_ByteToInt` (`self.State`)))
  (return _json))

(fn `UserConstructionScript`
  (`parent.UserConstructionScript`))
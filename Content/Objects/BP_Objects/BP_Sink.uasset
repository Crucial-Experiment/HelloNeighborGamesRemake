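; Interactive sink that fills objects placed under its running water and speeds up their cooling.
; Interacting with either handle rotates it via timeline, while the root toggles water effects and overlap detection through RemoteSink and notifies the tutorial.
; While on, Tick calls Filling on overlapping BP_Objects with a WaterComponent.
; Paired DoOnce gates enable fast cooling for the first overlapped object and revert it after shutoff.
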(event `Remote Sink`
  (bind _sink (`self.Sink`))
  (bind _water_zone (`self.Water Zone`))
  ;[1 1 1] Remote Sink
  (switch `/Game/Objects/Enum/TumblerStateEnum` (`self.State`)
    (:`NewEnumerator0`
      (`ActorComponent.Deactivate` _sink)
      (`ActorComponent.Deactivate` (`self.Water Sequence`))
      (set `self.State` "NewEnumerator1")
      (set `PrimitiveComponent.bGenerateOverlapEvents` false _water_zone))
    (:`NewEnumerator1`
      (`ActorComponent.Activate` _sink false)
      (`ActorComponent.Activate` (`self.Water Sequence`) false)
      (set `self.State` "NewEnumerator0")
      (set `PrimitiveComponent.bGenerateOverlapEvents` true _water_zone))))

(event `/Game/Function/BP_Interface.Interact`
  (params (Component :type "PrimitiveComponent Object Reference") (Location :type "Vector Structure"))
  ;[1 1 1] Interact
  (`|ExecutionSequence`
    (:`then_0`
      (if (== Component (`self.Right`))
        (`/Engine/EditorBlueprintResources/StandardMacros.FlipFlop`
          (:`A`
            (bind (_direction _alpha) (`Timeline|Rotate Right Timeline` :!label _label)
              (:`Update`
                (`SceneComponent.K2_SetRelativeRotation` (`self.Right`) (`KismetMathLibrary.RLerp` (struct) (struct :`Yaw` 100.0) _alpha) false false))))
          (:`B`
            (goto _label :!via `Reverse`)))))
    (:`then_1`
      (if (== Component (`self.Left`))
        (`/Engine/EditorBlueprintResources/StandardMacros.FlipFlop`
          (:`A`
            (bind (_direction_2 _alpha_2) (`Timeline|Rotate Left Timeline` :!label _label_2)
              (:`Update`
                (`SceneComponent.K2_SetRelativeRotation` (`self.Left`) (`KismetMathLibrary.RLerp` (struct) (struct :`Yaw` -100.0) _alpha_2) false false))))
          (:`B`
            (goto _label_2 :!via `Reverse`)))))
    (:`then_2`
      (if (== Component (`self.Root`))
        (`self.Remote Sink`)
        (`/Game/Objects/Tutorial/TutorialComponent.Check Use Type` (`self.TutorialComponent`) "NewEnumerator6")))))

(event `self.ReceiveTick`
  (params (DeltaSeconds :type "Float (single-precision)"))
  ;[1 1 1] Water Zone
  (if (`|EnumEquality` (`self.State`) "NewEnumerator0")
    (for _array_element (`PrimitiveComponent.GetOverlappingActors` (`self.Water Zone`) "/Game/Objects/Structurs/BP_Object.BP_Object_C")
      (`|ExecutionSequence`
        (:`then_0`
          (bind _returnvalue (`self.GetComponentByClass` _array_element "/Game/Objects/Structurs/WaterComponent.WaterComponent_C"))
          (`/Engine/EditorBlueprintResources/StandardMacros.IsValid` _returnvalue
            (:`Is Valid`
              (`/Game/Objects/Structurs/WaterComponent.Filling` _returnvalue))))
        (:`then_1`
          (`/Engine/EditorBlueprintResources/StandardMacros.DoOnce` false :!label _label_3
            (:`Completed`
              (`|ExecutionSequence`
                (:`then_0`
                  (bind _output_get (set `self.Actor Temperature` _array_element))
                  (`/Game/Objects/Structurs/WaterComponent.Update Temperature` (`self.WaterComponent`) _output_get true))
                (:`then_1`
                  (goto _label_4 :!via `Reset`))))))))
    (else
      (`|ExecutionSequence`
        (:`then_0`
          (goto _label_3 :!via `Reset`))
        (:`then_1`
          (`/Engine/EditorBlueprintResources/StandardMacros.DoOnce` false :!label _label_4
            (:`Completed`
              (bind _actor_temperature (`self.Actor Temperature`)
                (:`then`
                  (`/Game/Objects/Structurs/WaterComponent.Update Temperature` (`self.WaterComponent`) _actor_temperature false)
                  (set `self.Actor Temperature` null))
                (:`else`)))))))))

(fn `UserConstructionScript`)
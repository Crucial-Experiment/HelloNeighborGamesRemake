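; A handheld TV remote item that operates the BP_TV it is pointed at.
; VR use, or a left click while the player holds this item, fires a line trace and continues only if it hits a TV.
; The hit TV passes through a server event to an all-clients event, which calls RemoteTV on it and reports the use to the tutorial and GameJolt components.
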(event `self.On VR Use`
  (`parent.On VR Use`)
  (bind _actor (`self.Line Trace` 1500.0 :!label _label))
  (bind _asbp_tv (cast `/Game/Objects/BP_Objects/BP_TV` _actor))
  (`self.Interact (Server)` _asbp_tv))

(event `self.ReceiveBeginPlay`
  (`parent.ReceiveBeginPlay`))

(event `On Press LMB_1`
  (bind _player (`/Game/Function/BP_MacroLibrary.Find Player`)
    (:`Is Valid`
      (bind _item (`/Game/Player/BP_Player.Get Item` _player))
      (if (== _item self)
        (goto _label)))))

(event `Interact (Server)`
  (params (TV :type "/Game/Objects/BP_Objects/BP_TV Object Reference"))
  (`self.Interact (All)` TV))

(event `Interact (All)`
  (params (TV :type "/Game/Objects/BP_Objects/BP_TV Object Reference"))
  (`/Game/Objects/BP_Objects/BP_TV.RemoteTV` TV false)
  (`/Game/Objects/Tutorial/TutorialComponent.Check Use Type` (`self.TutorialComponent`) "NewEnumerator6")
  (`/Game/Objects/GameJolt/GameJoltComponent.Check Use Type` (`self.GameJoltComponent`) "NewEnumerator6"))

(fn `UserConstructionScript`
  (`parent.UserConstructionScript`))
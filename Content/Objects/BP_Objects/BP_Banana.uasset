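; BP_Banana is an edible banana object that turns into a peel when eaten.
; On the VROnly EventEat event for itself, if it has not been eaten yet, it swaps the root static mesh to the peel and sets the FlatComponent icon to the peel image.
; The construction script only calls the parent's.
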(event `/Game/Function/BP_Interface.Eat (VR Only)`
  (params (Actor :type "/Game/Objects/Structurs/BP_Object Object Reference"))
  (if (and (== Actor self) (not (`self.Eat?`)))
    (`StaticMeshComponent.SetStaticMesh` (`self.Root`) "/Game/Objects/Meshes/banana_peel.banana_peel")
    (set `/Game/Objects/Structurs/FlatComponent.Icon` "/Game/UMG/Inv_Icons/Banana__Peel_.Banana__Peel_" (`self.FlatComponent`))))

(fn `UserConstructionScript`
  (`parent.UserConstructionScript`))
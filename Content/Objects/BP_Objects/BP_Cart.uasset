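; Rail cart that travels along a Rails actor's spline when the player touches its top or bottom trigger, unless Blocking is set.
; Each trigger drives a movement timeline in opposite directions, positioning and orienting the cart along the spline.
; A timer or another touch while moving halts it, with DoOnce gates guarding retriggers.
; A products box tracks overlapping BP_Objects, and construction snaps the cart to Rails.
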(event `self.Box Top.OnComponentBeginOverlap`
  (params (OverlappedComponent :type "PrimitiveComponent Object Reference") (OtherActor :type "Actor Object Reference") (OtherComp :type "PrimitiveComponent Object Reference") (OtherBodyIndex :type Integer) (bFromSweep :type Boolean) (SweepResult :type "HitResult Structure (by ref)"))
  (bind _stopping (`self.Stopping`))
  (bind _impact (`self.Impact`))
  (bind _returnvalue (`KismetMathLibrary.RandomFloatInRange` (`self.Stop After Min`) (`self.Stop After Min`)))
  (bind _spline (`/Game/Objects/BP_Objects/BP_Rails.Spline` (`self.Rails`)))
  (bind _returnvalue_2 (`SplineComponent.GetSplineLength` _spline))
  (if (not (`self.Blocking`))
    (cast `/Game/Player/BP_Player` OtherActor)
    (`/Engine/EditorBlueprintResources/StandardMacros.DoOnce` false :!label _label
      (:`Completed`
        (`|ExecutionSequence`
          (:`then_0`
            (`AudioComponent.Play` _impact 0.0)
            (if _stopping
              (set `self.Stopping` false)
              (`KismetSystemLibrary.K2_SetTimerDelegate` (delegate `Stop`) _returnvalue)
              (bind (_direction _alpha) (`Timeline|Movement Timeline` :!via `Reverse` :!label _label_2)
                (:`Update`
                  (bind _output_get (set `self.DistanceAlongSpline` (`KismetMathLibrary.FClamp` (* _alpha _returnvalue_2) 0.0 _returnvalue_2)))
                  (`self.K2_SetActorLocation` (`SplineComponent.GetLocationAtDistanceAlongSpline` _spline _output_get "World"))
                  (bind (_returnvalue_roll _returnvalue_pitch _returnvalue_yaw) (`KismetMathLibrary.BreakRotator` (`KismetMathLibrary.Conv_VectorToRotator` (`SplineComponent.GetTangentAtDistanceAlongSpline` _spline _output_get "World"))))
                  (bind _result (`/Engine/EditorBlueprintResources/StandardMacros.NegateFloat` _returnvalue_pitch)
                    (:`  `
                      (`self.K2_SetActorRotation` (`KismetMathLibrary.MakeRotator` _returnvalue_roll _result (- _returnvalue_yaw 180.0))))))
                (:`Finished`
                  (set `self.Stopping` true)
                  (`|ExecutionSequence` :!label _label_3
                    (:`then_0`
                      (goto _label :!via `Reset`))
                    (:`then_1`
                      (goto _label_5 :!via `Reset`)))))
              (else
                (`self.Stop` :!label _label_4))))
          (:`then_1`
            (goto _label_5 :!via `Reset`)))))))

(event `self.Box Bottom.OnComponentBeginOverlap`
  (params (OverlappedComponent :type "PrimitiveComponent Object Reference") (OtherActor :type "Actor Object Reference") (OtherComp :type "PrimitiveComponent Object Reference") (OtherBodyIndex :type Integer) (bFromSweep :type Boolean) (SweepResult :type "HitResult Structure (by ref)"))
  (if (not (`self.Blocking`))
    (cast `/Game/Player/BP_Player` OtherActor)
    (`/Engine/EditorBlueprintResources/StandardMacros.DoOnce` false :!label _label_5
      (:`Completed`
        (`|ExecutionSequence`
          (:`then_0`
            (`AudioComponent.Play` (`self.Impact`) 0.0)
            (if (`self.Stopping`)
              (set `self.Stopping` false)
              (`KismetSystemLibrary.K2_SetTimerDelegate` (delegate `Stop`) (`KismetMathLibrary.RandomFloatInRange` (`self.Stop After Min`) (`self.Stop After Min`)))
              (goto _label_2)
              (else
                (goto _label_4))))
          (:`then_1`
            (goto _label :!via `Reset`)))))))

(event `Stop`
  (`|ExecutionSequence`
    (:`then_0`
      (set `self.Stopping` true)
      (goto _label_2 :!via `Stop`))
    (:`then_1`
      (goto _label_3))))

(event `self.Box Products.OnComponentBeginOverlap`
  (params (OverlappedComponent :type "PrimitiveComponent Object Reference") (OtherActor :type "Actor Object Reference") (OtherComp :type "PrimitiveComponent Object Reference") (OtherBodyIndex :type Integer) (bFromSweep :type Boolean) (SweepResult :type "HitResult Structure (by ref)"))
  (bind _asbp_object (cast `/Game/Objects/Structurs/BP_Object` OtherActor))
  (`KismetArrayLibrary.Array_Add` (`self.Products`) _asbp_object)
  (`KismetSystemLibrary.PrintString` (`KismetStringLibrary.Concat_StrStr` "Add: " (`KismetSystemLibrary.GetDisplayName` _asbp_object))))

(event `self.Box Products.OnComponentEndOverlap`
  (params (OverlappedComponent :type "PrimitiveComponent Object Reference") (OtherActor :type "Actor Object Reference") (OtherComp :type "PrimitiveComponent Object Reference") (OtherBodyIndex :type Integer))
  (bind _asbp_object (cast `/Game/Objects/Structurs/BP_Object` OtherActor))
  (`KismetArrayLibrary.Array_RemoveItem` (`self.Products`) _asbp_object)
  (`KismetSystemLibrary.PrintString` (`KismetStringLibrary.Concat_StrStr` "Remove: " (`KismetSystemLibrary.GetDisplayName` _asbp_object))))

(fn `UserConstructionScript`
  (bind _rails (`self.Rails`))
  (`parent.UserConstructionScript`)
  (`/Engine/EditorBlueprintResources/StandardMacros.IsValid` _rails
    (:`Is Valid`
      (`self.K2_SetActorLocation` (`self.K2_GetActorLocation` _rails) false true)
      (`self.K2_SetActorRotation` (`self.Rotation`)))))
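; Player car prop whose trunk, left door and right door open and close when interacted with.
; The Interact event matches the passed component, and a FlipFlop per part alternately plays or reverses that part's timeline to lerp its relative rotation.
; Open sounds play as movement starts, while closed sounds wait until the reverse finishes, with both doors sharing the same cues.
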(event `/Game/Function/BP_Interface.Interact`
  (params (Component :type "PrimitiveComponent Object Reference") (Location :type "Vector Structure"))
  (`|ExecutionSequence`
    (:`then_0`
      (if (== Component (`self.Trunk`))
        (bind _isa (`/Engine/EditorBlueprintResources/StandardMacros.FlipFlop`)
          (:`A`
            (`|ExecutionSequence`
              (:`then_0`
                (bind (_direction _alpha) (`Timeline|Trunk Rotation` :!label _label)
                  (:`Update`
                    (`SceneComponent.K2_SetRelativeRotation` (`self.Trunk`) (`KismetMathLibrary.RLerp` (struct) (struct :`Roll` 70.0) _alpha) false false))
                  (:`Finished`
                    (if (not _isa)
                      (`GameplayStatics.PlaySoundAtLocation` "/Game/Sounds/Objects/OpenClosed/car_trunk_closed_Cue.car_trunk_closed_Cue" (`self.K2_GetActorLocation`) (struct) 1.0 1.0 0.0 null null null null)))))
              (:`then_1`
                (`GameplayStatics.PlaySoundAtLocation` "/Game/Sounds/Objects/OpenClosed/car_trunk_open_Cue.car_trunk_open_Cue" (`self.K2_GetActorLocation`) (struct) 1.0 1.0 0.0 null null null null))))
          (:`B`
            (goto _label :!via `Reverse`)))))
    (:`then_1`
      (if (== Component (`self.Door Left`))
        (bind _isa_2 (`/Engine/EditorBlueprintResources/StandardMacros.FlipFlop`)
          (:`A`
            (`|ExecutionSequence`
              (:`then_0`
                (bind (_direction_2 _alpha_2) (`Timeline|Left Door Rotation` :!label _label_2)
                  (:`Update`
                    (`SceneComponent.K2_SetRelativeRotation` (`self.Door Left`) (`KismetMathLibrary.RLerp` (struct) (struct :`Yaw` 50.0) _alpha_2) false false))
                  (:`Finished`
                    (if (not _isa_2)
                      (`GameplayStatics.PlaySoundAtLocation` "/Game/Sounds/Objects/OpenClosed/car_door_player_closed_Cue.car_door_player_closed_Cue" (`self.K2_GetActorLocation`) (struct) 1.0 1.0 0.0 null null null null :!label _label_3)))))
              (:`then_1`
                (`GameplayStatics.PlaySoundAtLocation` "/Game/Sounds/Objects/OpenClosed/car_door_player_open_Cue.car_door_player_open_Cue" (`self.K2_GetActorLocation`) (struct) 1.0 1.0 0.0 null null null null :!label _label_4))))
          (:`B`
            (goto _label_2 :!via `Reverse`)))))
    (:`then_2`
      (if (== Component (`self.Door Right`))
        (bind _isa_3 (`/Engine/EditorBlueprintResources/StandardMacros.FlipFlop`)
          (:`A`
            (`|ExecutionSequence`
              (:`then_0`
                (bind (_direction_3 _alpha_3) (`Timeline|Шкала времени` :!label _label_5)
                  (:`Update`
                    (`SceneComponent.K2_SetRelativeRotation` (`self.Door Right`) (`KismetMathLibrary.RLerp` (struct) (struct :`Yaw` -50.0) _alpha_3) false false))
                  (:`Finished`
                    (if (not _isa_3)
                      (goto _label_3)))))
              (:`then_1`
                (goto _label_4))))
          (:`B`
            (goto _label_5 :!via `Reverse`)))))))

(fn `UserConstructionScript`)
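; BP_Train is an interactive train that rides a Rails spline when powered by electricity or a generator.
; Interact toggles sliding doors, sets start/stop state and flips a direction lever, with Moving driving a timeline that plays or reverses along the spline.
; At timeline end it restarts if looping or a trace finds BP_Rails, otherwise derails with physics and an impulse.
; State, direction and rotation are saved to JSON.
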(event `self.Enable`
  ;[1 1 1] Electricity
  (`parent.Enable`)
  (`self.Moving` (`self.State`) :!label _label))

(event `self.Disable`
  ;[1 1 1] Electricity
  (`parent.Disable`)
  (goto _label))

(event `/Game/Function/BP_Interface.Interact`
  (params (Component :type "PrimitiveComponent Object Reference") (Location :type "Vector Structure"))
  (bind _returnvalue (`self.K2_GetActorLocation`))
  (bind _lever (`self.Lever`))
  ;[1 1 1] Electricity
  (`|ExecutionSequence`
    (:`then_0`
      (if (or (== Component (`self.Door 4`)) (== Component (`self.Door 3`)))
        (`/Engine/EditorBlueprintResources/StandardMacros.FlipFlop`
          (:`A`
            (bind (_direction _alpha) (`Timeline|Door 3-4 Timeline` :!label _label_2)
              (:`Update`
                (`SceneComponent.K2_SetRelativeLocation` (`self.Door 3`) (`KismetMathLibrary.VLerp` (-18.75 -431.25 1162.5) (-37.5 -662.5 1162.5) _alpha) false false)
                (`SceneComponent.K2_SetRelativeLocation` (`self.Door 4`) (`KismetMathLibrary.VLerp` (-18.75 -181.25 1162.5) (-43.75 50.0 1162.5) _alpha) false false))))
          (:`B`
            (goto _label_2 :!via `Reverse`)))
        (elif (or (== Component (`self.Door 1`)) (== Component (`self.Door 2`)))
          (`/Engine/EditorBlueprintResources/StandardMacros.FlipFlop`
            (:`A`
              (bind (_direction_2 _alpha_2) (`Timeline|Door 1-2 Timeline` :!label _label_3)
                (:`Update`
                  (`SceneComponent.K2_SetRelativeLocation` (`self.Door 1`) (`KismetMathLibrary.VLerp` (0.0 -162.5 1162.5) (237.5 -137.5 1162.5) _alpha_2) false false)
                  (`SceneComponent.K2_SetRelativeLocation` (`self.Door 2`) (`KismetMathLibrary.VLerp` (0.0 -162.5 1162.5) (-231.25 -131.25 1162.5) _alpha_2) false false))))
            (:`B`
              (goto _label_3 :!via `Reverse`))))))
    (:`then_1`
      (if (== Component (`self.Start Button`))
        (set `self.State` "NewEnumerator0")
        (`self.Moving` (`self.State`) :!label _label_4)
        (elif (== Component (`self.Stop Button`))
          (set `self.State` "NewEnumerator1")
          (goto _label_4))))
    (:`then_2`
      (if (== Component (`self.Box_0`))
        (if (`self.Move Back`)
          (set `self.Move Back` false)
          (`GameplayStatics.PlaySoundAtLocation` "/Game/Sounds/Objects/TurnOnOff/train_switch_on_Cue.train_switch_on_Cue" _returnvalue (struct) 1.0 1.0 0.0 "/Game/Sounds/Attenuation/Silent.Silent" null null null)
          (`SceneComponent.K2_SetRelativeRotation` _lever (struct :`Roll` 35.0) false false)
          (else
            (set `self.Move Back` true)
            (`GameplayStatics.PlaySoundAtLocation` "/Game/Sounds/Objects/TurnOnOff/train_switch_off_Cue.train_switch_off_Cue" _returnvalue (struct) 1.0 1.0 0.0 "/Game/Sounds/Attenuation/Silent.Silent" null null null)
            (`SceneComponent.K2_SetRelativeRotation` _lever (struct :`Roll` -35.0) false false)))
        (`self.Moving` (`self.State`))))))

(event `self.ReceiveBeginPlay`
  ;[1 1 1] Begin Play
  (`parent.ReceiveBeginPlay`)
  (`self.Moving` (`self.State`)))

(event `Moving`
  (params (State :type "/Game/Objects/Enum/TumblerStateEnum Enum" :default "NewEnumerator0"))
  (bind _move (`self.Move`))
  (bind _rails_check (`self.Rails Check`))
  (bind _train (`self.Train`))
  (bind _returnvalue (`SceneComponent.K2_GetComponentLocation` _rails_check))
  (bind _spline (`/Game/Objects/BP_Objects/BP_Rails.Spline` (`self.Rails`)))
  (bind _spline_2 (`/Game/Objects/BP_Objects/BP_Rails.Spline` (`self.Rails`)))
  ;[1 1 1] Moving
  (`TimelineComponent.SetPlayRate` (`self.Move Timeline`) (/ 1.0 (`self.Speed`)))
  (if (or (`self.Has Electricity`) (`self.Generator`))
    (switch `/Game/Objects/Enum/TumblerStateEnum` State
      (:`NewEnumerator0`
        (`AudioComponent.Play` _move 0.0)
        (if (not (`self.Move Back`))
          (bind (_direction _alpha) (`Timeline|Move Timeline` :!label _label_5)
            (:`Update`
              (bind _returnvalue_2 (`KismetMathLibrary.Lerp` 0.0 (`SplineComponent.GetDistanceAlongSplineAtSplinePoint` _spline (- (`SplineComponent.GetNumberOfSplinePoints` _spline) 1)) _alpha))
              (`self.K2_SetActorLocation` (`SplineComponent.GetLocationAtDistanceAlongSpline` _spline_2 _returnvalue_2 "World"))
              (bind (_returnvalue_roll _returnvalue_pitch _returnvalue_yaw) (`KismetMathLibrary.BreakRotator` (`KismetMathLibrary.Conv_VectorToRotator` (`SplineComponent.GetTangentAtDistanceAlongSpline` _spline_2 _returnvalue_2 "World"))))
              (bind _result (`/Engine/EditorBlueprintResources/StandardMacros.NegateFloat` _returnvalue_pitch)
                (:`  `
                  (`self.K2_SetActorRotation` (`KismetMathLibrary.MakeRotator` _result _returnvalue_roll (- _returnvalue_yaw 90.0))))))
            (:`Finished`
              (if (not (`self.Again From Start Rails?`))
                (if (or (`self.Has Electricity`) (`self.Generator`))
                  (bind (_outhit _returnvalue_3) (`KismetSystemLibrary.LineTraceSingle` :`Start` _returnvalue :`End` (+ _returnvalue (* (`SceneComponent.GetForwardVector` _rails_check) 50)) :`TraceChannel` "TraceTypeQuery1" :`DrawDebugType` (`self.Draw Debug`)))
                  (if _returnvalue_3
                    (cast `/Game/Objects/BP_Objects/BP_Rails` (`.HitActor` (`GameplayStatics.BreakHitResult` _outhit))
                      (:`then`
                        (`self.Play from Start`))
                      (:`CastFailed`
                        (`self.Set Flat Mode` "NewEnumerator0" :!label _label_6)
                        (set `self.Rails` null)
                        (`AudioComponent.Stop` (`self.Move`))
                        (`PrimitiveComponent.SetSimulatePhysics` _train true)
                        (`PrimitiveComponent.AddImpulse` _train (+ (* (`self.GetActorForwardVector`) 1000000.0) (`self.K2_GetActorLocation`)) "None" false)))
                    (else
                      (goto _label_6))))
                (else
                  (`self.Play from Start`)))))
          (else
            (goto _label_5 :!via `Reverse`))))
      (:`NewEnumerator1`
        (`AudioComponent.Stop` _move :!label _label_7)
        (goto _label_5 :!via `Stop`)))
    (else
      (goto _label_7))))

(event `Play from Start`
  ;[1 1 1] Moving
  (if (not (`self.Move Back`))
    (goto _label_5 :!via `PlayFromStart`)
    (else
      (goto _label_5 :!via `ReverseFromEnd`))))

(fn `Load Data`
  (params (JSON :type String))
  (returns (Object :type "VaRestJsonObject Object Reference"))
  (bind _object (`parent.Load Data` JSON))
  (`|ExecutionSequence`
    (:`then_0`
      (bind (_has_field_ _return_value) (`/Game/Function/BP_JSON_FunctionLibrary.Get Value As Bool` _object "Move Back"))
      (if _has_field_
        (set `self.Move Back` _return_value)))
    (:`then_1`
      (bind (_has_field__2 _return_value_2) (`/Game/Function/BP_JSON_FunctionLibrary.Get Value As Int` _object "State"))
      (if (and _has_field__2 (!= _return_value_2 (`KismetMathLibrary.Conv_ByteToInt` (`self.State`))))
        (`self.Moving` (cast `/Game/Objects/Enum/TumblerStateEnum` (`KismetMathLibrary.Conv_IntToByte` _return_value_2)))))
    (:`then_2`
      (bind (_has_field__3 _return_value_3) (`/Game/Function/BP_JSON_FunctionLibrary.Get Value As Rotator` _object "Rotation"))
      (if _has_field__3
        (set `self.Rotation` _return_value_3)))
    (:`then_3`
      (return _object))))

(fn `Save Data`
  (returns (JSON :type "VaRestJsonObject Object Reference"))
  (bind _json (`parent.Save Data`))
  (`VaRestJsonObject.SetIntegerField` _json "State" (`KismetMathLibrary.Conv_ByteToInt` (`self.State`)))
  (`VaRestJsonObject.SetBoolField` _json "Move Back" (`self.Move Back`))
  (`/Game/Function/BP_JSON_FunctionLibrary.Set Rotator Field` _json "Rotation" (`self.Rotation`))
  (return _json))

(fn `UserConstructionScript`
  (bind _rails (`self.Rails`))
  (bind _lever (`self.Lever`))
  (`parent.UserConstructionScript`)
  (`|ExecutionSequence`
    (:`then_0`
      (`/Engine/EditorBlueprintResources/StandardMacros.IsValid` _rails
        (:`Is Valid`
          (`self.K2_SetActorLocation` (`self.K2_GetActorLocation` _rails) false true)
          (`self.K2_SetActorRotation` (`self.Rotation`)))))
    (:`then_1`
      (if (`self.Move Back`)
        (`SceneComponent.K2_SetRelativeRotation` _lever (struct :`Roll` -35.0) false false)
        (else
          (`SceneComponent.K2_SetRelativeRotation` _lever (struct :`Roll` 35.0) false false))))))
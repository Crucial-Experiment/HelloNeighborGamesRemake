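; Lamp object Blueprint that extends a parent class with a second spark effect and an optional linked Bulb actor.
; The construction script snaps a valid Bulb to the Scene component's transform and disables PSparks1 auto-activation; without a Bulb, PSparks1 auto-activates.
; At runtime, PSparks1 mirrors PSparks through its activation and deactivation events, while Enable and Disable simply defer to the parent.
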(event `/Game/Objects/Structurs/BP_Electricity.Enable`
  ;[1 1 1] Set State
  (`parent.Enable`))

(event `/Game/Objects/Structurs/BP_Electricity.Disable`
  ;[1 1 1] Set State
  (`parent.Disable`))

(event `self.ReceiveBeginPlay`
  ;[1 1 1] Begin Play
  (`parent.ReceiveBeginPlay`)
  (add `ActorComponent.OnComponentActivated` (`self.P_Sparks`) (delegate `On Activated`))
  (add `ActorComponent.OnComponentDeactivated` (`self.P_Sparks`) (delegate `On Deactivated`)))

(event `On Activated`
  (params (Component :type "ActorComponent Object Reference") (bReset :type Boolean))
  ;[1 1 1] Begin Play
  (`ActorComponent.Activate` (`self.P_Sparks1`) bReset))

(event `On Deactivated`
  (params (Component :type "ActorComponent Object Reference"))
  ;[1 1 1] Begin Play
  (`ActorComponent.Deactivate` (`self.P_Sparks1`)))

(fn `UserConstructionScript`
  (bind _p_sparks1 (`self.P_Sparks1`))
  (bind (_returnvalue_location _returnvalue_rotation) (`KismetMathLibrary.BreakTransform` (`SceneComponent.K2_GetComponentToWorld` (`self.Scene`))))
  (`parent.UserConstructionScript`)
  (`/Engine/EditorBlueprintResources/StandardMacros.IsValid` (`self.Bulb`)
    (:`Is Valid`
      (`ActorComponent.SetAutoActivate` _p_sparks1 false)
      (`self.K2_SetActorLocationAndRotation` (`self.Bulb`) _returnvalue_location _returnvalue_rotation false false))
    (:`Is Not Valid`
      (`ActorComponent.SetAutoActivate` _p_sparks1 true))))
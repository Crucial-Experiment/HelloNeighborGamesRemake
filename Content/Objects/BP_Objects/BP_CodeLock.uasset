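; BP_CodeLock is a ten-button keypad lock that unlocks when the pressed digit sequence matches KeyCode.
; Interactions route through a server event to an All event, which toggles the button's material and adds or removes its index in Code, using the current material as pressed state.
; Each press compares the joined digits with KeyCode, resetting on a full-length mismatch.
; A match runs the parent unlock, disables pickup and sets flat mode.
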(event `Check Code`
  (bind _temp_code (`self.Temp Code`))
  ;[1 1 1] Check Code
  (set `self.Temp Code` "")
  (for _array_element (`self.Code`)
    (set `self.Temp Code` (`KismetStringLibrary.Concat_StrStr` (`self.Temp Code`) _array_element)))
  (if (`KismetStringLibrary.EqualEqual_StrStr` (`self.Key Code`) _temp_code)
    (`self.Unlock`)
    (elif (<= (`KismetStringLibrary.Len` (`self.Key Code`)) (`KismetStringLibrary.Len` _temp_code))
      (for _array_element_2 (`self.Get Buttons`)
        (`PrimitiveComponent.SetMaterial` _array_element_2 0 (`self.Button Off`)))
      (set `self.Temp Code` "")
      (set `self.Code` (`|MakeArray`)))))

(event `self.Unlock`
  ;[1 1 1] Unlock
  (`parent.Unlock`)
  (set `self.CanPickUp` false)
  (`self.Set Flat Mode` "NewEnumerator1"))

(event `Interact (All)`
  (params (Component :type "PrimitiveComponent Object Reference"))
  (bind _code (`self.Code`))
  ;[1 1 1] Logic
  (if (!= Component (`self.Root`))
    (bind (_return _index) (`self.Component` Component))
    (if (!= (`PrimitiveComponent.GetMaterial` _return 0) "/Game/Objects/Materials/panel_light_m_inst.panel_light_m_inst")
      (`PrimitiveComponent.SetMaterial` _return 0 (`self.Button On`))
      (bind _returnvalue (`KismetStringLibrary.Conv_IntToString` _index))
      (`KismetArrayLibrary.Array_Add` _code _returnvalue)
      (else
        (`PrimitiveComponent.SetMaterial` _return 0 (`self.Button Off`))
        (`KismetArrayLibrary.Array_RemoveItem` _code _returnvalue)))
    (`self.Check Code`)))

(event `Interact (Server)`
  (params (Component :type "PrimitiveComponent Object Reference"))
  ;[1 1 1] Logic
  (`self.Interact (All)` Component))

(event `/Game/Function/BP_Interface.Interact`
  (params (Component :type "PrimitiveComponent Object Reference") (Location :type "Vector Structure"))
  ;[1 1 1] Logic
  (`self.Interact (Server)` Component))

(fn `Component`
  (params (Comp :type "PrimitiveComponent Object Reference"))
  (returns (Return :type "StaticMeshComponent Object Reference") (Index :type Integer))
  (for (_array_element _array_index) (`self.Get Buttons`)
    (if (== Comp _array_element)
      (return _array_element _array_index))))

(fn `Get Buttons`
  (returns (Buttons :type "Array of StaticMeshComponent Object Reference"))
  (return (`|MakeArray` (`self.button_0`) (`self.button_1`) (`self.button_2`) (`self.button_3`) (`self.button_4`) (`self.button_5`) (`self.button_6`) (`self.button_7`) (`self.button_8`) (`self.button_9`))))

(fn `UserConstructionScript`
  (`parent.UserConstructionScript`))
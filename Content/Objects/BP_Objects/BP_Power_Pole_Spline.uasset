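; Spline-driven power line actor that builds a row of connected power poles in its construction script.
; A BP_Power_Pole child actor is spawned at each spline point, matching its location and rotation, and stored in an array.
; A second pass attaches both cables of each pole to the next pole's anchors, setting lengths to the gap plus random slack.
; The last pole's cable lengths are zeroed.
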(fn `UserConstructionScript`
  (bind _spline (`self.Spline`))
  (bind _index_of_loop (`self.Index of loop`))
  (bind _output (`|GetArrayItem` (`self.All child actors of power pone`) (`self.Index of loop 2`)))
  (bind _output_2 (`|GetArrayItem` (`self.All child actors of power pone`) (`self.Number of spline points`)))
  (bind _output_3 (`|GetArrayItem` (`self.All child actors of power pone`) (`self.Index of loop 2`)))
  (bind _cable_1 (`/Game/Objects/BP_Objects/BP_Power_Pole.Cable 1` _output_3))
  (bind _cable_2 (`/Game/Objects/BP_Objects/BP_Power_Pole.Cable 2` _output))
  (bind _cable_1_pos (`/Game/Objects/BP_Objects/BP_Power_Pole.Cable 1 Pos` (`|GetArrayItem` (`self.All child actors of power pone`) (+ (`self.Index of loop 2`) 1))))
  (bind _cable_2_pos (`/Game/Objects/BP_Objects/BP_Power_Pole.Cable 2 Pos` (`|GetArrayItem` (`self.All child actors of power pone`) (+ (`self.Index of loop 2`) 1))))
  (bind _output_get (set `self.Number of spline points` (- (`SplineComponent.GetNumberOfSplinePoints` (`self.Spline`)) 1)))
  (for _index (range (+ _output_get 1))
    (set `self.Index of loop` _index)
    (bind _returnvalue (`AddComponent|NODE_AddChildActorComponent-2` :`RelativeTransform` (`KismetMathLibrary.Conv_VectorToTransform` (`SplineComponent.GetLocationAtSplinePoint` _spline _index_of_loop "Local"))))
    (`ChildActorComponent.SetChildActorClass` _returnvalue "/Game/Objects/BP_Objects/BP_Power_Pole.BP_Power_Pole_C")
    (bind _asbp_power_pole (cast `/Game/Objects/BP_Objects/BP_Power_Pole` (`ChildActorComponent.ChildActor` _returnvalue)))
    (`KismetArrayLibrary.Array_Add` (`self.All child actors of power pone`) _asbp_power_pole)
    (`SceneComponent.K2_SetRelativeRotation` _returnvalue (`SplineComponent.GetRotationAtSplinePoint` _spline _index_of_loop "Local") false false))
  (for _index_2 (range (+ (`self.Number of spline points`) 1))
    (set `self.Index of loop 2` _index_2)
    (`|ExecutionSequence`
      (:`then_0`
        (`SceneComponent.K2_AttachToComponent` _cable_1 _cable_1_pos "None" "SnapToTarget" "SnapToTarget" "SnapToTarget" true)
        (set `CableComponent.CableLength` (+ (`KismetMathLibrary.RandomFloatInRange` 0.0 120.0) (`KismetMathLibrary.VSize` (- (`SceneComponent.K2_GetComponentLocation` (`/Game/Objects/BP_Objects/BP_Power_Pole.Cable 1 Pos` _output_3)) (`SceneComponent.K2_GetComponentLocation` _cable_1_pos)))) _cable_1)
        (set `CableComponent.CableLength` 0.0 (`/Game/Objects/BP_Objects/BP_Power_Pole.Cable 1` _output_2)))
      (:`then_1`
        (`SceneComponent.K2_AttachToComponent` _cable_2 _cable_2_pos "None" "SnapToTarget" "SnapToTarget" "SnapToTarget" true)
        (set `CableComponent.CableLength` (+ (`KismetMathLibrary.RandomFloatInRange` 0.0 120.0) (`KismetMathLibrary.VSize` (- (`SceneComponent.K2_GetComponentLocation` (`/Game/Objects/BP_Objects/BP_Power_Pole.Cable 2 Pos` _output)) (`SceneComponent.K2_GetComponentLocation` _cable_2_pos)))) _cable_2)
        (set `CableComponent.CableLength` 0.0 (`/Game/Objects/BP_Objects/BP_Power_Pole.Cable 2` _output_2))))))
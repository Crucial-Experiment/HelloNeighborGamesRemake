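; BP_Phone is a usable phone item whose call rings a linked ParentPhone to lure the neighbour AI.
; CallPhone toggles call and delayed bell sounds, writing a check task and location to the AI blackboard unless its state excludes it.
; Using the held phone, or VR use, line-traces for a BP_Phone_Base to dock on, stopping the call.
; Otherwise it toggles the call and reports to tutorial and GameJolt components.
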(event `Call Phone`
  (bind _parent_phone (`self.Parent Phone`))
  (bind _parent_phone_2 (`self.Parent Phone`))
  (bind _call (`self.Call`))
  ;[1 1 1] Call
  (`/Engine/EditorBlueprintResources/StandardMacros.FlipFlop`
    (:`A`
      (`AudioComponent.Play` _call 0.0)
      (`/Engine/EditorBlueprintResources/StandardMacros.IsValid` _parent_phone_2
        (:`Is Valid`
          (`KismetSystemLibrary.Delay` 1.0)
          (`AudioComponent.Play` (`/Game/Objects/BP_Objects/BP_Phone.Bell` _parent_phone_2) 0.0)
          (bind _sosed (`/Game/Function/BP_MacroLibrary.Find Sosed`)
            (:`Is Valid`
              (if (`|EnumInequality` (`/Game/Sosed/BP_Sosed.Current State` _sosed) "NewEnumerator2")
                (bind _returnvalue (`AIBlueprintHelperLibrary.GetBlackboard` _sosed))
                (`BlackboardComponent.SetValueAsInt` _returnvalue "CheckTask" 5)
                (`BlackboardComponent.SetValueAsVector` _returnvalue "Check Location" (`SceneComponent.K2_GetComponentLocation` (`/Game/Objects/BP_Objects/BP_Phone.Arrow` _parent_phone_2)))
                (`BlackboardComponent.SetValueAsObject` _returnvalue "Phone" self)
                (`/Game/Sosed/BP_Sosed.Set State` _sosed "NewEnumerator3")))))))
    (:`B`
      (`AudioComponent.Stop` _call)
      (`/Engine/EditorBlueprintResources/StandardMacros.IsValid` _parent_phone
        (:`Is Valid`
          (`KismetSystemLibrary.Delay` 0.5)
          (`AudioComponent.Stop` (`/Game/Objects/BP_Objects/BP_Phone.Bell` _parent_phone)))))))

(event `self.ReceiveBeginPlay`
  ;[1 1 1] Begin Play and Use
  (`parent.ReceiveBeginPlay`))

(event `On Press LMB_1`
  (bind _parent_phone (`self.Parent Phone`))
  ;[1 1 1] Begin Play and Use
  (bind _player (`/Game/Function/BP_MacroLibrary.Find Player`)
    (:`Is Valid`
      (bind _item (`/Game/Player/BP_Player.Get Item` _player))
      (if (== _item self)
        (bind _actor (`self.Line Trace` 300.0 :!label _label))
        (`/Engine/EditorBlueprintResources/StandardMacros.IsValid` _actor
          (:`Is Valid`
            (bind _asbp_phone_base (cast `/Game/Objects/BP_Objects/BP_Phone_Base` _actor)
              (:`then`
                (`self.Try Release`)
                (`KismetArrayLibrary.Array_RemoveItem` (`/Game/UMG/Inventory/WB_Inventory.Inventory` (`/Game/Player/BP_Player.Inventory` _player)) self)
                (bind _scene (`/Game/Objects/BP_Objects/BP_Phone_Base.Scene` _asbp_phone_base))
                (`self.K2_SetActorLocationAndRotation` (`SceneComponent.K2_GetComponentLocation` _scene) (`SceneComponent.K2_GetComponentRotation` _scene))
                (set `/Game/Objects/BP_Objects/BP_Phone_Base.Phone` self _asbp_phone_base)
                (`PrimitiveComponent.SetSimulatePhysics` (`self.Root`) false)
                (`AudioComponent.Stop` (`self.Call`))
                (`/Engine/EditorBlueprintResources/StandardMacros.IsValid` _parent_phone
                  (:`Is Valid`
                    (`KismetSystemLibrary.Delay` 0.5)
                    (`AudioComponent.Stop` (`/Game/Objects/BP_Objects/BP_Phone.Bell` _parent_phone)))))
              (:`CastFailed`
                (`self.Call Phone` :!label _label_2)
                (`/Game/Objects/Tutorial/TutorialComponent.Check Use Type` (`self.TutorialComponent`) "NewEnumerator6")
                (`/Game/Objects/GameJolt/GameJoltComponent.Check Use Type` (`self.GameJoltComponent`) "NewEnumerator6"))))
          (:`Is Not Valid`
            (goto _label_2)))))))

(event `self.On VR Use`
  ;[1 1 1] Begin Play and Use
  (`parent.On VR Use`)
  (goto _label))

(fn `UserConstructionScript`)
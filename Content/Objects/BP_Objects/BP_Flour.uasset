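; BP_Flour is a flour object that makes the player leave a trail of flour footprints after stepping out of it.
; Exiting its Box starts a looping timer that spawns footprint actors below the player, matching their rotation.
; At the maximum count, the timer clears and the count and player reference reset.
; Re-entering the Box stops the timer but keeps the current count.
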(event `self.Box.OnComponentBeginOverlap`
  (params (OverlappedComponent :type "PrimitiveComponent Object Reference") (OtherActor :type "Actor Object Reference") (OtherComp :type "PrimitiveComponent Object Reference") (OtherBodyIndex :type Integer) (bFromSweep :type Boolean) (SweepResult :type "HitResult Structure (by ref)"))
  (cast `/Game/Player/BP_Player` OtherActor)
  (`KismetSystemLibrary.K2_ClearAndInvalidateTimerHandle` (`self.Player Out`)))

(event `self.Box.OnComponentEndOverlap`
  (params (OverlappedComponent :type "PrimitiveComponent Object Reference") (OtherActor :type "Actor Object Reference") (OtherComp :type "PrimitiveComponent Object Reference") (OtherBodyIndex :type Integer))
  (bind _asbp_player (cast `/Game/Player/BP_Player` OtherActor))
  (set `self.Player` _asbp_player)
  (bind _returnvalue (`KismetSystemLibrary.K2_SetTimerDelegate` (delegate `Spawn Flour Footprint`) (`self.Spawn Time`) true true))
  (set `self.Player Out` _returnvalue))

(event `Spawn Flour Footprint`
  (bind _player (`self.Player`))
  (if (< (`self.Flour Footprint Count`) (`self.Flour Footprint Count Max`))
    (`|SpawnActorFromClass` (`self.Flour Footprint Class`) (`KismetMathLibrary.MakeTransform` (- (`self.K2_GetActorLocation` _player) (0.0 0.0 90.0)) (`self.K2_GetActorRotation` _player)) "Undefined" "MultiplyWithRoot" null null)
    (`/Engine/EditorBlueprintResources/StandardMacros.IncrementInt` (`self.Flour Footprint Count`))
    (else
      (set `self.Flour Footprint Count` 0)
      (`KismetSystemLibrary.K2_ClearAndInvalidateTimerHandle` (`self.Player Out`))
      (set `self.Player` null))))

(fn `UserConstructionScript`)
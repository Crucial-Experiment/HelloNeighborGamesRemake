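; Interactable stereo record player that plays the sound of its assigned vinyl and drives linked speaker objects (Dynamics).
; Construction snaps the vinyl onto Part, whose children spin on Tick while playing.
; Direct or remote interaction toggles playback when a vinyl is present and electricity or a generator is available, also notifying tutorial and GameJolt components.
; Toggling or disabling propagates power state to each speaker, passing along the vinyl's sound.
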(event `self.ReceiveBeginPlay`
  (bind _vinyl (`self.Vinyl`))
  (`/Engine/EditorBlueprintResources/StandardMacros.IsValid` _vinyl
    (:`Is Valid`
      (set `/Game/Objects/BP_Objects/BP_Vinyl.Stereo System` self _vinyl)
      (`self.Set Flat Mode` _vinyl "NewEnumerator1")
      (`AudioComponent.SetSound` (`self.Music`) (`/Game/Objects/BP_Objects/BP_Vinyl.Sound` (`self.Vinyl`))))))

(event `self.ReceiveTick`
  (params (DeltaSeconds :type "Float (single-precision)"))
  (switch `/Game/Objects/Enum/TumblerStateEnum` (`self.State`)
    (:`NewEnumerator0`
      (`SceneComponent.K2_AddRelativeRotation` (`SceneComponent.GetChildrenComponents` (`self.Part`) false) (struct :`Yaw` 1.0) false false))))

(event `Remote Interact`
  (bind _music (`self.Music`))
  (`/Engine/EditorBlueprintResources/StandardMacros.IsValid` (`self.Vinyl`) :!label _label
    (:`Is Valid`
      (if (or (`self.Has Electricity`) (`self.Generator`))
        (`/Game/Objects/Tutorial/TutorialComponent.Check Use Type` (`self.TutorialComponent`) "NewEnumerator6")
        (`/Game/Objects/GameJolt/GameJoltComponent.Check Use Type` (`self.GameJoltComponent`) "NewEnumerator6")
        (switch `/Game/Objects/Enum/TumblerStateEnum` (`self.State`)
          (:`NewEnumerator0`
            (set `self.State` "NewEnumerator1")
            (`AudioComponent.Stop` _music)
            (`self.Set Dynamics State` "NewEnumerator1"))
          (:`NewEnumerator1`
            (set `self.State` "NewEnumerator0")
            (`AudioComponent.Play` _music 0.0)
            (`self.Set Dynamics State` "NewEnumerator0")))))))

(event `/Game/Function/BP_Interface.Interact`
  (params (Component :type "PrimitiveComponent Object Reference") (Location :type "Vector Structure"))
  (goto _label))

(event `self.Disable`
  (`parent.Disable`)
  (set `self.State` "NewEnumerator1")
  (`AudioComponent.Stop` (`self.Music`))
  (`self.Set Dynamics State` "NewEnumerator1"))

(event `Set Dynamics State`
  (params (State :type "/Game/Objects/Enum/TumblerStateEnum Enum" :default "NewEnumerator0"))
  (bind _dynamics (`self.Dynamics`))
  (for _array_element _dynamics
    (bind _vinyl (`self.Vinyl`)
      (:`then`
        (`AudioComponent.SetSound` (`/Game/Objects/BP_Objects/BP_Stereo_System_Dynamic.Music` _array_element) (`/Game/Objects/BP_Objects/BP_Vinyl.Sound` _vinyl)))
      (:`else`)))
  (for _array_element_2 _dynamics
    (switch `/Game/Objects/Enum/TumblerStateEnum` State
      (:`NewEnumerator0`
        (set `/Game/Objects/Structurs/BP_Electricity.Has Electricity` true _array_element_2)
        (`self.Enable` _array_element_2))
      (:`NewEnumerator1`
        (set `/Game/Objects/Structurs/BP_Electricity.Has Electricity` false _array_element_2)
        (`self.Disable` _array_element_2)))))

(fn `OnRep_Dynamics`)

(fn `UserConstructionScript`
  (bind _vinyl (`self.Vinyl`))
  (`parent.UserConstructionScript`)
  (`/Engine/EditorBlueprintResources/StandardMacros.IsValid` _vinyl
    (:`Is Valid`
      (`self.K2_AttachToComponent` _vinyl (`self.Part`) "None" "SnapToTarget" "SnapToTarget" "SnapToTarget" true)
      (`AudioComponent.SetSound` (`self.Music`) (`/Game/Objects/BP_Objects/BP_Vinyl.Sound` (`self.Vinyl`))))))
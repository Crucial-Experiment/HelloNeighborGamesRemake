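; BP_Washer is a washer object whose door swings open and closed when the player interacts with it.
; A timeline drives the door's relative rotation, with a state variable gating toggles, paired open/close sounds and callbacks on completion.
; The construction script tags the door as interactive when enabled.
; The door state is saved, and loading replays the interaction when the saved state differs from the current one.
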(event `/Game/Function/BP_Interface.Interact`
  (params (Component :type "PrimitiveComponent Object Reference") (Location :type "Vector Structure"))
  (if (and (== Component (`self.Door`)) (`self.Interactive?`))
    (switch `/Game/Objects/Enum/RotateStateEnum` (`self.Rotate State`)
      (:`NewEnumerator0`
        (set `self.Rotate State` "NewEnumerator3")
        (`|ExecutionSequence`
          (:`then_0`
            (bind (_direction _alpha) (`Timeline|Rotation` :!via `Reverse` :!label _label)
              (:`Update`
                (`SceneComponent.K2_SetRelativeRotation` (`self.Door`) (`KismetMathLibrary.RLerp` (struct) (struct :`Yaw` -125.0) _alpha) false false))
              (:`Finished`
                (switch `/Game/Objects/Enum/RotateStateEnum` (`self.Rotate State`)
                  (:`NewEnumerator2`
                    (set `self.Rotate State` "NewEnumerator0")
                    (`self.Open`))
                  (:`NewEnumerator3`
                    (set `self.Rotate State` "NewEnumerator1")
                    (`self.Close`))))))
          (:`then_1`
            (`KismetSystemLibrary.Delay` 0.3)
            (`AudioComponent.Play` (`self.washer_close_Cue`) 0.0))))
      (:`NewEnumerator1`
        (set `self.Rotate State` "NewEnumerator2")
        (`AudioComponent.Play` (`self.washer_open_Cue`) 0.0)
        (goto _label)))))

(fn `Load Data`
  (params (JSON :type String))
  (returns (Object :type "VaRestJsonObject Object Reference"))
  (bind _object (`parent.Load Data` JSON))
  (`|ExecutionSequence`
    (:`then_0`
      (bind (_has_field_ _return_value) (`/Game/Function/BP_JSON_FunctionLibrary.Get Value As Int` _object "State"))
      (if (and _has_field_ (!= _return_value (`KismetMathLibrary.Conv_ByteToInt` (`self.Rotate State`))))
        (`self.Interact` (`self.Door`))))
    (:`then_1`
      (return _object))))

(fn `Save Data`
  (returns (JSON :type "VaRestJsonObject Object Reference"))
  (bind _json (`parent.Save Data`))
  (`VaRestJsonObject.SetIntegerField` _json "State" (`KismetMathLibrary.Conv_ByteToInt` (`self.Rotate State`)))
  (return _json))

(fn `UserConstructionScript`
  (bind _componenttags (`ActorComponent.ComponentTags` (`self.Door`)))
  (if (`self.Interactive?`)
    (`KismetArrayLibrary.Array_Set` _componenttags 0 "interactive")
    (else
      (`KismetArrayLibrary.Array_Set` _componenttags))))
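; BP_Video_Recorder is an interactive, pickable VCR that plays an inserted cassette's media on a linked TV.
; Injection attaches the cassette, animates it and the door by timelines, then swaps the TV's media source and shows playtime on a looping timer.
; Interacting reverses the same timeline to eject and restore the previous source.
; Interact and pickup replicate through Server-to-All events, with pickup unlinking the TV.
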(event `/Game/Function/BP_Interface.Interact`
  (params (Component :type "PrimitiveComponent Object Reference") (Location :type "Vector Structure"))
  (if (== Component (`self.Sphere`))
    (`self.Cassette`
      (:`then`
        (`self.Interact (Server)`))
      (:`else`))))

(event `Interact (Server)`
  (`self.Interact (All)`))

(event `/Game/Function/BP_Interface.PickUp`
  (`parent.PickUp`)
  (`self.Pick Up (Server)`))

(event `Pick Up (Server)`
  (`self.Pick Up (All)`))

(event `Pick Up (All)`
  (bind _tv (`self.TV`)
    (:`then`
      (set `/Game/Objects/BP_Objects/BP_TV.Media Source` (`self.Old Media Source`) _tv)
      (`/Game/Objects/BP_Objects/BP_TV.Open Media` _tv)
      (switch `/Game/Objects/Enum/TumblerStateEnum` (`/Game/Objects/BP_Objects/BP_TV.State` _tv)
        (:`NewEnumerator0`
          (`PrimitiveComponent.SetMaterial` (`/Game/Objects/Structurs/BP_Object.Root` _tv) (`/Game/Objects/BP_Objects/BP_TV.Display Mat Id` _tv) (`/Game/Objects/BP_Objects/BP_TV.Display On` _tv))
          (`AudioComponent.Play` (`/Game/Objects/BP_Objects/BP_TV.TV Sound` _tv) 0.0)
          (`MediaPlayer.Pause` (`/Game/Objects/BP_Objects/BP_TV.Media Player` _tv)))
        (:`NewEnumerator1`
          _))
      (set `self.TV` null)
      (`KismetSystemLibrary.K2_ClearAndInvalidateTimerHandle` (`self.Play Time`))
      (`TextRenderComponent.K2_SetText` (`self.TextRender`) ""))
    (:`else`)))

(event `Injection`
  (params (Cassette :type "/Game/Objects/BP_Objects/BP_Cassette Object Reference"))
  (bind _cassette (`self.Cassette`))
  (bind _returnvalue (not (`self.Reverse`)))
  (bind _returnvalue_2 (select `bool` _returnvalue :`false` (`self.Old Media Source`) :`true` (`/Game/Objects/BP_Objects/BP_Cassette.Media Source` Cassette)))
  (set `self.Cassette` Cassette)
  (`self.K2_AttachToComponent` Cassette (`self.Cassette Pos`) "None" "SnapToTarget" "SnapToTarget" "SnapToTarget" true)
  (`self.Set Flat Mode` Cassette "NewEnumerator1")
  (`self.SetActorEnableCollision` Cassette false)
  (set `self.Reverse` false)
  (`KismetSystemLibrary.Delay` 0.2)
  (`|ExecutionSequence`
    (:`then_0`
      (bind (_direction _alpha) (`Timeline|Cassette Injection` :!label _label)
        (:`Update`
          (`SceneComponent.K2_SetRelativeLocation` (`self.Cassette Pos`) (`KismetMathLibrary.VLerp` (-9.083368 23.0 9.27) (-9.083368 11.0 9.27) _alpha) false false))
        (:`Finished`
          (bind _tv (`self.TV`)
            (:`then`
              (if _returnvalue
                (set `self.Old Media Source` (`/Game/Objects/BP_Objects/BP_TV.Media Source` _tv)))
              (set `/Game/Objects/BP_Objects/BP_TV.Media Source` _returnvalue_2 _tv)
              (`/Game/Objects/BP_Objects/BP_TV.Open Media` _tv)
              (`GameplayStatics.PlaySound2D` "/Game/Sounds/Objects/Custom/video_recorder_start.video_recorder_start" 1.0 1.0 0.0 null null)
              (`|ExecutionSequence`
                (:`then_0`
                  (`KismetSystemLibrary.Delay` 0.6)
                  (switch `/Game/Objects/Enum/TumblerStateEnum` (`/Game/Objects/BP_Objects/BP_TV.State` _tv)
                    (:`NewEnumerator0`
                      (`/Engine/EditorBlueprintResources/StandardMacros.IsValid` _returnvalue_2
                        (:`Is Valid`
                          (bind _root (`/Game/Objects/Structurs/BP_Object.Root` _tv))
                          (bind _display_mat_id (`/Game/Objects/BP_Objects/BP_TV.Display Mat Id` _tv))
                          (`PrimitiveComponent.SetMaterial` _root _display_mat_id (`/Game/Objects/BP_Objects/BP_TV.Display Media Player` _tv))
                          (bind _tv_sound (`/Game/Objects/BP_Objects/BP_TV.TV Sound` _tv))
                          (`AudioComponent.Stop` _tv_sound)
                          (bind _media_player (`/Game/Objects/BP_Objects/BP_TV.Media Player` _tv))
                          (`MediaPlayer.Play` _media_player))
                        (:`Is Not Valid`
                          (`PrimitiveComponent.SetMaterial` _root _display_mat_id (`/Game/Objects/BP_Objects/BP_TV.Display On` _tv))
                          (`AudioComponent.Play` _tv_sound 0.0)
                          (`MediaPlayer.Pause` _media_player)))
                      (if (`self.Reverse`) :!label _label_2
                        (`self.Set Flat Mode` _cassette "NewEnumerator0")
                        (`self.SetActorEnableCollision` _cassette true)
                        (`self.K2_DetachFromActor` _cassette "KeepRelative" "KeepRelative" "KeepRelative")
                        (set `self.Cassette` null)))))
                (:`then_1`
                  (if (not (`self.Reverse`))
                    (bind _returnvalue_3 (`KismetSystemLibrary.K2_SetTimerDelegate` (delegate `Get Play Time`) 1.0 true true))
                    (set `self.Play Time` _returnvalue_3)
                    (else
                      (`KismetSystemLibrary.K2_ClearAndInvalidateTimerHandle` (`self.Play Time`))
                      (`TextRenderComponent.K2_SetText` (`self.TextRender`) ""))))))
            (:`else`
              (goto _label_2))))))
    (:`then_1`
      (`self.Open / Close Door` :!label _label_3))
    (:`then_2`
      (`GameplayStatics.PlaySound2D` "/Game/Sounds/Objects/Custom/video_recorder_injection.video_recorder_injection" 1.0 1.0 0.0 null null))))

(event `Interact (All)`
  (set `self.Reverse` true)
  (`|ExecutionSequence`
    (:`then_0`
      (goto _label :!via `Reverse`))
    (:`then_1`
      (`KismetSystemLibrary.Delay` 2.0)
      (goto _label_3))))

(event `Get Play Time`
  (bind (_returnvalue_days _returnvalue_hours _returnvalue_minutes _returnvalue_seconds) (`KismetMathLibrary.BreakTimespan` (`MediaPlayer.GetTime` (`/Game/Objects/BP_Objects/BP_TV.Media Player` (`self.TV`)))))
  (`TextRenderComponent.K2_SetText` (`self.TextRender`) (`KismetTextLibrary.Conv_StringToText` (`KismetStringLibrary.Concat_StrStr` (`KismetSystemLibrary.MakeLiteralString` (`KismetStringLibrary.Conv_IntToString` _returnvalue_hours)) " : " (`KismetSystemLibrary.MakeLiteralString` (`KismetStringLibrary.Conv_IntToString` _returnvalue_minutes)) " : " (`KismetSystemLibrary.MakeLiteralString` (`KismetStringLibrary.Conv_IntToString` _returnvalue_seconds))))))

(event `Open / Close Door`
  (`/Engine/EditorBlueprintResources/StandardMacros.FlipFlop`
    (:`A`
      (bind (_direction _alpha) (`Timeline|Door Rotation` :!label _label_4)
        (:`Update`
          (`SceneComponent.K2_SetRelativeRotation` (`self.Door`) (`KismetMathLibrary.RLerp` (struct) (struct :`Roll` 90.0) _alpha) false false))))
    (:`B`
      (goto _label_4 :!via `Reverse`))))

(fn `UserConstructionScript`
  (`parent.UserConstructionScript`))
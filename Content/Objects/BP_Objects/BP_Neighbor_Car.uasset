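; The neighbor's car, with an openable trunk and doors, that drives along a spline.
; Interact picks the part by component and toggles its rotation timeline with sounds; the trunk can be locked, and RemoteOpenLeftDoor toggles the left door externally.
; MoveTimeline moves and orients the car along DrivePoint's spline at a rate inverse to DriveSpeed, calling MoveCompleted after WaitTime.
; DriveRevers runs it backwards with yaw offset flipped; DriveStop halts it.
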(event `self.Interact`
  (params (Component :type "PrimitiveComponent Object Reference") (Location :type "Vector Structure"))
  (bind (_relativerotation_roll _relativerotation_pitch) (`KismetMathLibrary.BreakRotator` (`SceneComponent.RelativeRotation` (`self.Door Right`))))
  ;[1 1 1] Interact
  (`|ExecutionSequence`
    (:`then_0`
      (if (== Component (`self.Trunk`))
        (if (not (`self.Lock Trunk`))
          (bind _isa (`/Engine/EditorBlueprintResources/StandardMacros.FlipFlop`)
            (:`A`
              (`|ExecutionSequence`
                (:`then_0`
                  (bind (_direction _alpha) (`Timeline|Trunk Rotation` :!label _label)
                    (:`Update`
                      (`SceneComponent.K2_SetRelativeRotation` (`self.Trunk`) (`KismetMathLibrary.RLerp` (struct) (struct :`Roll` 70.0) _alpha) false false))
                    (:`Finished`
                      (if (not _isa)
                        (`GameplayStatics.PlaySoundAtLocation` "/Game/Sounds/Objects/OpenClosed/car_trunk_closed_Cue.car_trunk_closed_Cue" (`self.K2_GetActorLocation`) (struct) 1.0 1.0 0.0 null null null null)))))
                (:`then_1`
                  (`GameplayStatics.PlaySoundAtLocation` "/Game/Sounds/Objects/OpenClosed/car_trunk_open_Cue.car_trunk_open_Cue" (`self.K2_GetActorLocation`) (struct) 1.0 1.0 0.0 null null null null))))
            (:`B`
              (goto _label :!via `Reverse`)))
          (else
            (`GameplayStatics.PlaySoundAtLocation` "/Game/Sounds/Objects/Noise/car_trunk_lock_Cue.car_trunk_lock_Cue" (`self.K2_GetActorLocation`) (struct) 1.0 1.0 0.0 null null null null)))))
    (:`then_1`
      (if (== Component (`self.Door Left`))
        (bind _isa_2 (`/Engine/EditorBlueprintResources/StandardMacros.FlipFlop` :!label _label_2)
          (:`A`
            (`|ExecutionSequence`
              (:`then_0`
                (bind (_direction_2 _alpha_2) (`Timeline|Left Door Rotation` :!label _label_3)
                  (:`Update`
                    (`SceneComponent.K2_SetRelativeRotation` (`self.Door Left`) (`KismetMathLibrary.RLerp` (struct) (struct :`Yaw` 50.0) _alpha_2) false false))
                  (:`Finished`
                    (if (not _isa_2)
                      (`GameplayStatics.PlaySoundAtLocation` "/Game/Sounds/Objects/OpenClosed/car_door_player_closed_Cue.car_door_player_closed_Cue" (`self.K2_GetActorLocation`) (struct) 1.0 1.0 0.0 null null null null :!label _label_4)))))
              (:`then_1`
                (`GameplayStatics.PlaySoundAtLocation` "/Game/Sounds/Objects/OpenClosed/car_door_player_open_Cue.car_door_player_open_Cue" (`self.K2_GetActorLocation`) (struct) 1.0 1.0 0.0 null null null null :!label _label_5))))
          (:`B`
            (goto _label_3 :!via `Reverse`)))))
    (:`then_2`
      (if (== Component (`self.Door Right`))
        (bind _isa_3 (`/Engine/EditorBlueprintResources/StandardMacros.FlipFlop`)
          (:`A`
            (`|ExecutionSequence`
              (:`then_0`
                (bind (_direction_3 _alpha_3) (`Timeline|Шкала времени` :!label _label_6)
                  (:`Update`
                    (`SceneComponent.K2_SetRelativeRotation` (`self.Door Right`) (`KismetMathLibrary.RLerp` (`KismetMathLibrary.MakeRotator` 0.0 _relativerotation_pitch) (`KismetMathLibrary.MakeRotator` 0.0 _relativerotation_pitch -50.0) _alpha_3) false false))
                  (:`Finished`
                    (if (not _isa_3)
                      (goto _label_4)))))
              (:`then_1`
                (goto _label_5))))
          (:`B`
            (goto _label_6 :!via `Reverse`)))))))

(event `Remote Open Left Door`
  ;[1 1 1] Interact
  (goto _label_2))

(event `self.ReceiveBeginPlay`
  ;[1 1 1] Driving
  (`TimelineComponent.SetPlayRate` (`self.Move Timeline`) (/ 1.0 (`self.Drive Speed`))))

(event `Drive`
  (bind _spline (`/Game/Sosed/BP_Drive_Point.Spline` (`self.Drive Point`)))
  (bind _spline_2 (`/Game/Sosed/BP_Drive_Point.Spline` (`self.Drive Point`)))
  ;[1 1 1] Driving
  (bind (_direction _alpha) (`Timeline|Move Timeline` :!label _label_7)
    (:`Update`
      (bind _returnvalue (`KismetMathLibrary.Lerp` 0.0 (`SplineComponent.GetDistanceAlongSplineAtSplinePoint` _spline_2 (- (`SplineComponent.GetNumberOfSplinePoints` _spline_2) 1)) _alpha))
      (`self.K2_SetActorLocation` (`SplineComponent.GetLocationAtDistanceAlongSpline` _spline _returnvalue "World"))
      (bind (_returnvalue_roll _returnvalue_pitch _returnvalue_yaw) (`KismetMathLibrary.BreakRotator` (`KismetMathLibrary.Conv_VectorToRotator` (`SplineComponent.GetTangentAtDistanceAlongSpline` _spline _returnvalue "World"))))
      (bind _result (`/Engine/EditorBlueprintResources/StandardMacros.NegateFloat` _returnvalue_pitch)
        (:`  `
          (`self.K2_SetActorRotation` (`KismetMathLibrary.MakeRotator` _result _returnvalue_roll (select `bool` (`self.Drive Back`) :`false` (- _returnvalue_yaw 90.0) :`true` (+ _returnvalue_yaw 90.0) :!type "Float (single-precision)"))))))
    (:`Finished`
      (`KismetSystemLibrary.Delay` (`self.Wait Time`))
      (`self.Move Completed`))))

(event `Drive Revers`
  ;[1 1 1] Driving
  (set `self.Drive Back` true)
  (goto _label_7 :!via `Reverse`))

(event `Drive Stop`
  ;[1 1 1] Driving
  (set `self.Drive Back` false)
  (goto _label_7 :!via `Stop`))

(fn `UserConstructionScript`)
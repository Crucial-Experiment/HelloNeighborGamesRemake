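; A lift floor stop that opens and closes its LiftDoor and lets the Sosed AI ride the Lift.
; When BP_Sosed enters the Box and the lift's state allows, it runs timed state changes and loops over the lift's floors looking for itself.
; It then sends the lift to a random floor, re-entering the loop if the pick matches the loop index.
; MoveCompleted restores the AI's walking mode and unbinds itself.
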(event `Close Door`
  (bind _lift_door (`self.Lift Door`))
  (`/Engine/EditorBlueprintResources/StandardMacros.IsValid` _lift_door
    (:`Is Valid`
      (`/Game/Objects/BP_Objects/BP_LiftDoor.Close` _lift_door))))

(event `Open Door`
  (bind _lift_door (`self.Lift Door`))
  (`/Engine/EditorBlueprintResources/StandardMacros.IsValid` _lift_door
    (:`Is Valid`
      (`/Game/Objects/BP_Objects/BP_LiftDoor.Open` _lift_door))))

(event `self.Box.OnComponentBeginOverlap`
  (params (OverlappedComponent :type "PrimitiveComponent Object Reference") (OtherActor :type "Actor Object Reference") (OtherComp :type "PrimitiveComponent Object Reference") (OtherBodyIndex :type Integer) (bFromSweep :type Boolean) (SweepResult :type "HitResult Structure (by ref)"))
  (bind _lift (`self.Lift`))
  (bind _floors (`/Game/Objects/BP_Objects/BP_Lift.Floors` _lift))
  (bind (_outitem _outindex) (`KismetArrayLibrary.Array_Random` _floors))
  ;[1 1 1] Sosed Ai
  (bind _asbp_sosed (cast `/Game/Sosed/BP_Sosed` OtherActor))
  (`/Engine/EditorBlueprintResources/StandardMacros.IsValid` _lift
    (:`Is Valid`
      (if (`|EnumInequality` (`/Game/Objects/BP_Objects/BP_Lift.State` _lift) "NewEnumerator1")
        (`KismetSystemLibrary.Delay` 3.0)
        (`/Game/Objects/BP_Objects/BP_Lift.Set State` _lift "NewEnumerator3")
        (`KismetSystemLibrary.Delay` 1.6)
        (for (_array_element _array_index) _floors :!label _label
          (`/Engine/EditorBlueprintResources/StandardMacros.IsValid` _array_element
            (:`Is Valid`
              (if (== _array_element self)
                (`KismetSystemLibrary.Delay` 1.0)
                (`/Game/Objects/BP_Objects/BP_Lift.Set State` _lift "NewEnumerator2")
                (`CharacterMovementComponent.SetMovementMode` (`Character.CharacterMovement` _asbp_sosed) "MOVE_Walking" 0)
                (else
                  (break))))
            (:`Is Not Valid`
              (break))))
        (if (!= _outindex _array_index)
          (set `/Game/Objects/BP_Objects/BP_Lift.Flour` _outindex _lift)
          (`/Game/Objects/BP_Objects/BP_Lift.Set State` _lift "NewEnumerator1")
          (add `/Game/Objects/BP_Objects/BP_Lift.Move Completed` _lift (delegate `Move Completed`))
          (else
            (goto _label)))))))

(event `self.Box.OnComponentEndOverlap`
  (params (OverlappedComponent :type "PrimitiveComponent Object Reference") (OtherActor :type "Actor Object Reference") (OtherComp :type "PrimitiveComponent Object Reference") (OtherBodyIndex :type Integer))
  ;[1 1 1] Sosed Ai
  (cast `/Game/Sosed/BP_Sosed` OtherActor))

(event `Move Completed`
  ;[1 1 1] Sosed Ai
  (`CharacterMovementComponent.SetMovementMode` (`Character.CharacterMovement` (stale `self.Box.OnComponentBeginOverlap` _asbp_sosed)) "MOVE_Walking" 0)
  (clear `/Game/Objects/BP_Objects/BP_Lift.Move Completed` (`self.Lift`)))

(fn `UserConstructionScript`)
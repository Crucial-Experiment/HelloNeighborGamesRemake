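; BP_Scoreboard is a scoreboard object that keeps a count and shows it on a widget component.
; On BeginPlay it casts the component's widget to BPW_RR_Scoreboard and caches the reference.
; ResetCount zeroes the score and shows "000", while AddCount increments it and updates the text.
; The display prepends a fixed "00" to the score, so it grows past three digits from ten onward.
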(event `self.ReceiveBeginPlay`
  (bind _asbpw_rr_scoreboard (cast `/Game/UMG/BPW_RR_Scoreboard` (`WidgetComponent.GetWidget` (`self.Widget`))))
  (set `self.RR Scoreboard` _asbpw_rr_scoreboard))

(event `Reset Count`
  (set `self.Score` 0)
  (`TextBlock.SetText` (`/Game/UMG/BPW_RR_Scoreboard.Text` (`self.RR Scoreboard`)) "000"))

(event `Add Count`
  (`/Engine/EditorBlueprintResources/StandardMacros.IncrementInt` (`self.Score`)
    (:`  `
      (`TextBlock.SetText` (`/Game/UMG/BPW_RR_Scoreboard.Text` (`self.RR Scoreboard`)) (`KismetTextLibrary.Conv_StringToText` (`KismetStringLibrary.Concat_StrStr` "00" (`KismetStringLibrary.Conv_IntToString` (`self.Score`))))))))

(fn `UserConstructionScript`)
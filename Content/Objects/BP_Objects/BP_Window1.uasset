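; Breakable window that the neighbor AI (Sosed) investigates when broken and gets boarded up on restore after three breaks.
; A fast BP_Object hit or BrokeGlass call goes through a server-to-multicast event that hides the glass, spawns temporary shards and sends the neighbor's blackboard a Check task.
; The window spawns a nav link only while the neighbor is in Attack, and SosedJump shatters the glass without counting a break.
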(event `Neighbor Check`
  (params (Neighbor :type "/Game/Sosed/BP_Sosed Object Reference") (Damage :type "PrimitiveComponent Object Reference"))
  (bind _returnvalue (`AIBlueprintHelperLibrary.GetBlackboard` Neighbor))
  (bind _scene (`self.Scene`))
  ;[1 1 1] Check Window
  (if (`|EnumInequality` (`/Game/Sosed/BP_Sosed.Current State` Neighbor) "NewEnumerator2")
    (`BlackboardComponent.SetValueAsInt` _returnvalue "CheckTask" 0)
    (`BlackboardComponent.SetValueAsObject` _returnvalue "CheckActor" self)
    (`BlackboardComponent.SetValueAsVector` _returnvalue "Check Location" (`SceneComponent.K2_GetComponentLocation` Damage))
    (`BlackboardComponent.SetValueAsRotator` _returnvalue "Check Rotation" (`SceneComponent.K2_GetComponentRotation` Damage))
    (`BlackboardComponent.SetValueAsVector` _returnvalue "Check Point Location" (`SceneComponent.K2_GetComponentLocation` _scene))
    (`BlackboardComponent.SetValueAsVector` _returnvalue "Check Point Forward" (`SceneComponent.GetForwardVector` _scene))
    (`/Game/Sosed/BP_Sosed.Set State` Neighbor "NewEnumerator3")))

(event `Sosed Jump`
  (bind (_returnvalue_location _returnvalue_rotation) (`KismetMathLibrary.BreakTransform` (`SceneComponent.K2_GetComponentToWorld` (`self.Glass`))))
  ;[1 1 1] Sosed Jump
  (`self.Win Collision` false)
  (bind _returnvalue (`|SpawnActorFromClass` "/Game/Objects/Destroy/BP_GC_Glass.BP_GC_Glass_C" (`KismetMathLibrary.MakeTransform` _returnvalue_location _returnvalue_rotation) "Undefined" "MultiplyWithRoot" null null))
  (`KismetSystemLibrary.Delay` 2.5)
  (`self.K2_DestroyActor` _returnvalue))

(event `Broke Glass`
  ;[1 1 1] Window 1
  (`/Engine/EditorBlueprintResources/StandardMacros.DoOnce` false
    (:`Completed`
      (`self.Broke Glass (Server)` :!label _label))))

(event `Restoring Windows`
  ;[1 1 1] Restoring Windows
  (`self.Win Collision` true (`self.Glass`))
  (`self.Check Boarded`))

(event `self.Glass.OnComponentHit`
  (params (HitComponent :type "PrimitiveComponent Object Reference") (OtherActor :type "Actor Object Reference") (OtherComp :type "PrimitiveComponent Object Reference") (NormalImpulse :type "Vector Structure") (Hit :type "HitResult Structure (by ref)"))
  ;[1 1 1] Window 1
  (bind _asbp_object (cast `/Game/Objects/Structurs/BP_Object` OtherActor))
  (if (`self.Could Be Broken`)
    (if (>= (`KismetMathLibrary.VSize` (`self.GetVelocity` _asbp_object)) 200.0)
      (goto _label))))

(event `Broke Glass (All)`
  (bind _glass (`self.Glass`))
  (bind (_returnvalue_location _returnvalue_rotation) (`KismetMathLibrary.BreakTransform` (`SceneComponent.K2_GetComponentToWorld` _glass)))
  ;[1 1 1] Window 1
  (`self.Win Collision` false _glass)
  (bind _returnvalue (`|SpawnActorFromClass` (`self.Destroy Class`) (`KismetMathLibrary.MakeTransform` _returnvalue_location _returnvalue_rotation) "Undefined" "MultiplyWithRoot" null null))
  (`/Engine/EditorBlueprintResources/StandardMacros.IncrementInt` (`self.Broken Count`)
    (:`  `
      (set `/Game/Objects/Destroy/BP_GC_Glass.Glass Break` (`self.Glass Break`) _returnvalue)
      (`KismetSystemLibrary.Delay` 2.5)
      (`self.K2_DestroyActor` _returnvalue)
      (`/Game/Objects/Tutorial/TutorialComponent.Check Use Type` (`self.TutorialComponent`) "NewEnumerator7")
      (`/Game/Objects/GameJolt/GameJoltComponent.Check Use Type` (`self.GameJoltComponent`) "NewEnumerator7")
      (bind _sosed (`/Game/Function/BP_MacroLibrary.Find Sosed`)
        (:`Is Valid`
          (`self.Neighbor Check` _sosed (`self.Check Arrow`)))))))

(event `Broke Glass (Server)`
  ;[1 1 1] Window 1
  (`self.Broke Glass (All)`))

(event `self.ReceiveBeginPlay`
  (bind _childactor (`ChildActorComponent.ChildActor` (`self.Nav Link Proxy`)))
  (`|ExecutionSequence`
    (:`then_0`
      (if (`self.Start Boarded`)
        (`self.Add Boarded`)))
    (:`then_1`
      (bind _sosed (`/Game/Function/BP_MacroLibrary.Find Sosed`)
        (:`Is Valid`
          (add `/Game/Sosed/BP_Sosed.State Mode Change` _sosed (delegate `On Sosed State Mode Change`)))))
    (:`then_2`
      (`/Engine/EditorBlueprintResources/StandardMacros.IsValid` _childactor
        (:`Is Valid`
          (`self.K2_DestroyActor` _childactor))))))

(event `On Sosed State Mode Change`
  (params (`New State` :type "/Game/Sosed/Ai/Struct/Sosed_Stage_Enum Enum" :default "NewEnumerator0"))
  (bind _nav_temp (`self.Nav Temp`))
  (switch `/Game/Sosed/Ai/Struct/Sosed_Stage_Enum` `New State`
    (:`NewEnumerator0`
      (`/Engine/EditorBlueprintResources/StandardMacros.IsValid` _nav_temp :!label _label_2
        (:`Is Valid`
          (`self.K2_DestroyActor` _nav_temp))))
    (:`NewEnumerator1`
      (goto _label_2))
    (:`NewEnumerator2`
      (`/Engine/EditorBlueprintResources/StandardMacros.IsValid` _nav_temp
        (:`Is Not Valid`
          (bind _returnvalue (`|SpawnActorFromClass` "/Game/Objects/Structurs/BP_NavLinkProxy.BP_NavLinkProxy_C" (`self.Nav Temp Tranfs`) "Undefined" "MultiplyWithRoot" null null))
          (bind _output_get (set `self.Nav Temp` _returnvalue))
          (`/Game/Objects/Structurs/BP_NavLinkProxy.Set Nav Link` _output_get (`self.Left`) (`self.Right`) (`self.Direction`)))))
    (:`NewEnumerator3`
      (goto _label_2))))

(fn `Add Boarded`
  (bind _boarded_mesh (`self.Boarded Mesh`))
  (bind _returnvalue (or (`self.Boarded`) (`self.Start Boarded`)))
  (`SceneComponent.SetVisibility` (`self.Boarded Mesh`) _returnvalue false)
  (if _returnvalue
    (`PrimitiveComponent.SetCollisionEnabled` _boarded_mesh "QueryAndPhysics")
    (else
      (`PrimitiveComponent.SetCollisionEnabled` _boarded_mesh "NoCollision"))))

(fn `Check Boarded`
  (if (and (not (`self.Boarded`)) (>= (`self.Broken Count`) 3))
    (`SceneComponent.SetVisibility` (`self.Boarded Mesh`) true false)
    (`PrimitiveComponent.SetCollisionEnabled` (`self.Boarded Mesh`) "QueryAndPhysics")
    (set `self.Could Be Broken` false)
    (set `self.Boarded` true)))

(fn `UserConstructionScript`
  (bind _nav_link_proxy (`self.Nav Link Proxy`))
  (`self.Add Boarded`)
  (bind _asbp_nav_link_proxy (cast `/Game/Objects/Structurs/BP_NavLinkProxy` (`ChildActorComponent.ChildActor` _nav_link_proxy)))
  (`/Game/Objects/Structurs/BP_NavLinkProxy.Set Nav Link` _asbp_nav_link_proxy (`self.Left`) (`self.Right`) (`self.Direction`))
  (set `self.Nav Temp` _asbp_nav_link_proxy)
  (set `self.Nav Temp Tranfs` (`SceneComponent.K2_GetComponentToWorld` _nav_link_proxy)))

(fn `Win Collision`
  (params (`On / Off` :type Boolean) (`Win Mesh` :type "PrimitiveComponent Object Reference"))
  (`SceneComponent.SetVisibility` `Win Mesh` `On / Off` false)
  (`PrimitiveComponent.SetCollisionEnabled` `Win Mesh` (select `bool` `On / Off` :`false` "NoCollision" :`true` "QueryAndPhysics" :!type "ECollisionEnabled Enum")))
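; BP_Egg is a physical egg that breaks on impacts above a speed threshold, reusing tomato sound and splash assets.
; Hitting BP_Player shows a screen splash widget, hitting BP_Sosed just destroys the egg, and other surfaces get a BP_Egg_Splat.
; Window hits also alert the Sosed AI, unless in an excluded state, by writing a check task, window and splat to its Blackboard and switching state.
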(event `self.Root.OnComponentHit`
  (params (HitComponent :type "PrimitiveComponent Object Reference") (OtherActor :type "Actor Object Reference") (OtherComp :type "PrimitiveComponent Object Reference") (NormalImpulse :type "Vector Structure") (Hit :type "HitResult Structure (by ref)"))
  (bind (_returnvalue_roll _returnvalue_pitch _returnvalue_yaw) (`KismetMathLibrary.BreakRotator` (`self.K2_GetActorRotation`)))
  (bind (_bblockinghit _binitialoverlap _time _distance _location) (`GameplayStatics.BreakHitResult` Hit))
  (if (>= (`KismetMathLibrary.VSize` (`self.GetVelocity`)) 150.0)
    (`GameplayStatics.PlaySoundAtLocation` "/Game/Sounds/Human/tomato_fase_Cue.tomato_fase_Cue" _location (struct) 1.0 1.0 0.0 null null null null)
    (cast `/Game/Player/BP_Player` OtherActor
      (:`then`
        (bind _returnvalue (`|CreateWidget` "/Game/UMG/Other/BPW_Tomato_Splash.BPW_Tomato_Splash_C"))
        (`UserWidget.AddToViewport` _returnvalue 0)
        (`self.K2_DestroyActor` :!label _label))
      (:`CastFailed`
        (cast `/Game/Sosed/BP_Sosed` OtherActor
          (:`then`
            (goto _label))
          (:`CastFailed`
            (bind _returnvalue_2 (`|SpawnActorFromClass` "/Game/Objects/BP_Objects/BP_Egg_Splat.BP_Egg_Splat_C" (`KismetMathLibrary.MakeTransform` _location (`KismetMathLibrary.MakeRotator` 0.0 0.0 _returnvalue_yaw)) "Undefined" "OverrideRootScale" null null))
            (bind _asbp_window_1 (cast `/Game/Objects/BP_Objects/BP_Window1` OtherActor)
              (:`then`
                (bind _sosed (`/Game/Function/BP_MacroLibrary.Find Sosed`)
                  (:`Is Valid`
                    (if (`|EnumInequality` (`/Game/Sosed/BP_Sosed.Current State` _sosed) "NewEnumerator2")
                      (bind _returnvalue_3 (`AIBlueprintHelperLibrary.GetBlackboard` _sosed))
                      (`BlackboardComponent.SetValueAsInt` _returnvalue_3 "CheckTask" 7)
                      (`BlackboardComponent.SetValueAsObject` _returnvalue_3 "CheckActor" _asbp_window_1)
                      (`BlackboardComponent.SetValueAsObject` _returnvalue_3 "DestroyActor" _returnvalue_2)
                      (`/Game/Sosed/BP_Sosed.Set State` _sosed "NewEnumerator3")
                      (`self.K2_DestroyActor` :!label _label_2)))
                  (:`Is Not Valid`
                    (goto _label_2))))
              (:`CastFailed`
                (goto _label_2)))))))))

(fn `UserConstructionScript`
  (`parent.UserConstructionScript`))
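; BP_UV_Light is a holdable UV flashlight item that reveals BP_Invisibility objects it points at.
; VR use, or left-click while held, toggles it through a server-to-all state event driving light, sound, bulb material and tutorial/GameJolt checks; slot changes switch it off.
; Each Tick hides the last revealed object, then, while on, line-traces from the player camera or VR trace point to reveal the hit one.
; Its on/off state persists in JSON save data.
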(event `Set State (All)`
  (params (`New State` :type "/Game/Objects/Enum/TumblerStateEnum Enum" :default "NewEnumerator0"))
  (bind _root (`self.Root`))
  (bind _tutorialcomponent (`self.TutorialComponent`))
  (bind _gamejoltcomponent (`self.GameJoltComponent`))
  (bind _spotlight (`self.SpotLight`))
  (bind _output_get (set `self.State` `New State`))
  (switch `/Game/Objects/Enum/TumblerStateEnum` _output_get
    (:`NewEnumerator0`
      (`SceneComponent.SetVisibility` _spotlight true false)
      (set `self.State` "NewEnumerator0")
      (`AudioComponent.Play` (`self.flashlight_on`) 0.0)
      (`PrimitiveComponent.SetMaterial` _root 1 "/Game/Objects/Materials/dl_uv_bulb_m.dl_uv_bulb_m")
      (`/Game/Objects/Tutorial/TutorialComponent.Check Use Type` _tutorialcomponent "NewEnumerator4")
      (`/Game/Objects/GameJolt/GameJoltComponent.Check Use Type` _gamejoltcomponent "NewEnumerator4"))
    (:`NewEnumerator1`
      (`SceneComponent.SetVisibility` _spotlight false false)
      (set `self.State` "NewEnumerator1")
      (`AudioComponent.Play` (`self.flashlight_off`) 0.0)
      (`PrimitiveComponent.SetMaterial` _root 1 "/Game/Objects/Materials/bulb_glass_m.bulb_glass_m")
      (`/Game/Objects/Tutorial/TutorialComponent.Check Use Type` _tutorialcomponent "NewEnumerator3")
      (`/Game/Objects/GameJolt/GameJoltComponent.Check Use Type` _gamejoltcomponent "NewEnumerator3"))))

(event `Set State (Server)`
  (params (`New State` :type "/Game/Objects/Enum/TumblerStateEnum Enum" :default "NewEnumerator0"))
  (`self.Set State (All)` `New State`))

(event `On Slot Change_1`
  (`self.Set State (Server)` "NewEnumerator1"))

(event `self.On VR Use`
  (`parent.On VR Use`)
  (`self.Set State (Server)` (select `/Game/Objects/Enum/TumblerStateEnum` (`self.State`) :`NewEnumerator0` "NewEnumerator1" :`NewEnumerator1` "NewEnumerator0" :!type "/Game/Objects/Enum/TumblerStateEnum Enum") :!label _label))

(event `self.ReceiveBeginPlay`
  (`parent.ReceiveBeginPlay`))

(event `On Press LMB_1`
  (bind _player (`/Game/Function/BP_MacroLibrary.Find Player`)
    (:`Is Valid`
      (bind _item (`/Game/Player/BP_Player.Get Item` _player))
      (if (== _item self)
        (goto _label)))))

(event `self.ReceiveTick`
  (params (DeltaSeconds :type "Float (single-precision)"))
  (bind _invisibility (`self.Invisibility`))
  (`|ExecutionSequence`
    (:`then_0`
      (`/Engine/EditorBlueprintResources/StandardMacros.IsValid` _invisibility
        (:`Is Valid`
          (`/Game/Objects/BP_Objects/BP_Invisibility.Hidden` _invisibility)
          (set `self.Invisibility` null))))
    (:`then_1`
      (switch `/Game/Objects/Enum/TumblerStateEnum` (`self.State`)
        (:`NewEnumerator0`
          (bind _returnvalue (select `bool` (`/Game/Player/BP_Player.Start VR` (stale `On Press LMB_1` _player)) :`false` (select `/Game/Player/Functions/PlayerModel_Enum` (`/Game/Player/BP_Player.Model` (stale `On Press LMB_1` _player)) :`NewEnumerator0` (`/Game/Player/BP_Player.Camera` (stale `On Press LMB_1` _player)) :!type "SceneComponent Object Reference") :`true` (`self.Trace`)))
          (bind _returnvalue_2 (`SceneComponent.K2_GetComponentLocation` _returnvalue))
          (bind (_outhit _returnvalue_3) (`KismetSystemLibrary.LineTraceSingle` _returnvalue_2 (+ _returnvalue_2 (* (`SceneComponent.GetForwardVector` _returnvalue) 500.0)) "TraceTypeQuery1"))
          (if _returnvalue_3
            (bind _asbp_invisibility (cast `/Game/Objects/BP_Objects/BP_Invisibility` (`.HitActor` (`GameplayStatics.BreakHitResult` _outhit))))
            (`/Game/Objects/BP_Objects/BP_Invisibility.Visibility` _asbp_invisibility)
            (set `self.Invisibility` _asbp_invisibility)))))))

(fn `Load Data`
  (params (JSON :type String))
  (returns (Object :type "VaRestJsonObject Object Reference"))
  (bind _object (`parent.Load Data` JSON))
  (`|ExecutionSequence`
    (:`then_0`
      (bind (_has_field_ _return_value) (`/Game/Function/BP_JSON_FunctionLibrary.Get Value As Int` _object "State"))
      (if (and _has_field_ (!= _return_value (`KismetMathLibrary.Conv_ByteToInt` (`self.State`))))
        (`self.On VR Use`)))
    (:`then_1`
      (return _object))))

(fn `Save Data`
  (returns (JSON :type "VaRestJsonObject Object Reference"))
  (bind _json (`parent.Save Data`))
  (`VaRestJsonObject.SetIntegerField` _json "State" (`KismetMathLibrary.Conv_ByteToInt` (`self.State`)))
  (return _json))

(fn `UserConstructionScript`
  (`parent.UserConstructionScript`))
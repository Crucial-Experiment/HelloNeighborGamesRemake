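; BP_LiftCall is a call button that summons a linked lift to its floor.
; Interaction or VR hand overlap on the button goes through a server event to all clients, gated by a DoOnce that resets when the lift completes moving.
; A call notifies tutorial and GameJolt components, then sets lift state directly if already on that floor, otherwise changes state, waits briefly, assigns the floor and changes state again.
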(event `self.ReceiveBeginPlay`
  (`/Engine/EditorBlueprintResources/StandardMacros.IsValid` (`self.Lift`)
    (:`Is Valid`
      (add `/Game/Objects/BP_Objects/BP_Lift.Move Completed` (`self.Lift`) (delegate `Reset Do Once`)))))

(event `Reset Do Once`
  (bind _lift (`self.Lift`))
  (goto _label_2 :!via `Reset`))

(event `/Game/Function/BP_Interface.Interact`
  (params (Component :type "PrimitiveComponent Object Reference") (Location :type "Vector Structure"))
  (if (== Component (`self.Button`))
    (`self.Interact (Server)` :!label _label)))

(event `Interact (All)`
  (bind _lift (`self.Lift`))
  (`/Engine/EditorBlueprintResources/StandardMacros.IsValid` _lift
    (:`Is Valid`
      (`/Engine/EditorBlueprintResources/StandardMacros.DoOnce` false :!label _label_2
        (:`Completed`
          (`/Game/Objects/Tutorial/TutorialComponent.Check Use Type` (`self.TutorialComponent`) "NewEnumerator6")
          (`/Game/Objects/GameJolt/GameJoltComponent.Check Use Type` (`self.GameJoltComponent`) "NewEnumerator6")
          (if (== (`/Game/Objects/BP_Objects/BP_Lift.Flour` _lift) (`self.Flour`))
            (`/Game/Objects/BP_Objects/BP_Lift.Set State` _lift "NewEnumerator2")
            (else
              (`/Game/Objects/BP_Objects/BP_Lift.Set State` _lift "NewEnumerator3")
              (`KismetSystemLibrary.Delay` 1.6)
              (set `/Game/Objects/BP_Objects/BP_Lift.Flour` (`self.Flour`) _lift)
              (`/Game/Objects/BP_Objects/BP_Lift.Set State` _lift "NewEnumerator1"))))))))

(event `self.Button.OnComponentBeginOverlap`
  (params (OverlappedComponent :type "PrimitiveComponent Object Reference") (OtherActor :type "Actor Object Reference") (OtherComp :type "PrimitiveComponent Object Reference") (OtherBodyIndex :type Integer) (bFromSweep :type Boolean) (SweepResult :type "HitResult Structure (by ref)"))
  (if (`self.Overlap VR Hands` OtherActor OtherComp)
    (goto _label)))

(event `Interact (Server)`
  (`self.Interact (All)`))

(fn `UserConstructionScript`)
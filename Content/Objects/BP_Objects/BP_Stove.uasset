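; BP_Stove is an interactable stove that toggles on and off and heats actors standing in its hot zone.
; Interact switches fire, light and sounds, waiting for the start sound before igniting, and notifies the tutorial and GameJolt components.
; While lit, HotZone overlaps start a looping timer that plays a timeline writing Temperature to the overlapping actor's TemperatureComponent.
; Switching off or ending overlap resets that timer.
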(event `/Game/Function/BP_Interface.Interact`
  (params (Component :type "PrimitiveComponent Object Reference") (Location :type "Vector Structure"))
  (bind _start_cue (`self.Start Cue`))
  (`/Game/Objects/Tutorial/TutorialComponent.Check Use Type` (`self.TutorialComponent`) "NewEnumerator6")
  (`/Game/Objects/GameJolt/GameJoltComponent.Check Use Type` (`self.GameJoltComponent`) "NewEnumerator5")
  (switch `/Game/Objects/Enum/TumblerStateEnum` (`self.State`)
    (:`NewEnumerator0`
      (`SceneComponent.SetVisibility` (`self.Fire`) false false)
      (`SceneComponent.SetVisibility` (`self.PointLight`) false false)
      (`AudioComponent.Stop` (`self.Loop Cue`))
      (`AudioComponent.Play` (`self.End Cue`) 0.0)
      (set `PrimitiveComponent.bGenerateOverlapEvents` false (`self.Hot Zone`))
      (`KismetSystemLibrary.K2_SetTimerDelegate` (delegate `Make Hot`))
      (set `self.State` "NewEnumerator1"))
    (:`NewEnumerator1`
      (`AudioComponent.Play` _start_cue 0.0)
      (bind _returnvalue (message `AnimationDataModel.GetPlayLength` _start_cue))
      (`KismetSystemLibrary.Delay` _returnvalue)
      (`SceneComponent.SetVisibility` (`self.Fire`) true false)
      (`SceneComponent.SetVisibility` (`self.PointLight`) true false)
      (`AudioComponent.Play` (`self.Loop Cue`) 0.0)
      (set `PrimitiveComponent.bGenerateOverlapEvents` true (`self.Hot Zone`))
      (set `self.State` "NewEnumerator0"))))

(event `Make Hot`
  (bind (_direction _temperature) (`Timeline|Шкала времени`)
    (:`Update`
      (set `/Game/Objects/Structurs/TemperatureComponent.Temperature` _temperature (`self.GetComponentByClass` (stale `self.Hot Zone.OnComponentBeginOverlap` OtherActor) "/Game/Objects/Structurs/TemperatureComponent.TemperatureComponent_C")))))

(event `self.Hot Zone.OnComponentBeginOverlap`
  (params (OverlappedComponent :type "PrimitiveComponent Object Reference") (OtherActor :type "Actor Object Reference") (OtherComp :type "PrimitiveComponent Object Reference") (OtherBodyIndex :type Integer) (bFromSweep :type Boolean) (SweepResult :type "HitResult Structure (by ref)"))
  (`/Engine/EditorBlueprintResources/StandardMacros.IsValid` (`self.GetComponentByClass` OtherActor "/Game/Objects/Structurs/TemperatureComponent.TemperatureComponent_C")
    (:`Is Valid`
      (`KismetSystemLibrary.K2_SetTimerDelegate` (delegate `Make Hot`) 0.1 true true))))

(event `self.Hot Zone.OnComponentEndOverlap`
  (params (OverlappedComponent :type "PrimitiveComponent Object Reference") (OtherActor :type "Actor Object Reference") (OtherComp :type "PrimitiveComponent Object Reference") (OtherBodyIndex :type Integer))
  (`KismetSystemLibrary.K2_SetTimerDelegate` (delegate `Make Hot`))
  (`/Engine/EditorBlueprintResources/StandardMacros.IsValid` (`self.GetComponentByClass` OtherActor "/Game/Objects/Structurs/TemperatureComponent.TemperatureComponent_C")))

(fn `UserConstructionScript`)
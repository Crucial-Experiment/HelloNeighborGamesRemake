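; Kitchen cabinet actor with two doors that swing open and closed independently when interacted with.
; The Interact event checks which door component was hit and branches on that door's rotation state, acting only when it is fully open or closed.
; A timeline per door plays or reverses to lerp its relative rotation in mirrored directions, then settles the state on finish.
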(event `/Game/Function/BP_Interface.Interact`
  (params (Component :type "PrimitiveComponent Object Reference") (Location :type "Vector Structure"))
  (`|ExecutionSequence`
    (:`then_0`
      (if (== Component (`self.Door 1`))
        (switch `/Game/Objects/Enum/RotateStateEnum` (`self.Door 1 Rotate`)
          (:`NewEnumerator0`
            (set `self.Door 1 Rotate` "NewEnumerator3")
            (bind (_direction _alpha) (`Timeline|Door 1 Rotate Timeline` :!via `Reverse` :!label _label)
              (:`Update`
                (`SceneComponent.K2_SetRelativeRotation` (`self.Door 1`) (`KismetMathLibrary.RLerp` (struct) (struct :`Yaw` 100.0) _alpha) false false))
              (:`Finished`
                (switch `/Game/Objects/Enum/RotateStateEnum` (`self.Door 1 Rotate`)
                  (:`NewEnumerator2`
                    (set `self.Door 1 Rotate` "NewEnumerator0"))
                  (:`NewEnumerator3`
                    (set `self.Door 1 Rotate` "NewEnumerator1"))))))
          (:`NewEnumerator1`
            (set `self.Door 1 Rotate` "NewEnumerator2")
            (`|ExecutionSequence`
              (:`then_0`
                (goto _label)))))))
    (:`then_1`
      (if (== Component (`self.Door 2`))
        (switch `/Game/Objects/Enum/RotateStateEnum` (`self.Door 2 Rotate`)
          (:`NewEnumerator0`
            (set `self.Door 2 Rotate` "NewEnumerator3")
            (bind (_direction_2 _alpha_2) (`Timeline|Door 2 Rotate Timeline` :!via `Reverse` :!label _label_2)
              (:`Update`
                (`SceneComponent.K2_SetRelativeRotation` (`self.Door 2`) (`KismetMathLibrary.RLerp` (struct) (struct :`Yaw` -100.0) _alpha_2) false false))
              (:`Finished`
                (switch `/Game/Objects/Enum/RotateStateEnum` (`self.Door 2 Rotate`)
                  (:`NewEnumerator2`
                    (set `self.Door 2 Rotate` "NewEnumerator0"))
                  (:`NewEnumerator3`
                    (set `self.Door 2 Rotate` "NewEnumerator1"))))))
          (:`NewEnumerator1`
            (set `self.Door 2 Rotate` "NewEnumerator2")
            (`|ExecutionSequence`
              (:`then_0`
                (goto _label_2)))))))))

(fn `UserConstructionScript`)
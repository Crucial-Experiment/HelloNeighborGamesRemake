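; Powered elevator that moves between placed Floor actors, registering itself with them and an optional attached Panel on BeginPlay.
; SetState drives Stop, Move, Open Door and Close Door, operating the child-actor car door and current floor's door together.
; Moves use MoveComponentTo with optional rotation, opening doors after a short delay on arrival.
; Movement and doors require electricity or a generator; power changes halt or resume travel, and state and floor are saved.
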(event `Close Door`
  ;[1 1 1] Open / Close Door
  (bind _asbp_lift_door (cast `/Game/Objects/BP_Objects/BP_LiftDoor` (`ChildActorComponent.ChildActor` (`self.Door`))))
  (`/Game/Objects/BP_Objects/BP_LiftDoor.Close` _asbp_lift_door))

(event `Move`
  (params (Floor :type Integer))
  (bind _returnvalue (or (`self.Has Electricity`) (`self.Generator`)))
  (bind _output (`|GetArrayItem` (`self.Floors`) Floor))
  ;[1 1 1] Move
  (if _returnvalue
    (set `self.Flour` Floor)
    (`KismetSystemLibrary.MoveComponentTo` (`self.Root`) (`self.K2_GetActorLocation` _output) (select `bool` (`self.Use Rotation?`) :`false` (`self.K2_GetActorRotation`) :`true` (`self.K2_GetActorRotation` _output)) false false (`self.Speed`) :!label _label)
    (if _returnvalue
      (`KismetSystemLibrary.Delay` 1.0)
      (`self.Set State` "NewEnumerator2")
      (`self.Move Completed`))))

(event `Move Stop`
  ;[1 1 1] Move
  (goto _label :!via `Stop`))

(event `Open Door`
  ;[1 1 1] Open / Close Door
  (bind _asbp_lift_door (cast `/Game/Objects/BP_Objects/BP_LiftDoor` (`ChildActorComponent.ChildActor` (`self.Door`))))
  (`/Game/Objects/BP_Objects/BP_LiftDoor.Open` _asbp_lift_door))

(event `self.ReceiveBeginPlay`
  ;[1 1 1] Begin Play
  (`|ExecutionSequence`
    (:`then_0`
      (bind _panel (`self.Panel`)
        (:`then`
          (set `/Game/Objects/BP_Objects/BP_LiftButton.Lift` self _panel)
          (`/Game/Objects/BP_Objects/BP_LiftButton.Update Floors` _panel))
        (:`else`)))
    (:`then_1`
      (`self.Set State` (`self.State`)))
    (:`then_2`
      (for _array_element (`self.Floors`)
        (`/Engine/EditorBlueprintResources/StandardMacros.IsValid` _array_element
          (:`Is Valid`
            (set `/Game/Objects/BP_Objects/BP_LiftFloor.Lift` self _array_element)))))))

(event `self.Enable`
  ;[1 1 1] Electricity
  (`parent.Enable`)
  (if (`|EnumEquality` (`self.State`) "NewEnumerator1")
    (`self.Move` (`self.Flour`))))

(event `self.Disable`
  ;[1 1 1] Electricity
  (`parent.Disable`)
  (`self.Move Stop`))

(fn `Load Data`
  (params (JSON :type String))
  (returns (Object :type "VaRestJsonObject Object Reference"))
  (bind _object (`parent.Load Data` JSON))
  (`|ExecutionSequence`
    (:`then_0`
      (bind (_has_field_ _return_value) (`/Game/Function/BP_JSON_FunctionLibrary.Get Value As Int` _object "Flour"))
      (if _has_field_
        (set `self.Flour` _return_value)))
    (:`then_1`
      (bind (_has_field__2 _return_value_2) (`/Game/Function/BP_JSON_FunctionLibrary.Get Value As Int` _object "State"))
      (if (and _has_field__2 (!= _return_value_2 (`KismetMathLibrary.Conv_ByteToInt` (`self.State`))))
        (`self.Set State` (cast `/Game/Objects/Enum/ElevatorStateEnum` (`KismetMathLibrary.Conv_IntToByte` _return_value_2)))))
    (:`then_2`
      (return _object))))

(fn `Save Data`
  (returns (JSON :type "VaRestJsonObject Object Reference"))
  (bind _json (`parent.Save Data`))
  (`VaRestJsonObject.SetIntegerField` _json "State" (`KismetMathLibrary.Conv_ByteToInt` (`self.State`)))
  (`VaRestJsonObject.SetIntegerField` _json "Flour" (`self.Flour`))
  (return _json))

(fn `Set State`
  (params (`New State` :type "/Game/Objects/Enum/ElevatorStateEnum Enum" :default "NewEnumerator0"))
  (bind _returnvalue (or (`self.Has Electricity`) (`self.Generator`)))
  (bind _output (`|GetArrayItem` (`self.Floors`) (`self.Flour`)))
  (bind _output_get (set `self.State` `New State`))
  (switch `/Game/Objects/Enum/ElevatorStateEnum` _output_get
    (:`NewEnumerator0`
      (`self.Move Stop`))
    (:`NewEnumerator1`
      (`self.Move` (`self.Flour`)))
    (:`NewEnumerator2`
      (`/Engine/EditorBlueprintResources/StandardMacros.IsValid` _output
        (:`Is Valid`
          (if _returnvalue
            (`/Game/Objects/BP_Objects/BP_LiftFloor.Open Door` _output)
            (`self.Open Door`)
            (`self.Set State` "NewEnumerator0" :!label _label)))))
    (:`NewEnumerator3`
      (`/Engine/EditorBlueprintResources/StandardMacros.IsValid` _output
        (:`Is Valid`
          (if _returnvalue
            (`/Game/Objects/BP_Objects/BP_LiftFloor.Close Door` _output)
            (`self.Close Door`)
            (goto _label)))))))

(fn `UserConstructionScript`
  (bind _panel (`self.Panel`)
    (:`then`
      (`self.K2_AttachToComponent` _panel (`self.Panel Loc`) "None" "SnapToTarget" "SnapToTarget" "SnapToTarget" true))
    (:`else`)))
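; Umbrella item for desktop and VR that toggles open and closed, swapping its mesh and playing a sound.
; Pickup, grab and drop set or clear the player's Umbrella reference.
; LMB or VR use toggles it and notifies tutorial and GameJolt components; slot changes force it closed if it is the player's current item.
; State saves to JSON; loading replays the use toggle when it differs, side effects included.
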(event `self.GrabComponent.OnGrabbed`
  (params (`Self Ref` :type "/Game/Objects/Structurs/GrabComponent Object Reference"))
  (bind _player (`/Game/Function/BP_MacroLibrary.Find Player` :!label _label)
    (:`Is Valid`
      (set `/Game/Player/BP_Player.Umbrella` self _player))))

(event `/Game/Function/BP_Interface.PickUp`
  (`parent.PickUp`)
  (goto _label))

(event `On Item Dropped_1`
  (bind _player (`/Game/Function/BP_MacroLibrary.Find Player` :!label _label_2)
    (:`Is Valid`
      (set `/Game/Player/BP_Player.Umbrella` null _player))))

(event `self.GrabComponent.OnDropped`
  (params (`Self Ref` :type "/Game/Objects/Structurs/GrabComponent Object Reference"))
  (goto _label_2))

(event `On Slot Change_1`
  (bind _player (`/Game/Function/BP_MacroLibrary.Find Player`)
    (:`Is Valid`
      (bind _item (`/Game/Player/BP_Player.Get Item` _player))
      (if (== _item self)
        ;[1 1 1] Use
        (set `self.State` "NewEnumerator1" :!label _label_3)
        (`StaticMeshComponent.SetStaticMesh` (`self.Root`) "/Game/Objects/Meshes/umbrella_close_new.umbrella_close_new")
        (`GameplayStatics.PlaySound2D` "/Game/Sounds/Objects/OpenClosed/umbrella_close_Cue.umbrella_close_Cue" 1.0 1.0 0.0 null null)))))

(event `self.On VR Use`
  ;[1 1 1] Use
  (`parent.On VR Use`)
  (`/Game/Objects/Tutorial/TutorialComponent.Check Use Type` (`self.TutorialComponent`) "NewEnumerator6" :!label _label_4)
  (`/Game/Objects/GameJolt/GameJoltComponent.Check Use Type` (`self.GameJoltComponent`) "NewEnumerator6")
  (switch `/Game/Objects/Enum/TumblerStateEnum` (`self.State`)
    (:`NewEnumerator0`
      (goto _label_3))
    (:`NewEnumerator1`
      (set `self.State` "NewEnumerator0")
      (`StaticMeshComponent.SetStaticMesh` (`self.Root`) "/Game/Objects/Meshes/umbrella_new.umbrella_new")
      (`GameplayStatics.PlaySound2D` "/Game/Sounds/Objects/OpenClosed/umbrella_open_Cue.umbrella_open_Cue" 1.0 1.0 0.0 null null))))

(event `On Press LMB_1`
  ;[1 1 1] Use
  (bind _player (`/Game/Function/BP_MacroLibrary.Find Player`)
    (:`Is Valid`
      (bind _item (`/Game/Player/BP_Player.Get Item` _player))
      (if (== _item self)
        (goto _label_4)))))

(fn `Load Data`
  (params (JSON :type String))
  (returns (Object :type "VaRestJsonObject Object Reference"))
  (bind _object (`parent.Load Data` JSON))
  (`|ExecutionSequence`
    (:`then_0`
      (bind (_has_field_ _return_value) (`/Game/Function/BP_JSON_FunctionLibrary.Get Value As Int` _object "State"))
      (if (and _has_field_ (!= _return_value (`KismetMathLibrary.Conv_ByteToInt` (`self.State`))))
        (`self.On VR Use`)))
    (:`then_1`
      (return _object))))

(fn `Save Data`
  (returns (JSON :type "VaRestJsonObject Object Reference"))
  (bind _json (`parent.Save Data`))
  (`VaRestJsonObject.SetIntegerField` _json "State" (`KismetMathLibrary.Conv_ByteToInt` (`self.State`)))
  (return _json))

(fn `UserConstructionScript`
  (`parent.UserConstructionScript`))
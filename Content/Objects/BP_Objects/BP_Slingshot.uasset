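; BP_Slingshot is a usable slingshot that fires a random projectile from its SpawnClass list.
; VR use, or left click while the player holds it, updates tutorial and GameJolt checks, then calls a server shot.
; A DoOnce-gated timeline animates the Part with sound, then spawns the projectile and resets.
; The launch impulse follows player 0's camera forward, even though it runs on the server.
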(event `self.On VR Use`
  (`parent.On VR Use`)
  (`/Game/Objects/Tutorial/TutorialComponent.Check Use Type` (`self.TutorialComponent`) "NewEnumerator6" :!label _label)
  (`/Game/Objects/GameJolt/GameJoltComponent.Check Use Type` (`self.GameJoltComponent`) "NewEnumerator8")
  (`self.Shot (Server)`))

(event `Shot (Server)`
  (bind _part (`self.Part`))
  (bind _part_2 (`self.Part`))
  (`/Engine/EditorBlueprintResources/StandardMacros.DoOnce` false :!label _label_2
    (:`Completed`
      (`GameplayStatics.PlaySound2D` "/Game/Sounds/Objects/Loop/air_rifle_shot_Cue.air_rifle_shot_Cue" 1.0 1.0 0.0 null null)
      (bind (_direction _alpha) (`Timeline|Shot` :!via `PlayFromStart`)
        (:`Update`
          (`SceneComponent.K2_SetRelativeRotation` _part (struct :`Roll` 90.0) false false)
          (`SceneComponent.K2_SetRelativeLocation` _part (`KismetMathLibrary.VLerp` (0.0 -20.625184 18.15299) (0.0 -7.625184 22.15299) _alpha) false false))
        (:`Finished`
          (bind _returnvalue (`|SpawnActorFromClass` (`KismetArrayLibrary.Array_Random` (`self.Spawn Class`)) (`SceneComponent.K2_GetComponentToWorld` (`self.Scene`)) "Undefined" "MultiplyWithRoot" null null))
          (`PrimitiveComponent.AddImpulse` (`/Game/Objects/Structurs/BP_Object.Root` _returnvalue) (* (`self.GetActorForwardVector` (`GameplayStatics.GetPlayerCameraManager` 0)) (`self.Shot Power`)) "None" false)
          (`SceneComponent.K2_SetRelativeRotation` :`self` _part_2)
          (`SceneComponent.K2_SetRelativeLocation` _part_2 (0.0 -10.0 1.0) false false)
          (goto _label_2 :!via `Reset`))))))

(event `self.On Press LMB`
  (bind _player (`/Game/Function/BP_MacroLibrary.Find Player`)
    (:`Is Valid`
      (bind _item (`/Game/Player/BP_Player.Get Item` _player))
      (if (== _item self)
        (goto _label)))))

(fn `UserConstructionScript`
  (`parent.UserConstructionScript`))
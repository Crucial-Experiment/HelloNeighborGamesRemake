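; BP_Invisibility is a text actor that starts hidden in game and can be shown or hidden through events.
; The construction script applies the text, alignment, font, color and world size variables to its TextRender component.
; BeginPlay runs the parent logic and then calls Hidden, while the Visibility and Hidden events toggle the whole actor's in-game visibility.
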(event `self.ReceiveBeginPlay`
  (`parent.ReceiveBeginPlay`)
  (`self.Hidden`))

(event `Visibility`
  (`self.SetActorHiddenInGame` self false))

(event `Hidden`
  (`self.SetActorHiddenInGame` self true))

(fn `UserConstructionScript`
  (bind _textrender (`self.TextRender`))
  (`parent.UserConstructionScript`)
  (`TextRenderComponent.K2_SetText` _textrender (`KismetTextLibrary.Conv_StringToText` (`self.Text`)))
  (`TextRenderComponent.SetHorizontalAlignment` _textrender (`self.Horizontal Alignment`))
  (`TextRenderComponent.SetFont` _textrender (`self.Font`))
  (`TextRenderComponent.SetTextRenderColor` _textrender (`self.Color`))
  (`TextRenderComponent.SetWorldSize` _textrender (`self.World Size`)))
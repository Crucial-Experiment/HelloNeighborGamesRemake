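; BP_School_Clock is a school clock that acts like a bell schedule, switching linked electrical objects and the states of students and teachers.
; A looping timer, run while powered and paced by Speed, rotates the hand one degree per tick.
; Every other time pitch reaches 5 degrees, tracked by the Counting toggle, it powers the Electricity objects for WorkingTime and calls SetState on every BP_Student and BP_Teacher.
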(event `Count`
  (bind _part (`self.Part`))
  (bind _electricity (`self.Electricity`))
  (bind (_relativerotation_roll _relativerotation_pitch) (`KismetMathLibrary.BreakRotator` (`SceneComponent.RelativeRotation` _part)))
  (`SceneComponent.K2_AddLocalRotation` _part (struct :`Pitch` -1.0) false false)
  (if (`KismetMathLibrary.NearlyEqual_FloatFloat` _relativerotation_pitch 5.0)
    (if (`self.Counting`)
      (set `self.Counting` false)
      (`|ExecutionSequence`
        (:`then_0`
          (for _array_element _electricity
            (`self.Enable` _array_element))
          (`KismetSystemLibrary.Delay` (`self.Working Time`))
          (for _array_element_2 _electricity
            (`self.Disable` _array_element_2)))
        (:`then_1`
          (bind _outactors (`GameplayStatics.GetAllActorsOfClass` "/Game/Objects/NPC/BP_Student.BP_Student_C"))
          (for _array_element_3 _outactors
            (`/Game/Objects/NPC/BP_Student.Set State` _array_element_3)))
        (:`then_2`
          (bind _outactors_2 (`GameplayStatics.GetAllActorsOfClass` "/Game/Objects/NPC/BP_Teacher.BP_Teacher_C"))
          (for _array_element_4 _outactors_2
            (`/Game/Objects/NPC/BP_Teacher.Set State` _array_element_4))))
      (else
        (set `self.Counting` true)))))

(event `self.ReceiveBeginPlay`
  (`parent.ReceiveBeginPlay`)
  (if (`self.Has Electricity`)
    (bind _returnvalue (`KismetSystemLibrary.K2_SetTimerDelegate` (delegate `Count`) (/ (`self.Speed`) 10.0) true :!label _label))
    (set `self.Timer` _returnvalue)))

(event `self.Enable`
  (`parent.Enable`)
  (goto _label))

(event `self.Disable`
  (`parent.Disable`)
  (`KismetSystemLibrary.K2_ClearAndInvalidateTimerHandle` (`self.Timer`)))

(fn `UserConstructionScript`
  (`parent.UserConstructionScript`))
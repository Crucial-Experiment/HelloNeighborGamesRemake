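; BP_Teleport is a trigger actor that moves the player or the neighbor (BP_Sosed) to the world location of its Billboard component.
; Box overlap runs two checks, gated by the PlayerOnly and NeighborOnly flags, each casting to its character class before teleporting without sweep.
; The player branch also reports a use type to the TutorialComponent and GameJoltComponent before the move.
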(event `self.Box.OnComponentBeginOverlap`
  (params (OverlappedComponent :type "PrimitiveComponent Object Reference") (OtherActor :type "Actor Object Reference") (OtherComp :type "PrimitiveComponent Object Reference") (OtherBodyIndex :type Integer) (bFromSweep :type Boolean) (SweepResult :type "HitResult Structure (by ref)"))
  (`|ExecutionSequence`
    (:`then_0`
      (if (`self.Player Only`)
        (cast `/Game/Player/BP_Player` OtherActor)
        (`/Game/Objects/Tutorial/TutorialComponent.Check Use Type` (`self.TutorialComponent`) "NewEnumerator6")
        (`/Game/Objects/GameJolt/GameJoltComponent.Check Use Type` (`self.GameJoltComponent`) "NewEnumerator6")
        (`self.K2_SetActorLocation` OtherActor (`SceneComponent.K2_GetComponentLocation` (`self.Billboard`)) false true :!label _label)))
    (:`then_1`
      (if (`self.Neighbor Only`)
        (cast `/Game/Sosed/BP_Sosed` OtherActor)
        (goto _label)))))

(fn `UserConstructionScript`)
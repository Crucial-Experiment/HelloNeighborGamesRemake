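; BP_Crying_Neighbor is a crying neighbor object that reacts when the player enters its trigger box.
; On overlap with BP_Player, it runs a GameJolt component use-type check and adds the configured widget class to the viewport, if set.
; If a sound is assigned, it plays it at the actor's location and stops the Crying component.
; Nothing limits repeat triggers, so each overlap runs the sequence again.
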(event `self.Box.OnComponentBeginOverlap`
  (params (OverlappedComponent :type "PrimitiveComponent Object Reference") (OtherActor :type "Actor Object Reference") (OtherComp :type "PrimitiveComponent Object Reference") (OtherBodyIndex :type Integer) (bFromSweep :type Boolean) (SweepResult :type "HitResult Structure (by ref)"))
  (bind _widget (`self.Widget`))
  (bind _sound (`self.Sound`))
  (cast `/Game/Player/BP_Player` OtherActor)
  (`/Game/Objects/GameJolt/GameJoltComponent.Check Use Type` (`self.GameJoltComponent`) "NewEnumerator6")
  (if (`KismetSystemLibrary.IsValidClass` _widget)
    (bind _returnvalue (`|CreateWidget` _widget))
    (`UserWidget.AddToViewport` _returnvalue 0))
  (`/Engine/EditorBlueprintResources/StandardMacros.IsValid` _sound
    (:`Is Valid`
      (`GameplayStatics.PlaySoundAtLocation` _sound (`self.K2_GetActorLocation`) (struct) 1.0 1.0 0.0 null null null null)
      (`AudioComponent.Stop` (`self.Crying`)))))

(fn `UserConstructionScript`)
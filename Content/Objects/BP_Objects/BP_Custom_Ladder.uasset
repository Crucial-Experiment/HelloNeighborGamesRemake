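; Modular climbable ladder that supports both VR and non-VR players.
; The construction script stacks Count middle mesh segments and an optional top piece, each with a climb-tagged grab component, then fits the trigger boxes, end markers and nav link to the height.
; For non-VR players, entering BoxIn switches movement to Flying and sets IsLadder through server events, while leaving BoxIn or BoxOut restores Walking.
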(event `Box In (Server)`
  (params (Character :type "/Game/Player/BP_Player Object Reference"))
  (set `/Game/Player/BP_Player.Is Ladder` true Character)
  (`CharacterMovementComponent.SetMovementMode` (`Character.CharacterMovement` Character) "MOVE_Flying" 0))

(event `Box Out (Server)`
  (params (Character :type "/Game/Player/BP_Player Object Reference"))
  (set `/Game/Player/BP_Player.Is Ladder` false Character)
  (`CharacterMovementComponent.SetMovementMode` (`Character.CharacterMovement` Character) "MOVE_Walking" 0))

(event `self.Box In.OnComponentBeginOverlap`
  (params (OverlappedComponent :type "PrimitiveComponent Object Reference") (OtherActor :type "Actor Object Reference") (OtherComp :type "PrimitiveComponent Object Reference") (OtherBodyIndex :type Integer) (bFromSweep :type Boolean) (SweepResult :type "HitResult Structure (by ref)"))
  (bind _asbp_player (cast `/Game/Player/BP_Player` OtherActor))
  (if (not (`/Game/Player/BP_Player.Start VR` _asbp_player))
    (`self.Box In (Server)` _asbp_player)))

(event `self.Box Out.OnComponentEndOverlap`
  (params (OverlappedComponent :type "PrimitiveComponent Object Reference") (OtherActor :type "Actor Object Reference") (OtherComp :type "PrimitiveComponent Object Reference") (OtherBodyIndex :type Integer))
  (bind _asbp_player (cast `/Game/Player/BP_Player` OtherActor))
  (if (not (`/Game/Player/BP_Player.Start VR` _asbp_player))
    (`self.Box Out (Server)` _asbp_player)))

(event `self.Box In.OnComponentEndOverlap`
  (params (OverlappedComponent :type "PrimitiveComponent Object Reference") (OtherActor :type "Actor Object Reference") (OtherComp :type "PrimitiveComponent Object Reference") (OtherBodyIndex :type Integer))
  (bind _asbp_player (cast `/Game/Player/BP_Player` OtherActor))
  (if (not (`/Game/Player/BP_Player.Start VR` _asbp_player))
    (`self.Box Out (Server)` _asbp_player)))

(fn `UserConstructionScript`
  (bind _box_out (`self.Box Out`))
  (bind _box_in (`self.Box In`))
  (bind _box_out_2 (`self.Box Out`))
  (bind _end_top_point (`self.End Top Point`))
  (bind _bottom_direction (`self.Bottom Direction`))
  (bind _box_in_2 (`self.Box In`))
  (bind _returnvalue (`StaticMesh.GetBoundingBox` (`self.Middle Mesh`)))
  (bind (_relativelocation_x _relativelocation_y) (`KismetMathLibrary.BreakVector` (`SceneComponent.RelativeLocation` _box_in_2)))
  (bind (_boxextent_x _boxextent_y) (`KismetMathLibrary.BreakVector` (`BoxComponent.BoxExtent` _box_out_2)))
  (bind (_boxextent_x_2 _boxextent_y_2) (`KismetMathLibrary.BreakVector` (`BoxComponent.BoxExtent` _box_in)))
  (bind (_relativelocation_x_2 _relativelocation_y_2) (`KismetMathLibrary.BreakVector` (`SceneComponent.RelativeLocation` _bottom_direction)))
  (bind (_relativelocation_x_3 _relativelocation_y_3) (`KismetMathLibrary.BreakVector` (`SceneComponent.RelativeLocation` (`self.End Top Direction`))))
  (bind (_relativelocation_x_4 _relativelocation_y_4) (`KismetMathLibrary.BreakVector` (`SceneComponent.RelativeLocation` _box_out)))
  (bind (_relativelocation_x_5 _relativelocation_y_5) (`KismetMathLibrary.BreakVector` (`SceneComponent.RelativeLocation` _end_top_point)))
  (bind _returnvalue_2 (- (.z (`.Max` (break `Box` _returnvalue))) (.z (break `Box` _returnvalue))))
  (bind _returnvalue_3 (* (- (.x (`.Max` (break `Box` _returnvalue))) (.x (break `Box` _returnvalue))) 0.3))
  (bind _returnvalue_4 (* (`self.Count`) _returnvalue_2))
  (bind _returnvalue_5 (`KismetMathLibrary.Conv_IntToDouble` _returnvalue_4))
  (bind _returnvalue_6 (/ _returnvalue_4 2))
  (bind _returnvalue_7 (`KismetMathLibrary.Conv_IntToDouble` (- _returnvalue_6 0)))
  (for _index (range (`self.Count`))
    (bind _returnvalue_8 (`AddComponent|NODE_AddStaticMeshComponent-0` :`bManualAttachment` true :`RelativeTransform` (`KismetMathLibrary.MakeTransform` (`KismetMathLibrary.MakeVector` 0.0 0.0 (`KismetMathLibrary.Conv_IntToDouble` (* _index _returnvalue_2))))))
    (`StaticMeshComponent.SetStaticMesh` _returnvalue_8 (`self.Middle Mesh`))
    (`SceneComponent.K2_AttachToComponent` _returnvalue_8 (`self.Root`) "None" "KeepRelative" "KeepRelative" "KeepRelative" true)
    (bind _returnvalue_9 (`AddComponent|NODE_AddGrabComponent-0`))
    (`SceneComponent.K2_AttachToComponent` _returnvalue_9 _returnvalue_8 "None" "SnapToTarget" "SnapToTarget" "SnapToTarget" true)
    (set `/Game/Objects/Structurs/GrabComponent.GrabType` "NewEnumerator3" _returnvalue_9)
    (set `ActorComponent.ComponentTags` (`|MakeArray` "climb" :!type "Name") _returnvalue_9))
  (`SceneComponent.K2_SetRelativeLocation` _box_in_2 (`KismetMathLibrary.MakeVector` 0.0 _relativelocation_y (`KismetMathLibrary.Conv_IntToDouble` _returnvalue_6)) false false)
  (`BoxComponent.SetBoxExtent` _box_in (`KismetMathLibrary.MakeVector` _returnvalue_3 _boxextent_y_2 _returnvalue_7) true)
  (`SceneComponent.K2_SetRelativeLocation` _box_out (`KismetMathLibrary.MakeVector` 0.0 _relativelocation_y_4 (`KismetMathLibrary.Conv_IntToDouble` _returnvalue_6)) false false)
  (`BoxComponent.SetBoxExtent` _box_out_2 (`KismetMathLibrary.MakeVector` _returnvalue_3 _boxextent_y _returnvalue_7) true)
  (`SceneComponent.K2_SetRelativeLocation` (`self.End Top Direction`) (`KismetMathLibrary.MakeVector` _relativelocation_x_3 _relativelocation_y_3 (- _returnvalue_5 140.0)) false false)
  (`SceneComponent.K2_SetRelativeLocation` _bottom_direction (`KismetMathLibrary.MakeVector` _relativelocation_x_2 _relativelocation_y_2 _returnvalue_5) false false)
  (`SceneComponent.K2_SetRelativeLocation` _end_top_point (`KismetMathLibrary.MakeVector` _relativelocation_x_5 _relativelocation_y_5 (+ _returnvalue_5 100.0)) false false)
  (bind _asbp_nav_link_proxy (cast `/Game/Objects/Structurs/BP_NavLinkProxy` (`ChildActorComponent.ChildActor` (`self.Nav Link`)))
    (:`then`
      (`/Game/Objects/Structurs/BP_NavLinkProxy.Set Nav Link` _asbp_nav_link_proxy (0.0 70.0 20.0) (`KismetMathLibrary.MakeVector` 0.0 -70.0 (- _returnvalue_5 30.0)) "Auto"))
    (:`CastFailed`
      _))
  (if (`self.Top Attachment`)
    (bind _returnvalue_10 (`AddComponent|NODE_AddStaticMeshComponent-2` :`bManualAttachment` true :`RelativeTransform` (`KismetMathLibrary.MakeTransform` (`KismetMathLibrary.MakeVector` 0.0 0.0 _returnvalue_5))))
    (`SceneComponent.K2_AttachToComponent` _returnvalue_10 (`self.Root`) "None" "KeepRelative" "KeepRelative" "KeepRelative" true)
    (bind _returnvalue_11 (`AddComponent|NODE_AddGrabComponent-1`))
    (`SceneComponent.K2_AttachToComponent` _returnvalue_11 _returnvalue_10 "None" "SnapToTarget" "SnapToTarget" "SnapToTarget" true)
    (set `/Game/Objects/Structurs/GrabComponent.GrabType` "NewEnumerator3" _returnvalue_11)
    (set `ActorComponent.ComponentTags` (`|MakeArray` "climb" :!type "Name") _returnvalue_11)))
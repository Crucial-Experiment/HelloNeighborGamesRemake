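; BP_Hand_Wheel is a carryable valve wheel that players attach to a matching BP_Tube_Main and turn to toggle it open or closed.
; Using it while held line-traces for a tube, drops the wheel and snaps it to the tube's position and state-based rotation.
; Interacting plays the tube's animation and a rotation timeline, updating tube state when finished.
; Attach, interact and pickup replicate through Server-to-All events; pickup clears the tube link.
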(event `self.ReceiveBeginPlay`
  (`parent.ReceiveBeginPlay`))

(event `self.On VR Use`
  (`parent.On VR Use`)
  (bind _actor (`self.Line Trace` 300.0 "NewEnumerator1" :!label _label))
  (bind _asbp_tube_main (cast `/Game/Objects/Structurs/BP_Tube_Main` _actor))
  (`/Game/Objects/Tutorial/TutorialComponent.Check Use Type` (`self.TutorialComponent`) "NewEnumerator6")
  (`/Game/Objects/GameJolt/GameJoltComponent.Check Use Type` (`self.GameJoltComponent`) "NewEnumerator6")
  (if (== (`/Game/Objects/Structurs/BP_Tube_Main.Apply Class` _asbp_tube_main) (`GameplayStatics.GetObjectClass` self))
    (`/Game/Objects/Structurs/FlatComponent.Drop Item` (`self.FlatComponent`) 0.0)
    (`self.Try Release`)
    (if (`/Game/Function/BP_GameInstance.Online Mode` (`/Game/Function/BP_FunctionLibrary.Get Game Instance`))
      (`KismetSystemLibrary.Delay` 0.35))
    (`self.LMB (Server)` _asbp_tube_main)))

(event `self.On Press LMB`
  (`parent.On Press LMB`)
  (bind _player (`/Game/Function/BP_MacroLibrary.Find Player`)
    (:`Is Valid`
      (bind _item (`/Game/Player/BP_Player.Get Item` _player))
      (if (== _item self)
        (goto _label)))))

(event `LMB (Server)`
  (params (Tube :type "/Game/Objects/Structurs/BP_Tube_Main Object Reference"))
  (`self.LMB (All)` Tube))

(event `Interact (Server)`
  (`self.Interact (All)`))

(event `LMB (All)`
  (params (Tube :type "/Game/Objects/Structurs/BP_Tube_Main Object Reference"))
  (bind _scene (`/Game/Objects/Structurs/BP_Tube_Main.Scene` Tube))
  (bind _root (`self.Root`))
  (bind _state (`/Game/Objects/Structurs/BP_Tube_Main.State` Tube))
  (bind (_returnvalue_roll _returnvalue_pitch _returnvalue_yaw) (`KismetMathLibrary.BreakRotator` (select `/Game/Objects/Enum/HandWheelRotationEnum` (`/Game/Objects/Structurs/BP_Tube_Main.Apply Rotation` Tube) :`NewEnumerator0` (struct :`Yaw` 90.0) :`NewEnumerator1` (struct :`Yaw` 90.0 :`Roll` 90.0) :`NewEnumerator2` (struct :`Yaw` 90.0 :`Roll` 90.0) :`NewEnumerator3` (struct :`Yaw` 90.0 :`Roll` 180.0) :`NewEnumerator4` (`/Game/Objects/Structurs/BP_Tube_Main.Apply Custom Rotation End` Tube))))
  (`self.Set Flat Mode` "NewEnumerator1")
  (`SceneComponent.K2_SetWorldLocation` _root (`SceneComponent.K2_GetComponentLocation` _scene) false false)
  (`SceneComponent.K2_SetWorldRotation` _root (`KismetMathLibrary.MakeRotator` (select `/Game/Objects/Enum/TumblerStateEnum` _state :`NewEnumerator0` _returnvalue_roll :`NewEnumerator1` (.roll (`SceneComponent.K2_GetComponentRotation` _scene))) (select `/Game/Objects/Enum/TumblerStateEnum` _state :`NewEnumerator0` _returnvalue_pitch :`NewEnumerator1` (.pitch (`SceneComponent.K2_GetComponentRotation` _scene))) (select `/Game/Objects/Enum/TumblerStateEnum` _state :`NewEnumerator0` _returnvalue_yaw :`NewEnumerator1` (.yaw (`SceneComponent.K2_GetComponentRotation` _scene)))) false false)
  (set `self.Tube` Tube)
  (`/Game/Objects/Structurs/FlatComponent.Play Use Anim` (`self.FlatComponent`) false false))

(event `/Game/Function/BP_Interface.Interact`
  (params (Component :type "PrimitiveComponent Object Reference") (Location :type "Vector Structure"))
  (`self.Interact (Server)`))

(event `Interact (All)`
  (bind _tube (`self.Tube`))
  (bind _tube_2 (`self.Tube`))
  (bind _apply_rotation (`/Game/Objects/Structurs/BP_Tube_Main.Apply Rotation` _tube))
  (`/Engine/EditorBlueprintResources/StandardMacros.IsValid` _tube_2
    (:`Is Valid`
      (`AudioComponent.Play` (`/Game/Objects/Structurs/BP_Tube_Main.open_closed` _tube_2) 0.0)
      (switch `/Game/Objects/Enum/TumblerStateEnum` (`/Game/Objects/Structurs/BP_Tube_Main.State` _tube_2)
        (:`NewEnumerator0`
          (bind (_direction _alpha) (`Timeline|Rotation Timeline` :!via `Reverse` :!label _label_2)
            (:`Update`
              (`SceneComponent.K2_SetRelativeRotation` (`self.Root`) (`KismetMathLibrary.RLerp` (select `/Game/Objects/Enum/HandWheelRotationEnum` _apply_rotation :`NewEnumerator1` (struct :`Pitch` 90.0) :`NewEnumerator2` (struct :`Pitch` -90.0 :`Roll` 180.0) :`NewEnumerator3` (struct :`Roll` 180.0) :`NewEnumerator4` (`/Game/Objects/Structurs/BP_Tube_Main.Apply Custom Rotation Start` _tube)) (select `/Game/Objects/Enum/HandWheelRotationEnum` _apply_rotation :`NewEnumerator0` (struct :`Yaw` 90.0) :`NewEnumerator1` (struct :`Yaw` 90.0 :`Roll` 90.0) :`NewEnumerator2` (struct :`Yaw` 90.0 :`Roll` 90.0) :`NewEnumerator3` (struct :`Yaw` 90.0 :`Roll` 180.0) :`NewEnumerator4` (`/Game/Objects/Structurs/BP_Tube_Main.Apply Custom Rotation End` _tube)) _alpha true) false false))
            (:`Finished`
              (bind _tube_3 (`self.Tube`)
                (:`then`
                  (`/Game/Objects/Structurs/BP_Tube_Main.Set State` _tube_3))
                (:`else`)))))
        (:`NewEnumerator1`
          (goto _label_2))))))

(event `Pick Up (All)`
  (set `self.Tube` null)
  (goto _label_2 :!via `Stop`))

(event `/Game/Function/BP_Interface.PickUp`
  (`parent.PickUp`)
  (`self.Pick Up (Server)`))

(event `Pick Up (Server)`
  (`self.Pick Up (All)`))

(fn `UserConstructionScript`
  (`parent.UserConstructionScript`))
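; Interactive, networked boiler with a hinged door, valve spigot, temperature gauge and combustion trigger.
; Interactions replicate via server-to-all events; timelines animate door and spigot, whose state machine shifts the gauge temperature.
; Finished valve turns toggle the linked Water's frozen state (frozen when open) and notify tutorial and GameJolt components.
; BP_Burning actors entering the trigger burn after their combustion time unless they leave or cannot burn.
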(event `Interact (All)`
  (params (Component :type "PrimitiveComponent Object Reference"))
  (bind _returnvalue (`self.K2_GetActorLocation`))
  (bind _temperatire (`self.Temperatire`))
  (`|ExecutionSequence`
    (:`then_0`
      ;[1 1 1] Door
      (if (== Component (`self.Door`))
        (`/Engine/EditorBlueprintResources/StandardMacros.FlipFlop`
          (:`A`
            (bind (_direction _alpha) (`Timeline|Boiler Door Timeline` :!label _label)
              (:`Update`
                (`SceneComponent.K2_SetRelativeRotation` (`self.Door`) (`KismetMathLibrary.RLerp` (struct) (struct :`Yaw` -55.0) _alpha) false false))))
          (:`B`
            (goto _label :!via `Reverse`)))))
    (:`then_1`
      ;[1 1 1] Spigot
      (if (== Component (`self.Spigot`))
        (switch `/Game/Objects/Enum/RotateStateEnum` (`self.Spigot State`)
          (:`NewEnumerator0`
            (`GameplayStatics.PlaySoundAtLocation` "/Game/Sounds/Objects/TurnOnOff/valve_spin_on_Cue.valve_spin_on_Cue" _returnvalue (struct) 1.0 1.0 0.0 null null null null)
            (set `self.Spigot State` "NewEnumerator3")
            (bind (_direction_2 _alpha_2) (`Timeline|Spigot Timeline` :!via `Reverse` :!label _label_2)
              (:`Update`
                (`SceneComponent.K2_SetRelativeRotation` (`self.Spigot`) (`KismetMathLibrary.RLerp` (struct) (struct :`Roll` 180.0) _alpha_2) false false)
                (switch `/Game/Objects/Enum/RotateStateEnum` (`self.Spigot State`)
                  (:`NewEnumerator0`
                    (set `self.Temperatire` (`KismetMathLibrary.FClamp` (+ _temperatire 5.0) 0.0 70.0) :!label _label_3))
                  (:`NewEnumerator2`
                    (goto _label_3))
                  (:`NewEnumerator1`
                    (set `self.Temperatire` (`KismetMathLibrary.FClamp` (- _temperatire 5.0) -70.0 0.0) :!label _label_4))
                  (:`NewEnumerator3`
                    (goto _label_4))))
              (:`Finished`
                (switch `/Game/Objects/Enum/RotateStateEnum` (`self.Spigot State`)
                  (:`NewEnumerator2`
                    (set `self.Spigot State` "NewEnumerator0")
                    (`self.Frozen State (Server)` true))
                  (:`NewEnumerator3`
                    (set `self.Spigot State` "NewEnumerator1")
                    (`self.Frozen State (Server)` false)))
                (`/Game/Objects/Tutorial/TutorialComponent.Check Use Type` (`self.TutorialComponent`) "NewEnumerator6")
                (`/Game/Objects/GameJolt/GameJoltComponent.Check Use Type` (`self.GameJoltComponent`) "NewEnumerator6"))))
          (:`NewEnumerator1`
            (`GameplayStatics.PlaySoundAtLocation` "/Game/Sounds/Objects/TurnOnOff/valve_spin_off_Cue.valve_spin_off_Cue" _returnvalue (struct) 1.0 1.0 0.0 null null null null)
            (set `self.Spigot State` "NewEnumerator2")
            (goto _label_2)))))))

(event `self.ReceiveTick`
  (params (DeltaSeconds :type "Float (single-precision)"))
  (`SceneComponent.K2_SetRelativeRotation` (`self.Arrow`) (`KismetMathLibrary.MakeRotator` (`self.Temperatire`)) false false))

(event `Frozen State (Server)`
  (params (Frozen :type Boolean))
  ;[1 1 1] Server
  (`self.Frozen State (All)` Frozen))

(event `Interact (Server)`
  (params (Component :type "PrimitiveComponent Object Reference"))
  ;[1 1 1] Server
  (`self.Interact (All)` Component))

(event `self.Combustion Trigger.OnComponentBeginOverlap`
  (params (OverlappedComponent :type "PrimitiveComponent Object Reference") (OtherActor :type "Actor Object Reference") (OtherComp :type "PrimitiveComponent Object Reference") (OtherBodyIndex :type Integer) (bFromSweep :type Boolean) (SweepResult :type "HitResult Structure (by ref)"))
  ;[1 1 1] Combustion Trigger
  (bind _asbp_burning (cast `/Game/Objects/Structurs/BP_Burning` OtherActor))
  (set `/Game/Objects/Structurs/BP_Burning.Starting Burn` true _asbp_burning)
  (`KismetSystemLibrary.Delay` (`/Game/Objects/Structurs/BP_Burning.Combustion Time` _asbp_burning))
  (if (and (`/Game/Objects/Structurs/BP_Burning.Starting Burn` _asbp_burning) (`/Game/Objects/Structurs/BP_Burning.Can Be Burned` _asbp_burning))
    (`/Game/Objects/Structurs/BP_Burning.Burned` _asbp_burning)))

(event `Frozen State (All)`
  (params (Frozen :type Boolean))
  ;[1 1 1] Server
  (bind _water (`self.Water`)
    (:`then`
      (`/Game/Objects/BP_Objects/BP_Water.Frozen State` _water Frozen))
    (:`else`)))

(event `/Game/Function/BP_Interface.Interact`
  (params (Component :type "PrimitiveComponent Object Reference") (Location :type "Vector Structure"))
  ;[1 1 1] Server
  (`self.Interact (Server)` Component))

(event `self.Combustion Trigger.OnComponentEndOverlap`
  (params (OverlappedComponent :type "PrimitiveComponent Object Reference") (OtherActor :type "Actor Object Reference") (OtherComp :type "PrimitiveComponent Object Reference") (OtherBodyIndex :type Integer))
  ;[1 1 1] Combustion Trigger
  (bind _asbp_burning (cast `/Game/Objects/Structurs/BP_Burning` OtherActor))
  (set `/Game/Objects/Structurs/BP_Burning.Starting Burn` false _asbp_burning))

(fn `UserConstructionScript`
  (`SceneComponent.K2_SetRelativeRotation` (`self.Arrow`) (`KismetMathLibrary.MakeRotator` (`self.Temperatire`)) false false))
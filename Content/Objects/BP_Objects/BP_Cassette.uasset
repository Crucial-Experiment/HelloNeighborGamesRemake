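; BP_Cassette is a holdable cassette object that players insert into a video recorder.
; VR use, or left click while the player holds it, line-traces for a BP_Video_Recorder and, on a hit, releases the cassette.
; A server-to-all event chain then calls Injection on the recorder with the cassette and reports the use type to the tutorial and GameJolt components.
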(event `self.On VR Use`
  (`parent.On VR Use`)
  (bind _actor (`self.Line Trace` 1500.0 :!label _label))
  (bind _asbp_video_recorder (cast `/Game/Objects/BP_Objects/BP_Video_Recorder` _actor))
  (`self.Try Release`)
  (`self.Interact (Server)` _asbp_video_recorder))

(event `self.ReceiveBeginPlay`
  (`parent.ReceiveBeginPlay`))

(event `On Press LMB_1`
  (bind _player (`/Game/Function/BP_MacroLibrary.Find Player`)
    (:`Is Valid`
      (bind _item (`/Game/Player/BP_Player.Get Item` _player))
      (if (== _item self)
        (goto _label)))))

(event `Interact (Server)`
  (params (`Video Recorder` :type "/Game/Objects/BP_Objects/BP_Video_Recorder Object Reference"))
  (`self.Interact (All)` `Video Recorder`))

(event `Interact (All)`
  (params (`Video Recorder` :type "/Game/Objects/BP_Objects/BP_Video_Recorder Object Reference"))
  (`/Game/Objects/Tutorial/TutorialComponent.Check Use Type` (`self.TutorialComponent`) "NewEnumerator6")
  (`/Game/Objects/GameJolt/GameJoltComponent.Check Use Type` (`self.GameJoltComponent`) "NewEnumerator6")
  (`/Game/Objects/BP_Objects/BP_Video_Recorder.Injection` `Video Recorder` self))

(fn `UserConstructionScript`
  (`parent.UserConstructionScript`))
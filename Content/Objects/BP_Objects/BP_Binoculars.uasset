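; BP_Binoculars is a usable item that toggles a zoomed binocular view on and off.
; VR use, or left mouse press while the player holds it, reports to the Tutorial and GameJolt components, then adds or removes the BPW_Binoculars overlay and switches the player's field of view.
; Each toggle passes the state to a BP_Binoculars_Text actor.
; RemoveWidget forces the state off and clears the overlay without restoring field of view.
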(event `self.ReceiveBeginPlay`
  (`parent.ReceiveBeginPlay`))

(event `Text Check`
  (bind _returnvalue (`GameplayStatics.GetActorOfClass` "/Game/AngryNeighborFiles/BP_Binoculars_Text.BP_Binoculars_Text_C"))
  (`/Engine/EditorBlueprintResources/StandardMacros.IsValid` _returnvalue
    (:`Is Valid`
      (`/Game/AngryNeighborFiles/BP_Binoculars_Text.Set Text State` _returnvalue (`self.State`)))))

(event `self.On VR Use`
  (`parent.On VR Use`)
  (`/Game/Objects/Tutorial/TutorialComponent.Check Use Type` (`self.TutorialComponent`) "NewEnumerator6" :!label _label)
  (`/Game/Objects/GameJolt/GameJoltComponent.Check Use Type` (`self.GameJoltComponent`) "NewEnumerator6")
  (switch `/Game/Objects/Enum/TumblerStateEnum` (`self.State`)
    (:`NewEnumerator0`
      (`Widget.RemoveFromParent` (stale `self.On VR Use` _returnvalue))
      (`/Game/Player/BP_Player.Set Fiel Of View Back` (stale `On Press LMB_1` _player))
      (set `self.State` "NewEnumerator1"))
    (:`NewEnumerator1`
      (bind _returnvalue (`|CreateWidget` "/Game/UMG/Other/BPW_Binoculars.BPW_Binoculars_C"))
      (`UserWidget.AddToViewport` _returnvalue 1)
      (`/Game/Player/BP_Player.New Fiel Of View` (stale `On Press LMB_1` _player) 4.0)
      (set `self.State` "NewEnumerator0")))
  (`self.Text Check`))

(event `On Press LMB_1`
  (bind _player (`/Game/Function/BP_MacroLibrary.Find Player`)
    (:`Is Valid`
      (bind _item (`/Game/Player/BP_Player.Get Item` _player))
      (if (== _item self)
        (goto _label)))))

(event `Remove Widget`
  (set `self.State` "NewEnumerator1")
  (`/Engine/EditorBlueprintResources/StandardMacros.IsValid` (stale `self.On VR Use` _returnvalue)
    (:`Is Valid`
      (`Widget.RemoveFromParent` (stale `self.On VR Use` _returnvalue)))))

(fn `UserConstructionScript`
  (`parent.UserConstructionScript`))
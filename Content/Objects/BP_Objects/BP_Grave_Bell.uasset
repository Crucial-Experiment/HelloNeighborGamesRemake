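; BP_Grave_Bell is a holdable bell item, usable in VR and flat mode, that players install on a grave.
; On VR use or left click while held, a short line trace looks for a grave's BellBox, notifies tutorial and GameJolt components, and releases the bell.
; A server-to-all event then disables pickup and interaction, snaps it to the grave's Bell transform, and calls GraveBell on that grave.
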(event `Attach (Server)`
  (params (Grave :type "/Game/Objects/BP_Objects/BP_Grave Object Reference"))
  (`self.Attach (All)` Grave))

(event `self.ReceiveBeginPlay`
  (`parent.ReceiveBeginPlay`))

(event `self.On VR Use`
  (`parent.On VR Use`)
  (bind (_actor _component) (`self.Line Trace` 300.0 :!label _label))
  (bind _asbp_grave (cast `/Game/Objects/BP_Objects/BP_Grave` _actor))
  (bind _bell_box (`/Game/Objects/BP_Objects/BP_Grave.Bell Box` _asbp_grave))
  (`/Engine/EditorBlueprintResources/StandardMacros.IsValid` _bell_box
    (:`Is Valid`
      (if (== _component _bell_box)
        (`/Game/Objects/Tutorial/TutorialComponent.Check Use Type` (`self.TutorialComponent`) "NewEnumerator6")
        (`/Game/Objects/GameJolt/GameJoltComponent.Check Use Type` (`self.GameJoltComponent`) "NewEnumerator6")
        (`/Game/Objects/Structurs/FlatComponent.Drop Item` (`self.FlatComponent`) 0.0)
        (`self.Try Release`)
        (`self.Attach (Server)` _asbp_grave)
        (`/Game/Objects/Structurs/FlatComponent.Play Use Anim` (`self.FlatComponent`) false false)))))

(event `Attach (All)`
  (params (Grave :type "/Game/Objects/BP_Objects/BP_Grave Object Reference"))
  (bind _root (`self.Root`))
  (bind _bell (`/Game/Objects/BP_Objects/BP_Grave.Bell` Grave))
  (set `self.CanPickUp` false)
  (set `/Game/Objects/Structurs/GrabComponent.GrabType` "NewEnumerator0" (`self.GrabComponent`))
  (`self.Set Flat Mode` "NewEnumerator1")
  (`SceneComponent.K2_SetWorldLocation` _root (`SceneComponent.K2_GetComponentLocation` _bell) false false)
  (`SceneComponent.K2_SetWorldRotation` _root (`SceneComponent.K2_GetComponentRotation` _bell) false false)
  (`KismetArrayLibrary.Array_RemoveItem` (`ActorComponent.ComponentTags` _root) "interactive")
  (`/Game/Objects/BP_Objects/BP_Grave.Grave Bell` Grave))

(event `self.On Press LMB`
  (`parent.On Press LMB`)
  (bind _player (`/Game/Function/BP_MacroLibrary.Find Player`)
    (:`Is Valid`
      (bind _item (`/Game/Player/BP_Player.Get Item` _player))
      (if (== _item self)
        (goto _label)))))

(fn `UserConstructionScript`)
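; BP_Stereo_System_Dynamic is a stereo system object that plays the sound of an assigned Vinyl.
; The construction script snaps a valid Vinyl onto it by attachment and sets the Music component's sound from that Vinyl.
; Enable and Disable extend the parent's logic, starting the music from the beginning and stopping it.
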(event `self.Enable`
  (`parent.Enable`)
  (`AudioComponent.Play` (`self.Music`) 0.0))

(event `self.Disable`
  (`parent.Disable`)
  (`AudioComponent.Stop` (`self.Music`)))

(fn `UserConstructionScript`
  (bind _vinyl (`self.Vinyl`))
  (`parent.UserConstructionScript`)
  (`/Engine/EditorBlueprintResources/StandardMacros.IsValid` _vinyl
    (:`Is Valid`
      (`self.K2_AttachToComponent` _vinyl null "None" "SnapToTarget" "SnapToTarget" "SnapToTarget" true)
      (`AudioComponent.SetSound` (`self.Music`) (`/Game/Objects/BP_Objects/BP_Vinyl.Sound` (`self.Vinyl`))))))
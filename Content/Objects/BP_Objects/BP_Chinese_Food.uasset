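; BP_Chinese_Food is an edible Chinese food object that changes its look when eaten.
; It handles the VROnly EventEat event, acting only when the eaten actor is itself and its Eat flag is false.
; It then swaps the Root static mesh to a crumpled version and sets the FlatComponent icon to flattened noodles.
; The construction script only calls the parent's.
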(event `/Game/Function/BP_Interface.Eat (VR Only)`
  (params (Actor :type "/Game/Objects/Structurs/BP_Object Object Reference"))
  (if (and (== Actor self) (not (`self.Eat?`)))
    (`StaticMeshComponent.SetStaticMesh` (`self.Root`) "/Game/Objects/Meshes/crumpled_chinese_food_new.crumpled_chinese_food_new")
    (set `/Game/Objects/Structurs/FlatComponent.Icon` "/Game/UMG/Inv_Icons/Noodles_flattened.Noodles_flattened" (`self.FlatComponent`))))

(fn `UserConstructionScript`
  (`parent.UserConstructionScript`))
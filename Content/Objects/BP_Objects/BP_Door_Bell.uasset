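; BP_Door_Bell is an interactable doorbell that rings and draws the neighbor AI (Sosed) to check it.
; Interacting with its sphere, or touching it with VR hands, triggers the server interaction.
; The server plays the bell sound and reports the use to the tutorial and GameJolt components.
; Unless the neighbor is in an excluded state, it writes a check task at the arrow's location to its blackboard and switches its state.
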(event `Interact (Server)`
  (`GameplayStatics.SpawnSoundAtLocation` "/Game/Sounds/Maps/School/school_bell_1_Cue.school_bell_1_Cue" (`self.GetActorEyesViewPoint` self) (struct) 1.0 1.0 0.0 null null)
  (`/Game/Objects/Tutorial/TutorialComponent.Check Use Type` (`self.TutorialComponent`) "NewEnumerator6")
  (`/Game/Objects/GameJolt/GameJoltComponent.Check Use Type` (`self.GameJoltComponent`) "NewEnumerator6")
  (bind _sosed (`/Game/Function/BP_MacroLibrary.Find Sosed`)
    (:`Is Valid`
      (if (`|EnumInequality` (`/Game/Sosed/BP_Sosed.Current State` _sosed) "NewEnumerator2")
        (bind _returnvalue (`AIBlueprintHelperLibrary.GetBlackboard` _sosed))
        (`BlackboardComponent.SetValueAsInt` _returnvalue "CheckTask" 1)
        (`BlackboardComponent.SetValueAsVector` _returnvalue "Check Location" (`SceneComponent.K2_GetComponentLocation` (`self.Arrow`)))
        (`/Game/Sosed/BP_Sosed.Set State` _sosed "NewEnumerator3")))))

(event `/Game/Function/BP_Interface.Interact`
  (params (Component :type "PrimitiveComponent Object Reference") (Location :type "Vector Structure"))
  (if (== Component (`self.Sphere`))
    (`self.Interact (Server)` :!label _label)))

(event `self.Sphere.OnComponentBeginOverlap`
  (params (OverlappedComponent :type "PrimitiveComponent Object Reference") (OtherActor :type "Actor Object Reference") (OtherComp :type "PrimitiveComponent Object Reference") (OtherBodyIndex :type Integer) (bFromSweep :type Boolean) (SweepResult :type "HitResult Structure (by ref)"))
  (if (`self.Overlap VR Hands` OtherActor OtherComp)
    (goto _label)))

(fn `UserConstructionScript`)
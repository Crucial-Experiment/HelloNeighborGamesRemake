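; BP_Water is a water volume that switches between liquid water and solid ice.
; FrozenState swaps the cube's material and collision and stops or restarts any tracked shark; construction and BeginPlay apply the initial state.
; WaterBox overlaps drive splash feedback and shark attacks on the player when liquid, or change player and BP_Sosed friction and braking when frozen.
; EvaporationBox toggles post-processing for the player while unfrozen.
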(event `Frozen State`
  (params (Frozen :type Boolean))
  (bind _cube (`self.Cube`))
  (bind _cube_2 (`self.Cube`))
  ;[1 1 1] Frozen
  (bind _output_get (set `self.Frozen` Frozen))
  (if _output_get
    (`PrimitiveComponent.SetMaterial` _cube_2 0 (`self.Ice Material`))
    (`PrimitiveComponent.SetCollisionEnabled` _cube "QueryAndPhysics")
    (bind _shark (`self.Shark`)
      (:`then`
        (`/Game/Objects/BP_Objects/BP_Shark.Stop Shark` _shark))
      (:`else`))
    (else
      (`PrimitiveComponent.SetMaterial` _cube_2 0 (`self.Water Material`))
      (`PrimitiveComponent.SetCollisionEnabled` _cube "NoCollision")
      (bind _shark_2 (`self.Shark`)
        (:`then`
          (`/Game/Objects/BP_Objects/BP_Shark.Start Shark` _shark_2 self))
        (:`else`)))))

(event `self.ReceiveBeginPlay`
  (bind _cube (`self.Cube`))
  ;[1 1 1] Begin Play
  (if (`self.Frozen`)
    (`PrimitiveComponent.SetCollisionEnabled` _cube "QueryAndPhysics")
    (else
      (`PrimitiveComponent.SetCollisionEnabled` _cube "NoCollision"))))

(event `self.Water Box.OnComponentEndOverlap`
  (params (OverlappedComponent :type "PrimitiveComponent Object Reference") (OtherActor :type "Actor Object Reference") (OtherComp :type "PrimitiveComponent Object Reference") (OtherBodyIndex :type Integer))
  (bind _player_ground_friction (`self.Player Ground Friction`))
  (bind _player_braking_deceleration_walking (`self.Player Braking Deceleration Walking`))
  ;[1 1 1] Water Box
  (`|ExecutionSequence`
    (:`then_0`
      (bind _asbp_shark (cast `/Game/Objects/BP_Objects/BP_Shark` OtherActor))
      (`/Game/Objects/BP_Objects/BP_Shark.Stop Shark` _asbp_shark)
      (set `self.Shark` null))
    (:`then_1`
      (if (not (`self.Frozen`))
        (`|ExecutionSequence`
          (:`then_0`
            (`GameplayStatics.PlaySoundAtLocation` (`self.Water Sound`) (`self.K2_GetActorLocation`) (struct) 1.0 1.0 0.0 "/Game/Sounds/Attenuation/Silent.Silent" null null null))
          (:`then_1`
            (cast `/Game/Player/BP_Player` OtherActor)
            (bind _shark (`self.Shark`)
              (:`then`
                (set `/Game/Objects/BP_Objects/BP_Shark.Attack` false _shark))
              (:`else`))))
        (else
          (bind _asbp_player (cast `/Game/Player/BP_Player` OtherActor)
            (:`then`
              (bind _charactermovement (`Character.CharacterMovement` _asbp_player))
              (set `CharacterMovementComponent.GroundFriction` _player_ground_friction _charactermovement)
              (set `CharacterMovementComponent.BrakingDecelerationWalking` _player_braking_deceleration_walking _charactermovement))
            (:`CastFailed`
              (bind _asbp_sosed (cast `/Game/Sosed/BP_Sosed` OtherActor))
              (bind _charactermovement_2 (`Character.CharacterMovement` _asbp_sosed))
              (set `CharacterMovementComponent.GroundFriction` _player_ground_friction _charactermovement_2)
              (set `CharacterMovementComponent.BrakingDecelerationWalking` _player_braking_deceleration_walking _charactermovement_2))))))))

(event `self.Water Box.OnComponentBeginOverlap`
  (params (OverlappedComponent :type "PrimitiveComponent Object Reference") (OtherActor :type "Actor Object Reference") (OtherComp :type "PrimitiveComponent Object Reference") (OtherBodyIndex :type Integer) (bFromSweep :type Boolean) (SweepResult :type "HitResult Structure (by ref)"))
  (bind _returnvalue (`self.K2_GetActorLocation` OtherActor))
  (bind _ground_friction (`self.Ground Friction`))
  (bind _braking_deceleration_walking (`self.Braking Deceleration Walking`))
  (bind _returnvalue_2 (not (`self.Frozen`)))
  ;[1 1 1] Water Box
  (`|ExecutionSequence`
    (:`then_0`
      (if _returnvalue_2
        (bind _asbp_shark (cast `/Game/Objects/BP_Objects/BP_Shark` OtherActor))
        (bind _output_get (set `self.Shark` _asbp_shark))
        (`/Game/Objects/BP_Objects/BP_Shark.Start Shark` _output_get self)))
    (:`then_1`
      (if _returnvalue_2
        (`|ExecutionSequence`
          (:`then_0`
            (`GameplayStatics.SpawnEmitterAtLocation` (`self.Water Effect`) _returnvalue)
            (`GameplayStatics.PlaySoundAtLocation` (`self.Water Sound`) _returnvalue (struct) 1.0 1.0 0.0 null null null null))
          (:`then_1`
            (cast `/Game/Player/BP_Player` OtherActor)
            (bind _shark (`self.Shark`)
              (:`then`
                (set `/Game/Objects/BP_Objects/BP_Shark.Attack` true _shark))
              (:`else`))))
        (else
          (bind _asbp_player (cast `/Game/Player/BP_Player` OtherActor)
            (:`then`
              (bind _charactermovement (`Character.CharacterMovement` _asbp_player))
              (set `CharacterMovementComponent.GroundFriction` _ground_friction _charactermovement)
              (set `CharacterMovementComponent.BrakingDecelerationWalking` _braking_deceleration_walking _charactermovement))
            (:`CastFailed`
              (bind _asbp_sosed (cast `/Game/Sosed/BP_Sosed` OtherActor))
              (bind _charactermovement_2 (`Character.CharacterMovement` _asbp_sosed))
              (set `CharacterMovementComponent.GroundFriction` _ground_friction _charactermovement_2)
              (set `CharacterMovementComponent.BrakingDecelerationWalking` _braking_deceleration_walking _charactermovement_2))))))))

(event `self.Evaporation Box.OnComponentBeginOverlap`
  (params (OverlappedComponent :type "PrimitiveComponent Object Reference") (OtherActor :type "Actor Object Reference") (OtherComp :type "PrimitiveComponent Object Reference") (OtherBodyIndex :type Integer) (bFromSweep :type Boolean) (SweepResult :type "HitResult Structure (by ref)"))
  ;[1 1 1] Post Process
  (if (not (`self.Frozen`))
    (cast `/Game/Player/BP_Player` OtherActor)
    (set `PostProcessComponent.bEnabled` true (`self.PostProcess`))))

(event `self.Evaporation Box.OnComponentEndOverlap`
  (params (OverlappedComponent :type "PrimitiveComponent Object Reference") (OtherActor :type "Actor Object Reference") (OtherComp :type "PrimitiveComponent Object Reference") (OtherBodyIndex :type Integer))
  ;[1 1 1] Post Process
  (if (not (`self.Frozen`))
    (cast `/Game/Player/BP_Player` OtherActor)
    (set `PostProcessComponent.bEnabled` false (`self.PostProcess`))))

(fn `UserConstructionScript`
  (bind _cube (`self.Cube`))
  (if (`self.Frozen`)
    (`PrimitiveComponent.SetMaterial` _cube 0 (`self.Ice Material`))
    (else
      (`PrimitiveComponent.SetMaterial` _cube 0 (`self.Water Material`)))))
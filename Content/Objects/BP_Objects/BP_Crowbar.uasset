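; BP_Crowbar is a carryable tool that pulls out nails, including those holding door blocks.
; On left click while held, a short line trace unlocks the hit BP_Nail and reports the use to the tutorial and GameJolt components.
; In VR, overlap events, enabled from the player's StartVR flag, unlock a random nail on the touched BP_Door_Block.
; Shortly after pickup, a too-hot crowbar is released with a sizzle sound.
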(event `/Game/Function/BP_Interface.PickUp`
  ;[1 1 1] Pick Up
  (`parent.PickUp`)
  (`KismetSystemLibrary.Delay` 0.2)
  (if (> (`/Game/Objects/Structurs/TemperatureComponent.Temperature` (`self.TemperatureComponent`)) 0.2)
    (`self.Try Release`)
    (`GameplayStatics.PlaySound2D` "/Game/Sounds/Objects/Noise/sizzle_burn_Cue.sizzle_burn_Cue" 1.0 1.0 0.0 null null)))

(event `self.ReceiveBeginPlay`
  ;[1 1 1] Begin Play
  (`parent.ReceiveBeginPlay`)
  (bind _player (`/Game/Function/BP_MacroLibrary.Find Player`)
    (:`Is Valid`
      (set `PrimitiveComponent.bGenerateOverlapEvents` (`/Game/Player/BP_Player.Start VR` _player) (`self.VR Interact`)))))

(event `On Press LMB_1`
  ;[1 1 1] Begin Play
  (bind _player (`/Game/Function/BP_MacroLibrary.Find Player`)
    (:`Is Valid`
      (bind _item (`/Game/Player/BP_Player.Get Item` _player))
      (if (== _item self)
        (bind _actor (`self.Line Trace` 150.0 "NewEnumerator1"))
        (bind _asbp_nail (cast `/Game/Objects/BP_Objects/BP_Nail` _actor))
        (`/Game/Objects/BP_Objects/BP_Nail.Unlock` _asbp_nail)
        (`/Game/Objects/Tutorial/TutorialComponent.Check Use Type` (`self.TutorialComponent`) "NewEnumerator6")
        (`/Game/Objects/GameJolt/GameJoltComponent.Check Use Type` (`self.GameJoltComponent`) "NewEnumerator6")))))

(event `Unlock (Server)`
  (params (Nail :type "/Game/Objects/BP_Objects/BP_Nail Object Reference"))
  ;[1 1 1] Begin Play
  (`/Game/Objects/BP_Objects/BP_Nail.Unlock` Nail))

(event `self.On VR Use`
  ;[1 1 1] Begin Play
  (`parent.On VR Use`))

(event `self.VR Interact.OnComponentBeginOverlap`
  (params (OverlappedComponent :type "PrimitiveComponent Object Reference") (OtherActor :type "Actor Object Reference") (OtherComp :type "PrimitiveComponent Object Reference") (OtherBodyIndex :type Integer) (bFromSweep :type Boolean) (SweepResult :type "HitResult Structure (by ref)"))
  ;[1 1 1] VR Interact
  (bind _asbp_door_block (cast `/Game/Objects/BP_Objects/BP_Door_Block` OtherActor))
  (bind _nails (`/Game/Objects/BP_Objects/BP_Door_Block.Nails` _asbp_door_block))
  (if (`KismetArrayLibrary.Array_IsNotEmpty` _nails)
    (`GameplayStatics.PlaySound2D` "/Game/Sounds/Sosed/step_creaky_wood_Cue.step_creaky_wood_Cue" 1.0 1.0 0.0 null null)
    (`/Game/Objects/BP_Objects/BP_Nail.Unlock` (`KismetArrayLibrary.Array_Random` _nails))))

(fn `UserConstructionScript`
  (`parent.UserConstructionScript`)
  (set `/Game/Objects/Structurs/TemperatureComponent.Actor` (`self.Root`) (`self.TemperatureComponent`)))
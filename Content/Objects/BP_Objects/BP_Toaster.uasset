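; BP_Toaster is a toaster object that animates bread slices lowering and popping up, with sound.
; The SliceStart and SliceEnd events each play a cue at the actor's location and run a timeline that lerps the Scene component's relative location.
; SliceStart sinks it into the toaster, and SliceEnd raises it from there to above its original height.
; Nothing in this graph calls either event.
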(event `Slice Start`
  (`GameplayStatics.PlaySoundAtLocation` "/Game/Sounds/Maps/Darkness/toaster_down_Cue.toaster_down_Cue" (`self.K2_GetActorLocation`) (struct) 1.0 1.0 0.0 null null null null)
  (bind (_direction _alpha) (`Timeline|Slice` :!via `PlayFromStart`)
    (:`Update`
      (`SceneComponent.K2_SetRelativeLocation` (`self.Scene`) (`KismetMathLibrary.VLerp` (0.0 3.769433 22.0) (0.0 3.769433 7.0) _alpha) false false))))

(event `Slice End`
  (`GameplayStatics.PlaySoundAtLocation` "/Game/Sounds/Maps/Darkness/toaster_up_Cue.toaster_up_Cue" (`self.K2_GetActorLocation`) (struct) 1.0 1.0 0.0 null null null null)
  (bind (_direction _alpha) (`Timeline|Slice Fin` :!via `PlayFromStart`)
    (:`Update`
      (`SceneComponent.K2_SetRelativeLocation` (`self.Scene`) (`KismetMathLibrary.VLerp` (0.0 3.769433 7.0) (0.0 3.769433 35.0) _alpha) false false))))

(fn `UserConstructionScript`)
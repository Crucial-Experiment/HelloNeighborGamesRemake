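; Electric wires object that responds to power being enabled or disabled and can have a crowbar placed on it.
; Without a valid Crowbar, enabling starts spark effects and notifies the tutorial and GameJolt components; disabling stops sparks and notifies both.
; An assigned Crowbar is snapped to the Scene component at construction and set to a flat mode on BeginPlay.
; While powered, Tick holds that crowbar's temperature at maximum.
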(event `self.Disable`
  ;[1 1 1] Electricity
  (`parent.Disable`)
  (set `self.Tick` false)
  (`ActorComponent.Deactivate` (`self.Spark`))
  (`ActorComponent.Deactivate` (`self.P_Sparks`))
  (`/Game/Objects/Tutorial/TutorialComponent.Check Use Type` (`self.TutorialComponent`) "NewEnumerator4")
  (`/Game/Objects/GameJolt/GameJoltComponent.Check Use Type` (`self.GameJoltComponent`) "NewEnumerator4"))

(event `self.Enable`
  ;[1 1 1] Electricity
  (`parent.Enable`)
  (set `self.Tick` true)
  (`/Engine/EditorBlueprintResources/StandardMacros.IsValid` (`self.Crowbar`)
    (:`Is Not Valid`
      (`ActorComponent.Activate` (`self.Spark`) false)
      (`ActorComponent.Activate` (`self.P_Sparks`) false)
      (`/Game/Objects/Tutorial/TutorialComponent.Check Use Type` (`self.TutorialComponent`) "NewEnumerator3")
      (`/Game/Objects/GameJolt/GameJoltComponent.Check Use Type` (`self.GameJoltComponent`) "NewEnumerator3"))))

(event `self.ReceiveTick`
  (params (DeltaSeconds :type "Float (single-precision)"))
  (bind _crowbar (`self.Crowbar`))
  ;[1 1 1] Tick
  (if (or (`self.Has Electricity`) (`self.Generator`))
    (if (`self.Tick`)
      (`/Engine/EditorBlueprintResources/StandardMacros.IsValid` _crowbar
        (:`Is Valid`
          (set `/Game/Objects/Structurs/TemperatureComponent.Temperature` 1.0 (`/Game/Objects/BP_Objects/BP_Crowbar.TemperatureComponent` _crowbar)))
        (:`Is Not Valid`
          (set `self.Tick` false))))))

(event `self.ReceiveBeginPlay`
  (bind _crowbar (`self.Crowbar`))
  ;[1 1 1] Begin Play
  (`parent.ReceiveBeginPlay`)
  (`/Engine/EditorBlueprintResources/StandardMacros.IsValid` _crowbar
    (:`Is Valid`
      (`self.Set Flat Mode` _crowbar "NewEnumerator1")
      (set `self.Tick` true))))

(fn `UserConstructionScript`
  (`/Engine/EditorBlueprintResources/StandardMacros.IsValid` (`self.Crowbar`)
    (:`Is Valid`
      (`self.K2_SetActorTransform` (`self.Crowbar`) (`SceneComponent.K2_GetComponentToWorld` (`self.Scene`)) false false))))
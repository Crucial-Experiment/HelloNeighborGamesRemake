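; BP_Glue is a throwable glue jar that shatters on impact, with an explosion effect and crash sound.
; Throw builds a curved spline toward a point ahead of the target player at foot level, leading it by velocity, with debug drawing enabled.
; Tick moves the jar along that spline, then switches its flat mode.
; A fast or in-flight hit destroys it once, spawning a glue puddle on static, upward-facing surfaces.
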(event `self.Root.OnComponentHit`
  (params (HitComponent :type "PrimitiveComponent Object Reference") (OtherActor :type "Actor Object Reference") (OtherComp :type "PrimitiveComponent Object Reference") (NormalImpulse :type "Vector Structure") (Hit :type "HitResult Structure (by ref)"))
  (bind (_bblockinghit _binitialoverlap _time _distance _location _impactpoint _normal) (`GameplayStatics.BreakHitResult` Hit))
  (bind _returnvalue (`self.K2_GetActorLocation`))
  ;[1 1 1] Hit
  (if (or (> (`KismetMathLibrary.VSize` (`self.GetVelocity`)) 120.0) (`self.Is Move`))
    (set `self.Is Move` false)
    (`/Engine/EditorBlueprintResources/StandardMacros.DoOnce` false
      (:`Completed`
        (if (and (`|EnumEquality` (`SceneComponent.Mobility` OtherComp) "Static") (> (`KismetMathLibrary.Dot_VectorVector` _normal (0.0 0.0 1.0)) 0.5))
          (`|SpawnActorFromClass` "/Game/Objects/BP_Objects/BP_Puddle_Glue.BP_Puddle_Glue_C" (`KismetMathLibrary.MakeTransform` (+ _location (0.0 0.0 1.0))) "Undefined" "MultiplyWithRoot" null null))
        (`GameplayStatics.SpawnEmitterAtLocation` "/Game/Effects/Particle/P_Explosion_Glue.P_Explosion_Glue" _returnvalue)
        (`GameplayStatics.SpawnSoundAtLocation` "/Game/Sounds/Objects/Noise/crash_glue_jar_Cue.crash_glue_jar_Cue" _returnvalue (struct) 1.0 1.0 0.0 null null)
        (`self.K2_DestroyActor`)))))

(event `self.ReceiveTick`
  (params (DeltaSeconds :type "Float (single-precision)"))
  ;[1 1 1] Fly
  (`parent.ReceiveTick` DeltaSeconds)
  (if (`self.Is Move`)
    (`self.K2_SetActorLocation` (+ (`SplineComponent.GetLocationAtTime` (`self.Spline`) (`self.Time`) "Local" false) (`self.Start Pos`)))
    (bind _output_get (set `self.Time` (+ (`self.Time`) (* DeltaSeconds 4.0))))
    (if (>= _output_get 1.0)
      (set `self.Is Move` false)
      (`self.Set Flat Mode` "NewEnumerator0"))))

(fn `Throw`
  (params (Player :type "/Game/Player/BP_Player Object Reference"))
  (bind _returnvalue (`self.GetVelocity` Player))
  (bind _spline (`self.Spline`))
  (bind _returnvalue_2 (- (- (+ (`self.K2_GetActorLocation` Player) (* (`self.GetActorForwardVector` Player) 100.0) (* (`KismetMathLibrary.Normal` _returnvalue) (* (`KismetMathLibrary.VSize` _returnvalue) 0.7))) (`self.K2_GetActorLocation`)) (`KismetMathLibrary.MakeVector` 0.0 0.0 (`CapsuleComponent.GetScaledCapsuleHalfHeight` (`Character.CapsuleComponent` Player)))))
  (set `self.Is Move` true)
  (`SplineComponent.ClearSplinePoints` (`self.Spline`) false)
  (set `self.Start Pos` (`self.K2_GetActorLocation`))
  (`SplineComponent.SetSplinePoints` (`self.Spline`) (`|MakeArray` (0.0 0.0 0.0) _returnvalue_2) "Local" false)
  (`SplineComponent.SetTangentAtSplinePoint` _spline 1 (+ (`SplineComponent.GetArriveTangentAtSplinePoint` _spline 1 "Local") (* (`KismetMathLibrary.Normal` _returnvalue_2) 500.0) (0.0 0.0 -200.0)) "Local" true)
  (`SplineComponent.SetTangentAtSplinePoint` (`self.Spline`) 0 (`KismetMathLibrary.MakeVector` 0.0 0.0 -500.0) "Local" true)
  (`SplineComponent.SetDrawDebug` (`self.Spline`) true))

(fn `UserConstructionScript`
  (`parent.UserConstructionScript`))
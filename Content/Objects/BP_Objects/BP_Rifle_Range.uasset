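; Rifle range minigame actor with a lockable door and lights that track the mounted rifle and electricity.
; Pressing the button with a click or VR hand starts music and spawns warriors from a configured list, counting deaths on the scoreboard.
; Outside VR, the view blends to the range camera, player look input aims the rifle and left click fires.
; Reaching the target score spawns a "RifleRange" key; right click quits and clears warriors.
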(event `Rifle Taken`
  ;[1 1 1] Taken
  (set `self.Rifle` null)
  (`self.Rifle Transform`))

(event `self.Enable`
  (bind _lights (`self.Lights`))
  ;[1 1 1] Electricity
  (`parent.Enable`)
  (`self.Rifle` :!label _label
    (:`then`
      (`PrimitiveComponent.SetMaterial` _lights 0 "/Game/Objects/Materials/dl_bulb_m.dl_bulb_m" :!label _label_2))
    (:`else`
      (`PrimitiveComponent.SetMaterial` _lights 0 "/Game/Objects/Materials/dl_bulb_m_off.dl_bulb_m_off" :!label _label_3))))

(event `/Game/Function/BP_Interface.Interact`
  (params (Component :type "PrimitiveComponent Object Reference") (Location :type "Vector Structure"))
  ;[1 1 1] Interact
  (`self.Interact (Server)` Component))

(event `self.ReceiveBeginPlay`
  ;[1 1 1] Electricity
  (`parent.ReceiveBeginPlay`)
  (`|ExecutionSequence`
    (:`then_0`
      (if (or (`self.Has Electricity`) (`self.Generator`))
        (goto _label)
        (else
          (`self.Rifle` :!label _label_4
            (:`then`
              (goto _label_3))
            (:`else`)))))
    (:`then_1`
      (bind _player (`/Game/Function/BP_MacroLibrary.Find Player`)
        (:`Is Valid`
          (add `/Game/Player/BP_Player.Left Mouse Button` _player (delegate `Shot`)))))))

(event `Interact (Server)`
  (params (Component :type "PrimitiveComponent Object Reference"))
  ;[1 1 1] Interact
  (`|ExecutionSequence`
    (:`then_0`
      (bind _bool (`/Game/Function/BP_FunctionLibrary.Checking Object` Component (`self.Range Door`)))
      (if (and _bool (not (`self.Range Door Lock`)))
        (switch `/Game/Objects/Enum/RotateStateEnum` (`self.Range Rotate`)
          (:`NewEnumerator0`
            (set `self.Range Rotate` "NewEnumerator3")
            (bind (_direction _alpha) (`Timeline|Timeline_0` :!via `Reverse` :!label _label_5)
              (:`Update`
                (`SceneComponent.K2_SetRelativeRotation` (`self.Range Door`) (`KismetMathLibrary.RLerp` (struct) (struct :`Pitch` 90.0) _alpha) false false))
              (:`Finished`
                (switch `/Game/Objects/Enum/RotateStateEnum` (`self.Range Rotate`)
                  (:`NewEnumerator2`
                    (set `self.Range Rotate` "NewEnumerator0"))
                  (:`NewEnumerator3`
                    (set `self.Range Rotate` "NewEnumerator1"))))))
          (:`NewEnumerator1`
            (set `self.Range Rotate` "NewEnumerator2")
            (goto _label_5)))))
    (:`then_1`
      (bind _bool_2 (`/Game/Function/BP_FunctionLibrary.Checking Object` Component (`self.Button`)))
      (if (and _bool_2 (`KismetSystemLibrary.IsValid` (`self.Rifle`)))
        (bind _player (`/Game/Function/BP_MacroLibrary.Find Player`)
          (:`Is Valid`
            (add `/Game/Player/BP_Player.Right Mouse Button` _player (delegate `Stop Game`))
            (`self.Start Game` "NewEnumerator0" :!label _label_6)
            (bind _scoreboard (`self.Scoreboard`)
              (:`then`
                (set `self.Button Press` true)
                (`AudioComponent.Play` (`self.Music`) 0.0)
                (`/Game/Objects/BP_Objects/BP_Scoreboard.Reset Count` _scoreboard)
                (bind _player_2 (`/Game/Function/BP_MacroLibrary.Find Player`)
                  (:`Is Valid`
                    (if (not (`/Game/Player/BP_Player.Start VR` _player_2))
                      (`PlayerController.SetViewTargetWithBlend` (`GameplayStatics.GetPlayerController` 0) self 0.6 "VTBlend_Linear" 0.0 false))
                    (for _array_element (`self.Warrior Array`)
                      (add `/Game/Objects/BP_Objects/BP_Warrior.On Death` _array_element (delegate `Warrior Death`))))))
              (:`else`))))))))

(event `self.Disable`
  ;[1 1 1] Electricity
  (`parent.Disable`)
  (goto _label_4))

(event `Switch State`
  ;[1 1 1] Electricity
  (switch `/Game/Objects/Enum/TumblerStateEnum` (`self.State`)
    (:`NewEnumerator0`
      (goto _label_2))
    (:`NewEnumerator1`
      (goto _label_3))))

(event `Shot`
  ;[1 1 1] Rifle Shot
  (if (and (`self.Button Press`) (`KismetSystemLibrary.IsValid` (`self.Rifle`)))
    (`self.On VR Use` (`self.Rifle`))))

(event `self.Button.OnComponentBeginOverlap`
  (params (OverlappedComponent :type "PrimitiveComponent Object Reference") (OtherActor :type "Actor Object Reference") (OtherComp :type "PrimitiveComponent Object Reference") (OtherBodyIndex :type Integer) (bFromSweep :type Boolean) (SweepResult :type "HitResult Structure (by ref)"))
  ;[1 1 1] Interact
  (if (and (`self.Overlap VR Hands` OtherActor OtherComp) (`|EnumInequality` (`self.State`) "NewEnumerator0"))
    (goto _label_6)))

(event `Warrior Death`
  (bind (_returnvalue_location _returnvalue_rotation) (`KismetMathLibrary.BreakTransform` (`SceneComponent.K2_GetComponentToWorld` (`self.Billboard`))))
  ;[1 1 1] Interact
  (bind _scoreboard (`self.Scoreboard`)
    (:`then`
      (`/Game/Objects/BP_Objects/BP_Scoreboard.Add Count` _scoreboard)
      (if (>= (`/Game/Objects/BP_Objects/BP_Scoreboard.Score` _scoreboard) (`self.Spawn Count`))
        (bind _returnvalue (`|SpawnActorFromClass` (`self.Spawn Actor`) (`KismetMathLibrary.MakeTransform` _returnvalue_location _returnvalue_rotation) "Undefined" "SelectDefaultAtRuntime" null null))
        (bind _asbp_key (cast `/Game/Objects/Structurs/BP_Key` _returnvalue)
          (:`then`
            (set `/Game/Objects/Structurs/BP_Key.Code` "RifleRange" _asbp_key))
          (:`CastFailed`
            _))
        (if (not (`/Game/Player/BP_Player.Start VR` (stale `Interact (Server)` _player_2)))
          (`PlayerController.SetViewTargetWithBlend` (`GameplayStatics.GetPlayerController` 0) (stale `Interact (Server)` _player_2) 0.6 "VTBlend_Linear" 0.0 false))
        (set `self.Button Press` false)
        (`AudioComponent.Stop` (`self.Music`))))
    (:`else`)))

(event `self.ReceiveTick`
  (params (DeltaSeconds :type "Float (single-precision)"))
  (bind _rifle (`self.Rifle`))
  (bind (_returnvalue_roll _returnvalue_pitch _returnvalue_yaw) (`KismetMathLibrary.BreakRotator` (`self.K2_GetActorRotation` _rifle)))
  ;[1 1 1] Interact
  (bind _player (`/Game/Function/BP_MacroLibrary.Find Player`)
    (:`Is Valid`
      (if (and (`self.Button Press`) (`KismetSystemLibrary.IsValid` (`self.Rifle`)))
        (bind _returnvalue (- _returnvalue_pitch (`/Game/Player/BP_Player.Look Up` _player)))
        (bind _returnvalue_2 (+ _returnvalue_yaw (`/Game/Player/BP_Player.Get Turn` _player)))
        (`self.K2_SetActorRotation` _rifle (`KismetMathLibrary.MakeRotator` _returnvalue_roll _returnvalue _returnvalue_2) false)
        (`SceneComponent.K2_SetWorldRotation` (`self.Camera`) (`KismetMathLibrary.MakeRotator` 0.0 _returnvalue _returnvalue_2) false false)))))

(event `Unlock (Server)`
  (bind _lock_rr (`self.Lock RR`))
  ;[1 1 1] Unlock
  (`|ExecutionSequence`
    (:`then_0`
      (set `self.Range Door Lock` false))
    (:`then_1`
      (`PrimitiveComponent.SetSimulatePhysics` _lock_rr true)
      (`GameplayStatics.PlaySoundAtLocation` "/Game/Sounds/Maps/Act2/Main/lock_open_Cue.lock_open_Cue" (`self.K2_GetActorLocation`) (struct) 1.0 1.0 0.0 null null null null)
      (`KismetSystemLibrary.Delay` 1.5)
      (`ActorComponent.K2_DestroyComponent` _lock_rr))))

(event `Stop Game`
  ;[1 1 1] Interact
  (`PlayerController.SetViewTargetWithBlend` (`GameplayStatics.GetPlayerController` 0) (`GameplayStatics.GetPlayerPawn` 0) 0.6 "VTBlend_Linear" 0.0 false)
  (set `self.Button Press` false)
  (`AudioComponent.Stop` (`self.Music`))
  (bind _outactors (`GameplayStatics.GetAllActorsOfClass` "/Game/Objects/BP_Objects/BP_Warrior.BP_Warrior_C"))
  (for _array_element _outactors
    (`self.K2_DestroyActor` _array_element))
  (bind _player (`/Game/Function/BP_MacroLibrary.Find Player`)
    (:`Is Valid`
      (remove `/Game/Player/BP_Player.Right Mouse Button` _player (delegate `Stop Game`)))))

(event `self.Warrior Wall 1.OnComponentBeginOverlap`
  (params (OverlappedComponent :type "PrimitiveComponent Object Reference") (OtherActor :type "Actor Object Reference") (OtherComp :type "PrimitiveComponent Object Reference") (OtherBodyIndex :type Integer) (bFromSweep :type Boolean) (SweepResult :type "HitResult Structure (by ref)"))
  ;[1 1 1] Warrior Wall
  (bind _asbp_warrior (cast `/Game/Objects/BP_Objects/BP_Warrior` OtherActor))
  (`/Game/Objects/BP_Objects/BP_Warrior.New Action` :`self` _asbp_warrior))

(event `self.Warrior Wall 2.OnComponentBeginOverlap`
  (params (OverlappedComponent :type "PrimitiveComponent Object Reference") (OtherActor :type "Actor Object Reference") (OtherComp :type "PrimitiveComponent Object Reference") (OtherBodyIndex :type Integer) (bFromSweep :type Boolean) (SweepResult :type "HitResult Structure (by ref)"))
  ;[1 1 1] Warrior Wall
  (bind _asbp_warrior (cast `/Game/Objects/BP_Objects/BP_Warrior` OtherActor))
  (`/Game/Objects/BP_Objects/BP_Warrior.New Action` :`self` _asbp_warrior))

(fn `Rifle Transform`
  (bind (_returnvalue_location _returnvalue_rotation) (`KismetMathLibrary.BreakTransform` (`SceneComponent.K2_GetComponentToWorld` (`self.Scene`))))
  (bind _rifle (`self.Rifle`)
    (:`then`
      (`self.Set Flat Mode` _rifle "NewEnumerator1")
      (`self.K2_SetActorLocationAndRotation` _rifle _returnvalue_location _returnvalue_rotation false false)
      (set `/Game/Objects/BP_Objects/BP_Rifle.Rifle Range` self _rifle)
      (set `self.State` "NewEnumerator0"))
    (:`else`
      (set `self.State` "NewEnumerator1")))
  (`self.Switch State`))

(fn `Spawn Warriors`
  (for _array_element (`self.Warriors`)
    (if (`KismetSystemLibrary.IsValidClass` (break `/Game/Objects/Structurs/BP_WarriorStruct` _array_element))
      (bind _returnvalue (`|SpawnActorFromClass` "/Game/Objects/BP_Objects/BP_Warrior.BP_Warrior_C" (`KismetMathLibrary.MakeTransform` (select `/Game/Objects/Enum/PositionEnum` (`.Position_5_B6AA115344036490D575F7AF4A8B19A6` (break `/Game/Objects/Structurs/BP_WarriorStruct` _array_element)) :`NewEnumerator0` (`SceneComponent.K2_GetComponentLocation` (`KismetArrayLibrary.Array_Random` (`|MakeArray` (`self.Warrior Spawn 1`) (`self.Warrior Spawn 2`)))) :`NewEnumerator2` (`SceneComponent.K2_GetComponentLocation` (`KismetArrayLibrary.Array_Random` (`|MakeArray` (`self.Warrior Spawn 3`) (`self.Warrior Spawn 4`)))))) "Undefined" "OverrideRootScale" null null))
      (`/Game/Objects/BP_Objects/BP_Warrior.Set Mesh` _returnvalue (`.Skin_12_62E53D714B6860F59804D1BFA2F8AC18` (break `/Game/Objects/Structurs/BP_WarriorStruct` _array_element)))
      (set `/Game/Objects/BP_Objects/BP_Warrior.Animations` (`.Animations_16_38307D76413F6415B3565198129519C7` (break `/Game/Objects/Structurs/BP_WarriorStruct` _array_element)) _returnvalue)
      (`/Game/Objects/BP_Objects/BP_Warrior.Play Animation` _returnvalue)
      (`/Game/Objects/BP_Objects/BP_Warrior.New Action` _returnvalue (`.Action_8_0172792A4DB88A15EFA109903AFC1146` (break `/Game/Objects/Structurs/BP_WarriorStruct` _array_element)) (`.ActionStruct_20_E81C477F4C848FCC4432EDB5D45A6897` (break `/Game/Objects/Structurs/BP_WarriorStruct` _array_element)))
      (`KismetArrayLibrary.Array_Add` (`self.Warrior Array`) _returnvalue))))

(fn `Start Game`
  (params (`New State` :type "/Game/Objects/Enum/TumblerStateEnum Enum" :default "NewEnumerator0"))
  (bind _output_get (set `self.Game Status` `New State`))
  (switch `/Game/Objects/Enum/TumblerStateEnum` _output_get
    (:`NewEnumerator0`
      (`self.Spawn Warriors`))))

(fn `UserConstructionScript`
  (`self.Rifle Transform`))
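; BP_Fireworks is an interactable firework that players light or snuff, alternating on each interaction.
; Interact routes through a server event to an all-clients event, which also notifies the tutorial and GameJolt components.
; Lighting starts crackle audio, a fire emitter and the burning wick, then a delay.
; If still lit when the delay ends, it spawns the explosion effect and sound, then destroys itself.
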(event `Interact (All)`
  (bind _returnvalue (`self.K2_GetActorLocation`))
  (bind _crackle (`self.Crackle`))
  (`/Game/Objects/Tutorial/TutorialComponent.Check Use Type` (`self.TutorialComponent`) "NewEnumerator6")
  (`/Game/Objects/GameJolt/GameJoltComponent.Check Use Type` (`self.GameJoltComponent`) "NewEnumerator6")
  (`/Engine/EditorBlueprintResources/StandardMacros.FlipFlop`
    (:`A`
      (set `self.Couting` true)
      (`ActorComponent.Activate` _crackle false)
      (bind _returnvalue_2 (`GameplayStatics.SpawnEmitterAtLocation` "/Game/Effects/Particle/P_Fire.P_Fire" (`self.K2_GetActorLocation`) (struct :`Pitch` 90.0) (1.0 1.0 1.0) false))
      (`AudioComponent.Play` (`self.Burning Wick`) 0.0)
      (`KismetSystemLibrary.Delay` (`self.Delay`) :!label _label)
      (if (`self.Couting`)
        (`GameplayStatics.SpawnEmitterAtLocation` "/Game/Effects/Particle/P_Firework_new.P_Firework_new" _returnvalue)
        (`AudioComponent.Stop` (`self.Burning Wick`))
        (`GameplayStatics.PlaySoundAtLocation` "/Game/Sounds/Objects/Noise/firework_Cue.firework_Cue" _returnvalue (struct) 1.0 1.0 0.0 null null null null)
        (`ActorComponent.K2_DestroyComponent` _returnvalue_2)
        (`self.K2_DestroyActor`)))
    (:`B`
      (set `self.Couting` false)
      (`ActorComponent.Deactivate` _crackle)
      (`|ExecutionSequence`
        (:`then_0`
          (goto _label))
        (:`then_1`
          (`AudioComponent.Stop` (`self.Burning Wick`))
          (`/Engine/EditorBlueprintResources/StandardMacros.IsValid` _returnvalue_2
            (:`Is Valid`
              (`ActorComponent.K2_DestroyComponent` _returnvalue_2))))))))

(event `Interact (Server)`
  (`self.Interact (All)`))

(event `/Game/Function/BP_Interface.Interact`
  (params (Component :type "PrimitiveComponent Object Reference") (Location :type "Vector Structure"))
  (`parent.Interact` Component Location)
  (`self.Interact (Server)`))

(fn `UserConstructionScript`)
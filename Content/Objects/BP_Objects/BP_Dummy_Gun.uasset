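; BP_Dummy_Gun is an automatic gun that periodically fires bursts of dummy rifle bullets while enabled, recently rendered and near the player.
; Tick runs the cooldown, then loops through a burst with optional delays, launching bullets by impulse along the Sphere's facing with random spread.
; GetBullet pools projectiles, spawning up to MaxBullet, then recycling the first one in the matching flat mode and moving it to the array's end.
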(event `self.ReceiveTick`
  (params (DeltaSeconds :type "Float (single-precision)"))
  (bind _spread (`self.Spread`))
  (bind _delay_bullets (`self.Delay Bullets`))
  (bind _returnvalue (* _spread -1.0))
  (if (and (`self.WasRecentlyRendered` 0.2) (`self.Shoot?`))
    (if (<= (`self.Timer Shot`) 0.0)
      (set `self.Timer Shot` (`self.Shot Wait Time`))
      (bind _player (`/Game/Function/BP_MacroLibrary.Find Player`)
        (:`Is Valid`
          (if (<= (`KismetMathLibrary.VSize` (- (`self.K2_GetActorLocation` _player) (`self.K2_GetActorLocation`))) 1000.0)
            (bind _bullet (`self.Get Bullet` :!label _label))
            (`self.K2_SetActorLocation` _bullet (`SceneComponent.K2_GetComponentLocation` (`self.Sphere`)) false true)
            (`PrimitiveComponent.AddImpulse` (`/Game/Objects/Structurs/BP_Object.Root` _bullet) (+ (* (`KismetMathLibrary.GreaterGreater_VectorRotator` (1.0 0.0 0.0) (`SceneComponent.K2_GetComponentRotation` (`self.Sphere`))) (`self.Shot Power`)) (`KismetMathLibrary.MakeVector` (`KismetMathLibrary.RandomFloatInRange` _returnvalue _spread) (`KismetMathLibrary.RandomFloatInRange` _returnvalue _spread) (`KismetMathLibrary.RandomFloatInRange` _returnvalue _spread))) "None" false)
            (`AudioComponent.Play` (`self.Shot_Cue`) 0.0)
            (`/Engine/EditorBlueprintResources/StandardMacros.IncrementInt` (`self.Count`)
              (:`  `
                (if (> _delay_bullets 0.0)
                  (`KismetSystemLibrary.Delay` _delay_bullets))
                (if (>= (`self.Count`) (`self.Bullets Per Shot`))
                  (set `self.Count` 0)
                  (else
                    (goto _label))))))))
      (else
        (set `self.Timer Shot` (- (`self.Timer Shot`) DeltaSeconds))))))

(fn `Get Bullet`
  (returns (Bullet :type "/Game/Objects/BP_Objects/BP_RifleBullet Object Reference"))
  (bind _bullets (`self.Bullets`))
  (bind (_returnvalue_location _returnvalue_rotation) (`KismetMathLibrary.BreakTransform` (`SceneComponent.K2_GetComponentToWorld` (`self.Sphere`))))
  (if (< (`KismetArrayLibrary.Array_Length` (`self.Bullets`)) (`self.Max Bullet`))
    (bind _returnvalue (`|SpawnActorFromClass` "/Game/Objects/BP_Objects/BP_RifleBullet_Dummy.BP_RifleBullet_Dummy_C" (`KismetMathLibrary.MakeTransform` _returnvalue_location _returnvalue_rotation) "Undefined" "MultiplyWithRoot" null null))
    (`self.Set Flat Mode` _returnvalue "NewEnumerator0")
    (`KismetArrayLibrary.Array_Add` (`self.Bullets`) _returnvalue)
    (return _returnvalue)
    (else
      (for (_array_element _array_index) (`self.Bullets`)
        (if (`|EnumEquality` (`/Game/Objects/Structurs/FlatComponent.Mode` (`/Game/Objects/Structurs/BP_Object.FlatComponent` _array_element)) "NewEnumerator0")
          (`KismetArrayLibrary.Array_Add` _bullets _array_element)
          (`KismetArrayLibrary.Array_Remove` _bullets _array_index)
          (return (`|GetArrayItem` _bullets (`KismetArrayLibrary.Array_LastIndex` _bullets)))))
      (return null))))

(fn `UserConstructionScript`
  (`parent.UserConstructionScript`))
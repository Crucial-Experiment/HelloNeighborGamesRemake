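; BP_Brick is a brick object whose mesh is chosen from several single-brick and brick-block variants.
; The construction script switches on Model to set the Root static mesh, falling back to the first brick for unmatched values.
; A Destroy event removes the actor after a short delay, but only when its Destroy flag is set.
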(event `self.ReceiveBeginPlay`
  (`parent.ReceiveBeginPlay`))

(event `Destroy`
  (if (`self.Destroy?`)
    (`KismetSystemLibrary.Delay` 3.0)
    (`self.K2_DestroyActor`)))

(fn `UserConstructionScript`
  (bind _root (`self.Root`))
  (`parent.UserConstructionScript`)
  (switch `int` (`self.Model`)
    (:`Default`
      (`StaticMeshComponent.SetStaticMesh` _root "/Game/Objects/Meshes/brick_1_new.brick_1_new" :!label _label))
    (:`0`
      (goto _label))
    (:`1`
      (`StaticMeshComponent.SetStaticMesh` _root "/Game/Objects/Meshes/brick_2_new.brick_2_new"))
    (:`2`
      (`StaticMeshComponent.SetStaticMesh` _root "/Game/Objects/Meshes/brick_3_new.brick_3_new"))
    (:`3`
      (`StaticMeshComponent.SetStaticMesh` _root "/Game/Objects/Meshes/brick_block_1_new.brick_block_1_new"))
    (:`4`
      (`StaticMeshComponent.SetStaticMesh` _root "/Game/Objects/Meshes/brick_block_2_new.brick_block_2_new"))
    (:`5`
      (`StaticMeshComponent.SetStaticMesh` _root "/Game/Objects/Meshes/brick_block_3_new.brick_block_3_new"))
    (:`6`
      (`StaticMeshComponent.SetStaticMesh` _root "/Game/Objects/Meshes/brick_block_4_new.brick_block_4_new"))
    (:`7`
      (`StaticMeshComponent.SetStaticMesh` _root "/Game/Objects/Meshes/brick_block_5_new.brick_block_5_new"))))
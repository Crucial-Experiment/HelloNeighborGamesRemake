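; Shovel box object with a door that toggles open and closed and a placed spot for a linked shovel.
; The Open/Close event uses a FlipFlop to play or reverse a timeline that lerps the door's relative rotation.
; The Construction Script sets the flat mode of a valid Shovel reference and moves that actor to the box's ShovelScene transform.
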(event `Open / Close`
  (`/Engine/EditorBlueprintResources/StandardMacros.FlipFlop`
    (:`A`
      (bind (_direction _alpha) (`Timeline|Rotate Timeline` :!label _label)
        (:`Update`
          (`SceneComponent.K2_SetRelativeRotation` (`self.Door`) (`KismetMathLibrary.RLerp` (struct) (struct :`Roll` -100.0) _alpha) false false))))
    (:`B`
      (goto _label :!via `Reverse`))))

(fn `UserConstructionScript`
  (bind _shovel (`self.Shovel`)
    (:`then`
      (`/Game/Objects/Structurs/BP_Object.Set Flat Mode` _shovel "NewEnumerator1")
      (`self.K2_SetActorTransform` _shovel (`SceneComponent.K2_GetComponentToWorld` (`self.Shovel Scene`)) false false))
    (:`else`)))
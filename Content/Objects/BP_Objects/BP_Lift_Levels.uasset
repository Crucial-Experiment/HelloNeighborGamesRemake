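; BP_Lift_Levels is a floor indicator for a lift, with a rotating arrow and up to four level lights.
; BeginPlay unhides one light for each valid floor of the referenced Lift.
; Tick polls the lift's current floor and, on a change, lerps the arrow to that floor's preset rotation through a fixed-step Delay loop.
; Once the arrow arrives, the current floor's light gets the lit bulb material and the others the unlit one.
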(event `self.ReceiveBeginPlay`
  (bind _lift (`self.Lift`))
  (`/Engine/EditorBlueprintResources/StandardMacros.IsValid` _lift
    (:`Is Valid`
      (for (_array_element _array_index) (`/Game/Objects/BP_Objects/BP_Lift.Floors` _lift)
        (`/Engine/EditorBlueprintResources/StandardMacros.IsValid` _array_element
          (:`Is Valid`
            (`SceneComponent.SetHiddenInGame` (`|GetArrayItem` (`|MakeArray` (`self.Level 1`) (`self.Level 2`) (`self.Level 3`) (`self.Level 4`)) _array_index) false false)))))))

(event `self.ReceiveTick`
  (params (DeltaSeconds :type "Float (single-precision)"))
  (bind _lift (`self.Lift`)
    (:`then`
      (bind _flour (`/Game/Objects/BP_Objects/BP_Lift.Flour` _lift))
      (if (!= _flour (`self.Current Floar`))
        (set `self.Current Floar` _flour)
        (`self.Floor Changed`)))
    (:`else`)))

(event `Floor Changed`
  (set `self.Prev Rotation` (`SceneComponent.K2_GetComponentRotation` (`self.Arrow`)))
  (set `self.Alpha` 0.0)
  (`SceneComponent.K2_SetRelativeRotation` (`self.Arrow`) (`KismetMathLibrary.RLerp` (`self.Prev Rotation`) (`|GetArrayItem` (`self.Arrow Rotations`) (`self.Current Floar`)) (`self.Alpha`)) false false :!label _label)
  (set `self.Alpha` (+ (`self.Alpha`) (* (`self.Speed`) 0.0166)))
  (`KismetSystemLibrary.Delay` 0.0166)
  (if (>= (`self.Alpha`) 1.0)
    (for (_array_element _array_index) (`|MakeArray` (`self.Level 1`) (`self.Level 2`) (`self.Level 3`) (`self.Level 4`))
      (if (== _array_index (`self.Current Floar`))
        (`PrimitiveComponent.SetMaterial` _array_element 0 "/Game/Objects/Materials/dl_bulb_m.dl_bulb_m")
        (else
          (`PrimitiveComponent.SetMaterial` _array_element 0 "/Game/Objects/Materials/dl_bulb_m_off.dl_bulb_m_off"))))
    (else
      (goto _label))))

(fn `UserConstructionScript`)
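; BP_Terminal is a lockable terminal object that shows its state through red and green indicator lights and materials.
; The construction script starts it red when its Rotate reference is valid, otherwise green.
; Unlock extends the parent event: it sets a flat mode, switches materials and lights to green, plays an opening sound and disables pickup.
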(event `self.Unlock`
  (bind _root (`self.Root`))
  (`parent.Unlock`)
  (`self.Set Flat Mode` "NewEnumerator1")
  (`PrimitiveComponent.SetMaterial` _root 1 (`self.Off Red Material`))
  (`PrimitiveComponent.SetMaterial` _root 2 (`self.On Green Material`))
  (`SceneComponent.SetVisibility` (`self.Green Light`) true false)
  (`SceneComponent.SetVisibility` (`self.Red Light`) false false)
  (`GameplayStatics.PlaySoundAtLocation` "/Game/Sounds/Objects/OpenClosed/opening_opener_Cue.opening_opener_Cue" (`self.K2_GetActorLocation`) (struct) 1.0 1.0 0.0 null null null null)
  (set `self.CanPickUp` false))

(fn `UserConstructionScript`
  (bind _root (`self.Root`))
  (bind _red_light (`self.Red Light`))
  (`parent.UserConstructionScript`)
  (`self.Rotate`
    (:`then`
      (`PrimitiveComponent.SetMaterial` _root 1 (`self.On Red Material`))
      (`PrimitiveComponent.SetMaterial` _root 2 (`self.Off Green Material`))
      (`SceneComponent.SetVisibility` (`self.Green Light`) false false)
      (`SceneComponent.SetVisibility` _red_light true false))
    (:`else`
      (`PrimitiveComponent.SetMaterial` _root 1 (`self.Off Red Material`))
      (`PrimitiveComponent.SetMaterial` _root 2 (`self.On Green Material`))
      (`SceneComponent.SetVisibility` (`self.Green Light`) true false)
      (`SceneComponent.SetVisibility` _red_light false false))))
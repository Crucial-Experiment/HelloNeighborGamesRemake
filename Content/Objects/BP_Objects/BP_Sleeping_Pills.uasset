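; BP_Sleeping_Pills is a holdable item the player uses to poison a milk bottle.
; On left click while held, or on VR use, it line-traces for a BP_Milk_Bottle, swaps its material to poisoned milk, sets its poison flag and resets the poison timer.
; It then reports the use to tutorial and GameJolt components, releases itself and is destroyed.
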(event `self.ReceiveBeginPlay`
  (`parent.ReceiveBeginPlay`))

(event `On Press LMB_1`
  (bind _player (`/Game/Function/BP_MacroLibrary.Find Player`)
    (:`Is Valid`
      (bind _item (`/Game/Player/BP_Player.Get Item` _player))
      (if (== _item self)
        (bind _actor (`self.Line Trace` 200.0 "NewEnumerator1" :!label _label))
        (bind _asbp_milk_bottle (cast `/Game/Objects/BP_Objects/BP_Milk_Bottle` _actor))
        (`PrimitiveComponent.SetMaterial` (`/Game/Objects/Structurs/BP_Object.Root` _asbp_milk_bottle) 0 "/Game/Objects/Materials/bottle_milk_poisoned.bottle_milk_poisoned")
        (set `/Game/Objects/BP_Objects/BP_Milk_Bottle.Poisen` true _asbp_milk_bottle)
        (set `/Game/Objects/BP_Objects/BP_Milk_Bottle.Poisen Time Temp` 0 _asbp_milk_bottle)
        (`/Game/Objects/Tutorial/TutorialComponent.Check Use Type` (`self.TutorialComponent`) "NewEnumerator6")
        (`/Game/Objects/GameJolt/GameJoltComponent.Check Use Type` (`self.GameJoltComponent`) "NewEnumerator6")
        (`self.Try Release`)
        (`self.K2_DestroyActor`)))))

(event `self.On VR Use`
  (`parent.On VR Use`)
  (goto _label))

(fn `UserConstructionScript`)
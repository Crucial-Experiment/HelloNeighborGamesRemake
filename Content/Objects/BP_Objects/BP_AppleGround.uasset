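; Plantable ground plot that grows an apple tree from a planted, watered seed.
; Watering scales the tree up to sprout size, then Tick grows it to full size, teleports the Apple to its socket and enables Box overlaps.
; An overlap switches the Apple's flat mode and clears its reference.
; Save/load extends the parent's JSON with growth state, though "Is Pour" loads into IsSeed instead of IsPour.
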(event `self.ReceiveBeginPlay`
  (`parent.ReceiveBeginPlay`)
  (`SceneComponent.SetRelativeScale3D` (`self.Tree`) (0.0 0.0 0.0)))

(event `self.ReceiveTick`
  (params (DeltaSeconds :type "Float (single-precision)"))
  (if (and (`self.IsSeed`) (`self.IsPour`) (< (`self.Scale`) 1.0))
    (bind _output_get (set `self.Scale` (+ (`self.Scale`) (* DeltaSeconds (`self.SpeedScaleTree`)))))
    (if (>= _output_get 1.0)
      (set `self.Scale` 1.0)
      (`self.K2_SetActorLocation` (`self.Apple`) (`SceneComponent.K2_GetComponentLocation` (`self.Socket`)) false true)
      (`self.Set Flat Mode` (`self.Apple`) "NewEnumerator1")
      (set `PrimitiveComponent.bGenerateOverlapEvents` true (`self.Box`)))
    (`SceneComponent.SetRelativeScale3D` (`self.Tree`) (`KismetMathLibrary.Conv_DoubleToVector` (`self.Scale`)))))

(event `self.Box.OnComponentBeginOverlap`
  (params (OverlappedComponent :type "PrimitiveComponent Object Reference") (OtherActor :type "Actor Object Reference") (OtherComp :type "PrimitiveComponent Object Reference") (OtherBodyIndex :type Integer) (bFromSweep :type Boolean) (SweepResult :type "HitResult Structure (by ref)"))
  (`self.Set Flat Mode` (`self.Apple`) "NewEnumerator0")
  (set `self.Apple` null))

(fn `Has Seed`
  (returns (IsSeed :type Boolean))
  (return (`self.IsSeed`)))

(fn `Load Data`
  (params (JSON :type String))
  (returns (Object :type "VaRestJsonObject Object Reference"))
  (bind _object (`parent.Load Data` JSON))
  (`|ExecutionSequence`
    (:`then_0`
      (bind (_has_field_ _return_value) (`/Game/Function/BP_JSON_FunctionLibrary.Get Value As Bool` _object "Is Seed"))
      (if _has_field_
        (set `self.IsSeed` _return_value)))
    (:`then_1`
      (bind (_has_field__2 _return_value_2) (`/Game/Function/BP_JSON_FunctionLibrary.Get Value As Bool` _object "Is Pour"))
      (if _has_field__2
        (set `self.IsSeed` _return_value_2)))
    (:`then_2`
      (bind (_has_field__3 _return_value_3) (`/Game/Function/BP_JSON_FunctionLibrary.Get Value As Float` _object "Scale"))
      (if _has_field__3
        (set `self.Scale` _return_value_3)))
    (:`then_3`
      (return _object))))

(fn `Plant Seed`
  (set `self.IsSeed` true)
  (set `self.Scale` 0.0))

(fn `Save Data`
  (returns (JSON :type "VaRestJsonObject Object Reference"))
  (bind _json (`parent.Save Data`))
  (`VaRestJsonObject.SetBoolField` _json "Is Seed" (`self.IsSeed`))
  (`VaRestJsonObject.SetBoolField` _json "Is Pour" (`self.IsPour`))
  (`VaRestJsonObject.SetNumberField` _json "Scale" (`self.Scale`))
  (return _json))

(fn `UserConstructionScript`
  (`parent.UserConstructionScript`))

(fn `Watering`
  (if (and (`self.IsSeed`) (not (`self.IsPour`)))
    (bind _output_get (set `self.Scale` (+ (`self.Scale`) (* (`GameplayStatics.GetWorldDeltaSeconds`) (`self.SpeedScaleSprout`)))))
    (if (>= _output_get (`self.ScaleSprout`))
      (set `self.IsPour` true))
    (`SceneComponent.SetRelativeScale3D` (`self.Tree`) (`KismetMathLibrary.Conv_DoubleToVector` (`self.Scale`)))))
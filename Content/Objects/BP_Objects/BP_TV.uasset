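; Interactive TV that toggles screen, lights and sound or media playback, and can lure the Neighbor.
; Switching it on with electricity sends the Neighbor to check it through blackboard keys, depending on the Neighbor's current state.
; Toggles pass through server and all-client events, with a generator as alternative power.
; Saves store the on/off state, and loading calls the remote toggle when it differs.
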(event `RemoteTV`
  (params (`Neighbor?` :type Boolean))
  (if (not `Neighbor?`)
    (if (`|EnumInequality` (`self.State`) "NewEnumerator0") :!label _label
      (if (`self.Has Electricity`)
        ;[1 1 1] Neighbor coming to check
        (bind _sosed (`/Game/Function/BP_MacroLibrary.Find Sosed`)
          (:`Is Valid`
            (if (`|EnumInequality` (`/Game/Sosed/BP_Sosed.Current State` _sosed) "NewEnumerator2")
              (bind _returnvalue (`AIBlueprintHelperLibrary.GetBlackboard` _sosed))
              (`BlackboardComponent.SetValueAsInt` _returnvalue "CheckTask" 8)
              (`BlackboardComponent.SetValueAsVector` _returnvalue "Check Location" (`SceneComponent.K2_GetComponentLocation` (`self.Arrow`)))
              (`BlackboardComponent.SetValueAsObject` _returnvalue "CheckActor" self)
              (`/Game/Sosed/BP_Sosed.Set State` _sosed "NewEnumerator3")
              (if (or (`self.Has Electricity`) (`self.Generator`)) :!label _label_2
                (`self.Interact (Server)` (select `/Game/Objects/Enum/TumblerStateEnum` (`self.State`) :`NewEnumerator0` "NewEnumerator1" :`NewEnumerator1` "NewEnumerator0" :!type "/Game/Objects/Enum/TumblerStateEnum Enum"))
                (else
                  (`self.Interact (Server)` "NewEnumerator1")))))
          (:`Is Not Valid`
            (`/Game/Objects/Tutorial/TutorialComponent.Check Use Type` (`self.TutorialComponent`) "NewEnumerator6" :!label _label_3)
            (`/Game/Objects/GameJolt/GameJoltComponent.Check Use Type` (`self.GameJoltComponent`) "NewEnumerator6")
            (goto _label_2))))
      (else
        (goto _label_3)))
    (else
      (goto _label_3))))

(event `self.On VR Use`
  (`parent.On VR Use`)
  (goto _label))

(event `/Game/Function/BP_Interface.Interact`
  (params (Component :type "PrimitiveComponent Object Reference") (Location :type "Vector Structure"))
  (goto _label))

(event `self.On Press LMB`
  (`parent.On Press LMB`)
  (bind _player (`/Game/Function/BP_MacroLibrary.Find Player`)
    (:`Is Valid`
      (bind _item (`/Game/Player/BP_Player.Get Item` _player))
      (if (== _item self)
        (goto _label_2)))))

(event `Interact (All)`
  (params (`New State` :type "/Game/Objects/Enum/TumblerStateEnum Enum" :default "NewEnumerator0"))
  (bind _root (`self.Root`))
  (bind _media_player (`self.Media Player`))
  (bind _display_mat_id (`self.Display Mat Id`))
  (bind _tv_sound (`self.TV Sound`))
  (bind _rectlight (`self.RectLight`))
  (switch `/Game/Objects/Enum/TumblerStateEnum` `New State`
    (:`NewEnumerator0`
      (`self.Media Source`
        (:`then`
          _)
        (:`else`
          (`AudioComponent.Play` _tv_sound 0.0)))
      (`LightComponent.SetIntensity` _rectlight 14.0)
      (`LightComponent.SetIntensity` (`self.PointLight`) 14.0)
      (set `self.State` "NewEnumerator0")
      (`self.Media Source`
        (:`then`
          (`MediaPlayer.Play` _media_player)
          (`PrimitiveComponent.SetMaterial` (`self.Root`) (`self.Display Mat Id`) (`self.Display Media Player`)))
        (:`else`
          (`PrimitiveComponent.SetMaterial` _root _display_mat_id (`self.Display On`)))))
    (:`NewEnumerator1`
      (`AudioComponent.Stop` _tv_sound)
      (`LightComponent.SetIntensity` _rectlight 0.0)
      (`LightComponent.SetIntensity` (`self.PointLight`) 0.0)
      (set `self.State` "NewEnumerator1")
      (`PrimitiveComponent.SetMaterial` _root _display_mat_id (`self.Display Off`))
      (`MediaPlayer.Pause` _media_player))))

(event `Interact (Server)`
  (params (`New State` :type "/Game/Objects/Enum/TumblerStateEnum Enum" :default "NewEnumerator0"))
  (`self.Interact (All)` `New State`))

(event `Open Media`
  (bind _media_player (`self.Media Player`)
    (:`then`
      (`MediaSoundComponent.SetMediaPlayer` (`self.MediaSound`) _media_player)
      (bind _media_source (`self.Media Source`)
        (:`then`
          (`MediaPlayer.OpenSourceWithOptions` _media_player _media_source (make `MediaPlayerOptions` (struct :`Caption` -1 :`Metadata` -1 :`Script` -1 :`Subtitle` -1 :`Text` -1) "UseTrackOptionIndices" "+00000000.00:00:00.000000000" "RelativeToStartTime" "Disabled")))
        (:`else`)))
    (:`else`)))

(event `self.ReceiveBeginPlay`
  (`parent.ReceiveBeginPlay`)
  (`self.Open Media`))

(event `self.Disable`
  (`parent.Disable`)
  (`AudioComponent.Stop` (`self.TV Sound`))
  (`MediaPlayer.Pause` (`self.Media Player`))
  (`LightComponent.SetIntensity` (`self.RectLight`) 0.0)
  (`LightComponent.SetIntensity` (`self.PointLight`) 0.0)
  (`PrimitiveComponent.SetMaterial` (`self.Root`) (`self.Display Mat Id`) (`self.Display Off`)))

(event `self.Enable`
  (`parent.Enable`)
  (if (`|EnumEquality` (`self.State`) "NewEnumerator0")
    (`self.Media Source`
      (:`then`
        _)
      (:`else`
        (`AudioComponent.Play` (`self.TV Sound`) 0.0)))
    (`LightComponent.SetIntensity` (`self.RectLight`) 14.0)
    (`LightComponent.SetIntensity` (`self.PointLight`) 14.0)
    (`self.Media Source`
      (:`then`
        (`MediaPlayer.Play` (`self.Media Player`))
        (`PrimitiveComponent.SetMaterial` (`self.Root`) (`self.Display Mat Id`) (`self.Display Media Player`)))
      (:`else`
        (`PrimitiveComponent.SetMaterial` (`self.Root`) (`self.Display Mat Id`) (`self.Display On`))))))

(fn `Load Data`
  (params (JSON :type String))
  (returns (Object :type "VaRestJsonObject Object Reference"))
  (bind _object (`parent.Load Data` JSON))
  (if (!= (`VaRestJsonObject.GetIntegerField` _object "State") (`KismetMathLibrary.Conv_ByteToInt` (`self.State`)))
    (`self.RemoteTV` false)
    (return _object)))

(fn `Save Data`
  (returns (JSON :type "VaRestJsonObject Object Reference"))
  (bind _json (`parent.Save Data`))
  (`VaRestJsonObject.SetIntegerField` _json "State" (`KismetMathLibrary.Conv_ByteToInt` (`self.State`)))
  (return _json))

(fn `UserConstructionScript`)
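; BP_Grave is a grave object that reacts to bell and grave-top events by removing parts of itself.
; GraveBell destroys BellBox, then calls OpenClose on ShovelBox if it is valid.
; GraveTop destroys the Top component once GraveTopCount is zero or below; the count is only read here, never changed.
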(event `Grave Bell`
  (bind _shovel_box (`self.Shovel Box`))
  (`ActorComponent.K2_DestroyComponent` (`self.Bell Box`))
  (`/Engine/EditorBlueprintResources/StandardMacros.IsValid` _shovel_box
    (:`Is Valid`
      (`/Game/Objects/BP_Objects/BP_Shovel_Box.Open / Close` _shovel_box))))

(event `Grave Top`
  (if (<= (`self.Grave Top Count`) 0)
    (`ActorComponent.K2_DestroyComponent` (`self.Top`))))

(fn `UserConstructionScript`)
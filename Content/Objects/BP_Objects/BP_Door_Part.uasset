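; BP_Door_Part is a door piece whose surface material is chosen by a Material enum of default, white or red.
; The construction script applies the matching material to element 0 of the Root mesh after running the parent script, so the choice shows in the editor.
; A SetMaterial event stores a new value and repeats the same switch, allowing the look to change at runtime.
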(event `Set Material`
  (params (`New Material` :type "/Game/Objects/Enum/DoorMaterialEnim Enum" :default "NewEnumerator0"))
  (bind _root (`self.Root`))
  (bind _output_get (set `self.Material` `New Material`))
  (switch `/Game/Objects/Enum/DoorMaterialEnim` _output_get
    (:`NewEnumerator0`
      (`PrimitiveComponent.SetMaterial` _root 0 "/Game/Objects/Materials/door_m_new.door_m_new"))
    (:`NewEnumerator1`
      (`PrimitiveComponent.SetMaterial` _root 0 "/Game/Objects/Materials/door_white_Mat.door_white_Mat"))
    (:`NewEnumerator2`
      (`PrimitiveComponent.SetMaterial` _root 0 "/Game/Objects/Materials/door_red_Mat.door_red_Mat"))))

(fn `UserConstructionScript`
  (bind _root (`self.Root`))
  (`parent.UserConstructionScript`)
  (switch `/Game/Objects/Enum/DoorMaterialEnim` (`self.Material`)
    (:`NewEnumerator0`
      (`PrimitiveComponent.SetMaterial` _root 0 "/Game/Objects/Materials/door_m_new.door_m_new"))
    (:`NewEnumerator1`
      (`PrimitiveComponent.SetMaterial` _root 0 "/Game/Objects/Materials/door_white_Mat.door_white_Mat"))
    (:`NewEnumerator2`
      (`PrimitiveComponent.SetMaterial` _root 0 "/Game/Objects/Materials/door_red_Mat.door_red_Mat"))))
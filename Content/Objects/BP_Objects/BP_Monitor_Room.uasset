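; Monitor room object whose power button switches a bank of screens and every unbroken BP_Camera in the level on or off.
; A press by Interact, relayed through server to all clients, or by VR hand overlap requires electricity or a generator.
; A timeline animates the button, then applies screen materials, toggles the Room component and notifies tutorial and GameJolt components.
; Disable forces screens and cameras off, while Enable restores them if previously on.
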(event `self.ReceiveBeginPlay`
  ;[1 1 1] Begin Play and Electricity
  (switch `/Game/Objects/Enum/TumblerStateEnum` (`self.State`)
    (:`NewEnumerator0`
      (if (or (`self.Generator`) (`self.Has Electricity`))
        (`self.Set State` "NewEnumerator0")
        (else
          (`self.Set State` "NewEnumerator1"))))))

(event `/Game/Function/BP_Interface.Interact`
  (params (Component :type "PrimitiveComponent Object Reference") (Location :type "Vector Structure"))
  ;[1 1 1] Interact
  (`self.Interact (Server)` Component))

(event `Interact (Server)`
  (params (Component :type "PrimitiveComponent Object Reference"))
  ;[1 1 1] Interact
  (`self.Interact (All)` Component))

(event `Interact (All)`
  (params (Component :type "PrimitiveComponent Object Reference"))
  (bind _tutorialcomponent (`self.TutorialComponent`))
  (bind _gamejoltcomponent (`self.GameJoltComponent`))
  ;[1 1 1] Interact
  (if (== Component (`self.Button`))
    (if (or (`self.Has Electricity`) (`self.Generator`)) :!label _label
      (`/Game/Objects/Tutorial/TutorialComponent.Check Use Type` (`self.TutorialComponent`) "NewEnumerator6")
      (`/Game/Objects/GameJolt/GameJoltComponent.Check Use Type` (`self.GameJoltComponent`) "NewEnumerator6")
      (switch `/Game/Objects/Enum/RotateStateEnum` (`self.Button Loc State`)
        (:`NewEnumerator0`
          (set `self.Button Loc State` "NewEnumerator3")
          (`|ExecutionSequence`
            (:`then_0`
              (bind (_direction _alpha) (`Timeline|Button Timeline` :!via `PlayFromStart` :!label _label_2)
                (:`Update`
                  (`SceneComponent.K2_SetRelativeLocation` (`self.Button`) (`KismetMathLibrary.VLerp` (select `/Game/Objects/Enum/TumblerStateEnum` (`self.State`) :`NewEnumerator1` (0.0 0.0 -2.0) :!type "Vector Structure") (select `/Game/Objects/Enum/TumblerStateEnum` (`self.State`) :`NewEnumerator0` (0.0 0.0 -2.0) :`NewEnumerator1` (0.0 0.0 2.0) :!type "Vector Structure") _alpha) false false))
                (:`Finished`
                  (switch `/Game/Objects/Enum/RotateStateEnum` (`self.Button Loc State`)
                    (:`NewEnumerator2`
                      (set `self.Button Loc State` "NewEnumerator0")
                      (`self.Set State` "NewEnumerator0")
                      (set `self.State` "NewEnumerator0")
                      (`/Game/Objects/Tutorial/TutorialComponent.Check Use Type` _tutorialcomponent "NewEnumerator3")
                      (`/Game/Objects/GameJolt/GameJoltComponent.Check Use Type` _gamejoltcomponent "NewEnumerator3"))
                    (:`NewEnumerator3`
                      (set `self.Button Loc State` "NewEnumerator1")
                      (`self.Set State` "NewEnumerator1")
                      (set `self.State` "NewEnumerator1")
                      (`/Game/Objects/Tutorial/TutorialComponent.Check Use Type` _tutorialcomponent "NewEnumerator4")
                      (`/Game/Objects/GameJolt/GameJoltComponent.Check Use Type` _gamejoltcomponent "NewEnumerator4")))
                  (`self.Set Cameras State` (`self.State`)))))))
        (:`NewEnumerator1`
          (set `self.Button Loc State` "NewEnumerator2")
          (goto _label_2 :!via `PlayFromStart`))))))

(event `self.Disable`
  ;[1 1 1] Begin Play and Electricity
  (`parent.Disable`)
  (`self.Set State` "NewEnumerator1")
  (`self.Set Cameras State` "NewEnumerator1"))

(event `self.Button.OnComponentBeginOverlap`
  (params (OverlappedComponent :type "PrimitiveComponent Object Reference") (OtherActor :type "Actor Object Reference") (OtherComp :type "PrimitiveComponent Object Reference") (OtherBodyIndex :type Integer) (bFromSweep :type Boolean) (SweepResult :type "HitResult Structure (by ref)"))
  ;[1 1 1] Interact
  (if (`self.Overlap VR Hands` OtherActor OtherComp)
    (goto _label)))

(event `self.Enable`
  ;[1 1 1] Begin Play and Electricity
  (`parent.Enable`)
  (switch `/Game/Objects/Enum/TumblerStateEnum` (`self.State`)
    (:`NewEnumerator0`
      (`self.Set State` "NewEnumerator0")
      (`self.Set Cameras State` "NewEnumerator0"))))

(fn `Set Cameras State`
  (params (`New State` :type "/Game/Objects/Enum/TumblerStateEnum Enum" :default "NewEnumerator0"))
  (bind _outactors (`GameplayStatics.GetAllActorsOfClass` "/Game/Objects/BP_Objects/BP_Camera.BP_Camera_C"))
  (for _array_element _outactors
    (if (not (`/Game/Objects/BP_Objects/BP_Camera.Broken` _array_element))
      (`/Game/Objects/BP_Objects/BP_Camera.Set State` _array_element `New State`))))

(fn `Set State`
  (params (`New State` :type "/Game/Objects/Enum/TumblerStateEnum Enum" :default "NewEnumerator0"))
  (bind _root (`self.Root`))
  (bind _root_2 (`self.Root`))
  (switch `/Game/Objects/Enum/TumblerStateEnum` `New State`
    (:`NewEnumerator0`
      (`PrimitiveComponent.SetMaterial` _root 10 "/Game/Objects/Materials/tv_display_on.tv_display_on")
      (`PrimitiveComponent.SetMaterial` _root 11 "/Game/Objects/Materials/tv_display_on.tv_display_on")
      (`PrimitiveComponent.SetMaterial` _root 15 "/Game/Objects/Materials/tv_display_on.tv_display_on")
      (`PrimitiveComponent.SetMaterial` _root 17 "/Game/Objects/Materials/tv_display_on.tv_display_on")
      (`PrimitiveComponent.SetMaterial` _root 19 "/Game/Objects/Materials/tv_display_on.tv_display_on")
      (`PrimitiveComponent.SetMaterial` _root 21 "/Game/Objects/Materials/tv_display_on.tv_display_on")
      (`PrimitiveComponent.SetMaterial` _root 22 "/Game/Objects/Materials/tv_display_on.tv_display_on")
      (`PrimitiveComponent.SetMaterial` _root 25 "/Game/Objects/Materials/tv_display_on.tv_display_on")
      (`PrimitiveComponent.SetMaterial` _root 27 "/Game/Objects/Materials/tv_display_on.tv_display_on")
      (`ActorComponent.Activate` (`self.Room`) false))
    (:`NewEnumerator1`
      (`PrimitiveComponent.SetMaterial` _root_2 10 "/Game/Objects/Materials/monitor_display_off.monitor_display_off")
      (`PrimitiveComponent.SetMaterial` _root_2 11 "/Game/Objects/Materials/monitor_display_off.monitor_display_off")
      (`PrimitiveComponent.SetMaterial` _root_2 15 "/Game/Objects/Materials/monitor_display_off.monitor_display_off")
      (`PrimitiveComponent.SetMaterial` _root_2 17 "/Game/Objects/Materials/monitor_display_off.monitor_display_off")
      (`PrimitiveComponent.SetMaterial` _root_2 19 "/Game/Objects/Materials/monitor_display_off.monitor_display_off")
      (`PrimitiveComponent.SetMaterial` _root_2 21 "/Game/Objects/Materials/monitor_display_off.monitor_display_off")
      (`PrimitiveComponent.SetMaterial` _root_2 22 "/Game/Objects/Materials/monitor_display_off.monitor_display_off")
      (`PrimitiveComponent.SetMaterial` _root_2 25 "/Game/Objects/Materials/monitor_display_off.monitor_display_off")
      (`PrimitiveComponent.SetMaterial` _root_2 27 "/Game/Objects/Materials/monitor_display_off.monitor_display_off")
      (`ActorComponent.Deactivate` (`self.Room`)))))

(fn `UserConstructionScript`
  (`self.Set State` (`self.State`)))
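; School board puzzle actor that spawns a reward once when its 5, 3 and 8 slots hold the matching magnet classes.
; Construction snaps assigned magnets into place; BeginPlay changes their flat mode, links them to the board and disables their slot triggers.
; A one-second timer checks the classroom teacher; without one, assigned magnets are released and all triggers re-enabled.
; CheckBoard validates the slots, spawns the reward and notifies the tutorial and GameJolt components.
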(event `Check Board`
  (bind (_returnvalue_location _returnvalue_rotation) (`KismetMathLibrary.BreakTransform` (`SceneComponent.K2_GetComponentToWorld` (`self.Spawn Position`))))
  ;[1 1 1] Check
  (if (and (== (`GameplayStatics.GetObjectClass` (`self.5 Magnet`)) "/Game/Objects/BP_Objects/BP_5_Magnet.BP_5_Magnet_C") (== (`GameplayStatics.GetObjectClass` (`self.3 Magnet`)) "/Game/Objects/BP_Objects/BP_3_Magnet.BP_3_Magnet_C") (== (`GameplayStatics.GetObjectClass` (`self.8 Magnet`)) "/Game/Objects/BP_Objects/BP_8_Magnet.BP_8_Magnet_C") (not (`self.Given`)) (`KismetSystemLibrary.IsValidClass` (`self.Spawn`)))
    (`|SpawnActorFromClass` (`self.Spawn`) (`KismetMathLibrary.MakeTransform` _returnvalue_location _returnvalue_rotation) "Undefined" "SelectDefaultAtRuntime" null null)
    (set `self.Given` true)
    (`/Game/Objects/Tutorial/TutorialComponent.Check Use Type` (`self.TutorialComponent`) "NewEnumerator6")
    (`/Game/Objects/GameJolt/GameJoltComponent.Check Use Type` (`self.GameJoltComponent`) "NewEnumerator6")))

(event `self.ReceiveBeginPlay`
  ;[1 1 1] Begin Play
  (`|ExecutionSequence`
    (:`then_0`
      (bind _5_magnet (`self.5 Magnet`)
        (:`then`
          (`/Game/Objects/Structurs/BP_Object.Set Flat Mode` _5_magnet "NewEnumerator1")
          (`PrimitiveComponent.SetCollisionEnabled` (`self.5 Magnet Trigger`) "NoCollision")
          (set `/Game/Objects/BP_Objects/BP_1_Magnet.School Board` self (`self.5 Magnet`)))
        (:`else`)))
    (:`then_1`
      (bind _3_magnet (`self.3 Magnet`)
        (:`then`
          (`/Game/Objects/Structurs/BP_Object.Set Flat Mode` _3_magnet "NewEnumerator1")
          (`PrimitiveComponent.SetCollisionEnabled` (`self.3 Magnet Trigger`) "NoCollision")
          (set `/Game/Objects/BP_Objects/BP_1_Magnet.School Board` self (`self.3 Magnet`)))
        (:`else`)))
    (:`then_2`
      (bind _8_magnet (`self.8 Magnet`)
        (:`then`
          (`/Game/Objects/Structurs/BP_Object.Set Flat Mode` _8_magnet "NewEnumerator1")
          (`PrimitiveComponent.SetCollisionEnabled` (`self.8 Magnet Trigger`) "NoCollision")
          (set `/Game/Objects/BP_Objects/BP_1_Magnet.School Board` self (`self.8 Magnet`)))
        (:`else`)))
    (:`then_3`
      (`KismetSystemLibrary.K2_SetTimerDelegate` (delegate `Check Teacher`) 1.0 true))))

(event `Check Teacher`
  (bind _class_room (`self.Class Room`)
    (:`then`
      (`/Game/Objects/BP_Objects/BP_Class_Room.Teacher` _class_room
        (:`then`)
        (:`else`
          _)))
    (:`else`
      _))
  (`|ExecutionSequence`
    (:`then_0`
      (bind _5_magnet (`self.5 Magnet`)
        (:`then`
          (`/Game/Objects/Structurs/BP_Object.Set Flat Mode` _5_magnet "NewEnumerator0")
          (set `self.5 Magnet` null))
        (:`else`)))
    (:`then_1`
      (bind _3_magnet (`self.3 Magnet`)
        (:`then`
          (`/Game/Objects/Structurs/BP_Object.Set Flat Mode` _3_magnet "NewEnumerator0")
          (set `self.3 Magnet` null))
        (:`else`)))
    (:`then_2`
      (bind _8_magnet (`self.8 Magnet`)
        (:`then`
          (`/Game/Objects/Structurs/BP_Object.Set Flat Mode` _8_magnet "NewEnumerator0")
          (set `self.8 Magnet` null))
        (:`else`))))
  (`PrimitiveComponent.SetCollisionEnabled` (`self.8 Magnet Trigger`) "QueryAndPhysics")
  (`PrimitiveComponent.SetCollisionEnabled` (`self.3 Magnet Trigger`) "QueryAndPhysics")
  (`PrimitiveComponent.SetCollisionEnabled` (`self.5 Magnet Trigger`) "QueryAndPhysics"))

(fn `UserConstructionScript`
  (bind _5_magnet (`self.5 Magnet`))
  (bind _3_magnet (`self.3 Magnet`))
  (bind _8_magnet (`self.8 Magnet`))
  (`|ExecutionSequence`
    (:`then_0`
      (`/Engine/EditorBlueprintResources/StandardMacros.IsValid` _5_magnet
        (:`Is Valid`
          (`self.K2_SetActorTransform` _5_magnet (`SceneComponent.K2_GetComponentToWorld` (`self.5 Magnet Position`)) false false))))
    (:`then_1`
      (`/Engine/EditorBlueprintResources/StandardMacros.IsValid` _3_magnet
        (:`Is Valid`
          (`self.K2_SetActorTransform` _3_magnet (`SceneComponent.K2_GetComponentToWorld` (`self.3 Magnet Position`)) false false))))
    (:`then_2`
      (`/Engine/EditorBlueprintResources/StandardMacros.IsValid` _8_magnet
        (:`Is Valid`
          (`self.K2_SetActorTransform` _8_magnet (`SceneComponent.K2_GetComponentToWorld` (`self.8 Magnet Position`)) false false))))))
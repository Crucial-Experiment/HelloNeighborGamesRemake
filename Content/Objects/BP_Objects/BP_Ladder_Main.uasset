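; Climbable ladder that lets non-VR players move along it and carries a nav link.
; Overlapping LadderBox sends a server event that sets the player's IsLadder flag and switches movement to Flying; leaving restores Walking.
; VR players skip this switch, and BeginPlay sets the GrabComponent's grab type after the parent's logic.
; The construction script configures the child-actor BP_NavLinkProxy with fixed endpoints.
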(event `Box In (Server)`
  (params (Character :type "/Game/Player/BP_Player Object Reference"))
  (set `/Game/Player/BP_Player.Is Ladder` true Character)
  (`CharacterMovementComponent.SetMovementMode` (`Character.CharacterMovement` Character) "MOVE_Flying" 0))

(event `Box Out (Server)`
  (params (Character :type "/Game/Player/BP_Player Object Reference"))
  (set `/Game/Player/BP_Player.Is Ladder` false Character)
  (`CharacterMovementComponent.SetMovementMode` (`Character.CharacterMovement` Character) "MOVE_Walking" 0))

(event `self.ReceiveBeginPlay`
  (`parent.ReceiveBeginPlay`)
  (set `/Game/Objects/Structurs/GrabComponent.GrabType` "NewEnumerator3" (`self.GrabComponent`)))

(event `self.Ladder Box.OnComponentBeginOverlap`
  (params (OverlappedComponent :type "PrimitiveComponent Object Reference") (OtherActor :type "Actor Object Reference") (OtherComp :type "PrimitiveComponent Object Reference") (OtherBodyIndex :type Integer) (bFromSweep :type Boolean) (SweepResult :type "HitResult Structure (by ref)"))
  (bind _asbp_player (cast `/Game/Player/BP_Player` OtherActor))
  (if (not (`/Game/Player/BP_Player.Start VR` _asbp_player))
    (`self.Box In (Server)` _asbp_player)))

(event `self.Ladder Box.OnComponentEndOverlap`
  (params (OverlappedComponent :type "PrimitiveComponent Object Reference") (OtherActor :type "Actor Object Reference") (OtherComp :type "PrimitiveComponent Object Reference") (OtherBodyIndex :type Integer))
  (bind _asbp_player (cast `/Game/Player/BP_Player` OtherActor))
  (if (not (`/Game/Player/BP_Player.Start VR` _asbp_player))
    (`self.Box Out (Server)` _asbp_player)))

(fn `UserConstructionScript`
  (bind _asbp_nav_link_proxy (cast `/Game/Objects/Structurs/BP_NavLinkProxy` (`ChildActorComponent.ChildActor` (`self.Nav Link`))))
  (`/Game/Objects/Structurs/BP_NavLinkProxy.Set Nav Link` _asbp_nav_link_proxy (0.0 0.0 20.0) (0.0 -160.0 530.0) "Auto"))
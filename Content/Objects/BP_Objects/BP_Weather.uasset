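; Weather actor that keeps a rain particle effect and rain sound over the player.
; On BeginPlay it finds the player and starts a looping one-second timer that moves the actor to the player's X and Y while keeping its own height.
; Enable and Disable events activate or deactivate the rain particles and world audio cue together.
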(event `self.ReceiveBeginPlay`
  (bind _player (`/Game/Function/BP_MacroLibrary.Find Player`)
    (:`Is Valid`
      (set `self.Player` _player)
      (`KismetSystemLibrary.K2_SetTimerDelegate` (delegate `Set Weather Location`) 1.0 true true))))

(event `Set Weather Location`
  (bind (_returnvalue_x _returnvalue_y _returnvalue_z) (`KismetMathLibrary.BreakVector` (`self.K2_GetActorLocation`)))
  (bind (_returnvalue_x_2 _returnvalue_y_2) (`KismetMathLibrary.BreakVector` (`self.K2_GetActorLocation` (`self.Player`))))
  (`self.K2_SetActorLocation` (`KismetMathLibrary.MakeVector` _returnvalue_x_2 _returnvalue_y_2 _returnvalue_z)))

(event `Enable`
  (`ActorComponent.Activate` (`self.P_Rain`) false)
  (`ActorComponent.Activate` (`self.rain_world_Cue`) false))

(event `Disable`
  (`ActorComponent.Deactivate` (`self.P_Rain`))
  (`ActorComponent.Deactivate` (`self.rain_world_Cue`)))

(fn `UserConstructionScript`)
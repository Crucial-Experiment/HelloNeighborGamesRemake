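; BP_Vinyl is a grabbable vinyl record with its own sound and material that plays on BP_Stereo_System.
; Using it in VR, or left-clicking while holding it, line-traces for an empty stereo, snaps the record onto it, hands over the sound and reports to tutorial and GameJolt components.
; Picking up or grabbing it detaches it from the stereo's state, stopping the music and its linked speakers.
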(event `self.GrabComponent.OnDropped`
  (params (`Self Ref` :type "/Game/Objects/Structurs/GrabComponent Object Reference"))
  (`self.Stereo System`
    (:`then`)
    (:`else`
      (`self.Set Flat Mode` "NewEnumerator0"))))

(event `/Game/Function/BP_Interface.PickUp`
  (`parent.PickUp`)
  (bind _stereo_system (`self.Stereo System` :!label _label)
    (:`then`
      (set `/Game/Objects/BP_Objects/BP_Stereo_System.Vinyl` null _stereo_system)
      (set `/Game/Objects/BP_Objects/BP_Stereo_System.State` "NewEnumerator1" _stereo_system)
      (`AudioComponent.Stop` (`/Game/Objects/BP_Objects/BP_Stereo_System.Music` _stereo_system))
      (for _array_element (`/Game/Objects/BP_Objects/BP_Stereo_System.Dynamics` _stereo_system)
        (`AudioComponent.Stop` (`/Game/Objects/BP_Objects/BP_Stereo_System_Dynamic.Music` _array_element)))
      (set `self.Stereo System` null))
    (:`else`)))

(event `self.GrabComponent.OnGrabbed`
  (params (`Self Ref` :type "/Game/Objects/Structurs/GrabComponent Object Reference"))
  (goto _label))

(event `self.On VR Use`
  (`parent.On VR Use`)
  (bind _actor (`self.Line Trace` 300.0 "NewEnumerator1" :!label _label_2))
  (bind _asbp_stereo_system (cast `/Game/Objects/BP_Objects/BP_Stereo_System` _actor))
  (`/Engine/EditorBlueprintResources/StandardMacros.IsValid` (`/Game/Objects/BP_Objects/BP_Stereo_System.Vinyl` _asbp_stereo_system)
    (:`Is Not Valid`
      (`/Game/Objects/Tutorial/TutorialComponent.Check Use Type` (`self.TutorialComponent`) "NewEnumerator6")
      (`/Game/Objects/GameJolt/GameJoltComponent.Check Use Type` (`self.GameJoltComponent`) "NewEnumerator6")
      (bind _output_get (set `self.Stereo System` _asbp_stereo_system))
      (set `/Game/Objects/BP_Objects/BP_Stereo_System.Vinyl` self _output_get)
      (`self.Try Release`)
      (`self.K2_AttachToComponent` (`/Game/Objects/BP_Objects/BP_Stereo_System.Part` _output_get) "None" "SnapToTarget" "SnapToTarget" "SnapToTarget")
      (`self.Set Flat Mode` "NewEnumerator1")
      (`AudioComponent.SetSound` (`/Game/Objects/BP_Objects/BP_Stereo_System.Music` (`self.Stereo System`)) (`self.Sound`)))))

(event `On Press LMB_1`
  (bind _player (`/Game/Function/BP_MacroLibrary.Find Player`)
    (:`Is Valid`
      (bind _item (`/Game/Player/BP_Player.Get Item` _player))
      (if (== _item self)
        (goto _label_2)))))

(fn `UserConstructionScript`
  (`parent.UserConstructionScript`)
  (`PrimitiveComponent.SetMaterial` (`self.Root`) 0 (`self.Material`)))
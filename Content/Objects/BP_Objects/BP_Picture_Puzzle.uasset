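; BP_Picture_Puzzle is an electrical object that lights a bulb and spotlight and switches linked devices and an optional lock.
; Enable, Disable and BeginPlay set the bulb material and light visibility from the power state, then call Tumbler.
; With electricity or generator status, Tumbler On enables the Electricity array and unlocks the Lock.
; Off, or lack of power, disables and locks them, and both paths fire matching callbacks.
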(event `self.Enable`
  ;[1 1 1] Light
  (`parent.Enable`)
  (`PrimitiveComponent.SetMaterial` (`self.Root`) 0 "/Game/Objects/Materials/dl_bulb_m.dl_bulb_m" :!label _label)
  (`SceneComponent.SetVisibility` (`self.SpotLight`) true false)
  (`self.Tumbler` "NewEnumerator0"))

(event `self.ReceiveBeginPlay`
  ;[1 1 1] Light
  (`parent.ReceiveBeginPlay`)
  (if (or (`self.Has Electricity`) (`self.Generator`))
    (goto _label)
    (else
      (`PrimitiveComponent.SetMaterial` (`self.Root`) 0 "/Game/Objects/Materials/bulb_glass_m.bulb_glass_m" :!label _label_2)
      (`SceneComponent.SetVisibility` (`self.SpotLight`) false false)
      (`self.Tumbler` "NewEnumerator1"))))

(event `self.Disable`
  ;[1 1 1] Light
  (`parent.Disable`)
  (goto _label_2))

(event `Tumbler`
  (params (State :type "/Game/Objects/Enum/TumblerStateEnum Enum" :default "NewEnumerator0"))
  (bind _generator (`self.Generator`))
  ;[1 1 1] Tumbler
  (if (or (`self.Has Electricity`) _generator)
    (switch `/Game/Objects/Enum/TumblerStateEnum` State
      (:`NewEnumerator0`
        (for _array_element (`self.Electricity`)
          (`/Engine/EditorBlueprintResources/StandardMacros.IsValid` _array_element
            (:`Is Valid`
              (`self.Enable` _array_element))))
        (`self.On Enable`)
        (bind _lock (`self.Lock`)
          (:`then`
            (`/Game/Objects/Structurs/BP_Lock.Unlock` _lock)
            (`self.Set Flat Mode` _lock "NewEnumerator0"))
          (:`else`)))
      (:`NewEnumerator1`
        (for _array_element_2 (`self.Electricity`) :!label _label_3
          (`/Engine/EditorBlueprintResources/StandardMacros.IsValid` _array_element_2
            (:`Is Valid`
              (`self.Disable` _array_element_2))))
        (`self.On Disable`)
        (bind _lock_2 (`self.Lock`)
          (:`then`
            (`/Game/Objects/Structurs/BP_Lock.Lock` _lock_2)
            (`self.Set Flat Mode` _lock_2 "NewEnumerator0"))
          (:`else`))))
    (elif (not _generator)
      (goto _label_3))))

(fn `UserConstructionScript`
  (`parent.UserConstructionScript`))
(event `Remote Bath`
  (bind _water (`self.Water`))
  (bind _water_zone (`self.Water Zone`))
  (bind _tutorialcomponent (`self.TutorialComponent`))
  (bind _gamejoltcomponent (`self.GameJoltComponent`))
  ;[1 1 1] Interact
  (switch `/Game/Objects/Enum/TumblerStateEnum` (`self.State`) :!label _label
    (:`NewEnumerator0`
      (`ActorComponent.Deactivate` _water)
      (`ActorComponent.Deactivate` (`self.Shower Water`))
      (set `self.State` "NewEnumerator1")
      (set `PrimitiveComponent.bGenerateOverlapEvents` false _water_zone)
      (`/Game/Objects/Tutorial/TutorialComponent.Check Use Type` _tutorialcomponent "NewEnumerator4")
      (`/Game/Objects/GameJolt/GameJoltComponent.Check Use Type` _gamejoltcomponent "NewEnumerator4"))
    (:`NewEnumerator1`
      (`ActorComponent.Activate` _water false)
      (`ActorComponent.Activate` (`self.Shower Water`) false)
      (set `self.State` "NewEnumerator0")
      (set `PrimitiveComponent.bGenerateOverlapEvents` true _water_zone)
      (`/Game/Objects/Tutorial/TutorialComponent.Check Use Type` _tutorialcomponent "NewEnumerator3")
      (`/Game/Objects/GameJolt/GameJoltComponent.Check Use Type` _gamejoltcomponent "NewEnumerator3"))))

(event `/Game/Function/BP_Interface.Interact`
  (params (Component :type "PrimitiveComponent Object Reference") (Location :type "Vector Structure"))
  ;[1 1 1] Interact
  (goto _label))

(event `self.Water Zone.OnComponentBeginOverlap`
  (params (OverlappedComponent :type "PrimitiveComponent Object Reference") (OtherActor :type "Actor Object Reference") (OtherComp :type "PrimitiveComponent Object Reference") (OtherBodyIndex :type Integer) (bFromSweep :type Boolean) (SweepResult :type "HitResult Structure (by ref)"))
  (bind _returnvalue (`self.GetComponentByClass` OtherActor "/Game/Objects/Structurs/WaterComponent.WaterComponent_C"))
  ;[1 1 1] Water Zone
  (`|ExecutionSequence`
    (:`then_0`
      (`/Engine/EditorBlueprintResources/StandardMacros.IsValid` _returnvalue
        (:`Is Valid`
          (`|ExecutionSequence`
            (:`then_0`
              (bind (_direction _alpha) (`Timeline|Шкала времени` :`NewTime` (`/Game/Objects/Structurs/WaterComponent.Speed Fill` _returnvalue) :!via `SetNewTime` :!label _label_2)
                (:`Update`
                  (set `/Game/Objects/Structurs/WaterComponent.Fill` _alpha _returnvalue)
                  (`/Game/Objects/Structurs/WaterComponent.Update Water Box` _returnvalue))))
            (:`then_1`
              (goto _label_2))))))
    (:`then_1`
      (`/Game/Objects/Structurs/WaterComponent.Update Temperature` (`self.WaterComponent`) OtherActor true))))

(event `self.Water Zone.OnComponentEndOverlap`
  (params (OverlappedComponent :type "PrimitiveComponent Object Reference") (OtherActor :type "Actor Object Reference") (OtherComp :type "PrimitiveComponent Object Reference") (OtherBodyIndex :type Integer))
  ;[1 1 1] Water Zone
  (`|ExecutionSequence`
    (:`then_0`
      (`/Engine/EditorBlueprintResources/StandardMacros.IsValid` (`self.GetComponentByClass` OtherActor "/Game/Objects/Structurs/WaterComponent.WaterComponent_C")
        (:`Is Valid`
          (goto _label_2 :!via `Stop`))))
    (:`then_1`
      (`/Game/Objects/Structurs/WaterComponent.Update Temperature` (`self.WaterComponent`) OtherActor false))))

(event `self.ReceiveTick`
  (params (DeltaSeconds :type "Float (single-precision)")))

(fn `UserConstructionScript`)
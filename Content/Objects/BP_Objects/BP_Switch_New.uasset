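; Wall-style electrical switch that players flip by interaction or VR hand overlap to power linked Electricity objects on or off.
; A server-side interact plays a sound and a rotation timeline, then updates State and notifies Tutorial and GameJolt components.
; Tumbler propagates State to linked objects, enabling them only when the switch has electricity or is a generator.
; Saves store the rotation state, and loading replays the interaction when it differs.
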(event `/Game/Function/BP_Interface.Interact`
  (params (Component :type "PrimitiveComponent Object Reference") (Location :type "Vector Structure"))
  ;[1 1 1] Rotation
  (`self.Interact (Server)` Component))

(event `Interact (All)`
  (params (Component :type "PrimitiveComponent Object Reference"))
  ;[1 1 1] Rotation
)

(event `self.ReceiveBeginPlay`
  ;[1 1 1] Begin Play
  (`parent.ReceiveBeginPlay`)
  (`PrimitiveComponent.SetSimulatePhysics` (`self.Root`) false)
  (`self.Tumbler` (`self.State`)))

(event `Interact (Server)`
  (params (Component :type "PrimitiveComponent Object Reference"))
  (bind _state (`self.State`))
  (bind _tutorialcomponent (`self.TutorialComponent`))
  (bind _gamejoltcomponent (`self.GameJoltComponent`))
  ;[1 1 1] Rotation
  (if (== Component (`self.Switch`))
    (switch `/Game/Objects/Enum/RotateStateEnum` (`self.Rotate State`) :!label _label
      (:`NewEnumerator0`
        (set `self.Rotate State` "NewEnumerator3")
        (`|ExecutionSequence`
          (:`then_0`
            (bind (_direction _alpha) (`Timeline|Rotate Timeline` :!via `PlayFromStart` :!label _label_2)
              (:`Update`
                (`SceneComponent.K2_SetRelativeRotation` (`self.Switch`) (`KismetMathLibrary.RLerp` (select `/Game/Objects/Enum/TumblerStateEnum` _state :`NewEnumerator0` (struct :`Roll` -5.0) :`NewEnumerator1` (struct :`Roll` 5.0) :!type "Rotator Structure") (select `/Game/Objects/Enum/TumblerStateEnum` _state :`NewEnumerator0` (struct :`Roll` 5.0) :`NewEnumerator1` (struct :`Roll` -5.0) :!type "Rotator Structure") _alpha) false false))
              (:`Finished`
                (switch `/Game/Objects/Enum/RotateStateEnum` (`self.Rotate State`)
                  (:`NewEnumerator2`
                    (set `self.Rotate State` "NewEnumerator0")
                    (set `self.State` "NewEnumerator1")
                    (`/Game/Objects/Tutorial/TutorialComponent.Check Use Type` _tutorialcomponent "NewEnumerator4")
                    (`/Game/Objects/GameJolt/GameJoltComponent.Check Use Type` _gamejoltcomponent "NewEnumerator4"))
                  (:`NewEnumerator3`
                    (set `self.Rotate State` "NewEnumerator1")
                    (set `self.State` "NewEnumerator0")
                    (`/Game/Objects/Tutorial/TutorialComponent.Check Use Type` _tutorialcomponent "NewEnumerator3")
                    (`/Game/Objects/GameJolt/GameJoltComponent.Check Use Type` _gamejoltcomponent "NewEnumerator3")))
                (`self.Tumbler` (`self.State`)))))
          (:`then_1`
            (`GameplayStatics.PlaySoundAtLocation` "/Game/Sounds/Objects/TurnOnOff/switch_on_Cue.switch_on_Cue" (`self.K2_GetActorLocation`) (struct) 1.0 1.0 0.0 null null null null))))
      (:`NewEnumerator1`
        (set `self.Rotate State` "NewEnumerator2")
        (`|ExecutionSequence`
          (:`then_0`
            (goto _label_2 :!via `PlayFromStart`))
          (:`then_1`
            (`GameplayStatics.PlaySoundAtLocation` "/Game/Sounds/Objects/TurnOnOff/switch_off_Cue.switch_off_Cue" (`self.K2_GetActorLocation`) (struct) 1.0 1.0 0.0 null null null null)))))))

(event `self.Enable`
  ;[1 1 1] Tumbler
  (`parent.Enable`)
  (switch `/Game/Objects/Enum/TumblerStateEnum` (`self.State`) :!label _label_3
    (:`NewEnumerator0`
      (for _array_element (`self.Electricity`)
        (`/Engine/EditorBlueprintResources/StandardMacros.IsValid` _array_element
          (:`Is Valid`
            (`self.Enable` _array_element)))))))

(event `Tumbler`
  (params (State :type "/Game/Objects/Enum/TumblerStateEnum Enum" :default "NewEnumerator0"))
  (bind _generator (`self.Generator`))
  ;[1 1 1] Tumbler
  (if (or (`self.Has Electricity`) _generator)
    (switch `/Game/Objects/Enum/TumblerStateEnum` State
      (:`NewEnumerator0`
        (goto _label_3))
      (:`NewEnumerator1`
        (for _array_element (`self.Electricity`) :!label _label_4
          (`/Engine/EditorBlueprintResources/StandardMacros.IsValid` _array_element
            (:`Is Valid`
              (`self.Disable` _array_element))))))
    (elif (not _generator)
      (goto _label_4))))

(event `self.VR Interact.OnComponentBeginOverlap`
  (params (OverlappedComponent :type "PrimitiveComponent Object Reference") (OtherActor :type "Actor Object Reference") (OtherComp :type "PrimitiveComponent Object Reference") (OtherBodyIndex :type Integer) (bFromSweep :type Boolean) (SweepResult :type "HitResult Structure (by ref)"))
  ;[1 1 1] Rotation
  (if (`self.Overlap VR Hands` OtherActor OtherComp)
    (goto _label)))

(event `self.Disable`
  ;[1 1 1] Tumbler
  (`parent.Disable`)
  (goto _label_4))

(fn `Load Data`
  (params (JSON :type String))
  (returns (Object :type "VaRestJsonObject Object Reference"))
  (bind _object (`parent.Load Data` JSON))
  (`|ExecutionSequence`
    (:`then_0`
      (bind (_has_field_ _return_value) (`/Game/Function/BP_JSON_FunctionLibrary.Get Value As Int` _object "State"))
      (if (and _has_field_ (!= _return_value (`KismetMathLibrary.Conv_ByteToInt` (`self.Rotate State`))))
        (`self.Interact` (`self.Switch`))))
    (:`then_1`
      (return _object))))

(fn `Save Data`
  (returns (JSON :type "VaRestJsonObject Object Reference"))
  (bind _json (`parent.Save Data`))
  (`VaRestJsonObject.SetIntegerField` _json "State" (`KismetMathLibrary.Conv_ByteToInt` (`self.Rotate State`)))
  (return _json))

(fn `UserConstructionScript`
  (bind _switch (`self.Switch`))
  (`parent.UserConstructionScript`)
  (switch `/Game/Objects/Enum/TumblerStateEnum` (`self.State`)
    (:`NewEnumerator0`
      (`SceneComponent.K2_SetRelativeRotation` _switch (struct :`Roll` -5.0) false false)
      (set `self.Rotate State` "NewEnumerator1"))
    (:`NewEnumerator1`
      (`SceneComponent.K2_SetRelativeRotation` _switch (struct :`Roll` 5.0) false false)
      (set `self.Rotate State` "NewEnumerator0"))))
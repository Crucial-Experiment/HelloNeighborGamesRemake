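; BP_DL_Bulb is a bulb object that shows its lit or unlit state by swapping the material in slot 1 of its Root mesh.
; It extends a parent's Light event, calling the parent and then applying the on or off bulb material.
; On BeginPlay it shows the lit material if Lamp is valid, otherwise it switches the light off.
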(event `self.ReceiveBeginPlay`
  (bind _root (`self.Root`))
  ;[1 1 1] Begin Play
  (`parent.ReceiveBeginPlay`)
  (`|ExecutionSequence`
    (:`then_0`
      (`/Engine/EditorBlueprintResources/StandardMacros.IsValid` (`self.Lamp`)
        (:`Is Valid`
          (`PrimitiveComponent.SetMaterial` _root 1 "/Game/Objects/Materials/dl_bulb_m.dl_bulb_m"))
        (:`Is Not Valid`
          (`self.Light` false)
          (`PrimitiveComponent.SetMaterial` _root 1 "/Game/Objects/Materials/dl_bulb_m_off.dl_bulb_m_off"))))))

(event `self.Light`
  (params (State :type Boolean))
  (bind _root (`self.Root`))
  ;[1 1 1] Light
  (`parent.Light` State)
  (if State
    (`PrimitiveComponent.SetMaterial` _root 1 "/Game/Objects/Materials/dl_bulb_m.dl_bulb_m")
    (else
      (`PrimitiveComponent.SetMaterial` _root 1 "/Game/Objects/Materials/dl_bulb_m_off.dl_bulb_m_off"))))

(fn `UserConstructionScript`
  (`parent.UserConstructionScript`))
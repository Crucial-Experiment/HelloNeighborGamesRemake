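; Big door variant of a parent door Blueprint that can hand its interaction over to a cutscene.
; Interact sets the CutsceneManager state when the door has no locks, AutoLock and StartLook are off and a manager is valid; otherwise the parent interaction runs.
; The construction script extends the parent's, picking a wood material for the Border and Rotate components from the Material setting.
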(event `self.Interact`
  (params (Component :type "PrimitiveComponent Object Reference") (Location :type "Vector Structure"))
  (if (and (== (`KismetArrayLibrary.Array_Length` (`self.Locks`)) 0) (not (`self.Auto Lock`)) (`KismetSystemLibrary.IsValid` (`self.Cutscene Manager`)) (not (`self.Start Look`)))
    (`/Game/Objects/Cutscene/BP_Cutscene_Manager.Set State` (`self.Cutscene Manager`) "NewEnumerator0")
    (else
      (`parent.Interact` Component Location))))

(fn `UserConstructionScript`
  (bind _border (`self.Border`))
  (`parent.UserConstructionScript`)
  (switch `/Game/Objects/Enum/DoorMaterialEnim` (`self.Material`)
    (:`NewEnumerator0`
      (`PrimitiveComponent.SetMaterial` _border 0 "/Game/Objects/Materials/white_wood_mat.white_wood_mat")
      (`PrimitiveComponent.SetMaterial` (`self.Rotate`) 0 "/Game/Objects/Materials/white_wood_mat.white_wood_mat"))
    (:`NewEnumerator1`
      (`PrimitiveComponent.SetMaterial` _border 0 "/Game/Objects/Materials/wood_4_mat.wood_4_mat")
      (`PrimitiveComponent.SetMaterial` (`self.Rotate`) 0 "/Game/Objects/Materials/wood_4_mat.wood_4_mat"))
    (:`NewEnumerator2`
      (`PrimitiveComponent.SetMaterial` _border 0 "/Game/Objects/Materials/red_dark_wood.red_dark_wood")
      (`PrimitiveComponent.SetMaterial` (`self.Rotate`) 0 "/Game/Objects/Materials/red_dark_wood.red_dark_wood"))))
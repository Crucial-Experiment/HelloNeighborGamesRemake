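; BP_Bulb is a holdable light bulb that players screw into and remove from lamps.
; LMB or VR use line-traces for an allowed lamp class, links both actors, then releases the bulb.
; Server-to-All events snap it into the socket, lighting spotlight and glass if powered, and notify tutorial and GameJolt components.
; Pickup or VR grab unlinks and darkens it, reactivating sparks on powered lamps.
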(event `LMB (All)`
  (params (Lamp :type "/Game/Objects/BP_Objects/BP_Lamp Object Reference"))
  (bind _scene (`/Game/Objects/BP_Objects/BP_Lamp.Scene` Lamp))
  ;[1 1 1] Begin Play and Use
  (`self.Set Flat Mode` "NewEnumerator1")
  (`self.K2_SetActorLocation` (`SceneComponent.K2_GetComponentLocation` _scene))
  (`self.K2_SetActorRotation` (`SceneComponent.K2_GetComponentRotation` _scene))
  (`self.Light` (`/Game/Objects/Structurs/BP_Electricity.Has Electricity` Lamp))
  (`ActorComponent.Deactivate` (`/Game/Objects/BP_Objects/BP_Lamp.Spark` (`self.Lamp`)))
  (`ActorComponent.Deactivate` (`/Game/Objects/BP_Objects/BP_Lamp.P_Sparks` (`self.Lamp`)))
  (`GameplayStatics.SpawnSoundAtLocation` (select `int` (`KismetMathLibrary.RandomIntegerInRange` 0 3) :`0` "/Game/Sounds/Objects/Noise/bulb_screw_1_Cue.bulb_screw_1_Cue" :`1` "/Game/Sounds/Objects/Noise/bulb_screw_2_Cue.bulb_screw_2_Cue" :`2` "/Game/Sounds/Objects/Noise/bulb_screw_3_Cue.bulb_screw_3_Cue" :`3` "/Game/Sounds/Objects/Noise/bulb_screw_4_Cue.bulb_screw_4_Cue" :!type "SoundBase Object Reference") (`self.K2_GetActorLocation`) (struct) 1.0 1.0 0.0 null null)
  (`self.SetActorEnableCollision` true)
  (`/Game/Objects/Tutorial/TutorialComponent.Check Use Type` (`self.TutorialComponent`) "NewEnumerator6")
  (`/Game/Objects/GameJolt/GameJoltComponent.Check Use Type` (`self.GameJoltComponent`) "NewEnumerator6"))

(event `On Press LMB_1`
  ;[1 1 1] Begin Play and Use
  (bind _player (`/Game/Function/BP_MacroLibrary.Find Player`)
    (:`Is Valid`
      (bind _item (`/Game/Player/BP_Player.Get Item` _player))
      (if (== _item self)
        (bind _actor (`self.Line Trace` 300.0 "NewEnumerator1" :!label _label))
        (for _array_element (`self.Lamp Class`)
          (if (== _array_element (`GameplayStatics.GetObjectClass` _actor))
            (bind _asbp_lamp (cast `/Game/Objects/BP_Objects/BP_Lamp` _actor))
            (set `/Game/Objects/BP_Objects/BP_Lamp.Bulb` self _asbp_lamp)
            (set `self.Lamp` _asbp_lamp)
            (`self.Try Release`)
            (`self.LMB (Server)` _asbp_lamp)))))))

(event `self.On VR Use`
  ;[1 1 1] Begin Play and Use
  (goto _label))

(event `self.ReceiveBeginPlay`
  ;[1 1 1] Begin Play and Use
  (`parent.ReceiveBeginPlay`)
  (`/Engine/EditorBlueprintResources/StandardMacros.IsValid` (`self.Lamp`)
    (:`Is Not Valid`
      (`self.Light` false))))

(event `LMB (Server)`
  (params (Lamp :type "/Game/Objects/BP_Objects/BP_Lamp Object Reference"))
  ;[1 1 1] Begin Play and Use
  (`self.LMB (All)` Lamp))

(event `Light`
  (params (State :type Boolean))
  (bind _root (`self.Root`))
  ;[1 1 1] Light
  (`SceneComponent.SetVisibility` (`self.SpotLight`) State false)
  (if State
    (`PrimitiveComponent.SetMaterial` _root 0 "/Game/Objects/Materials/dl_bulb_m.dl_bulb_m")
    (else
      (`PrimitiveComponent.SetMaterial` _root 0 "/Game/Objects/Materials/bulb_glass_m.bulb_glass_m"))))

(event `Pick Up (Server)`
  ;[1 1 1] Pick Up
  (`self.Pick Up (All)`))

(event `Pick Up (All)`
  (bind _lamp (`self.Lamp`))
  ;[1 1 1] Pick Up
  (`/Engine/EditorBlueprintResources/StandardMacros.IsValid` _lamp
    (:`Is Valid`
      (set `/Game/Objects/BP_Objects/BP_Lamp.Bulb` null _lamp)
      (if (`/Game/Objects/Structurs/BP_Electricity.Has Electricity` _lamp)
        (`ActorComponent.Activate` (`/Game/Objects/BP_Objects/BP_Lamp.Spark` _lamp) false)
        (`ActorComponent.Activate` (`/Game/Objects/BP_Objects/BP_Lamp.P_Sparks` _lamp) false))
      (set `self.Lamp` null)
      (`self.Light` false)
      (`GameplayStatics.SpawnSoundAtLocation` (select `int` (`KismetMathLibrary.RandomIntegerInRange` 0 3) :`0` "/Game/Sounds/Objects/Noise/bulb_screw_1_Cue.bulb_screw_1_Cue" :`1` "/Game/Sounds/Objects/Noise/bulb_screw_2_Cue.bulb_screw_2_Cue" :`2` "/Game/Sounds/Objects/Noise/bulb_screw_3_Cue.bulb_screw_3_Cue" :`3` "/Game/Sounds/Objects/Noise/bulb_screw_4_Cue.bulb_screw_4_Cue" :!type "SoundBase Object Reference") (`self.K2_GetActorLocation`) (struct) 1.0 1.0 0.0 null null))))

(event `/Game/Function/BP_Interface.PickUp`
  ;[1 1 1] Pick Up
  (`parent.PickUp`)
  (`self.Pick Up (Server)` :!label _label_2))

(event `self.GrabComponent.OnGrabbed`
  (params (`Self Ref` :type "/Game/Objects/Structurs/GrabComponent Object Reference"))
  ;[1 1 1] Pick Up
  (goto _label_2))

(fn `UserConstructionScript`
  (`parent.UserConstructionScript`)
  (`LightComponent.SetLightColor` (`self.SpotLight`) (`KismetMathLibrary.Conv_ColorToLinearColor` (`self.Color`)) true))
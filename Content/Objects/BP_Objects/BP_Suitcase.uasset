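; BP_Suitcase is an interactive suitcase whose lid opens and closes with sound when its Part component receives Interact.
; A PartRotate state drives one timeline that lerps the lid's rotation and settles on Open or Close, ignoring interaction while moving.
; A trigger box reports other BP_Object actors entering or leaving to the tutorial and GameJolt components.
; Construction tags the root "interactive" when CanPickUp is set.
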(event `/Game/Function/BP_Interface.Interact`
  (params (Component :type "PrimitiveComponent Object Reference") (Location :type "Vector Structure"))
  (bind _part_rotate (`self.Part Rotate`))
  ;[1 1 1] Interact
  (if (== Component (`self.Part`))
    (switch `/Game/Objects/Enum/RotateStateEnum` (`self.Part Rotate`)
      (:`NewEnumerator0`
        (set `self.Part Rotate` "NewEnumerator3")
        (`|ExecutionSequence`
          (:`then_0`
            (bind (_direction _alpha) (`Timeline|Rotate Timeline` :!via `PlayFromStart` :!label _label)
              (:`Update`
                (`SceneComponent.K2_SetRelativeRotation` (`self.Part`) (`KismetMathLibrary.RLerp` (select `/Game/Objects/Enum/RotateStateEnum` _part_rotate :`NewEnumerator1` (struct :`Roll` 120.0) :`NewEnumerator3` (struct :`Roll` 120.0) :!type "Rotator Structure") (select `/Game/Objects/Enum/RotateStateEnum` _part_rotate :`NewEnumerator0` (struct :`Roll` 120.0) :`NewEnumerator2` (struct :`Roll` 120.0) :!type "Rotator Structure") _alpha) false false))
              (:`Finished`
                (switch `/Game/Objects/Enum/RotateStateEnum` (`self.Part Rotate`)
                  (:`NewEnumerator2`
                    (set `self.Part Rotate` "NewEnumerator0"))
                  (:`NewEnumerator3`
                    (set `self.Part Rotate` "NewEnumerator1"))))))
          (:`then_1`
            (`GameplayStatics.PlaySoundAtLocation` "/Game/Sounds/Objects/OpenClosed/suitcase_close_Cue.suitcase_close_Cue" (`self.K2_GetActorLocation`) (struct) 1.0 1.0 0.0 null null null null))))
      (:`NewEnumerator1`
        (set `self.Part Rotate` "NewEnumerator2")
        (`|ExecutionSequence`
          (:`then_0`
            (goto _label :!via `PlayFromStart`))
          (:`then_1`
            (`GameplayStatics.PlaySoundAtLocation` "/Game/Sounds/cutscenes/suitcase_open_Cue.suitcase_open_Cue" (`self.K2_GetActorLocation`) (struct) 1.0 1.0 0.0 null null null null)))))))

(event `self.Box.OnComponentBeginOverlap`
  (params (OverlappedComponent :type "PrimitiveComponent Object Reference") (OtherActor :type "Actor Object Reference") (OtherComp :type "PrimitiveComponent Object Reference") (OtherBodyIndex :type Integer) (bFromSweep :type Boolean) (SweepResult :type "HitResult Structure (by ref)"))
  ;[1 1 1] Trigger
  (if (!= OtherActor self)
    (cast `/Game/Objects/Structurs/BP_Object` OtherActor)
    (`/Game/Objects/Tutorial/TutorialComponent.Check Use Type` (`self.TutorialComponent`) "NewEnumerator3")
    (`/Game/Objects/GameJolt/GameJoltComponent.Check Use Type` (`self.GameJoltComponent`) "NewEnumerator3")))

(event `self.Box.OnComponentEndOverlap`
  (params (OverlappedComponent :type "PrimitiveComponent Object Reference") (OtherActor :type "Actor Object Reference") (OtherComp :type "PrimitiveComponent Object Reference") (OtherBodyIndex :type Integer))
  ;[1 1 1] Trigger
  (if (!= OtherActor self)
    (cast `/Game/Objects/Structurs/BP_Object` OtherActor)
    (`/Game/Objects/Tutorial/TutorialComponent.Check Use Type` (`self.TutorialComponent`) "NewEnumerator4")
    (`/Game/Objects/GameJolt/GameJoltComponent.Check Use Type` (`self.GameJoltComponent`) "NewEnumerator4")))

(fn `UserConstructionScript`
  (`parent.UserConstructionScript`)
  (set `ActorComponent.ComponentTags` (`|MakeArray` (select `bool` (`self.CanPickUp`) :`true` "interactive" :!type "Name")) (`self.Root`)))
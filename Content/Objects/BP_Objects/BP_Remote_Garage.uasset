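; BP_Remote_Garage is a usable remote item that toggles a garage door the player aims at.
; VR use, or left mouse while the local item is held, line traces for a BP_Garage_Door.
; A hit is relayed through a server event to all clients, which enable or disable the door by its state and notify the tutorial and GameJolt components of the use.
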(event `self.ReceiveBeginPlay`
  (`parent.ReceiveBeginPlay`))

(event `self.On VR Use`
  (`parent.On VR Use`)
  (bind _actor (`self.Line Trace` 1500.0 :!label _label))
  (bind _asbp_garage_door (cast `/Game/Objects/BP_Objects/BP_Garage_Door` _actor))
  (`self.Interact (Server)` _asbp_garage_door))

(event `On Press LMB_1`
  (bind _player (`/Game/Function/BP_MacroLibrary.Find Player`)
    (:`Is Valid`
      (bind _item (`/Game/Player/BP_Player.Get Item` _player))
      (if (== _item self)
        (goto _label)))))

(event `Interact (Server)`
  (params (`Garage Door` :type "/Game/Objects/BP_Objects/BP_Garage_Door Object Reference"))
  (`self.Interact (All)` `Garage Door`))

(event `Interact (All)`
  (params (`Garage Door` :type "/Game/Objects/BP_Objects/BP_Garage_Door Object Reference"))
  (`/Game/Objects/Tutorial/TutorialComponent.Check Use Type` (`self.TutorialComponent`) "NewEnumerator6")
  (`/Game/Objects/GameJolt/GameJoltComponent.Check Use Type` (`self.GameJoltComponent`) "NewEnumerator6")
  (switch `/Game/Objects/Enum/TumblerStateEnum` (`/Game/Objects/BP_Objects/BP_Garage_Door.State` `Garage Door`)
    (:`NewEnumerator0`
      (`/Game/Objects/Structurs/BP_Electricity.Disable` `Garage Door`))
    (:`NewEnumerator1`
      (`/Game/Objects/Structurs/BP_Electricity.Enable` `Garage Door`))))

(fn `UserConstructionScript`
  (`parent.UserConstructionScript`))
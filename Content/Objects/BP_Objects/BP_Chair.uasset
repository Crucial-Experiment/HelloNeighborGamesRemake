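; BP_Chair is a grabbable chair for VR and flat-screen play that mounts onto a BP_Rotate actor.
; VR use or left-click while held line-traces for a free mount, checks its rotate state, then links and snaps the chair, notifying tutorial and GameJolt components.
; Grabbing or picking it up unlinks it through a server event; BeginPlay re-attaches linked chairs.
; Placement runs inline, leaving the duplicate server add event's call unwired.
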(event `self.On VR Use`
  (`parent.On VR Use`)
  (bind _actor (`self.Line Trace` 250.0 :!label _label))
  (bind _asbp_rotate (cast `/Game/Objects/Structurs/BP_Rotate` _actor))
  (`/Game/Objects/Structurs/BP_Rotate.Chair` _asbp_rotate
    (:`then`)
    (:`else`
      (`/Game/Objects/Tutorial/TutorialComponent.Check Use Type` (`self.TutorialComponent`) "NewEnumerator6")
      (`/Game/Objects/GameJolt/GameJoltComponent.Check Use Type` (`self.GameJoltComponent`) "NewEnumerator6")
      (if (and (`|EnumEquality` (`/Game/Objects/Structurs/BP_Rotate.Rotate State` _asbp_rotate) "NewEnumerator1") (`/Game/Objects/Structurs/BP_Rotate.Can Place Chair` _asbp_rotate))
        (set `/Game/Objects/Structurs/BP_Rotate.Chair` self _asbp_rotate)
        (set `self.Rotate` _asbp_rotate)
        (`self.Try Release`)
        (`self.Set Flat Mode` "NewEnumerator1")
        (bind (_returnvalue_location _returnvalue_rotation) (`KismetMathLibrary.BreakTransform` (`SceneComponent.K2_GetComponentToWorld` (`/Game/Objects/Structurs/BP_Rotate.Scene` _asbp_rotate))))
        (`self.K2_SetActorLocationAndRotation` _returnvalue_location _returnvalue_rotation)
        (`GameplayStatics.PlaySound2D` "/Game/Sounds/Objects/OpenClosed/prop_door_close_Cue.prop_door_close_Cue" 1.0 1.0 0.0 null null)))))

(event `On Press LMB_1`
  (bind _player (`/Game/Function/BP_MacroLibrary.Find Player`)
    (:`Is Valid`
      (bind _item (`/Game/Player/BP_Player.Get Item` _player))
      (if (== _item self)
        (goto _label)))))

(event `self.ReceiveBeginPlay`
  (bind _rotate (`self.Rotate`))
  (`parent.ReceiveBeginPlay`)
  (`/Engine/EditorBlueprintResources/StandardMacros.IsValid` _rotate
    (:`Is Valid`
      (`self.Set Flat Mode` "NewEnumerator1")
      (`self.K2_AttachToComponent` (`/Game/Objects/Structurs/BP_Rotate.Scene` _rotate) "None" "SnapToTarget" "SnapToTarget" "SnapToTarget"))))

(event `Add Chair (Server)`
  (params (Actor :type "/Game/Objects/Structurs/BP_Rotate Object Reference"))
  (bind (_returnvalue_location _returnvalue_rotation) (`KismetMathLibrary.BreakTransform` (`SceneComponent.K2_GetComponentToWorld` (`/Game/Objects/Structurs/BP_Rotate.Scene` Actor))))
  (`/Game/Objects/Structurs/BP_Rotate.Chair` Actor
    (:`then`)
    (:`else`
      (`/Game/Objects/Tutorial/TutorialComponent.Check Use Type` (`self.TutorialComponent`) "NewEnumerator6")
      (`/Game/Objects/GameJolt/GameJoltComponent.Check Use Type` (`self.GameJoltComponent`) "NewEnumerator6")
      (if (and (`|EnumEquality` (`/Game/Objects/Structurs/BP_Rotate.Rotate State` Actor) "NewEnumerator1") (`/Game/Objects/Structurs/BP_Rotate.Can Place Chair` Actor))
        (set `/Game/Objects/Structurs/BP_Rotate.Chair` self Actor)
        (set `self.Rotate` Actor)
        (`self.Set Flat Mode` "NewEnumerator1")
        (`self.K2_SetActorLocationAndRotation` _returnvalue_location _returnvalue_rotation)))))

(event `self.GrabComponent.OnDropped`
  (params (`Self Ref` :type "/Game/Objects/Structurs/GrabComponent Object Reference"))
  (`self.Rotate`
    (:`then`)
    (:`else`
      (`self.Set Flat Mode` "NewEnumerator0"))))

(event `self.GrabComponent.OnGrabbed`
  (params (`Self Ref` :type "/Game/Objects/Structurs/GrabComponent Object Reference"))
  (`self.Rotate` :!label _label_2
    (:`then`
      (`GameplayStatics.PlaySound2D` "/Game/Sounds/Objects/OpenClosed/prop_door_open_Cue.prop_door_open_Cue" 1.0 1.0 0.0 null null)
      (`self.Remove Chair (Server)`))
    (:`else`)))

(event `/Game/Function/BP_Interface.PickUp`
  (`parent.PickUp`)
  (goto _label_2))

(event `Remove Chair (Server)`
  (bind _rotate (`self.Rotate`)
    (:`then`
      (set `/Game/Objects/Structurs/BP_Rotate.Chair` null _rotate)
      (set `self.Rotate` null))
    (:`else`)))

(fn `UserConstructionScript`
  (`parent.UserConstructionScript`))
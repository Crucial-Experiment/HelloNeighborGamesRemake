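; BP_Electromagnet is a usable item, for desktop and VR, that toggles on to pull magnetable physics objects toward it and toggles off to release them.
; Use, click and slot-change inputs go through server and multicast events, with slot changes or clicks while not held forcing a stop.
; While on, a delay loop retraces forward until it finds a target, then a self-restarting timeline lerps it to the magnet, with sound and distortion effects.
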(event `Interact (Server)`
  (params (`Stop?` :type Boolean))
  (`self.Interact (All)` `Stop?`))

(event `Move Target`
  (`PrimitiveComponent.SetSimulatePhysics` (`self.Magnet Target`) false)
  (`TimelineComponent.SetPlayRate` (`self.Move Timeline`) 0.3)
  (bind (_direction _alpha) (`Timeline|Move Timeline` :!via `PlayFromStart`)
    (:`Update`
      (set `self.Magnet Position` (`SceneComponent.K2_GetComponentLocation` (`self.Scene`)))
      (`SceneComponent.K2_SetWorldLocation` (`self.Magnet Target`) (`KismetMathLibrary.VLerp` (`SceneComponent.K2_GetComponentLocation` (`self.Magnet Target`)) (`self.Magnet Position`) _alpha) false false))
    (:`Finished`
      (`self.Move Target`))))

(event `On Slot Change_1`
  (`self.Interact (Server)` true))

(event `self.On VR Use`
  (`parent.On VR Use`)
  (`self.Interact (Server)` false :!label _label))

(event `Interact (All)`
  (params (`Stop?` :type Boolean))
  (if (not `Stop?`)
    (`/Game/Objects/Tutorial/TutorialComponent.Check Use Type` (`self.TutorialComponent`) "NewEnumerator6")
    (`/Game/Objects/GameJolt/GameJoltComponent.Check Use Type` (`self.GameJoltComponent`) "NewEnumerator6")
    (switch `/Game/Objects/Enum/TumblerStateEnum` (`self.Switch`)
      (:`NewEnumerator0`
        (set `self.Switch` "NewEnumerator1" :!label _label_2)
        (`TimelineComponent.Stop` (`self.Move Timeline`))
        (`/Engine/EditorBlueprintResources/StandardMacros.IsValid` (`self.Magnet Target`)
          (:`Is Valid`
            (`PrimitiveComponent.SetSimulatePhysics` (`self.Magnet Target`) true)
            (`AudioComponent.Stop` (`self.Loop`))
            (`GameplayStatics.PlaySoundAtLocation` "/Game/Sounds/Objects/Noise/electromagnetic_end_Cue.electromagnetic_end_Cue" (`self.K2_GetActorLocation`) (struct) 1.0 1.0 0.0 null null null null)
            (`ActorComponent.Deactivate` (`self.P_Magnet_Distortion`))
            (set `self.Magnet Target` null))))
      (:`NewEnumerator1`
        (`ActorComponent.Activate` (`self.P_Magnet_Distortion`) false)
        (set `self.Switch` "NewEnumerator0")
        (bind _start_vr (`/Game/Player/BP_Player.Start VR` (stale `On Press LMB_1` _player)))
        (bind _returnvalue (select `bool` _start_vr :`false` (select `/Game/Player/Functions/PlayerModel_Enum` (`/Game/Player/BP_Player.Model` (stale `On Press LMB_1` _player)) :`NewEnumerator0` (`/Game/Player/BP_Player.Camera` (stale `On Press LMB_1` _player)) :!type "SceneComponent Object Reference") :`true` (`self.Scene`)))
        (bind _returnvalue_2 (`SceneComponent.K2_GetComponentLocation` _returnvalue))
        (bind (_outhit _returnvalue_3) (`KismetSystemLibrary.LineTraceSingle` :`Start` _returnvalue_2 :`End` (+ _returnvalue_2 (* (`SceneComponent.GetForwardVector` _returnvalue) 1500.0)) :`TraceChannel` "TraceTypeQuery1" :`DrawDebugType` (select `bool` _start_vr :`true` "ForDuration" :!type "EDrawDebugTrace Enum") :!label _label_3))
        (if (`|EnumEquality` (`self.Switch`) "NewEnumerator0")
          (if _returnvalue_3
            (bind (_bblockinghit _binitialoverlap _time _distance _location _impactpoint _normal _impactnormal _physmat _hitactor _hitcomponent) (`GameplayStatics.BreakHitResult` _outhit))
            (bind _asbp_object (cast `/Game/Objects/Structurs/BP_Object` _hitactor)
              (:`then`
                (if (and (`SceneComponent.IsAnySimulatingPhysics` _hitcomponent) (`/Game/Objects/Structurs/FlatComponent.Can Be Magneted?` (`/Game/Objects/Structurs/BP_Object.FlatComponent` _asbp_object)))
                  (set `self.Magnet Target` _hitcomponent)
                  (`self.Move Target`)
                  (`GameplayStatics.PlaySoundAtLocation` "/Game/Sounds/Objects/Noise/electromagnetic_start_Cue.electromagnetic_start_Cue" (`self.K2_GetActorLocation`) (struct) 1.0 1.0 0.0 null null null null)
                  (`AudioComponent.Play` (`self.Loop`) 0.0)
                  (else
                    (`KismetSystemLibrary.Delay` 0.0001 :!label _label_4)
                    (goto _label_3))))
              (:`CastFailed`
                (goto _label_4)))
            (else
              (goto _label_4))))))
    (else
      (goto _label_2))))

(event `On Press LMB_1`
  (bind _player (`/Game/Function/BP_MacroLibrary.Find Player`)
    (:`Is Valid`
      (bind _item (`/Game/Player/BP_Player.Get Item` _player))
      (if (== _item self)
        (goto _label)
        (else
          (`self.Interact (Server)` true))))))

(fn `UserConstructionScript`)
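; Big double door, a child Blueprint that adds a second swinging leaf (Rotate2) to the parent door's behavior.
; RemoteOpen and Interact toggle that leaf through a state-driven timeline with open/close sounds; locks, a chair, AutoLock or StartLook block interaction with a lock sound.
; A bound SpawnDoor event swaps the leaf for an impulse-launched BP_Door_Part.
; The construction script applies the wood material and starting rotation.
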(event `self.Remote Open`
  (bind _open_sound (`self.Open Sound`))
  (bind _close_sound (`self.Close Sound`))
  (`parent.Remote Open`)
  (switch `/Game/Objects/Enum/RotateStateEnum` (`self.Rotate 2 State`) :!label _label
    (:`NewEnumerator0`
      (set `self.Rotate 2 State` "NewEnumerator3")
      (bind (_direction _alpha) (`Timeline|Rotate 2 Timeline` :!via `Reverse` :!label _label_2)
        (:`Update`
          (`SceneComponent.K2_SetRelativeRotation` (`self.Rotate 2`) (`KismetMathLibrary.RLerp` (`self.Rotate 2 A`) (`self.Rotate 2 B`) _alpha) false false))
        (:`Finished`
          (switch `/Game/Objects/Enum/RotateStateEnum` (`self.Rotate 2 State`)
            (:`NewEnumerator2`
              (set `self.Rotate 2 State` "NewEnumerator0"))
            (:`NewEnumerator3`
              (set `self.Rotate 2 State` "NewEnumerator1")
              ;[1 1 1] Close Sound
              (`/Engine/EditorBlueprintResources/StandardMacros.IsValid` _close_sound
                (:`Is Valid`
                  (`GameplayStatics.PlaySoundAtLocation` _close_sound (`self.K2_GetActorLocation`) (struct) 1.0 1.0 0.0 null null null null))))))))
    (:`NewEnumerator1`
      (set `self.Rotate 2 State` "NewEnumerator2")
      (`|ExecutionSequence`
        (:`then_0`
          (goto _label_2))
        (:`then_1`
          ;[1 1 1] Open Sound
          (`/Engine/EditorBlueprintResources/StandardMacros.IsValid` _open_sound
            (:`Is Valid`
              (`GameplayStatics.PlaySoundAtLocation` _open_sound (`self.K2_GetActorLocation`) (struct) 1.0 1.0 0.0 null null null null))))))))

(event `self.Interact`
  (params (Component :type "PrimitiveComponent Object Reference") (Location :type "Vector Structure"))
  (`parent.Interact` Component Location)
  (if (== Component (`self.Rotate 2`))
    (if (and (== (`KismetArrayLibrary.Array_Length` (`self.Locks`)) 0) (not (`KismetSystemLibrary.IsValid` (`self.Chair`))) (not (`self.Auto Lock`)) (not (`self.Start Look`)))
      (goto _label)
      (else
        (`GameplayStatics.PlaySoundAtLocation` (`self.Lock Sound`) (`self.K2_GetActorLocation`) (struct) 1.0 1.0 0.0 null null null null)))))

(event `self.ReceiveBeginPlay`
  (`parent.ReceiveBeginPlay`)
  (add `self.Spawn Door Part` (delegate `Spawn Door`))
  (`SceneComponent.K2_AttachToComponent` (`self.Latch Part`) (`self.Rotate 2`) "None" "KeepWorld" "KeepWorld" "KeepWorld" true))

(event `Spawn Door`
  (bind _rotate_2 (`self.Rotate 2`))
  (bind _returnvalue_location (`KismetMathLibrary.BreakTransform` (`SceneComponent.K2_GetComponentToWorld` _rotate_2)))
  (bind (_returnvalue_x _returnvalue_y _returnvalue_z) (`KismetMathLibrary.BreakVector` (`SceneComponent.GetForwardVector` _rotate_2)))
  (bind _returnvalue (`|SpawnActorFromClass` "/Game/Objects/BP_Objects/BP_Door_Part.BP_Door_Part_C" (`KismetMathLibrary.MakeTransform` (+ _returnvalue_location (`KismetMathLibrary.MakeVector` _returnvalue_x (+ _returnvalue_y (`self.Impulse`)) _returnvalue_z))) "Undefined" "OverrideRootScale" null null))
  (`ActorComponent.K2_DestroyComponent` (`self.Rotate 2`))
  (`PrimitiveComponent.AddImpulse` (`/Game/Objects/Structurs/BP_Object.Root` _returnvalue) (* (`SceneComponent.GetForwardVector` (`Actor.RootComponent` _returnvalue)) 150.0) "None" false)
  (`/Game/Objects/BP_Objects/BP_Door_Part.Set Material` _returnvalue (`self.Material`)))

(fn `UserConstructionScript`
  (bind _rotate_2 (`self.Rotate 2`))
  (bind _border (`self.Border`))
  (`parent.UserConstructionScript`)
  (`|ExecutionSequence`
    (:`then_0`
      (switch `/Game/Objects/Enum/DoorMaterialEnim` (`self.Material`)
        (:`NewEnumerator0`
          (`PrimitiveComponent.SetMaterial` _border 0 "/Game/Objects/Materials/white_wood_mat.white_wood_mat")
          (`PrimitiveComponent.SetMaterial` (`self.Rotate`) 0 "/Game/Objects/Materials/white_wood_mat.white_wood_mat")
          (`PrimitiveComponent.SetMaterial` (`self.Rotate 2`) 0 "/Game/Objects/Materials/white_wood_mat.white_wood_mat"))
        (:`NewEnumerator1`
          (`PrimitiveComponent.SetMaterial` _border 0 "/Game/Objects/Materials/wood_4_mat.wood_4_mat")
          (`PrimitiveComponent.SetMaterial` (`self.Rotate`) 0 "/Game/Objects/Materials/wood_4_mat.wood_4_mat")
          (`PrimitiveComponent.SetMaterial` (`self.Rotate 2`) 0 "/Game/Objects/Materials/wood_4_mat.wood_4_mat"))
        (:`NewEnumerator2`
          (`PrimitiveComponent.SetMaterial` _border 0 "/Game/Objects/Materials/red_dark_wood.red_dark_wood")
          (`PrimitiveComponent.SetMaterial` (`self.Rotate`) 0 "/Game/Objects/Materials/red_dark_wood.red_dark_wood")
          (`PrimitiveComponent.SetMaterial` (`self.Rotate 2`) 0 "/Game/Objects/Materials/red_dark_wood.red_dark_wood"))))
    (:`then_1`
      (switch `/Game/Objects/Enum/RotateStateEnum` (`self.Rotate 2 State`)
        (:`NewEnumerator0`
          (`SceneComponent.K2_SetRelativeRotation` _rotate_2 (struct :`Yaw` -100.0) false false))
        (:`NewEnumerator1`
          (`SceneComponent.K2_SetRelativeRotation` _rotate_2 (struct) false false))))))
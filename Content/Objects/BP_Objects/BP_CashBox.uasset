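; Checkout box that stops an overlapping shopping cart and checks its products against a required purchase list.
; On overlap it blocks the cart, disables the Electricity objects and runs the check after a two-second timer.
; Matches light five bulbs green by count, with the rest red, alongside OK or error signals.
; All green re-enables Electricity, also enabled at start; otherwise Catch plays, player input is disabled and the level reloads.
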(event `self.Box.OnComponentBeginOverlap`
  (params (OverlappedComponent :type "PrimitiveComponent Object Reference") (OtherActor :type "Actor Object Reference") (OtherComp :type "PrimitiveComponent Object Reference") (OtherBodyIndex :type Integer) (bFromSweep :type Boolean) (SweepResult :type "HitResult Structure (by ref)"))
  (bind _asbp_cart (cast `/Game/Objects/BP_Objects/BP_Cart` OtherActor))
  (bind _output_get (set `self.Cart` _asbp_cart))
  (`/Game/Objects/BP_Objects/BP_Cart.Stop` _output_get)
  (set `/Game/Objects/BP_Objects/BP_Cart.Blocking` true _output_get)
  (bind _returnvalue (`KismetSystemLibrary.K2_SetTimerDelegate` (delegate `Check Items`) 2.0 true true))
  (set `self.Check Timer` _returnvalue)
  (for _array_element (`self.Electricity`)
    (`/Game/Objects/Structurs/BP_Electricity.Disable` _array_element)))

(event `Check Items`
  (bind _array (`|MakeArray` (`self.Bulb 5`) (`self.Bulb 4`) (`self.Bulb 3`) (`self.Bulb 2`) (`self.Bulb 1`)))
  (for (_array_element _array_index) (`self.Need Purchases`)
    (for _array_element_2 (`/Game/Objects/BP_Objects/BP_Cart.Products` (`self.Cart`))
      (if (== (`GameplayStatics.GetObjectClass` _array_element_2) _array_element)
        (`KismetArrayLibrary.Array_Add` (`self.Item`) _array_index))))
  (for (_array_element_3 _array_index_2) _array
    (if (`KismetArrayLibrary.Array_IsValidIndex` (`self.Item`) _array_index_2)
      (`PrimitiveComponent.SetMaterial` _array_element_3 0 "/Game/Objects/Materials/Green_light_ON_inst.Green_light_ON_inst")
      (`AudioComponent.Play` (`self.Signal OK`) 0.0)
      (else
        (`PrimitiveComponent.SetMaterial` _array_element_3 0 "/Game/Objects/Materials/Red_light_ON_inst.Red_light_ON_inst")
        (`AudioComponent.Play` (`self.Signal ERR`) 0.0))))
  (for _array_element_4 _array
    (if (== (`PrimitiveComponent.GetMaterial` _array_element_4 0) "/Game/Objects/Materials/Green_light_ON_inst.Green_light_ON_inst")
      (set `self.Purchased` true)
      (else
        (set `self.Purchased` false)
        (break))))
  (`KismetSystemLibrary.K2_ClearAndInvalidateTimerHandle` (`self.Check Timer`))
  (if (`self.Purchased`)
    (for _array_element_5 (`self.Electricity`) :!label _label
      (`/Game/Objects/Structurs/BP_Electricity.Enable` _array_element_5))
    (else
      (`AudioComponent.Play` (`self.Catch`) 0.0)
      (bind _player (`/Game/Function/BP_MacroLibrary.Find Player`)
        (:`Is Valid`
          (`self.DisableInput` _player (`GameplayStatics.GetPlayerController` 0))
          (`KismetSystemLibrary.Delay` 2.0)
          (bind _returnvalue (`GameplayStatics.GetCurrentLevelName` true))
          (`GameplayStatics.OpenLevel` (`KismetStringLibrary.Conv_StringToName` _returnvalue)))))))

(event `self.ReceiveBeginPlay`
  (goto _label))

(fn `UserConstructionScript`)
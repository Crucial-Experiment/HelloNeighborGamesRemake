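; Radio item that players toggle on and off to play a sound, via left click while held, Interact or VR use.
; Toggles and slot changes, which force it off, go through a server event that stores the state and multicasts it.
; The multicast plays or stops the sound cue and notifies tutorial and GameJolt components of the use.
; The construction script assigns the configurable radio sound.
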(event `self.ReceiveBeginPlay`
  (`parent.ReceiveBeginPlay`))

(event `On Press LMB_1`
  (bind _player (`/Game/Function/BP_MacroLibrary.Find Player`)
    (:`Is Valid`
      (bind _item (`/Game/Player/BP_Player.Get Item` _player))
      (if (== _item self)
        (`self.Interact (Server)` (select `/Game/Objects/Enum/TumblerStateEnum` (`self.State`) :`NewEnumerator0` "NewEnumerator1" :`NewEnumerator1` "NewEnumerator0" :!type "/Game/Objects/Enum/TumblerStateEnum Enum") :!label _label)))))

(event `/Game/Function/BP_Interface.Interact`
  (params (Component :type "PrimitiveComponent Object Reference") (Location :type "Vector Structure"))
  (goto _label))

(event `Interact (Server)`
  (params (`New State` :type "/Game/Objects/Enum/TumblerStateEnum Enum" :default "NewEnumerator0"))
  (bind _output_get (set `self.State` `New State`))
  (`self.Interact (All)` _output_get))

(event `On Slot Change_1`
  (`self.Interact (Server)` "NewEnumerator1"))

(event `self.On VR Use`
  (`parent.On VR Use`)
  (goto _label))

(event `Interact (All)`
  (params (`New State` :type "/Game/Objects/Enum/TumblerStateEnum Enum" :default "NewEnumerator0"))
  (bind _radiosoundcue (`self.RadioSoundCue`))
  (`/Game/Objects/Tutorial/TutorialComponent.Check Use Type` (`self.TutorialComponent`) "NewEnumerator6")
  (`/Game/Objects/GameJolt/GameJoltComponent.Check Use Type` (`self.GameJoltComponent`) "NewEnumerator6")
  (switch `/Game/Objects/Enum/TumblerStateEnum` `New State`
    (:`NewEnumerator0`
      (`AudioComponent.Play` _radiosoundcue 0.0))
    (:`NewEnumerator1`
      (`AudioComponent.Stop` _radiosoundcue))))

(fn `UserConstructionScript`
  (`AudioComponent.SetSound` (`self.RadioSoundCue`) (`self.Radio Sound`)))
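; BP_School_Bell is a switchable school bell object that plays sound and animates while enabled.
; Enable starts the Bell component and the Call timeline, which tilts Part and slightly squashes and stretches Root.
; The timeline restarts itself on finish, looping the ringing motion.
; Disable stops both and resets the rotation and scale, with both events also calling their parent versions.
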(event `Play from Start`
  (bind (_direction _alpha) (`Timeline|Call` :!via `PlayFromStart` :!label _label)
    (:`Update`
      (`SceneComponent.K2_SetRelativeRotation` (`self.Part`) (`KismetMathLibrary.RLerp` (struct) (struct :`Pitch` -10.0) _alpha) false false)
      (`SceneComponent.SetRelativeScale3D` (`self.Root`) (`KismetMathLibrary.VLerp` (1.0 1.0 1.0) (1.1 1.0 0.9) _alpha)))
    (:`Finished`
      (`self.Play from Start`))))

(event `self.Enable`
  (`parent.Enable`)
  (`AudioComponent.Play` (`self.Bell`) 0.0)
  (goto _label))

(event `self.Disable`
  (`parent.Disable`)
  (`AudioComponent.Stop` (`self.Bell`))
  (`SceneComponent.K2_SetRelativeRotation` :`self` (`self.Part`))
  (`SceneComponent.SetRelativeScale3D` (`self.Root`) (1.0 1.0 1.0))
  (goto _label :!via `Stop`))

(fn `UserConstructionScript`
  (`parent.UserConstructionScript`))
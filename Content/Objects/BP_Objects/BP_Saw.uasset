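; BP_Saw is a usable item that cuts through cuttable BP_Door_Block locks, triggered by VR use or by left click while held.
; A short line trace finds the block, then chained timelines move the saw to its SawPosition and lower it while player input is disabled.
; A server event then unlocks the block and replaces it with two part actors, and the saw returns to its saved relative transform.
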(event `Unlock (Server)`
  (params (Lock :type "/Game/Objects/BP_Objects/BP_Door_Block Object Reference"))
  (bind _returnvalue (`SceneComponent.K2_GetComponentToWorld` (`/Game/Objects/Structurs/BP_Object.Root` Lock)))
  (`/Game/Objects/Structurs/BP_Lock.Unlock` Lock)
  (`|SpawnActorFromClass` "/Game/Objects/BP_Objects/BP_Door_Block_Part1.BP_Door_Block_Part1_C" _returnvalue "Undefined" "MultiplyWithRoot" null null)
  (`|SpawnActorFromClass` "/Game/Objects/BP_Objects/BP_Door_Block_Part2.BP_Door_Block_Part2_C" _returnvalue "Undefined" "MultiplyWithRoot" null null)
  (`self.K2_DestroyActor` Lock))

(event `self.On VR Use`
  (bind (_relative_transform_location _relative_transform_rotation) (`KismetMathLibrary.BreakTransform` (`self.Relative Transform`)))
  (bind _returnvalue (`SceneComponent.K2_GetComponentLocation` (`self.Root`)))
  (`parent.On VR Use`)
  (bind _actor (`self.Line Trace` 150.0 "NewEnumerator1" :!label _label))
  (bind _asbp_door_block (cast `/Game/Objects/BP_Objects/BP_Door_Block` _actor))
  (if (`/Game/Objects/BP_Objects/BP_Door_Block.Can Be Cut?` _asbp_door_block)
    (`self.DisableInput` (`GameplayStatics.GetPlayerPawn` 0) (`GameplayStatics.GetPlayerController` 0))
    (set `self.Relative Transform` (`SceneComponent.GetRelativeTransform` (`self.Root`)))
    (bind (_direction _alpha) (`Timeline|Location Timeline` :!via `PlayFromStart`)
      (:`Update`
        (bind _saw_position (`/Game/Objects/BP_Objects/BP_Door_Block.Saw Position` _asbp_door_block))
        (`SceneComponent.K2_SetWorldLocationAndRotation` (`self.Root`) (`KismetMathLibrary.VLerp` (`SceneComponent.K2_GetComponentLocation` (`self.Root`)) (`SceneComponent.K2_GetComponentLocation` _saw_position) _alpha) (`SceneComponent.K2_GetComponentRotation` _saw_position) false false))
      (:`Finished`
        (bind (_direction_2 _alpha_2) (`Timeline|Cutting Timeline` :!via `PlayFromStart`)
          (:`Update`
            (`SceneComponent.K2_SetWorldLocation` (`self.Root`) (`KismetMathLibrary.VLerp` _returnvalue (- _returnvalue (0.0 0.0 0.78)) _alpha_2) false false))
          (:`Finished`
            (`self.Unlock (Server)` _asbp_door_block)
            (`SceneComponent.K2_SetRelativeLocationAndRotation` (`self.Root`) _relative_transform_location _relative_transform_rotation false false)
            (`self.EnableInput` (`GameplayStatics.GetPlayerPawn` 0) (`GameplayStatics.GetPlayerController` 0))))))))

(event `self.On Press LMB`
  (bind _player (`/Game/Function/BP_MacroLibrary.Find Player`)
    (:`Is Valid`
      (bind _item (`/Game/Player/BP_Player.Get Item` _player))
      (if (== _item self)
        (goto _label)))))

(fn `UserConstructionScript`
  (`parent.UserConstructionScript`))
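; BP_Rifle is a grabbable rifle, usable by mouse click or VR use, that fires physical bullets or docks onto a rifle range stand.
; On use it notifies tutorial and GameJolt components, then line-traces: hitting the range's stand releases and docks it, otherwise it fires.
; The server shot spawns a BP_RifleBullet at the Sphere component and launches it with a forward impulse.
; Grabbing clears the range link, while dropping unlinked sets flat mode.
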(event `self.GrabComponent.OnDropped`
  (params (`Self Ref` :type "/Game/Objects/Structurs/GrabComponent Object Reference"))
  (`/Engine/EditorBlueprintResources/StandardMacros.IsValid` (`self.Rifle Range`)
    (:`Is Not Valid`
      (`self.Set Flat Mode` "NewEnumerator0"))))

(event `Shot (Server)`
  (bind _sphere (`self.Sphere`))
  (bind _returnvalue (`|SpawnActorFromClass` "/Game/Objects/BP_Objects/BP_RifleBullet.BP_RifleBullet_C" (`KismetMathLibrary.MakeTransform` (`SceneComponent.K2_GetComponentLocation` _sphere) (`SceneComponent.K2_GetComponentRotation` _sphere)) "Undefined" "OverrideRootScale" null null))
  (`PrimitiveComponent.AddImpulse` (`/Game/Objects/Structurs/BP_Object.Root` _returnvalue) (* (`SceneComponent.GetForwardVector` (`self.Sphere`)) 200000.0) "None" false))

(event `self.GrabComponent.OnGrabbed`
  (params (`Self Ref` :type "/Game/Objects/Structurs/GrabComponent Object Reference"))
  (bind _rifle_range (`self.Rifle Range`)
    (:`then`
      (`/Game/Objects/BP_Objects/BP_Rifle_Range.Rifle Taken` _rifle_range)
      (set `self.Rifle Range` null))
    (:`else`)))

(event `self.ReceiveBeginPlay`
  (`parent.ReceiveBeginPlay`))

(event `On Press LMB_1`
  (bind _player (`/Game/Function/BP_MacroLibrary.Find Player`)
    (:`Is Valid`
      (bind _item (`/Game/Player/BP_Player.Get Item` _player))
      (if (== _item self)
        (`/Game/Objects/Tutorial/TutorialComponent.Check Use Type` (`self.TutorialComponent`) "NewEnumerator6" :!label _label)
        (`/Game/Objects/GameJolt/GameJoltComponent.Check Use Type` (`self.GameJoltComponent`) "NewEnumerator6")
        (bind (_actor _component) (`self.Line Trace` 500.0))
        (bind _asbp_rifle_range (cast `/Game/Objects/BP_Objects/BP_Rifle_Range` _actor)
          (:`then`
            (bind _bool (`/Game/Function/BP_FunctionLibrary.Checking Object` _component (`/Game/Objects/BP_Objects/BP_Rifle_Range.Rifle Stand` _asbp_rifle_range)))
            (if _bool
              (set `/Game/Objects/BP_Objects/BP_Rifle_Range.Rifle` self _asbp_rifle_range)
              (set `self.Rifle Range` _asbp_rifle_range)
              (`self.Try Release`)
              (`/Game/Objects/BP_Objects/BP_Rifle_Range.Rifle Transform` _asbp_rifle_range)
              (else
                (`AudioComponent.Play` (`self.Shot`) 0.0 :!label _label_2)
                (`self.Shot (Server)`))))
          (:`CastFailed`
            (goto _label_2)))))))

(event `self.On VR Use`
  (`parent.On VR Use`)
  (goto _label))

(fn `UserConstructionScript`)
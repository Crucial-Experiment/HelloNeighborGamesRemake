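; BP_Picture_Set is a grabbable painting set object with five selectable mesh variants.
; The construction script runs the parent's script, then uses the Model value to assign the matching painting set mesh to Root.
; When the GrabComponent reports a drop, it calls SetFlatMode with a fixed enum value.
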(event `self.GrabComponent.OnDropped`
  (params (`Self Ref` :type "/Game/Objects/Structurs/GrabComponent Object Reference"))
  (`self.Set Flat Mode` "NewEnumerator0"))

(fn `UserConstructionScript`
  (bind _root (`self.Root`))
  (`parent.UserConstructionScript`)
  (switch `int` (`self.Model`)
    (:`0`
      (`StaticMeshComponent.SetStaticMesh` _root "/Game/Objects/Meshes/paintings_set_1_new.paintings_set_1_new"))
    (:`1`
      (`StaticMeshComponent.SetStaticMesh` _root "/Game/Objects/Meshes/paintings_set_2_new.paintings_set_2_new"))
    (:`2`
      (`StaticMeshComponent.SetStaticMesh` _root "/Game/Objects/Meshes/paintings_set_3_new.paintings_set_3_new"))
    (:`3`
      (`StaticMeshComponent.SetStaticMesh` _root "/Game/Objects/Meshes/paintings_set_4_new.paintings_set_4_new"))
    (:`4`
      (`StaticMeshComponent.SetStaticMesh` _root "/Game/Objects/Meshes/paintings_set_5_new.paintings_set_5_new"))))
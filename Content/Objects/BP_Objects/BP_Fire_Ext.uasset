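; Fire extinguisher item that toggles a spray to put out BP_Fire actors.
; While active, Tick runs a short line trace and subtracts Speed from the hit fire's Health each frame, unscaled by delta time.
; LMB while held or VR use toggles the spray components and notifies the tutorial, plus GameJolt on activation.
; Dropping, grab release and slot changes reuse the switch-off path, including its tutorial notification.
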(event `self.ReceiveTick`
  (params (DeltaSeconds :type "Float (single-precision)"))
  ;[1 1 1] Begin Play
  (if (`self.Activate`)
    (bind _actor (`self.Line Trace` 250.0))
    (bind _asbp_fire (cast `/Game/Objects/BP_Objects/BP_Fire` _actor))
    (`/Game/Objects/BP_Objects/BP_Fire.Set Health` _asbp_fire (- (`/Game/Objects/BP_Objects/BP_Fire.Health` _asbp_fire) (`self.Speed`)))))

(event `self.ReceiveBeginPlay`
  ;[1 1 1] Begin Play
  (`parent.ReceiveBeginPlay`))

(event `On Press LMB_1`
  (bind _tutorialcomponent (`self.TutorialComponent`))
  (bind _p_spray (`self.P_Spray`))
  ;[1 1 1] Begin Play
  (bind _player (`/Game/Function/BP_MacroLibrary.Find Player`)
    (:`Is Valid`
      (bind _item (`/Game/Player/BP_Player.Get Item` _player))
      (if (== _item self)
        (if (`self.Activate`) :!label _label
          (set `self.Activate` false :!label _label_2)
          (`ActorComponent.Deactivate` _p_spray)
          (`ActorComponent.Deactivate` (`self.Spray`))
          (`/Game/Objects/Tutorial/TutorialComponent.Check Use Type` _tutorialcomponent "NewEnumerator6")
          (else
            (set `self.Activate` true)
            (`ActorComponent.Activate` _p_spray false)
            (`ActorComponent.Activate` (`self.Spray`) false)
            (`/Game/Objects/Tutorial/TutorialComponent.Check Use Type` _tutorialcomponent "NewEnumerator6")
            (`/Game/Objects/GameJolt/GameJoltComponent.Check Use Type` (`self.GameJoltComponent`) "NewEnumerator6")))))))

(event `self.On VR Use`
  ;[1 1 1] Begin Play
  (`parent.On VR Use`)
  (goto _label))

(event `On Item Dropped_1`
  ;[1 1 1] Begin Play
  (goto _label_2))

(event `On Slot Change_1`
  ;[1 1 1] Begin Play
  (goto _label_2))

(event `self.GrabComponent.OnDropped`
  (params (`Self Ref` :type "/Game/Objects/Structurs/GrabComponent Object Reference"))
  ;[1 1 1] Begin Play
  (goto _label_2))

(fn `UserConstructionScript`)
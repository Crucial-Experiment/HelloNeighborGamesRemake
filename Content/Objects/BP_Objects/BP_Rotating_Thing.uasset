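; BP_Rotating_Thing is an electrically driven mechanism that spins around its yaw axis and plays machinery sounds.
; While it has electricity or is flagged as Generator, Tick rotates the root by Speed, and BeginPlay starts the buzz loop under the same check.
; Enable and Disable extend the parent's logic, switching between a start cue with delayed buzz and a crash cue on shutdown.
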(event `self.Enable`
  (`parent.Enable`)
  (`AudioComponent.Stop` (`self.mechanism_crash_Cue`))
  (`AudioComponent.Play` (`self.mechanism_start_Cue`) 0.0)
  (`KismetSystemLibrary.Delay` 1.4)
  (`AudioComponent.Play` (`self.mechanism_buzz_Cue`) 0.0))

(event `self.Disable`
  (`parent.Disable`)
  (`AudioComponent.Stop` (`self.mechanism_buzz_Cue`))
  (`AudioComponent.Play` (`self.mechanism_crash_Cue`) 0.0)
  (`AudioComponent.Stop` (`self.mechanism_start_Cue`)))

(event `self.ReceiveBeginPlay`
  (if (or (`self.Has Electricity`) (`self.Generator`))
    (`AudioComponent.Play` (`self.mechanism_buzz_Cue`) 0.0)))

(event `self.ReceiveTick`
  (params (DeltaSeconds :type "Float (single-precision)"))
  (if (or (`self.Has Electricity`) (`self.Generator`))
    (`SceneComponent.K2_AddWorldRotation` (`self.Root`) (`KismetMathLibrary.MakeRotator` 0.0 0.0 (`self.Speed`)) false false)))

(fn `UserConstructionScript`
  (`parent.UserConstructionScript`))
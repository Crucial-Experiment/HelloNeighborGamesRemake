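; BP_Latch is an interactive latch that snaps onto a linked Rotate object's latch position, starting closed when linked and open otherwise.
; Interacting with its boxes toggles it, only while that object isn't open, through server-to-all events that play timed animations and call parent lock logic with a rattle sound.
; Toggling also disables pickup and notifies tutorial and GameJolt components.
; The latch destroys itself when the linked object's SpawnDoorPart event fires.
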(event `self.Lock`
  (`parent.Lock`)
  (`GameplayStatics.PlaySoundAtLocation` "/Game/Sounds/Maps/Act2/Main/metal_rattle_off_Cue.metal_rattle_off_Cue" (`self.K2_GetActorLocation`) (struct) 1.0 1.0 0.0 null null null null :!label _label))

(event `self.Unlock`
  (`parent.Unlock`)
  (goto _label))

(event `self.ReceiveBeginPlay`
  (bind _rotate (`self.Rotate`)
    (:`then`
      (set `self.State` "NewEnumerator1")
      (`self.Play Animation` "/Game/Objects/Meshes/Animations/Latch/latch_close.latch_close")
      (`self.Lock`)
      (`SceneComponent.SetHiddenInGame` (`/Game/Objects/Structurs/BP_Rotate.Latch Part` _rotate) false false)
      (`self.K2_AttachToComponent` (`/Game/Objects/Structurs/BP_Rotate.Latch Pos` _rotate) "None" "SnapToTarget" "SnapToTarget" "SnapToTarget")
      (add `/Game/Objects/Structurs/BP_Rotate.Spawn Door Part` _rotate (delegate `Destroy`)))
    (:`else`
      (set `self.State` "NewEnumerator0")
      (`self.Play Animation` "/Game/Objects/Meshes/Animations/Latch/latch_open.latch_open")
      (`self.Unlock`))))

(event `Destroy`
  (`SceneComponent.SetHiddenInGame` (`/Game/Objects/Structurs/BP_Rotate.Latch Part` (stale `self.ReceiveBeginPlay` _rotate)) true false)
  (`self.K2_DestroyActor`))

(event `Lock (Server)`
  (`self.Lock (all)`))

(event `Lock (All)`
  (`self.Lock`)
  (bind _play_length (`self.Play Animation` "/Game/Objects/Meshes/Animations/Latch/latch_lock.latch_lock"))
  (`KismetSystemLibrary.Delay` _play_length)
  (`self.Play Animation` "/Game/Objects/Meshes/Animations/Latch/latch_close.latch_close")
  (set `self.State` "NewEnumerator1")
  (`self.Set Flat Mode` "NewEnumerator1" :!label _label_2)
  (set `/Game/Objects/Structurs/GrabComponent.GrabType` "NewEnumerator0" (`self.GrabComponent`))
  (set `self.CanPickUp` false)
  (`/Game/Objects/Tutorial/TutorialComponent.Check Use Type` (`self.TutorialComponent`) "NewEnumerator6")
  (`/Game/Objects/GameJolt/GameJoltComponent.Check Use Type` (`self.GameJoltComponent`) "NewEnumerator6"))

(event `/Game/Function/BP_Interface.Interact`
  (params (Component :type "PrimitiveComponent Object Reference") (Location :type "Vector Structure"))
  (if (or (== Component (`self.Box`)) (== Component (`self.Box1`)))
    (switch `/Game/Objects/Enum/RotateStateEnum` (`self.State`)
      (:`NewEnumerator0`
        (bind _rotate (`self.Rotate`)
          (:`then`
            (if (`|EnumInequality` (`/Game/Objects/Structurs/BP_Rotate.Rotate State` _rotate) "NewEnumerator0")
              (`self.Lock (Server)`)))
          (:`else`)))
      (:`NewEnumerator1`
        (bind _rotate_2 (`self.Rotate`)
          (:`then`
            (if (`|EnumInequality` (`/Game/Objects/Structurs/BP_Rotate.Rotate State` _rotate_2) "NewEnumerator0")
              (`self.Unlock (Server)`)))
          (:`else`))))))

(event `Unlock (All)`
  (bind _play_length (`self.Play Animation` "/Game/Objects/Meshes/Animations/Latch/latch_unlock.latch_unlock"))
  (`KismetSystemLibrary.Delay` _play_length)
  (`self.Play Animation` "/Game/Objects/Meshes/Animations/Latch/latch_open.latch_open")
  (`self.Unlock`)
  (set `self.State` "NewEnumerator0")
  (goto _label_2))

(event `Unlock (Server)`
  (`self.Unlock (All)`))

(fn `Play Animation`
  (params (Anim :type "AnimSequence Object Reference") (Loop :type Boolean))
  (returns (`Play Length` :type "Float (double-precision)"))
  (`SkeletalMeshComponent.PlayAnimation` (`self.Latch Mesh`) Anim Loop)
  (return (`AnimSequenceBase.GetPlayLength` Anim)))

(fn `UserConstructionScript`
  (`parent.UserConstructionScript`)
  (bind _rotate (`self.Rotate`)
    (:`then`
      (set `self.State` "NewEnumerator1")
      (`self.Play Animation` "/Game/Objects/Meshes/Animations/Latch/latch_close.latch_close")
      (`self.K2_AttachToComponent` (`/Game/Objects/Structurs/BP_Rotate.Latch Pos` _rotate) "None" "SnapToTarget" "SnapToTarget" "SnapToTarget"))
    (:`else`
      (set `self.State` "NewEnumerator0")
      (`self.Play Animation` "/Game/Objects/Meshes/Animations/Latch/latch_open.latch_open"))))
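; BP_Lattice is an electricity-driven barrier that closes while powered and opens when power is lost.
; Tick polls HasElectricity and switches a four-state machine, restarting OpenClose playback on each reversal, even mid-motion.
; MovingPlatform steps Alpha by Speed and delta time to lerp the Lattice's relative location and rotation between start (open) and end (closed).
; Enable and Disable extend parent behavior by reporting use types to the tutorial and GameJolt components.
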(event `self.Enable`
  ;[1 1 1] Begin Play and Electricity
  (`parent.Enable`)
  (`/Game/Objects/Tutorial/TutorialComponent.Check Use Type` (`self.TutorialComponent`) "NewEnumerator3")
  (`/Game/Objects/GameJolt/GameJoltComponent.Check Use Type` (`self.GameJoltComponent`) "NewEnumerator3"))

(event `self.ReceiveBeginPlay`
  ;[1 1 1] Begin Play and Electricity
  (`parent.ReceiveBeginPlay`))

(event `self.ReceiveTick`
  (params (DeltaSeconds :type "Float (single-precision)"))
  (bind _state (`self.State`))
  ;[1 1 1] Event Tick
  (`self.Moving Platform` DeltaSeconds)
  (if (`self.Has Electricity`)
    (switch `/Game/Objects/Enum/RotateStateEnum` _state
      (:`NewEnumerator0`
        (`AudioComponent.Stop` (`self.Open / Close`)))
      (:`NewEnumerator2`
        _))
    (set `self.State` "NewEnumerator3")
    (else
      (switch `/Game/Objects/Enum/RotateStateEnum` _state
        (:`NewEnumerator1`
          (`AudioComponent.Stop` (`self.Open / Close`)))
        (:`NewEnumerator3`
          _))
      (set `self.State` "NewEnumerator2")))
  (`AudioComponent.Play` (`self.Open / Close`) 0.0))

(event `self.Disable`
  ;[1 1 1] Begin Play and Electricity
  (`parent.Disable`)
  (`/Game/Objects/Tutorial/TutorialComponent.Check Use Type` (`self.TutorialComponent`) "NewEnumerator4")
  (`/Game/Objects/GameJolt/GameJoltComponent.Check Use Type` (`self.GameJoltComponent`) "NewEnumerator4"))

(fn `Moving Platform`
  (params (`Delta Time` :type "Float (double-precision)"))
  (bind _lattice (`self.Lattice`))
  (switch `/Game/Objects/Enum/RotateStateEnum` (`self.State`)
    (:`NewEnumerator2`
      (if (< (`self.Alpha`) 0.0)
        (`SceneComponent.K2_SetRelativeLocationAndRotation` _lattice (`self.Start Position`) (`self.Start Rotation`) false false)
        (set `self.Alpha` 0.0)
        (set `self.State` "NewEnumerator0")
        (else
          (`SceneComponent.K2_SetRelativeLocationAndRotation` _lattice (`KismetMathLibrary.VLerp` (`self.Start Position`) (`self.End Position`) (`self.Alpha`)) (`KismetMathLibrary.RLerp` (`self.Start Rotation`) (`self.End Rotation`) (`self.Alpha`)) false false)
          (set `self.Alpha` (- (`self.Alpha`) (* (`self.Speed`) `Delta Time`))))))
    (:`NewEnumerator3`
      (if (> (`self.Alpha`) 1.0)
        (`SceneComponent.K2_SetRelativeLocationAndRotation` (`self.Lattice`) (`self.End Position`) (`self.End Rotation`) false false)
        (set `self.Alpha` 1.0)
        (set `self.State` "NewEnumerator1")
        (else
          (`SceneComponent.K2_SetRelativeLocationAndRotation` (`self.Lattice`) (`KismetMathLibrary.VLerp` (`self.Start Position`) (`self.End Position`) (`self.Alpha`)) (`KismetMathLibrary.RLerp` (`self.Start Rotation`) (`self.End Rotation`) (`self.Alpha`)) false false)
          (set `self.Alpha` (+ (* (`self.Speed`) `Delta Time`) (`self.Alpha`))))))))

(fn `UserConstructionScript`
  (`parent.UserConstructionScript`))
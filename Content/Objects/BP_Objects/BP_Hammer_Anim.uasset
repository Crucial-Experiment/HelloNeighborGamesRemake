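; BP_Hammer_Anim is a usable hammer item that unlocks BP_Door_Block_Anim door blocks and BP_HammerTrigger actors.
; In VR, overlapping either target unlocks it, with a creak sound for blocks.
; On left click while held, a short line trace finds the target; triggers unlock immediately.
; Blocks first play a nail-puller animation with input disabled while a timeline moves the mesh, and successful uses report to tutorial and GameJolt components.
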(event `self.VR Interact.OnComponentBeginOverlap`
  (params (OverlappedComponent :type "PrimitiveComponent Object Reference") (OtherActor :type "Actor Object Reference") (OtherComp :type "PrimitiveComponent Object Reference") (OtherBodyIndex :type Integer) (bFromSweep :type Boolean) (SweepResult :type "HitResult Structure (by ref)"))
  ;[1 1 1] VR Interact
  (bind _asbp_door_block_anim (cast `/Game/Objects/BP_Objects/BP_Door_Block_Anim` OtherActor)
    (:`then`
      (if (not (`/Game/Objects/Structurs/BP_Object.CanPickUp` _asbp_door_block_anim))
        (`/Game/Objects/Structurs/BP_Lock.Unlock` _asbp_door_block_anim)
        (`GameplayStatics.PlaySound2D` "/Game/Sounds/Sosed/step_creaky_wood_Cue.step_creaky_wood_Cue" 1.0 1.0 0.0 null null)))
    (:`CastFailed`
      (bind _asbp_hammer_trigger (cast `/Game/PrototypeFiles/BP_HammerTrigger` OtherActor))
      (`|ExecutionSequence`
        (:`then_0`
          (`/Game/Objects/Structurs/BP_Lock.Unlock` _asbp_hammer_trigger))))))

(event `self.On VR Use`
  (`parent.On VR Use`))

(event `On Press LMB_2`
  (bind (_relative_transform_location _relative_transform_rotation) (`KismetMathLibrary.BreakTransform` (`self.Relative Transform`)))
  (bind _player (`/Game/Function/BP_MacroLibrary.Find Player`)
    (:`Is Valid`
      (bind _item (`/Game/Player/BP_Player.Get Item` _player))
      (if (== _item self)
        (bind _actor (`self.Line Trace` 150.0))
        (bind _asbp_door_block_anim (cast `/Game/Objects/BP_Objects/BP_Door_Block_Anim` _actor)
          (:`then`
            (if (not (`/Game/Objects/Structurs/BP_Object.CanPickUp` _asbp_door_block_anim))
              (`/Engine/EditorBlueprintResources/StandardMacros.DoOnce` false :!label _label
                (:`Completed`
                  (set `self.Relative Transform` (`SceneComponent.GetRelativeTransform` (`self.SkeletalMesh`)))
                  (`SkeletalMeshComponent.PlayAnimation` (`self.SkeletalMesh`) "/Game/Objects/Meshes/Animations/Nailpuller/nailpuller_Anim.nailpuller_Anim" false)
                  (`self.DisableInput` (`GameplayStatics.GetPlayerPawn` 0) (`GameplayStatics.GetPlayerController` 0))
                  (bind (_direction _alpha) (`Timeline|Location Timeline` :!via `PlayFromStart`)
                    (:`Update`
                      (`SceneComponent.K2_SetWorldLocationAndRotation` :`self` (`self.SkeletalMesh`) :`NewLocation` (`KismetMathLibrary.VLerp` (`SceneComponent.K2_GetComponentLocation` (`Actor.RootComponent` _asbp_door_block_anim)) (`SceneComponent.K2_GetComponentLocation` (`/Game/Objects/BP_Objects/BP_Door_Block_Anim.Scene` _asbp_door_block_anim)) _alpha)))
                    (:`Finished`
                      (`/Game/Objects/Structurs/BP_Lock.Unlock` _asbp_door_block_anim)
                      (`SceneComponent.K2_SetRelativeLocationAndRotation` (`self.SkeletalMesh`) _relative_transform_location _relative_transform_rotation false false)
                      (`self.EnableInput` (`GameplayStatics.GetPlayerPawn` 0) (`GameplayStatics.GetPlayerController` 0))
                      (`/Game/Objects/Tutorial/TutorialComponent.Check Use Type` (`self.TutorialComponent`) "NewEnumerator6")
                      (`/Game/Objects/GameJolt/GameJoltComponent.Check Use Type` (`self.GameJoltComponent`) "NewEnumerator6")
                      (goto _label :!via `Reset`)))))))
          (:`CastFailed`
            (bind _asbp_hammer_trigger (cast `/Game/PrototypeFiles/BP_HammerTrigger` _actor))
            (`/Game/Objects/Structurs/BP_Lock.Unlock` _asbp_hammer_trigger)
            (`/Game/Objects/Tutorial/TutorialComponent.Check Use Type` (`self.TutorialComponent`) "NewEnumerator6")
            (`/Game/Objects/GameJolt/GameJoltComponent.Check Use Type` (`self.GameJoltComponent`) "NewEnumerator6")))))))

(fn `UserConstructionScript`
  (`parent.UserConstructionScript`))
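; BP_Switcher_Picture is an interactable picture that works as a hidden electrical switch, with mesh and material chosen in the construction script.
; Server interaction plays or reverses a rotation timeline with a sound, then flips State and notifies the tutorial and GameJolt components.
; Tumbler enables or disables linked Electricity actors, depending on power or generator status.
; Rotation state is saved to JSON, and loading replays Interact when it differs.
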(event `Interact (Server)`
  (bind _tutorialcomponent (`self.TutorialComponent`))
  (bind _gamejoltcomponent (`self.GameJoltComponent`))
  ;[1 1 1] Rotation
  (`|ExecutionSequence`
    (:`then_0`
      (switch `/Game/Objects/Enum/RotateStateEnum` (`self.Rotate`)
        (:`NewEnumerator0`
          (bind (_direction _alpha) (`Timeline|Picture Rotate` :!via `Reverse` :!label _label)
            (:`Update`
              (`SceneComponent.K2_SetRelativeRotation` (`self.Picture`) (`KismetMathLibrary.RLerp` (struct :`Pitch` -20.0) (struct) _alpha) false false))
            (:`Finished`
              (switch `/Game/Objects/Enum/RotateStateEnum` (`self.Rotate`)
                (:`NewEnumerator0`
                  (set `self.Rotate` "NewEnumerator1")
                  (set `self.State` "NewEnumerator1")
                  (`/Game/Objects/Tutorial/TutorialComponent.Check Use Type` _tutorialcomponent "NewEnumerator4")
                  (`/Game/Objects/GameJolt/GameJoltComponent.Check Use Type` _gamejoltcomponent "NewEnumerator4"))
                (:`NewEnumerator1`
                  (set `self.Rotate` "NewEnumerator0")
                  (set `self.State` "NewEnumerator0")
                  (`/Game/Objects/Tutorial/TutorialComponent.Check Use Type` _tutorialcomponent "NewEnumerator3")
                  (`/Game/Objects/GameJolt/GameJoltComponent.Check Use Type` _gamejoltcomponent "NewEnumerator3")))
              (`self.Tumbler` (`self.State`)))))
        (:`NewEnumerator1`
          (goto _label))))
    (:`then_1`
      (`GameplayStatics.PlaySoundAtLocation` "/Game/Sounds/Objects/TurnOnOff/on_off_switch_Cue.on_off_switch_Cue" (`self.K2_GetActorLocation`) (struct) 1.0 1.0 0.0 null null null null))))

(event `/Game/Function/BP_Interface.Interact`
  (params (Component :type "PrimitiveComponent Object Reference") (Location :type "Vector Structure"))
  ;[1 1 1] Rotation
  (`parent.Interact` Component Location)
  (`self.Interact (Server)`))

(event `self.Enable`
  ;[1 1 1] Tumbler
  (`parent.Enable`)
  (switch `/Game/Objects/Enum/TumblerStateEnum` (`self.State`) :!label _label_2
    (:`NewEnumerator0`
      (for _array_element (`self.Electricity`)
        (`/Engine/EditorBlueprintResources/StandardMacros.IsValid` _array_element
          (:`Is Valid`
            (`self.Enable` _array_element)))))))

(event `Tumbler`
  (params (State :type "/Game/Objects/Enum/TumblerStateEnum Enum" :default "NewEnumerator0"))
  (bind _generator (`self.Generator`))
  ;[1 1 1] Tumbler
  (if (or (`self.Has Electricity`) _generator)
    (switch `/Game/Objects/Enum/TumblerStateEnum` State
      (:`NewEnumerator0`
        (goto _label_2))
      (:`NewEnumerator1`
        (for _array_element (`self.Electricity`) :!label _label_3
          (`/Engine/EditorBlueprintResources/StandardMacros.IsValid` _array_element
            (:`Is Valid`
              (`self.Disable` _array_element))))))
    (elif (not _generator)
      (goto _label_3))))

(event `self.Disable`
  ;[1 1 1] Tumbler
  (`parent.Disable`)
  (goto _label_3))

(fn `Load Data`
  (params (JSON :type String))
  (returns (Object :type "VaRestJsonObject Object Reference"))
  (bind _object (`parent.Load Data` JSON))
  (`|ExecutionSequence`
    (:`then_0`
      (bind (_has_field_ _return_value) (`/Game/Function/BP_JSON_FunctionLibrary.Get Value As Int` _object "State"))
      (if (and _has_field_ (!= _return_value (`KismetMathLibrary.Conv_ByteToInt` (`self.Rotate`))))
        (`self.Interact` (`self.Picture`))))
    (:`then_1`
      (return _object))))

(fn `Save Data`
  (returns (JSON :type "VaRestJsonObject Object Reference"))
  (bind _json (`parent.Save Data`))
  (`VaRestJsonObject.SetIntegerField` _json "State" (`KismetMathLibrary.Conv_ByteToInt` (`self.Rotate`)))
  (return _json))

(fn `UserConstructionScript`
  (bind _material_instance (`self.Material Instance`))
  (bind _picture (`self.Picture`))
  (`parent.UserConstructionScript`)
  (`PrimitiveComponent.SetMaterial` (`self.Picture`) 0 (select `bool` (`KismetSystemLibrary.IsValid` _material_instance) :`false` (`self.Material`) :`true` _material_instance :!type "MaterialInterface Object Reference"))
  (switch `/Game/Objects/Enum/PictureTypeEnum` (`self.Type`)
    (:`NewEnumerator0`
      (`StaticMeshComponent.SetStaticMesh` _picture (`self.Dark Mesh`)))
    (:`NewEnumerator1`
      (`StaticMeshComponent.SetStaticMesh` _picture (`self.White Mesh`)))))
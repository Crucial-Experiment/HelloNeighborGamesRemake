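; BP_1_Magnet is a grabbable magnet that players place into slots on a school board.
; Using it while held line-traces to the board; a matching trigger makes the server snap the magnet to that slot, disable physics and the trigger, and run CheckBoard.
; Picking it up or grabbing it in VR clears its slot and re-enables the trigger.
; Placement also notifies the tutorial and GameJolt components.
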(event `/Game/Function/BP_Interface.PickUp`
  (bind _school_board (`self.School Board`))
  (bind _school_board_2 (`self.School Board`))
  (bind _school_board_3 (`self.School Board`))
  (bind _8_magnet (`/Game/Objects/BP_Objects/BP_School_Board.8 Magnet` (`self.School Board`)))
  (bind _5_magnet (`/Game/Objects/BP_Objects/BP_School_Board.5 Magnet` _school_board))
  (bind _3_magnet (`/Game/Objects/BP_Objects/BP_School_Board.3 Magnet` (`self.School Board`)))
  (`parent.PickUp`)
  (`/Engine/EditorBlueprintResources/StandardMacros.IsValid` _school_board :!label _label
    (:`Is Valid`
      (`|ExecutionSequence`
        (:`then_0`
          (`/Engine/EditorBlueprintResources/StandardMacros.IsValid` _5_magnet
            (:`Is Valid`
              (if (== _5_magnet self)
                (set `/Game/Objects/BP_Objects/BP_School_Board.5 Magnet` null _school_board)
                (`PrimitiveComponent.SetCollisionEnabled` (`/Game/Objects/BP_Objects/BP_School_Board.5 Magnet Trigger` _school_board) "QueryAndPhysics")
                (set `self.School Board` null)))))
        (:`then_1`
          (`/Engine/EditorBlueprintResources/StandardMacros.IsValid` _3_magnet
            (:`Is Valid`
              (if (== _3_magnet self)
                (set `/Game/Objects/BP_Objects/BP_School_Board.3 Magnet` null _school_board_2)
                (`PrimitiveComponent.SetCollisionEnabled` (`/Game/Objects/BP_Objects/BP_School_Board.3 Magnet Trigger` _school_board_2) "QueryAndPhysics")
                (set `self.School Board` null)))))
        (:`then_2`
          (`/Engine/EditorBlueprintResources/StandardMacros.IsValid` _8_magnet
            (:`Is Valid`
              (if (== _8_magnet self)
                (set `/Game/Objects/BP_Objects/BP_School_Board.8 Magnet` null _school_board_3)
                (`PrimitiveComponent.SetCollisionEnabled` (`/Game/Objects/BP_Objects/BP_School_Board.8 Magnet Trigger` _school_board_3) "QueryAndPhysics")
                (set `self.School Board` null)))))))))

(event `self.GrabComponent.OnGrabbed`
  (params (`Self Ref` :type "/Game/Objects/Structurs/GrabComponent Object Reference"))
  (goto _label))

(event `Drop (Owner)`
  (`self.Try Release`))

(event `Interact (Server)`
  (params (Actor :type "Actor Object Reference") (Component :type "PrimitiveComponent Object Reference"))
  (bind _root (`self.Root`))
  (bind _asbp_school_board (cast `/Game/Objects/BP_Objects/BP_School_Board` Actor))
  (`|ExecutionSequence`
    (:`then_0`
      (bind _8_magnet_trigger (`/Game/Objects/BP_Objects/BP_School_Board.8 Magnet Trigger` _asbp_school_board))
      (if (== _8_magnet_trigger Component)
        (set `/Game/Objects/BP_Objects/BP_School_Board.8 Magnet` self _asbp_school_board)
        (set `self.School Board` _asbp_school_board)
        (`self.Try Release`)
        (`PrimitiveComponent.SetSimulatePhysics` _root false)
        (`self.K2_SetActorTransform` (`SceneComponent.K2_GetComponentToWorld` (`/Game/Objects/BP_Objects/BP_School_Board.8 Magnet Position` _asbp_school_board)))
        (`PrimitiveComponent.SetCollisionEnabled` _8_magnet_trigger "NoCollision")
        (`/Game/Objects/BP_Objects/BP_School_Board.Check Board` (`self.School Board`))
        (`/Game/Objects/Tutorial/TutorialComponent.Check Use Type` (`self.TutorialComponent`) "NewEnumerator6" :!label _label_2)
        (`/Game/Objects/GameJolt/GameJoltComponent.Check Use Type` (`self.GameJoltComponent`) "NewEnumerator6")))
    (:`then_1`
      (bind _5_magnet_trigger (`/Game/Objects/BP_Objects/BP_School_Board.5 Magnet Trigger` _asbp_school_board))
      (if (== Component _5_magnet_trigger)
        (set `/Game/Objects/BP_Objects/BP_School_Board.5 Magnet` self _asbp_school_board)
        (set `self.School Board` _asbp_school_board)
        (`self.Try Release`)
        (`PrimitiveComponent.SetSimulatePhysics` _root false)
        (`self.K2_SetActorTransform` (`SceneComponent.K2_GetComponentToWorld` (`/Game/Objects/BP_Objects/BP_School_Board.5 Magnet Position` _asbp_school_board)))
        (`PrimitiveComponent.SetCollisionEnabled` _5_magnet_trigger "NoCollision")
        (`/Game/Objects/BP_Objects/BP_School_Board.Check Board` (`self.School Board`))
        (goto _label_2)))
    (:`then_2`
      (bind _3_magnet_trigger (`/Game/Objects/BP_Objects/BP_School_Board.3 Magnet Trigger` _asbp_school_board))
      (if (== _3_magnet_trigger Component)
        (set `/Game/Objects/BP_Objects/BP_School_Board.3 Magnet` self _asbp_school_board)
        (set `self.School Board` _asbp_school_board)
        (`self.Try Release`)
        (`PrimitiveComponent.SetSimulatePhysics` (`self.Root`) false)
        (`self.K2_SetActorTransform` (`SceneComponent.K2_GetComponentToWorld` (`/Game/Objects/BP_Objects/BP_School_Board.3 Magnet Position` _asbp_school_board)))
        (`PrimitiveComponent.SetCollisionEnabled` _3_magnet_trigger "NoCollision")
        (`/Game/Objects/BP_Objects/BP_School_Board.Check Board` (`self.School Board`))
        (goto _label_2)))))

(event `On Press LMB_1`
  (bind _player (`/Game/Function/BP_MacroLibrary.Find Player`)
    (:`Is Valid`
      (bind _item (`/Game/Player/BP_Player.Get Item` _player))
      (if (== _item self)
        (bind (_actor _component) (`self.Line Trace` 250.0 "NewEnumerator1" :!label _label_3))
        (`self.Interact (Server)` _actor _component)))))

(event `self.On VR Use`
  (`parent.On VR Use`)
  (goto _label_3))

(fn `UserConstructionScript`)
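; BP_Puddle_Glue is a temporary glue puddle that waits, rescales and then removes itself.
; Tick drives a state machine: Dry counts down Delay, Scaled changes the root's X and Y scale by SpeedScale, and Destroy follows once either drops below zero.
; Box overlap events are empty; disconnected logic would slow BP_Player through a custom movement mode and restore walking afterwards.
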(event `self.ReceiveTick`
  (params (DeltaSeconds :type "Float (single-precision)"))
  (bind _root (`self.Root`))
  (bind _returnvalue (* DeltaSeconds (`self.Speed Scale`)))
  (bind (_relativescale3d_x _relativescale3d_y) (`KismetMathLibrary.BreakVector` (`SceneComponent.RelativeScale3D` (`self.Root`))))
  (bind (_relativescale3d_x_2 _relativescale3d_y_2 _relativescale3d_z) (`KismetMathLibrary.BreakVector` (`SceneComponent.RelativeScale3D` _root)))
  (switch `/Game/Objects/Enum/EnumGlueState` (`self.State`)
    (:`NewEnumerator0`
      (bind _output_get (set `self.Delay` (- (`self.Delay`) DeltaSeconds)))
      (if (< _output_get 0.0)
        (set `self.State` "NewEnumerator1")))
    (:`NewEnumerator1`
      (`SceneComponent.SetRelativeScale3D` _root (`KismetMathLibrary.MakeVector` (+ _relativescale3d_x_2 _returnvalue) (+ _relativescale3d_y_2 _returnvalue) _relativescale3d_z))
      (if (or (< _relativescale3d_x 0.0) (< _relativescale3d_y 0.0))
        (set `self.State` "NewEnumerator2")))
    (:`NewEnumerator2`
      (`self.K2_DestroyActor`))))

(event `self.Box.OnComponentBeginOverlap`
  (params (OverlappedComponent :type "PrimitiveComponent Object Reference") (OtherActor :type "Actor Object Reference") (OtherComp :type "PrimitiveComponent Object Reference") (OtherBodyIndex :type Integer) (bFromSweep :type Boolean) (SweepResult :type "HitResult Structure (by ref)")))

(event `self.Box.OnComponentEndOverlap`
  (params (OverlappedComponent :type "PrimitiveComponent Object Reference") (OtherActor :type "Actor Object Reference") (OtherComp :type "PrimitiveComponent Object Reference") (OtherBodyIndex :type Integer)))

(fn `UserConstructionScript`)
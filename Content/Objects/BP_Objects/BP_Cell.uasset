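; Crow cage that acts as an alarm, spotting pawns along a forward line trace and drawing the Neighbor to investigate.
; Each Tick traces while ignoring the Neighbor, with paired DoOnce nodes resetting each other so spotted and lost transitions fire once.
; Spotting starts croaking and sends the hit location to the Neighbor's blackboard; losing sight restores idle, and both notify Tutorial and GameJolt components.
; Construction snaps the linked Crow into the cage.
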(event `self.ReceiveTick`
  (params (DeltaSeconds :type "Float (single-precision)"))
  (bind _gamejoltcomponent (`self.GameJoltComponent`))
  (bind _tutorialcomponent (`self.TutorialComponent`))
  (bind _line (`self.Line`))
  (bind _crow_loud (`self.Crow Loud`))
  (bind _crow (`self.Crow`))
  (bind _returnvalue (`SceneComponent.K2_GetComponentLocation` _line))
  (bind (_outhit _returnvalue_2) (`KismetSystemLibrary.LineTraceSingleForObjects` _returnvalue (+ _returnvalue (* (`SceneComponent.GetForwardVector` _line) 500.0)) (`|MakeArray` "ObjectTypeQuery3" :!type "EObjectTypeQuery Enum") false (`|MakeArray` (stale `self.ReceiveBeginPlay` _sosed) :!type "Actor Object Reference")))
  (set `/Game/Objects/BP_Objects/BP_Crow.Player Spotted` _returnvalue_2 (`self.Crow`))
  (if _returnvalue_2
    (`|ExecutionSequence`
      (:`then_0`
        (`/Engine/EditorBlueprintResources/StandardMacros.DoOnce` false :!label _label
          (:`Completed`
            (`AudioComponent.Play` _crow_loud 0.0)
            (`SkeletalMeshComponent.PlayAnimation` (`/Game/Objects/BP_Objects/BP_Crow.Crow` _crow) (`/Game/Objects/BP_Objects/BP_Crow.Croaks` _crow) true)
            (`/Game/Objects/Tutorial/TutorialComponent.Check Use Type` _tutorialcomponent "NewEnumerator3")
            (`/Game/Objects/GameJolt/GameJoltComponent.Check Use Type` _gamejoltcomponent "NewEnumerator3")
            ;[1 1 1] Neighbor coming to check
            (bind _neighbor (`self.Neighbor`)
              (:`then`
                (if (`|EnumInequality` (`/Game/Sosed/BP_Sosed.Current State` _neighbor) "NewEnumerator2")
                  (bind _returnvalue_3 (`AIBlueprintHelperLibrary.GetBlackboard` _neighbor))
                  (`BlackboardComponent.SetValueAsInt` _returnvalue_3 "CheckTask" 3)
                  (`BlackboardComponent.SetValueAsVector` _returnvalue_3 "Check Location" (`.Location` (`GameplayStatics.BreakHitResult` _outhit)))
                  (`/Game/Sosed/BP_Sosed.Set State` _neighbor "NewEnumerator3")))
              (:`else`)))))
      (:`then_1`
        (goto _label_2 :!via `Reset`)))
    (else
      (`|ExecutionSequence`
        (:`then_0`
          (`/Engine/EditorBlueprintResources/StandardMacros.DoOnce` false :!label _label_2
            (:`Completed`
              (`AudioComponent.Stop` _crow_loud)
              (`/Game/Objects/BP_Objects/BP_Crow.Play Idle Anim` (`self.Crow`))
              (`/Game/Objects/Tutorial/TutorialComponent.Check Use Type` _tutorialcomponent "NewEnumerator4")
              (`/Game/Objects/GameJolt/GameJoltComponent.Check Use Type` _gamejoltcomponent "NewEnumerator4"))))
        (:`then_1`
          (goto _label :!via `Reset`))))))

(event `self.ReceiveBeginPlay`
  (`parent.ReceiveBeginPlay`)
  (bind _sosed (`/Game/Function/BP_MacroLibrary.Find Sosed`)
    (:`Is Valid`
      (set `self.Neighbor` _sosed))))

(fn `UserConstructionScript`
  (bind (_returnvalue_location _returnvalue_rotation) (`KismetMathLibrary.BreakTransform` (`SceneComponent.K2_GetComponentToWorld` (`self.Scene`))))
  (`parent.UserConstructionScript`)
  (bind _crow (`self.Crow`)
    (:`then`
      (`self.K2_SetActorLocationAndRotation` _crow _returnvalue_location _returnvalue_rotation false false)
      (set `/Game/Objects/BP_Objects/BP_Crow.Cell` self _crow))
    (:`else`)))
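; BP_Windmill is a windmill object that runs when it is a generator or has electricity.
; While powered, Tick spins the Wheel in pitch and the Shaft in yaw at a shared Speed.
; Smoke and a rusty windmill sound activate or deactivate at BeginPlay and on the inherited Enable and Disable events.
; The construction script hides the platform, bridge and support when OldVersion is set.
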(event `self.ReceiveTick`
  (params (DeltaSeconds :type "Float (single-precision)"))
  (bind _speed (`self.Speed`))
  (if (or (`self.Generator`) (`self.Has Electricity`))
    (`SceneComponent.K2_AddWorldRotation` (`self.Wheel`) (`KismetMathLibrary.MakeRotator` 0.0 _speed) false false)
    (`SceneComponent.K2_AddWorldRotation` (`self.Shaft`) (`KismetMathLibrary.MakeRotator` 0.0 0.0 _speed) false false)))

(event `self.ReceiveBeginPlay`
  (bind _smoke (`self.Smoke`))
  (`parent.ReceiveBeginPlay`)
  (if (or (`self.Generator`) (`self.Has Electricity`))
    (`ActorComponent.Activate` _smoke false :!label _label)
    (`ActorComponent.Activate` (`self.Windmill_Rusty_Cue`) false)
    (else
      (`ActorComponent.Deactivate` _smoke :!label _label_2)
      (`ActorComponent.Deactivate` (`self.Windmill_Rusty_Cue`)))))

(event `self.Enable`
  (`parent.Enable`)
  (goto _label))

(event `self.Disable`
  (`parent.Disable`)
  (goto _label_2))

(fn `UserConstructionScript`
  (`parent.UserConstructionScript`)
  (`SceneComponent.SetVisibility` (`self.Platform`) (not (`self.Old Version`)) false)
  (`SceneComponent.SetVisibility` (`self.Bridge`) (not (`self.Old Version`)) false)
  (`SceneComponent.SetVisibility` (`self.Support`) (not (`self.Old Version`)) false))
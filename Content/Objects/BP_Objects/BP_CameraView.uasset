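; BP_CameraView is a camera view object that pairs a RenderCamera scene capture with a Display component.
; The construction script assigns the capture's render target, applies DisplayMaterial to the display, and copies the capture-every-frame and capture-on-movement settings.
; BeginPlay forces per-frame capture on, overriding that setting, then sets it on again after a half-second delay.
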(event `self.ReceiveBeginPlay`
  (bind _render_camera (`self.Render Camera`))
  (set `SceneCaptureComponent.bCaptureEveryFrame` true _render_camera)
  (`KismetSystemLibrary.Delay` 0.5)
  (set `SceneCaptureComponent.bCaptureEveryFrame` true _render_camera))

(fn `UserConstructionScript`
  (bind _render_camera (`self.Render Camera`))
  (set `SceneCaptureComponent2D.TextureTarget` (`self.Texture Target`) (`self.Render Camera`))
  (`PrimitiveComponent.SetMaterial` (`self.Display`) 0 (`self.Display Material`))
  (set `SceneCaptureComponent.bCaptureEveryFrame` (`self.Capture Every Frame`) _render_camera)
  (set `SceneCaptureComponent.bCaptureOnMovement` (`self.Capture On Movement`) _render_camera))
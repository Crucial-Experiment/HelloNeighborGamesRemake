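; Security camera that detects the player and sends the Neighbor to investigate.
; While on, it line-traces forward each tick; a new player hit plays a sound, notifies GameJolt and tutorial components, and sets the Neighbor's blackboard check location and state.
; Initial state follows the monitor room when the Neighbor exists.
; A fast impact or CameraBroke event breaks it, swapping material, sparking and making it pickable.
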(event `self.ReceiveTick`
  (params (DeltaSeconds :type "Float (single-precision)"))
  (bind _line (`self.Line`))
  (bind _returnvalue (`SceneComponent.K2_GetComponentLocation` _line))
  ;[1 1 1] Tick
  (switch `/Game/Objects/Enum/TumblerStateEnum` (`self.State`)
    (:`NewEnumerator0`
      (bind (_outhit _returnvalue_2) (`KismetSystemLibrary.LineTraceSingleForObjects` _returnvalue (+ _returnvalue (* (`SceneComponent.GetForwardVector` _line) 500.0)) (`|MakeArray` "ObjectTypeQuery3" :!type "EObjectTypeQuery Enum") false (`|MakeArray` (stale `self.ReceiveBeginPlay` _sosed) :!type "Actor Object Reference") "ForOneFrame"))
      (if _returnvalue_2
        (`/Engine/EditorBlueprintResources/StandardMacros.DoOnce` false :!label _label
          (:`Completed`
            (bind (_bblockinghit _binitialoverlap _time _distance _location _impactpoint _normal _impactnormal _physmat _hitactor) (`GameplayStatics.BreakHitResult` _outhit))
            (cast `/Game/Player/BP_Player` _hitactor)
            (`GameplayStatics.PlaySoundAtLocation` "/Game/Sounds/Objects/Noise/camera_detect_Cue.camera_detect_Cue" (`self.K2_GetActorLocation`) (struct) 1.0 1.0 0.0 null null null null)
            (`/Game/Objects/GameJolt/GameJoltComponent.Check Use Type` (`self.GameJoltComponent`) "NewEnumerator6")
            (`/Game/Objects/Tutorial/TutorialComponent.Check Use Type` (`self.TutorialComponent`) "NewEnumerator6")
            ;;[1 1 1] Neighbor coming to check
            (bind _neighbor (`self.Neighbor`)
              (:`then`
                (if (`|EnumInequality` (`/Game/Sosed/BP_Sosed.Current State` _neighbor) "NewEnumerator2")
                  (bind _returnvalue_3 (`AIBlueprintHelperLibrary.GetBlackboard` _neighbor))
                  (`BlackboardComponent.SetValueAsInt` _returnvalue_3 "CheckTask" 3)
                  (`BlackboardComponent.SetValueAsVector` _returnvalue_3 "Check Location" _location)
                  (`/Game/Sosed/BP_Sosed.Set State` _neighbor "NewEnumerator3")))
              (:`else`))))
        (else
          (goto _label :!via `Reset`))))))

(event `self.ReceiveBeginPlay`
  ;[1 1 1] Tick
  (`parent.ReceiveBeginPlay`)
  (bind _sosed (`/Game/Function/BP_MacroLibrary.Find Sosed`)
    (:`Is Valid`
      (set `self.Neighbor` _sosed)
      (`|ExecutionSequence`
        (:`then_0`
          (bind _returnvalue (`GameplayStatics.GetActorOfClass` "/Game/Objects/BP_Objects/BP_Monitor_Room.BP_Monitor_Room_C"))
          (`/Engine/EditorBlueprintResources/StandardMacros.IsValid` _returnvalue
            (:`Is Valid`
              (set `self.State` (`/Game/Objects/BP_Objects/BP_Monitor_Room.State` _returnvalue)))))
        (:`then_1`
          (if (`self.Broken`)
            (`AudioComponent.Stop` (`self.Loop`))
            (`AudioComponent.Play` (`self.Spark`) 0.0)
            (`self.Set State` "NewEnumerator1")
            (set `self.CanPickUp` true)))))))

(event `self.Root.OnComponentHit`
  (params (HitComponent :type "PrimitiveComponent Object Reference") (OtherActor :type "Actor Object Reference") (OtherComp :type "PrimitiveComponent Object Reference") (NormalImpulse :type "Vector Structure") (Hit :type "HitResult Structure (by ref)"))
  ;[1 1 1] Hit
  (if (>= (`KismetMathLibrary.VSize` (`self.GetVelocity` OtherActor)) 500.0)
    (`AudioComponent.Stop` (`self.Loop`) :!label _label_2)
    (`AudioComponent.Play` (`self.Spark`) 0.0)
    (`ActorComponent.Activate` (`self.P_Sparks`) false)
    (set `self.Broken` true)
    (`self.Set State` "NewEnumerator1")
    (set `self.CanPickUp` true)))

(event `Camera Broke`
  ;[1 1 1] Hit
  (goto _label_2))

(fn `Set State`
  (params (`New State` :type "/Game/Objects/Enum/TumblerStateEnum Enum" :default "NewEnumerator0"))
  (bind _root (`self.Root`))
  (bind _output_get (set `self.State` `New State`))
  (switch `/Game/Objects/Enum/TumblerStateEnum` _output_get
    (:`NewEnumerator0`
      (`PrimitiveComponent.SetMaterial` _root 1 "/Game/Objects/Materials/camera2_m.camera2_m"))
    (:`NewEnumerator1`
      (`PrimitiveComponent.SetMaterial` _root 1 "/Game/Objects/Materials/camera3_m.camera3_m"))))

(fn `UserConstructionScript`
  (`ActorComponent.SetAutoActivate` (`self.P_Sparks`) (`self.Broken`)))
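; BP_Picture_Rectangular is a grabbable rectangular picture object with Dark and White variants.
; The construction script sets the Root mesh from Type and applies MaterialInstance to the first material slot, falling back to Material if it is not valid.
; When the GrabComponent reports a drop, it calls SetFlatMode with a fixed enum value.
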(event `self.GrabComponent.OnDropped`
  (params (`Self Ref` :type "/Game/Objects/Structurs/GrabComponent Object Reference"))
  (`self.Set Flat Mode` "NewEnumerator0"))

(fn `UserConstructionScript`
  (bind _material_instance (`self.Material Instance`))
  (bind _root (`self.Root`))
  (`parent.UserConstructionScript`)
  (`PrimitiveComponent.SetMaterial` (`self.Root`) 0 (select `bool` (`KismetSystemLibrary.IsValid` _material_instance) :`false` (`self.Material`) :`true` _material_instance :!type "MaterialInterface Object Reference"))
  (switch `/Game/Objects/Enum/PictureTypeEnum` (`self.Type`)
    (:`NewEnumerator0`
      (`StaticMeshComponent.SetStaticMesh` _root (`self.Dark Mesh`)))
    (:`NewEnumerator1`
      (`StaticMeshComponent.SetStaticMesh` _root (`self.White Mesh`)))))
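; BP_Teacher_Table is an interactable teacher's table with four sliding parts, likely drawers, arranged two per side at two heights.
; The Interact event receives a component and compares it against each part to decide which one moves.
; Each part has its own FlipFlop and Timeline, which lerps its relative location along local Y, alternately playing to slide it out and reversing to return it.
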(event `/Game/Function/BP_Interface.Interact`
  (params (Component :type "PrimitiveComponent Object Reference") (Location :type "Vector Structure"))
  (`|ExecutionSequence`
    (:`then_0`
      (if (== Component (`self.teacher_table_part1_new`))
        (`/Engine/EditorBlueprintResources/StandardMacros.FlipFlop`
          (:`A`
            (bind (_direction _alpha) (`Timeline|Timeline_0` :!label _label)
              (:`Update`
                (`SceneComponent.K2_SetRelativeLocation` (`self.teacher_table_part1_new`) (`KismetMathLibrary.VLerp` (-57.0 -3.0 55.0) (-57.0 -48.0 55.0) _alpha) false false))))
          (:`B`
            (goto _label :!via `Reverse`)))))
    (:`then_1`
      (if (== Component (`self.teacher_table_part2_new`))
        (`/Engine/EditorBlueprintResources/StandardMacros.FlipFlop`
          (:`A`
            (bind (_direction_2 _alpha_2) (`Timeline|Timeline_1` :!label _label_2)
              (:`Update`
                (`SceneComponent.K2_SetRelativeLocation` (`self.teacher_table_part2_new`) (`KismetMathLibrary.VLerp` (-57.0 -3.0 29.0) (-57.0 -48.0 29.0) _alpha_2) false false))))
          (:`B`
            (goto _label_2 :!via `Reverse`)))))
    (:`then_2`
      (if (== Component (`self.teacher_table_part1_new1`))
        (`/Engine/EditorBlueprintResources/StandardMacros.FlipFlop`
          (:`A`
            (bind (_direction_3 _alpha_3) (`Timeline|Timeline_2` :!label _label_3)
              (:`Update`
                (`SceneComponent.K2_SetRelativeLocation` (`self.teacher_table_part1_new1`) (`KismetMathLibrary.VLerp` (61.0 -3.0 55.0) (61.0 -48.0 55.0) _alpha_3) false false))))
          (:`B`
            (goto _label_3 :!via `Reverse`)))))
    (:`then_3`
      (if (== Component (`self.teacher_table_part2_new1`))
        (`/Engine/EditorBlueprintResources/StandardMacros.FlipFlop`
          (:`A`
            (bind (_direction_4 _alpha_4) (`Timeline|Timeline_3` :!label _label_4)
              (:`Update`
                (`SceneComponent.K2_SetRelativeLocation` (`self.teacher_table_part2_new1`) (`KismetMathLibrary.VLerp` (61.0 -3.0 29.0) (61.0 -48.0 29.0) _alpha_4) false false))))
          (:`B`
            (goto _label_4 :!via `Reverse`)))))))

(fn `UserConstructionScript`)
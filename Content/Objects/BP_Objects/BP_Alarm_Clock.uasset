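; Alarm clock item that, when its countdown ends, rings and lures the Neighbor to its location.
; VR use, Interact or left-click while held toggles the countdown; stopping it or changing slot also silences the alarm.
; A looping one-second timer drives the countdown, then writes a check task and location to the Neighbor's Blackboard and switches its state, unless a particular state blocks it.
; Use actions also report to tutorial and GameJolt components.
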(event `Count Down`
  (if (`self.Countdown`)
    (bind _output_get (set `self.Temp Clock` (- (`self.Temp Clock`) 1.0)))
    (if (<= _output_get 0.0)
      (set `self.Countdown` false)
      (`AudioComponent.Play` (`self.Alarm`) 0.0)
      ;[1 1 1] Neighbor coming to check
      (bind _sosed (`/Game/Function/BP_MacroLibrary.Find Sosed`)
        (:`Is Valid`
          (if (`|EnumInequality` (`/Game/Sosed/BP_Sosed.Current State` _sosed) "NewEnumerator2")
            (bind _returnvalue (`AIBlueprintHelperLibrary.GetBlackboard` _sosed))
            (`BlackboardComponent.SetValueAsInt` _returnvalue "CheckTask" 3)
            (`BlackboardComponent.SetValueAsVector` _returnvalue "Check Location" (`SceneComponent.K2_GetComponentLocation` (`self.Arrow`)))
            (`/Game/Sosed/BP_Sosed.Set State` _sosed "NewEnumerator3")))))))

(event `self.On VR Use`
  (bind _tutorialcomponent (`self.TutorialComponent`))
  (`parent.On VR Use`)
  (`/Game/Objects/Tutorial/TutorialComponent.Check Use Type` (`self.TutorialComponent`) "NewEnumerator0" :!label _label)
  (`/Game/Objects/GameJolt/GameJoltComponent.Check Use Type` (`self.GameJoltComponent`) "NewEnumerator6")
  (set `self.Temp Clock` (`self.Second`))
  (if (not (`self.Countdown`))
    (set `self.Countdown` true)
    (`KismetSystemLibrary.K2_SetTimerDelegate` (delegate `Count Down`) 1.0 true)
    (`/Game/Objects/Tutorial/TutorialComponent.Check Use Type` _tutorialcomponent "NewEnumerator3")
    (else
      (set `self.Countdown` false :!label _label_2)
      (`AudioComponent.Stop` (`self.Alarm`))
      (`/Game/Objects/Tutorial/TutorialComponent.Check Use Type` _tutorialcomponent "NewEnumerator4"))))

(event `/Game/Function/BP_Interface.Interact`
  (params (Component :type "PrimitiveComponent Object Reference") (Location :type "Vector Structure"))
  (goto _label))

(event `self.ReceiveBeginPlay`
  (`parent.ReceiveBeginPlay`))

(event `self.On Press LMB`
  (bind _player (`/Game/Function/BP_MacroLibrary.Find Player`)
    (:`Is Valid`
      (bind _item (`/Game/Player/BP_Player.Get Item` _player))
      (if (== _item self)
        (goto _label)))))

(event `self.On Slot Change`
  (goto _label_2))

(fn `UserConstructionScript`
  (`parent.UserConstructionScript`))
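; Four-button elevator panel that sends its linked Lift to the selected floor, usable through Interact or VR hand overlap.
; UpdateFloors, run at BeginPlay, unhides buttons for valid Lift floors and removes their "interactive" tag.
; Presses route through the server to an all-clients event that changes Lift state and target floor, delaying first if the current floor has a door.
; The construction script gives three buttons dynamic materials with differing "V" values.
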(event `self.ReceiveBeginPlay`
  (`self.Update Floors`))

(event `Update Floors`
  (bind _lift (`self.Lift`))
  (`/Engine/EditorBlueprintResources/StandardMacros.IsValid` _lift
    (:`Is Valid`
      (for (_array_element _array_index) (`/Game/Objects/BP_Objects/BP_Lift.Floors` _lift)
        (`/Engine/EditorBlueprintResources/StandardMacros.IsValid` _array_element
          (:`Is Valid`
            (bind _output (`|GetArrayItem` (`|MakeArray` (`self.Button_1`) (`self.Button_2`) (`self.Button_3`) (`self.Button_4`)) _array_index))
            (`SceneComponent.SetHiddenInGame` _output false false)
            (`KismetArrayLibrary.Array_RemoveItem` (`ActorComponent.ComponentTags` _output) "interactive")))))))

(event `/Game/Function/BP_Interface.Interact`
  (params (Component :type "PrimitiveComponent Object Reference") (Location :type "Vector Structure"))
  (`self.Interact (Server)` (select `bool` (stale `VR Use` Index) :`false` Component :`true` (stale `VR Use` Component)) :!label _label))

(event `VR Use`
  (params (Component :type "PrimitiveComponent Object Reference") (Index :type Boolean))
  (goto _label))

(event `Interact (All)`
  (params (Component :type "PrimitiveComponent Object Reference"))
  (bind _lift (`self.Lift`))
  (for (_array_element _array_index) (`|MakeArray` (`self.Button_1`) (`self.Button_2`) (`self.Button_3`) (`self.Button_4`))
    (if (and (== Component _array_element) (not (`SceneComponent.bHiddenInGame` _array_element)))
      (`/Engine/EditorBlueprintResources/StandardMacros.IsValid` (`/Game/Objects/BP_Objects/BP_LiftFloor.Lift Door` (`|GetArrayItem` (`/Game/Objects/BP_Objects/BP_Lift.Floors` _lift) (`/Game/Objects/BP_Objects/BP_Lift.Flour` _lift)))
        (:`Is Valid`
          (`/Game/Objects/BP_Objects/BP_Lift.Set State` (`self.Lift`) "NewEnumerator3")
          (`|ExecutionSequence`
            (:`then_0`
              (`KismetSystemLibrary.Delay` 1.6))
            (:`then_1`
              (break))))
        (:`Is Not Valid`
          (`|ExecutionSequence`
            (:`then_0`
              (`/Game/Objects/BP_Objects/BP_Lift.Set State` (`self.Lift`) "NewEnumerator3"))
            (:`then_1`
              (break)))))
      (set `/Game/Objects/BP_Objects/BP_Lift.Flour` _array_index _lift)
      (`/Game/Objects/BP_Objects/BP_Lift.Set State` _lift "NewEnumerator1"))))

(event `Interact (Server)`
  (params (Component :type "PrimitiveComponent Object Reference"))
  (`self.Interact (All)` Component))

(event `self.Button_1.OnComponentBeginOverlap`
  (params (OverlappedComponent :type "PrimitiveComponent Object Reference") (OtherActor :type "Actor Object Reference") (OtherComp :type "PrimitiveComponent Object Reference") (OtherBodyIndex :type Integer) (bFromSweep :type Boolean) (SweepResult :type "HitResult Structure (by ref)"))
  (if (`self.Overlap VR Hands` OtherActor OtherComp)
    (`self.VR Use` (`self.Button_1`) true)))

(event `self.Button_2.OnComponentBeginOverlap`
  (params (OverlappedComponent :type "PrimitiveComponent Object Reference") (OtherActor :type "Actor Object Reference") (OtherComp :type "PrimitiveComponent Object Reference") (OtherBodyIndex :type Integer) (bFromSweep :type Boolean) (SweepResult :type "HitResult Structure (by ref)"))
  (if (`self.Overlap VR Hands` OtherActor OtherComp)
    (`self.VR Use` (`self.Button_2`) true)))

(event `self.Button_3.OnComponentBeginOverlap`
  (params (OverlappedComponent :type "PrimitiveComponent Object Reference") (OtherActor :type "Actor Object Reference") (OtherComp :type "PrimitiveComponent Object Reference") (OtherBodyIndex :type Integer) (bFromSweep :type Boolean) (SweepResult :type "HitResult Structure (by ref)"))
  (if (`self.Overlap VR Hands` OtherActor OtherComp)
    (`self.VR Use` (`self.Button_3`) true)))

(event `self.Button_4.OnComponentBeginOverlap`
  (params (OverlappedComponent :type "PrimitiveComponent Object Reference") (OtherActor :type "Actor Object Reference") (OtherComp :type "PrimitiveComponent Object Reference") (OtherBodyIndex :type Integer) (bFromSweep :type Boolean) (SweepResult :type "HitResult Structure (by ref)"))
  (if (`self.Overlap VR Hands` OtherActor OtherComp)
    (`self.VR Use` (`self.Button_4`) true)))

(fn `UserConstructionScript`
  (bind _button_1 (`self.Button_1`))
  (bind _button_3 (`self.Button_3`))
  (bind _button_2 (`self.Button_2`))
  (`|ExecutionSequence`
    (:`then_0`
      (bind _returnvalue (`PrimitiveComponent.CreateDynamicMaterialInstance` _button_2 0 "/Game/Objects/Materials/elevator_panel_Inst.elevator_panel_Inst" "None"))
      (`PrimitiveComponent.SetMaterial` _button_2 0 _returnvalue)
      (`MaterialInstanceDynamic.SetScalarParameterValue` _returnvalue "V" 0.62))
    (:`then_1`
      (bind _returnvalue_2 (`PrimitiveComponent.CreateDynamicMaterialInstance` _button_3 0 "/Game/Objects/Materials/elevator_panel_Inst.elevator_panel_Inst" "None"))
      (`PrimitiveComponent.SetMaterial` _button_3 0 _returnvalue_2)
      (`MaterialInstanceDynamic.SetScalarParameterValue` _returnvalue_2 "V" 0.805))
    (:`then_2`
      (bind _returnvalue_3 (`PrimitiveComponent.CreateDynamicMaterialInstance` _button_1 0 "/Game/Objects/Materials/elevator_panel_Inst.elevator_panel_Inst" "None"))
      (`PrimitiveComponent.SetMaterial` _button_1 0 _returnvalue_3)
      (`MaterialInstanceDynamic.SetScalarParameterValue` _returnvalue_3 "V" 0.44))))
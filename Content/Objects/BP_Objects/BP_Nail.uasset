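; BP_Nail is a nail object that can start fixed to a Border and later be ejected as a grabbable pickup.
; At BeginPlay it registers with the Border and disables pickup; Unlock switches flat mode and grab type, deregisters, notifies the Border and plays a sound.
; The construction script picks one of two meshes from Model.
; Save data stores the locked state, and loading an unlocked state replays Unlock.
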(event `Unlock`
  (bind _border (`self.Border`))
  (`/Engine/EditorBlueprintResources/StandardMacros.IsValid` _border
    (:`Is Valid`
      (`self.Set Flat Mode` "NewEnumerator0")
      (set `self.CanPickUp` true)
      (set `/Game/Objects/Structurs/GrabComponent.GrabType` "NewEnumerator4" (`self.GrabComponent`))
      (`KismetArrayLibrary.Array_RemoveItem` (`/Game/Objects/BP_Objects/BP_Door_Block.Nails` _border) self)
      (`/Game/Objects/BP_Objects/BP_Door_Block.Nail Status` (`self.Border`))
      (set `self.Border` null)
      (`GameplayStatics.PlaySoundAtLocation` "/Game/Sounds/Objects/Noise/nail_eject_Cue.nail_eject_Cue" (`self.K2_GetActorLocation`) (struct) 1.0 1.0 0.0 null null null null))))

(event `self.ReceiveBeginPlay`
  (bind _border (`self.Border`))
  (`parent.ReceiveBeginPlay`)
  (`/Engine/EditorBlueprintResources/StandardMacros.IsValid` _border
    (:`Is Valid`
      (`self.Set Flat Mode` "NewEnumerator1")
      (set `self.CanPickUp` false)
      (set `/Game/Objects/Structurs/GrabComponent.GrabType` "NewEnumerator0" (`self.GrabComponent`))
      (`KismetArrayLibrary.Array_Add` (`/Game/Objects/BP_Objects/BP_Door_Block.Nails` _border) self)
      (`/Game/Objects/BP_Objects/BP_Door_Block.Nail Status` (`self.Border`)))))

(fn `Load Data`
  (params (JSON :type String))
  (returns (Object :type "VaRestJsonObject Object Reference"))
  (bind _object (`parent.Load Data` JSON))
  (`|ExecutionSequence`
    (:`then_0`
      (bind (_has_field_ _return_value) (`/Game/Function/BP_JSON_FunctionLibrary.Get Value As Bool` _object "State"))
      (if (and _has_field_ (not _return_value))
        (`self.Unlock`)))
    (:`then_1`
      (return _object))))

(fn `Save Data`
  (returns (JSON :type "VaRestJsonObject Object Reference"))
  (bind _json (`parent.Save Data`))
  (`VaRestJsonObject.SetBoolField` _json "State" (and (`|EnumEquality` (`/Game/Objects/Structurs/FlatComponent.Mode` (`self.FlatComponent`)) "NewEnumerator1") (not (`self.CanPickUp`))))
  (return _json))

(fn `UserConstructionScript`
  (bind _root (`self.Root`))
  (`parent.UserConstructionScript`)
  (switch `int` (`self.Model`)
    (:`Default`
      (`StaticMeshComponent.SetStaticMesh` _root "/Game/Objects/Meshes/nail_1_new.nail_1_new" :!label _label))
    (:`0`
      (goto _label))
    (:`1`
      (`StaticMeshComponent.SetStaticMesh` _root "/Game/Objects/Meshes/nail_2_new.nail_2_new"))))
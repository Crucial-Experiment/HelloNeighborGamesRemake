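; BP_Seed is a usable seed item that plants itself in apple ground and is consumed.
; VR use, or left click while it is the player's held item, line-traces for a BP_AppleGround, releases the seed and calls the server interact.
; The server multicasts to notify GameJolt and tutorial components, plant and, as a marked temporary step, immediately water the ground, then destroys the seed.
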(event `self.On VR Use`
  (`parent.On VR Use`)
  (bind _actor (`self.Line Trace` 1500.0 :!label _label))
  (bind _asbp_apple_ground (cast `/Game/Objects/BP_Objects/BP_AppleGround` _actor))
  (`self.Try Release`)
  (`self.Interact (Server)` _asbp_apple_ground))

(event `self.ReceiveBeginPlay`
  (`parent.ReceiveBeginPlay`))

(event `On Press LMB_1`
  (bind _player (`/Game/Function/BP_MacroLibrary.Find Player`)
    (:`Is Valid`
      (bind _item (`/Game/Player/BP_Player.Get Item` _player))
      (if (== _item self)
        (goto _label)))))

(event `Interact (Server)`
  (params (Ground :type "/Game/Objects/BP_Objects/BP_AppleGround Object Reference"))
  (`self.Interact (All)` Ground)
  (`self.K2_DestroyActor` self))

(event `Interact (All)`
  (params (Ground :type "/Game/Objects/BP_Objects/BP_AppleGround Object Reference"))
  (`/Game/Objects/GameJolt/GameJoltComponent.Check Use Type` (`self.GameJoltComponent`) "NewEnumerator6")
  (`/Game/Objects/Tutorial/TutorialComponent.Check Use Type` (`self.TutorialComponent`) "NewEnumerator6")
  (`/Game/Objects/BP_Objects/BP_AppleGround.Plant Seed` Ground)
  (`/Game/Objects/BP_Objects/BP_AppleGround.Watering` Ground) ; Временно!!!
)

(fn `UserConstructionScript`
  (`parent.UserConstructionScript`))
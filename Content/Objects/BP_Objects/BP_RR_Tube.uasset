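; BP_RR_Tube is a transport tube actor that sucks in actors entering its Box and ejects them at an exit point.
; Overlapping actors, filtered against an Ignored class list, join a queue, and each addition triggers processing of the first entry.
; A timeline lerps that actor toward InScene while shrinking it, then the tube animation plays.
; After a delay the actor jumps to OutScene, scales to its size, and Next repeats.
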(event `self.ReceiveBeginPlay`
  ;[1 1 1] Box
  (`parent.ReceiveBeginPlay`))

(event `Next`
  (bind _tube (`self.Tube`))
  ;[1 1 1] Box
  (if (!= (`KismetArrayLibrary.Array_Length` (`self.Queue`)) 0) :!label _label
    (bind _output_get (set `self.RR Actor` (`|GetArrayItem` (`self.Queue`))))
    (bind (_direction _alpha) (`Timeline|Move Timeline` :!via `PlayFromStart`)
      (:`Update`
        (`self.K2_SetActorRelativeLocation` _output_get (`KismetMathLibrary.VLerp` (`self.K2_GetActorLocation` _output_get) (`SceneComponent.K2_GetComponentLocation` (`self.In Scene`)) _alpha) false false)
        (`self.SetActorRelativeScale3D` _output_get (`KismetMathLibrary.VLerp` (`self.GetActorScale3D` _output_get) (0.25 0.25 0.25) _alpha)))
      (:`Finished`
        (`SkeletalMeshComponent.PlayAnimation` _tube "/Game/Objects/Meshes/Animations/RifleRange/RR_tube_in_out_new.RR_tube_in_out_new" false)
        (`KismetSystemLibrary.Delay` (`SkeletalMeshComponent.GetPlayRate` _tube))
        (`self.K2_SetActorRelativeLocation` _output_get (`SceneComponent.K2_GetComponentLocation` (`self.Out Scene`)) false false)
        (bind (_direction_2 _alpha_2) (`Timeline|Scale Timeline` :!via `PlayFromStart`)
          (:`Update`
            (`self.SetActorRelativeScale3D` _output_get (`KismetMathLibrary.VLerp` (`self.GetActorScale3D` _output_get) (`SceneComponent.K2_GetComponentScale` (`self.Out Scene`)) _alpha_2)))
          (:`Finished`
            (`KismetArrayLibrary.Array_RemoveItem` (`self.Queue`) _output_get)
            (set `self.RR Actor` null)
            (`self.Next`)))))))

(event `self.Box.OnComponentBeginOverlap`
  (params (OverlappedComponent :type "PrimitiveComponent Object Reference") (OtherActor :type "Actor Object Reference") (OtherComp :type "PrimitiveComponent Object Reference") (OtherBodyIndex :type Integer) (bFromSweep :type Boolean) (SweepResult :type "HitResult Structure (by ref)"))
  ;[1 1 1] Box
  (bind _status (`/Game/Function/BP_FunctionLibrary.Checking Class` (`GameplayStatics.GetObjectClass` OtherActor) (`self.Ignored`)))
  (if _status
    _
    (elif (== (`KismetArrayLibrary.Array_Find` (`self.Queue`)) -1)
      (`KismetArrayLibrary.Array_Add` (`self.Queue`) OtherActor)
      (goto _label))))

(event `self.Box.OnComponentEndOverlap`
  (params (OverlappedComponent :type "PrimitiveComponent Object Reference") (OtherActor :type "Actor Object Reference") (OtherComp :type "PrimitiveComponent Object Reference") (OtherBodyIndex :type Integer))
  ;[1 1 1] Box
  (if (!= (`self.RR Actor`) OtherActor)
    (`KismetArrayLibrary.Array_RemoveItem` (`self.Queue`) OtherActor)))

(fn `UserConstructionScript`)
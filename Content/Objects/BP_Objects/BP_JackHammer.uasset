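; BP_JackHammer is a usable item that destroys bricks the player aims at.
; A left-click while it is the held item, or a VR use action, fires a short line trace and passes any BP_Brick hit to a server crush event.
; That event sets the brick's flat mode, reports the use type to the tutorial and GameJolt components, then destroys the brick.
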(event `self.ReceiveBeginPlay`
  (`parent.ReceiveBeginPlay`))

(event `On Press LMB_1`
  (bind _player (`/Game/Function/BP_MacroLibrary.Find Player`)
    (:`Is Valid`
      (bind _item (`/Game/Player/BP_Player.Get Item` _player))
      (if (== _item self)
        (bind _actor (`self.Line Trace` 300.0 "NewEnumerator1" :!label _label))
        (bind _asbp_brick (cast `/Game/Objects/BP_Objects/BP_Brick` _actor))
        (`self.Crush (Server)` _asbp_brick)))))

(event `self.On VR Use`
  (`parent.On VR Use`)
  (goto _label))

(event `Crush (Server)`
  (params (Brick :type "/Game/Objects/BP_Objects/BP_Brick Object Reference"))
  (`self.Set Flat Mode` Brick "NewEnumerator0")
  (`/Game/Objects/Tutorial/TutorialComponent.Check Use Type` (`self.TutorialComponent`) "NewEnumerator6")
  (`/Game/Objects/GameJolt/GameJoltComponent.Check Use Type` (`self.GameJoltComponent`) "NewEnumerator6")
  (`/Game/Objects/BP_Objects/BP_Brick.Destroy` Brick))

(fn `UserConstructionScript`
  (`parent.UserConstructionScript`))
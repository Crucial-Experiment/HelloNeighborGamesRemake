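; Lamp post object that lights up when it has electricity or its Generator property is set.
; On BeginPlay and on the Enable and Disable electricity events, it calls the parent logic, then toggles the spotlight and swaps the bulb material between lit and plain glass.
; The construction script sets spotlight visibility from Generator alone, leaving the bulb material untouched.
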(event `self.ReceiveBeginPlay`
  (bind _bulb (`self.Bulb`))
  (bind _spotlight (`self.SpotLight`))
  ;[1 1 1] Begin Play
  (`parent.ReceiveBeginPlay`)
  (if (or (`self.Has Electricity`) (`self.Generator`))
    (`SceneComponent.SetVisibility` _spotlight true false)
    (`PrimitiveComponent.SetMaterial` _bulb 0 "/Game/Objects/Materials/dl_bulb_m.dl_bulb_m")
    (else
      (`SceneComponent.SetVisibility` _spotlight false false)
      (`PrimitiveComponent.SetMaterial` _bulb 0 "/Game/Objects/Materials/bulb_glass_m.bulb_glass_m"))))

(event `self.Enable`
  ;[1 1 1] Electricity
  (`parent.Enable`)
  (`SceneComponent.SetVisibility` (`self.SpotLight`) true false)
  (`PrimitiveComponent.SetMaterial` (`self.Bulb`) 0 "/Game/Objects/Materials/dl_bulb_m.dl_bulb_m"))

(event `self.Disable`
  ;[1 1 1] Electricity
  (`parent.Disable`)
  (`SceneComponent.SetVisibility` (`self.SpotLight`) false false)
  (`PrimitiveComponent.SetMaterial` (`self.Bulb`) 0 "/Game/Objects/Materials/bulb_glass_m.bulb_glass_m"))

(fn `UserConstructionScript`
  (bind _spotlight (`self.SpotLight`))
  (`parent.UserConstructionScript`)
  (if (`self.Generator`)
    (`SceneComponent.SetVisibility` _spotlight true false)
    (else
      (`SceneComponent.SetVisibility` _spotlight false false))))
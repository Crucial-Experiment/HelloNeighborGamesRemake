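; BP_Bolt is a bolt object linked to another actor through its Rotate reference.
; Its construction script checks whether that reference is a BP_Ladder and, if so, makes the ladder's Bolt component visible in game.
; The event graph holds only disabled default events, so the Blueprint adds no runtime logic of its own.
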(fn `UserConstructionScript`
  (`parent.UserConstructionScript`)
  (bind _rotate (`self.Rotate`)
    (:`then`
      (if (== (`GameplayStatics.GetObjectClass` _rotate) "/Game/Objects/BP_Objects/BP_Ladder.BP_Ladder_C")
        (bind _asbp_ladder (cast `/Game/Objects/BP_Objects/BP_Ladder` (`self.Rotate`)))
        (`SceneComponent.SetHiddenInGame` (`/Game/Objects/BP_Objects/BP_Ladder.Bolt` _asbp_ladder) false false)))
    (:`else`)))
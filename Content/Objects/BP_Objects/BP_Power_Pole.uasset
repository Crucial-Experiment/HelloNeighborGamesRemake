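; Power pole prop that picks one of three static mesh variants at random in the Construction Script.
; A random index also selects preset attachment offsets, with the third variant differing from the other two.
; These offsets position both cable components and their position markers, and set each cable's EndLocation.
; The event graph holds only disabled placeholder events, so the Blueprint adds no runtime logic.
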(fn `UserConstructionScript`
  (bind _returnvalue (`KismetMathLibrary.MakeVector` 13.556257 -85.833885 642.026272))
  (bind _returnvalue_2 (`KismetMathLibrary.MakeVector` 13.556257 30.71415 655.13725))
  (bind _returnvalue_3 (`KismetMathLibrary.MakeVector` 13.556257 44.468831 651.263213))
  (bind _returnvalue_4 (`KismetMathLibrary.MakeVector` 13.556257 -72.670173 651.263214))
  (bind _cable_1 (`self.Cable 1`))
  (bind (_outitem _outindex) (`KismetArrayLibrary.Array_Random` (`|MakeArray` "/Game/Objects/Meshes/pole1_new.pole1_new" "/Game/Objects/Meshes/pole2_new.pole2_new" "/Game/Objects/Meshes/pole3_new.pole3_new" :!type "StaticMesh Object Reference")))
  (`StaticMeshComponent.SetStaticMesh` (`self.Static Mesh`) _outitem)
  (switch `int` _outindex
    (:`Default`
      (`SceneComponent.K2_SetRelativeLocation` _cable_1 _returnvalue_3 false false :!label _label)
      (`SceneComponent.K2_SetRelativeLocation` (`self.Cable 1 Pos`) _returnvalue_3 false false)
      (set `CableComponent.EndLocation` _returnvalue_3 _cable_1)
      (`SceneComponent.K2_SetRelativeLocation` (`self.Cable 2 Pos`) _returnvalue_4 false false)
      (`SceneComponent.K2_SetRelativeLocation` (`self.Cable 2`) _returnvalue_4 false false)
      (set `CableComponent.EndLocation` _returnvalue_4 (`self.Cable 2`)))
    (:`0`
      (goto _label))
    (:`1`
      (goto _label))
    (:`2`
      (`SceneComponent.K2_SetRelativeLocation` (`self.Cable 1 Pos`) _returnvalue_2 false false)
      (`SceneComponent.K2_SetRelativeLocation` (`self.Cable 1`) _returnvalue_2 false false)
      (set `CableComponent.EndLocation` _returnvalue_2 (`self.Cable 1`))
      (`SceneComponent.K2_SetRelativeLocation` (`self.Cable 2 Pos`) _returnvalue false false)
      (`SceneComponent.K2_SetRelativeLocation` (`self.Cable 2`) _returnvalue false false)
      (set `CableComponent.EndLocation` _returnvalue (`self.Cable 2`)))))
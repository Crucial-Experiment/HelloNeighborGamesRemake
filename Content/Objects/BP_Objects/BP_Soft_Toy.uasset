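; BP_Soft_Toy is a burnable toy object that carries a linked actor and releases it when burned.
; The construction script attaches that actor to the toy's root and snaps it to the Scene component's transform.
; On BeginPlay it sets the actor's flat mode and disables its collision.
; The inherited burned event reapplies that flat mode, re-enables collision and makes the actor visible.
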(event `self.ReceiveBeginPlay`
  ;[1 1 1] Begin Play
  (`parent.ReceiveBeginPlay`)
  (bind _actor (`self.Actor`)
    (:`then`
      (`self.Set Flat Mode` _actor "NewEnumerator1")
      (`self.SetActorEnableCollision` _actor false))
    (:`else`)))

(event `self.Burned Event`
  ;[1 1 1] Burned
  (`parent.Burned Event`)
  (bind _actor (`self.Actor`)
    (:`then`
      (`self.Set Flat Mode` _actor "NewEnumerator1")
      (`self.SetActorEnableCollision` _actor true)
      (`self.SetActorHiddenInGame` _actor false))
    (:`else`)))

(fn `UserConstructionScript`
  (bind _actor (`self.Actor`)
    (:`then`
      (`self.K2_AttachToComponent` _actor (`self.Root`) "None" "KeepRelative" "KeepRelative" "KeepRelative" true)
      (`self.K2_SetActorTransform` _actor (`SceneComponent.K2_GetComponentToWorld` (`self.Scene`)) false false))
    (:`else`)))
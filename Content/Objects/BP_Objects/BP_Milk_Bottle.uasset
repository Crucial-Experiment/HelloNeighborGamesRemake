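; BP_Milk_Bottle is a milk bottle object that can be poisoned, with the poison wearing off over time.
; The construction script applies the poisoned or normal milk material to Root based on the Poisen flag.
; Tick runs through a one-second Delay, counting PoisenTimeTemp up to PoisenTime while poisoned.
; At the limit it clears Poisen and sets material slot 0 with no material specified.
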(event `self.ReceiveTick`
  (params (DeltaSeconds :type "Float (single-precision)"))
  (`KismetSystemLibrary.Delay` 1.0)
  (if (`self.Poisen`)
    (if (>= (`self.Poisen Time Temp`) (`self.Poisen Time`))
      (set `self.Poisen` false)
      (`PrimitiveComponent.SetMaterial` (`self.Root`) 0 null)
      (else
        (`/Engine/EditorBlueprintResources/StandardMacros.IncrementInt` (`self.Poisen Time Temp`))))))

(fn `UserConstructionScript`
  (bind _root (`self.Root`))
  (if (`self.Poisen`)
    (`PrimitiveComponent.SetMaterial` _root 0 "/Game/Objects/Materials/bottle_milk_poisoned.bottle_milk_poisoned")
    (else
      (`PrimitiveComponent.SetMaterial` _root 0 "/Game/Objects/Materials/bottle_milk_m_inst.bottle_milk_m_inst"))))
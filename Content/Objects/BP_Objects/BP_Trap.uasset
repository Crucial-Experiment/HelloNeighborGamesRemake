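; BP_Trap is a throwable bear trap that Interact arms and that snaps shut on the player, an attacking Neighbor or other objects.
; SetState drives animation, mesh, overlap, pickup and sound, returning animation length for delays.
; A caught player is pinned with a UI widget until escaping or being caught by the Neighbor.
; Player and object triggers send a non-attacking Neighbor to investigate via Blackboard, while an attacking one is briefly held.
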(event `/Game/Function/BP_Interface.Interact`
  (params (Component :type "PrimitiveComponent Object Reference") (Location :type "Vector Structure"))
  ;[1 1 1] Begin Play and Interact
  (`parent.Interact` Component Location)
  (switch `/Game/Objects/Enum/RotateStateEnum` (`self.State`)
    (:`NewEnumerator1`
      (bind _anim_play_length (`self.Set State` "NewEnumerator2"))
      (`KismetSystemLibrary.Delay` _anim_play_length)
      (set `self.State` "NewEnumerator0"))))

(event `self.ReceiveBeginPlay`
  ;[1 1 1] Begin Play and Interact
  (`parent.ReceiveBeginPlay`)
  (`self.Set State` (`self.State`))
  (bind _sosed (`/Game/Function/BP_MacroLibrary.Find Sosed`)
    (:`Is Valid`
      (set `self.Neighbor` _sosed)
      (add `/Game/Sosed/BP_Sosed.On Player Catch` _sosed (delegate `Player Out Trap`)))))

(event `self.Trap Box.OnComponentBeginOverlap`
  (params (OverlappedComponent :type "PrimitiveComponent Object Reference") (OtherActor :type "Actor Object Reference") (OtherComp :type "PrimitiveComponent Object Reference") (OtherBodyIndex :type Integer) (bFromSweep :type Boolean) (SweepResult :type "HitResult Structure (by ref)"))
  (bind (_returnvalue_x _returnvalue_y) (`KismetMathLibrary.BreakVector` (`self.K2_GetActorLocation`)))
  ;[1 1 1] Main Logic
  (bind (_is_player _is_neighbor _is_bp_object) (`self.Check Object` OtherActor))
  (`|ExecutionSequence`
    (:`then_0`
      (`/Engine/EditorBlueprintResources/StandardMacros.IsValid` _is_player
        (:`Is Valid`
          (`self.Set State` "NewEnumerator3")
          (set `/Game/Player/BP_Player.Is Trap` true _is_player)
          (`self.SetActorEnableCollision` false)
          (set `self.Player Is Here?` true)
          (add `/Game/Player/BP_Player.Out Trap` _is_player (delegate `Player Out Trap`))
          (`UserWidget.AddToViewport` (`/Game/Player/BP_Player.In Trap` _is_player) 0)
          (bind (_returnvalue_x_2 _returnvalue_y_2 _returnvalue_z) (`KismetMathLibrary.BreakVector` (`self.K2_GetActorLocation` _is_player)))
          (`self.K2_SetActorLocation` _is_player (`KismetMathLibrary.MakeVector` _returnvalue_x _returnvalue_y _returnvalue_z) false true)
          ;[1 1 1] Neighbor Run to Trap
          (bind _sosed (`/Game/Function/BP_MacroLibrary.Find Sosed` :!label _label)
            (:`Is Valid`
              (if (`|EnumInequality` (`/Game/Sosed/BP_Sosed.Current State` _sosed) "NewEnumerator2")
                (bind _returnvalue (`AIBlueprintHelperLibrary.GetBlackboard` _sosed))
                (`BlackboardComponent.SetValueAsInt` _returnvalue "CheckTask" 2)
                (`BlackboardComponent.SetValueAsVector` _returnvalue "Check Location" (`SceneComponent.K2_GetComponentLocation` (`self.Root`)))
                (`BlackboardComponent.SetValueAsObject` _returnvalue "Trap" self)
                (`/Game/Sosed/BP_Sosed.Set State` _sosed "NewEnumerator3")))))))
    (:`then_1`
      (`/Engine/EditorBlueprintResources/StandardMacros.IsValid` _is_neighbor
        (:`Is Valid`
          (`self.Neighbor in Trap` _is_neighbor))))
    (:`then_2`
      (`/Engine/EditorBlueprintResources/StandardMacros.IsValid` _is_bp_object
        (:`Is Valid`
          (`self.Actor in Trap`)
          (goto _label))))))

(event `Player Out Trap`
  ;[1 1 1] Main Logic
  (`self.Set State` "NewEnumerator1")
  (set `self.Player Is Here?` false)
  (`self.SetActorEnableCollision` true)
  (bind _in_trap (`/Game/Player/BP_Player.In Trap` (stale `self.Trap Box.OnComponentBeginOverlap` _is_player)))
  (`/Engine/EditorBlueprintResources/StandardMacros.IsValid` _in_trap
    (:`Is Valid`
      (`Widget.RemoveFromParent` _in_trap))))

(fn `Set State`
  (params (NewState :type "/Game/Objects/Enum/RotateStateEnum Enum" :default "NewEnumerator0"))
  (returns (`Anim Play Length` :type "Float (double-precision)"))
  (bind _trap_sm (`self.Trap SM`))
  (bind _trap_sm_2 (`self.Trap SM`))
  (bind _trap_box (`self.Trap Box`))
  (bind _grabcomponent (`self.GrabComponent`))
  (bind _tutorialcomponent (`self.TutorialComponent`))
  (bind _gamejoltcomponent (`self.GameJoltComponent`))
  (bind _output_get (set `self.State` NewState))
  (switch `/Game/Objects/Enum/RotateStateEnum` _output_get
    (:`NewEnumerator0`
      (`SkeletalMeshComponent.PlayAnimation` _trap_sm_2 "/Game/Objects/Meshes/Animations/Trap/trap_Anim_Armature_open.trap_Anim_Armature_open" false)
      (`StaticMeshComponent.SetStaticMesh` (`self.Root`) "/Game/Objects/Meshes/trap_new.trap_new" :!label _label)
      (set `PrimitiveComponent.bGenerateOverlapEvents` true _trap_box)
      (set `self.CanPickUp` false)
      (set `/Game/Objects/Structurs/GrabComponent.GrabType` "NewEnumerator0" _grabcomponent)
      (`AudioComponent.Play` (`self.Trap Reload`) 0.0)
      (`/Game/Objects/Tutorial/TutorialComponent.Check Use Type` _tutorialcomponent "NewEnumerator1")
      (`/Game/Objects/GameJolt/GameJoltComponent.Check Use Type` _gamejoltcomponent "NewEnumerator1"))
    (:`NewEnumerator2`
      (`SkeletalMeshComponent.PlayAnimation` _trap_sm_2 "/Game/Objects/Meshes/Animations/Trap/trap_Anim_Armature_opening.trap_Anim_Armature_opening" false)
      (goto _label))
    (:`NewEnumerator1`
      (`SkeletalMeshComponent.PlayAnimation` _trap_sm "/Game/Objects/Meshes/Animations/Trap/trap_Anim_Armature_closed.trap_Anim_Armature_closed" false)
      (`StaticMeshComponent.SetStaticMesh` (`self.Root`) "/Game/Objects/Meshes/trap_closed_new.trap_closed_new" :!label _label_2)
      (set `PrimitiveComponent.bGenerateOverlapEvents` false _trap_box)
      (set `self.CanPickUp` true)
      (set `/Game/Objects/Structurs/GrabComponent.GrabType` "NewEnumerator4" _grabcomponent)
      (`AudioComponent.Play` (`self.Mantrap`) 0.0)
      (`/Game/Objects/Tutorial/TutorialComponent.Check Use Type` _tutorialcomponent "NewEnumerator2")
      (`/Game/Objects/GameJolt/GameJoltComponent.Check Use Type` _gamejoltcomponent "NewEnumerator2"))
    (:`NewEnumerator3`
      (`SkeletalMeshComponent.PlayAnimation` _trap_sm "/Game/Objects/Meshes/Animations/Trap/trap_Anim_Armature_closing.trap_Anim_Armature_closing" false)
      (goto _label_2)))
  (`self.Set Flat Mode` "NewEnumerator1")
  (bind _returnvalue (message `AnimationDataModel.GetPlayLength` (`self.Trap SM`)))
  (return _returnvalue))

(fn `Throw`
  (params (Player :type "/Game/Player/BP_Player Object Reference"))
  (`self.Set State` "NewEnumerator0")
  (`self.Set Flat Mode` "NewEnumerator0")
  (`self.K2_SetActorRelativeRotation` (struct :`Roll` 90.0))
  (`PrimitiveComponent.AddImpulse` (`self.Root`) (* (`KismetMathLibrary.Normal` (- (+ (`self.K2_GetActorLocation` Player) (0.0 0.0 30.0)) (`self.K2_GetActorLocation`))) 150000.0) "None" false))

(fn `UserConstructionScript`
  (`self.Set State` (`self.State`)))
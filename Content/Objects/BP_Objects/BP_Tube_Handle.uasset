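; BP_Tube_Handle is an interactable handle whose lever rotates when toggled between On and Off.
; Interact calls its parent, then a server event that plays the OpenClosed component and reports the use type to the Tutorial and GameJolt components.
; The current State chooses whether one timeline plays forward or in reverse.
; That timeline lerps the Level component's relative rotation over a quarter turn and calls SetState when finished.
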(event `Interact (Server)`
  (bind _gamejoltcomponent (`self.GameJoltComponent`))
  (bind _tutorialcomponent (`self.TutorialComponent`))
  (`AudioComponent.Play` (`self.open_closed`) 0.0)
  (switch `/Game/Objects/Enum/TumblerStateEnum` (`self.State`)
    (:`NewEnumerator0`
      (`/Game/Objects/Tutorial/TutorialComponent.Check Use Type` _tutorialcomponent "NewEnumerator4")
      (`/Game/Objects/GameJolt/GameJoltComponent.Check Use Type` _gamejoltcomponent "NewEnumerator4")
      (bind (_direction _alpha) (`Timeline|Шкала времени` :!via `Reverse` :!label _label)
        (:`Update`
          (`SceneComponent.K2_SetRelativeRotation` (`self.Level`) (`KismetMathLibrary.RLerp` (struct :`Pitch` 90.0) (struct :`Pitch` 90.0 :`Roll` -90.0) _alpha) false false))
        (:`Finished`
          (`self.Set State`))))
    (:`NewEnumerator1`
      (`/Game/Objects/Tutorial/TutorialComponent.Check Use Type` _tutorialcomponent "NewEnumerator3")
      (`/Game/Objects/GameJolt/GameJoltComponent.Check Use Type` _gamejoltcomponent "NewEnumerator3")
      (goto _label))))

(event `/Game/Function/BP_Interface.Interact`
  (params (Component :type "PrimitiveComponent Object Reference") (Location :type "Vector Structure"))
  (`parent.Interact` Component Location)
  (`self.Interact (Server)`))

(fn `UserConstructionScript`
  (`parent.UserConstructionScript`))
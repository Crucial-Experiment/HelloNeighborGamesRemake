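; BP_Warrior is a skinned-mesh character object that idles or slides left or right and can be knocked down.
; NewAction drives movement timelines, and overlapping another warrior sets both to Idle.
; A hard enough hit destroys its collision box, tips it over, calls OnDeath, then removes the actor.
; The construction script picks the mesh from Skin, and animations play from an array without waiting, so the last valid one wins.
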(event `New Action`
  (params (`New Action` :type "/Game/Objects/Enum/WarriorActionEnum Enum" :default "NewEnumerator0") (`New Struct` :type "/Game/Objects/Structurs/BP_Warrior_Action_Struct Structure"))
  (bind _returnvalue (`self.K2_GetActorLocation`))
  (bind _returnvalue_2 (`self.K2_GetActorLocation`))
  (bind (_struct_movetoleft _struct_movetoright) (break `/Game/Objects/Structurs/BP_Warrior_Action_Struct` (`self.Struct`)))
  (bind _struct_movetoleft_2 (break `/Game/Objects/Structurs/BP_Warrior_Action_Struct` (`self.Struct`)))
  (set `self.Struct` `New Struct`)
  (bind _output_get (set `self.Action` `New Action`))
  (switch `/Game/Objects/Enum/WarriorActionEnum` _output_get
    (:`NewEnumerator0`
      (`|ExecutionSequence`
        (:`then_0`
          (bind (_direction _alpha) (`Timeline|Move to Left` :!via `Stop` :!label _label)
            (:`Update`
              (`self.K2_SetActorRelativeLocation` (`KismetMathLibrary.VLerp` _returnvalue_2 (+ _returnvalue_2 _struct_movetoleft_2) _alpha)))))
        (:`then_1`
          (bind (_direction_2 _alpha_2) (`Timeline|Move to Right` :!via `Stop` :!label _label_2)
            (:`Update`
              (`self.K2_SetActorRelativeLocation` (`KismetMathLibrary.VLerp` _returnvalue (+ _returnvalue _struct_movetoright) _alpha_2)))))))
    (:`NewEnumerator1`
      (goto _label :!via `PlayFromStart`))
    (:`NewEnumerator2`
      (goto _label_2 :!via `PlayFromStart`))))

(event `self.Box.OnComponentHit`
  (params (HitComponent :type "PrimitiveComponent Object Reference") (OtherActor :type "Actor Object Reference") (OtherComp :type "PrimitiveComponent Object Reference") (NormalImpulse :type "Vector Structure") (Hit :type "HitResult Structure (by ref)"))
  (`/Engine/EditorBlueprintResources/StandardMacros.CompareFloat` (`KismetMathLibrary.VSize` NormalImpulse) 1200.0
    (:`>`
      (`ActorComponent.K2_DestroyComponent` (`self.Box`))
      (bind (_direction _alpha) (`Timeline|Rotate Timeline`)
        (:`Update`
          (`self.K2_SetActorRelativeRotation` (`KismetMathLibrary.RLerp` (struct) (struct :`Roll` -90.0) _alpha)))
        (:`Finished`
          (`self.On Death`)
          (`KismetSystemLibrary.Delay` 1.5)
          (`self.K2_DestroyActor`))))))

(event `self.ReceiveBeginPlay`
  (`parent.ReceiveBeginPlay`)
  (`self.New Action` (`self.Action`) (`self.Struct`))
  (for _array_element (`self.Animations`) :!label _label_3
    (`/Engine/EditorBlueprintResources/StandardMacros.IsValid` (break `/Game/Sosed/Ai/Struct/AnimPoint` _array_element)
      (:`Is Valid`
        (`SkeletalMeshComponent.PlayAnimation` (`self.Mesh`) (break `/Game/Sosed/Ai/Struct/AnimPoint` _array_element) (`.Loop_8_419914E846BCFCE562A09F91144AA8AF` (break `/Game/Sosed/Ai/Struct/AnimPoint` _array_element)))))))

(event `Play Animation`
  (goto _label_3))

(event `self.Box.OnComponentBeginOverlap`
  (params (OverlappedComponent :type "PrimitiveComponent Object Reference") (OtherActor :type "Actor Object Reference") (OtherComp :type "PrimitiveComponent Object Reference") (OtherBodyIndex :type Integer) (bFromSweep :type Boolean) (SweepResult :type "HitResult Structure (by ref)"))
  (bind _asbp_warrior (cast `/Game/Objects/BP_Objects/BP_Warrior` OtherActor))
  (`self.New Action` :`self` _asbp_warrior)
  (`self.New Action` "NewEnumerator0"))

(fn `Set Mesh`
  (params (Index :type Integer))
  (switch `int` Index
    (:`Default`
      (set `self.New Mesh` "/Game/Objects/Meshes/Animations/RifleRange/warrior_1_new.warrior_1_new" :!label _label))
    (:`0`
      (goto _label))
    (:`1`
      (set `self.New Mesh` "/Game/Objects/Meshes/Animations/RifleRange/warrior_2_new.warrior_2_new"))
    (:`2`
      (set `self.New Mesh` "/Game/Objects/Meshes/Animations/RifleRange/target_mirror_new.target_mirror_new"))
    (:`3`
      (set `self.New Mesh` "/Game/Objects/Meshes/Animations/RifleRange/target_pride_new.target_pride_new")))
  (`SkinnedMeshComponent.SetSkinnedAssetAndUpdate` (`self.Mesh`) (`self.New Mesh`) true))

(fn `UserConstructionScript`
  (`self.Set Mesh` (`self.Skin`)))
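; BP_LiftDoor is a two-panel lift door that slides open and closed through its Open and Close events.
; Open plays DoorsTimeline and Close reverses it.
; The timeline's Alpha interpolates each panel's relative location between its start and end vectors, moving both doors together without sweep.
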(event `Open`
  (bind (_direction _alpha) (`Timeline|Doors Timeline` :!label _label)
    (:`Update`
      (`SceneComponent.K2_SetRelativeLocation` (`self.Door 1`) (`KismetMathLibrary.VLerp` (`self.Left Door Start`) (`self.Left Door End`) _alpha) false false)
      (`SceneComponent.K2_SetRelativeLocation` (`self.Door 2`) (`KismetMathLibrary.VLerp` (`self.Right Door Start`) (`self.Right Door End`) _alpha) false false))))

(event `Close`
  (goto _label :!via `Reverse`))

(fn `UserConstructionScript`)
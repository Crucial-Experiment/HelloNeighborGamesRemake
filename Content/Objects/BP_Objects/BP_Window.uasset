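; Breakable window object that extends a parent glass blueprint with two more panes, GlassWin1 and GlassWin3.
; A fast BP_Object hit on a breakable pane, or the inherited BrokeGlass event (once, both panes), triggers a server-to-multicast break.
; Breaking disables the pane, spawns a short-lived destruction actor, counts the break, then updates tutorial and GameJolt checks and runs NeighborCheck.
; RestoringWindows re-enables both panes alongside the parent's restore.
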(event `Broke Glass 2 (All)`
  (bind _glass_win_1 (`self.Glass Win 1`))
  (bind (_returnvalue_location _returnvalue_rotation) (`KismetMathLibrary.BreakTransform` (`SceneComponent.K2_GetComponentToWorld` _glass_win_1)))
  ;[1 1 1] Window 1
  (`self.Win Collision` false _glass_win_1)
  (bind _returnvalue (`|SpawnActorFromClass` (`self.Destroy Class`) (`KismetMathLibrary.MakeTransform` _returnvalue_location _returnvalue_rotation) "Undefined" "MultiplyWithRoot" null null))
  (`/Engine/EditorBlueprintResources/StandardMacros.IncrementInt` (`self.Broken Count`)
    (:`  `
      (set `/Game/Objects/Destroy/BP_GC_Glass.Glass Break` (`self.Glass Break`) _returnvalue)
      (`KismetSystemLibrary.Delay` 2.5)
      (`self.K2_DestroyActor` _returnvalue)
      (`/Game/Objects/Tutorial/TutorialComponent.Check Use Type` (`self.TutorialComponent`) "NewEnumerator7")
      (`/Game/Objects/GameJolt/GameJoltComponent.Check Use Type` (`self.GameJoltComponent`) "NewEnumerator7")
      (bind _sosed (`/Game/Function/BP_MacroLibrary.Find Sosed`)
        (:`Is Valid`
          (`self.Neighbor Check` _sosed (`self.Arrow Win 1`)))))))

(event `self.Glass Win 1.OnComponentHit`
  (params (HitComponent :type "PrimitiveComponent Object Reference") (OtherActor :type "Actor Object Reference") (OtherComp :type "PrimitiveComponent Object Reference") (NormalImpulse :type "Vector Structure") (Hit :type "HitResult Structure (by ref)"))
  ;[1 1 1] Window 1
  (bind _asbp_object (cast `/Game/Objects/Structurs/BP_Object` OtherActor))
  (if (`self.Could Be Broken`)
    (if (>= (`KismetMathLibrary.VSize` (`self.GetVelocity` _asbp_object)) 200.0)
      (`self.Broke Glass 2 (Server)` :!label _label))))

(event `Broke Glass 2 (Server)`
  ;[1 1 1] Window 1
  (`self.Broke Glass 2 (All)`))

(event `self.Broke Glass`
  (`parent.Broke Glass`)
  (`/Engine/EditorBlueprintResources/StandardMacros.DoOnce` false
    (:`Completed`
      (`|ExecutionSequence`
        (:`then_0`
          (goto _label))
        (:`then_1`
          ;[1 1 1] Window 3
          (`self.Broke Glass 3 (Server)` :!label _label_2))))))

(event `Broke Glass 3 (All)`
  (bind _glass_win_3 (`self.Glass Win 3`))
  (bind (_returnvalue_location _returnvalue_rotation) (`KismetMathLibrary.BreakTransform` (`SceneComponent.K2_GetComponentToWorld` _glass_win_3)))
  ;[1 1 1] Window 3
  (`self.Win Collision` false _glass_win_3)
  (bind _returnvalue (`|SpawnActorFromClass` (`self.Destroy Class`) (`KismetMathLibrary.MakeTransform` _returnvalue_location _returnvalue_rotation) "Undefined" "MultiplyWithRoot" null null))
  (`/Engine/EditorBlueprintResources/StandardMacros.IncrementInt` (`self.Broken Count`)
    (:`  `
      (set `/Game/Objects/Destroy/BP_GC_Glass.Glass Break` (`self.Glass Break`) _returnvalue)
      (`KismetSystemLibrary.Delay` 2.5)
      (`self.K2_DestroyActor` _returnvalue)
      (`/Game/Objects/Tutorial/TutorialComponent.Check Use Type` (`self.TutorialComponent`) "NewEnumerator7")
      (`/Game/Objects/GameJolt/GameJoltComponent.Check Use Type` (`self.GameJoltComponent`) "NewEnumerator7")
      (bind _sosed (`/Game/Function/BP_MacroLibrary.Find Sosed`)
        (:`Is Valid`
          (`self.Neighbor Check` _sosed (`self.Arrow Win 3`)))))))

(event `self.Glass Win 3.OnComponentHit`
  (params (HitComponent :type "PrimitiveComponent Object Reference") (OtherActor :type "Actor Object Reference") (OtherComp :type "PrimitiveComponent Object Reference") (NormalImpulse :type "Vector Structure") (Hit :type "HitResult Structure (by ref)"))
  ;[1 1 1] Window 3
  (bind _asbp_object (cast `/Game/Objects/Structurs/BP_Object` OtherActor))
  (if (`self.Could Be Broken`)
    (if (>= (`KismetMathLibrary.VSize` (`self.GetVelocity` _asbp_object)) 200.0)
      (goto _label_2))))

(event `Broke Glass 3 (Server)`
  ;[1 1 1] Window 3
  (`self.Broke Glass 3 (All)`))

(event `self.Restoring Windows`
  ;[1 1 1] Restoring Windows
  (`parent.Restoring Windows`)
  (`self.Win Collision` true (`self.Glass Win 3`))
  (`self.Win Collision` true (`self.Glass Win 1`)))

(fn `UserConstructionScript`
  (`parent.UserConstructionScript`))
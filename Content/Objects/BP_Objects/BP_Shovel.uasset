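; BP_Shovel is a held item that digs away the top of a BP_Grave.
; LMB while held, or VR use, runs a short line trace and, on the grave's Top component, calls a server event and plays a dirt sound.
; The server relays to an all-clients event that lowers Top, decrements its count and notifies tutorial and GameJolt components.
; Dropping resets the shovel's scale, and a grab-component drop also sets flat mode.
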(event `self.GrabComponent.OnDropped`
  (params (`Self Ref` :type "/Game/Objects/Structurs/GrabComponent Object Reference"))
  (`self.Set Flat Mode` "NewEnumerator0")
  (`self.SetActorScale3D` (1.5 1.5 1.5) :!label _label))

(event `On Item Dropped_1`
  (goto _label))

(event `self.ReceiveBeginPlay`
  (`parent.ReceiveBeginPlay`))

(event `On Press LMB_1`
  (bind _player (`/Game/Function/BP_MacroLibrary.Find Player`)
    (:`Is Valid`
      (bind _item (`/Game/Player/BP_Player.Get Item` _player))
      (if (== _item self)
        (bind (_actor _component) (`self.Line Trace` 300.0 "NewEnumerator1" :!label _label_2))
        (bind _asbp_grave (cast `/Game/Objects/BP_Objects/BP_Grave` _actor))
        (bind _top (`/Game/Objects/BP_Objects/BP_Grave.Top` _asbp_grave))
        (`/Engine/EditorBlueprintResources/StandardMacros.IsValid` _top
          (:`Is Valid`
            (if (== _component _top)
              (`self.Interact (Server)` _asbp_grave)
              (`GameplayStatics.PlaySoundAtLocation` "/Game/Sounds/cutscenes/Act1/shovel_impact_dirt_1_Cue.shovel_impact_dirt_1_Cue" (`self.K2_GetActorLocation`) (struct) 1.0 1.0 0.0 null null null null))))))))

(event `self.On VR Use`
  (`parent.On VR Use`)
  (goto _label_2))

(event `Interact (All)`
  (params (Grave :type "/Game/Objects/BP_Objects/BP_Grave Object Reference"))
  (bind _top (`/Game/Objects/BP_Objects/BP_Grave.Top` Grave))
  (bind (_returnvalue_x _returnvalue_y _returnvalue_z) (`KismetMathLibrary.BreakVector` (`SceneComponent.K2_GetComponentLocation` _top)))
  (`SceneComponent.K2_SetWorldLocation` _top (`KismetMathLibrary.MakeVector` _returnvalue_x _returnvalue_y (- _returnvalue_z 25.0)) false false)
  (`/Engine/EditorBlueprintResources/StandardMacros.DecrementInt` (`/Game/Objects/BP_Objects/BP_Grave.Grave Top Count` Grave)
    (:`  `
      (`/Game/Objects/BP_Objects/BP_Grave.Grave Top` Grave)
      (`/Game/Objects/Tutorial/TutorialComponent.Check Use Type` (`self.TutorialComponent`) "NewEnumerator6")
      (`/Game/Objects/GameJolt/GameJoltComponent.Check Use Type` (`self.GameJoltComponent`) "NewEnumerator6"))))

(event `Interact (Server)`
  (params (Grave :type "/Game/Objects/BP_Objects/BP_Grave Object Reference"))
  (`self.Interact (All)` Grave))

(fn `UserConstructionScript`
  (`parent.UserConstructionScript`))
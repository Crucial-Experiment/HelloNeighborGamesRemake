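; BP_NeighborLift is a floor trigger that works a referenced Lift for the neighbour character (BP_Sosed).
; On box overlap it compares the lift's floor to its own and, if they match, just switches the lift's state.
; Otherwise it freezes the neighbour's movement, changes lift state, then after a short delay sends the lift its floor and another state.
; The lift's MoveCompleted event restores walking and unbinds itself.
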(event `self.Box.OnComponentBeginOverlap`
  (params (OverlappedComponent :type "PrimitiveComponent Object Reference") (OtherActor :type "Actor Object Reference") (OtherComp :type "PrimitiveComponent Object Reference") (OtherBodyIndex :type Integer) (bFromSweep :type Boolean) (SweepResult :type "HitResult Structure (by ref)"))
  (bind _lift (`self.Lift`))
  (bind _lift_2 (`self.Lift`))
  (bind _asbp_sosed (cast `/Game/Sosed/BP_Sosed` OtherActor))
  (`/Engine/EditorBlueprintResources/StandardMacros.IsValid` _lift
    (:`Is Valid`
      (if (== (`/Game/Objects/BP_Objects/BP_Lift.Flour` _lift) (`self.Floor`))
        (`/Game/Objects/BP_Objects/BP_Lift.Set State` _lift_2 "NewEnumerator2")
        (else
          (`CharacterMovementComponent.SetMovementMode` (`Character.CharacterMovement` _asbp_sosed) "MOVE_None" 0)
          (add `/Game/Objects/BP_Objects/BP_Lift.Move Completed` _lift_2 (delegate `Move Completed`))
          (`/Game/Objects/BP_Objects/BP_Lift.Set State` _lift_2 "NewEnumerator3")
          (`KismetSystemLibrary.Delay` 1.6)
          (set `/Game/Objects/BP_Objects/BP_Lift.Flour` (`self.Floor`) _lift_2)
          (`/Game/Objects/BP_Objects/BP_Lift.Set State` _lift_2 "NewEnumerator1"))))))

(event `Move Completed`
  (`CharacterMovementComponent.SetMovementMode` (`Character.CharacterMovement` (stale `self.Box.OnComponentBeginOverlap` _asbp_sosed)) "MOVE_Walking" 0)
  (clear `/Game/Objects/BP_Objects/BP_Lift.Move Completed` (`self.Lift`)))

(fn `UserConstructionScript`)
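; BP_Fridge is an electricity-aware fridge with a looping or ambient tone and an interactive hinged door.
; The tone plays while powered and stops on Disable, while Interact toggles the door through a rotation timeline with open and delayed close sounds.
; Power and door changes report use types to the tutorial and GameJolt components.
; Door state is saved to JSON, and loading replays Interact when the saved state differs.
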(event `self.ReceiveBeginPlay`
  (`parent.ReceiveBeginPlay`)
  (if (or (`self.Has Electricity`) (`self.Generator`))
    (`AudioComponent.Play` (`self.Tone`) 0.0 :!label _label)
    (`/Game/Objects/Tutorial/TutorialComponent.Check Use Type` (`self.TutorialComponent`) "NewEnumerator3")
    (`/Game/Objects/GameJolt/GameJoltComponent.Check Use Type` (`self.GameJoltComponent`) "NewEnumerator3")))

(event `self.Enable`
  (`parent.Enable`)
  (goto _label))

(event `self.Disable`
  (`parent.Disable`)
  (`AudioComponent.Stop` (`self.Tone`))
  (`/Game/Objects/Tutorial/TutorialComponent.Check Use Type` (`self.TutorialComponent`) "NewEnumerator4")
  (`/Game/Objects/GameJolt/GameJoltComponent.Check Use Type` (`self.GameJoltComponent`) "NewEnumerator4"))

(event `/Game/Function/BP_Interface.Interact`
  (params (Component :type "PrimitiveComponent Object Reference") (Location :type "Vector Structure"))
  (bind _tutorialcomponent (`self.TutorialComponent`))
  (bind _gamejoltcomponent (`self.GameJoltComponent`))
  (if (== Component (`self.Door`))
    (switch `/Game/Objects/Enum/RotateStateEnum` (`self.Door State`)
      (:`NewEnumerator0`
        (`/Game/Objects/Tutorial/TutorialComponent.Check Use Type` _tutorialcomponent "NewEnumerator2")
        (`/Game/Objects/GameJolt/GameJoltComponent.Check Use Type` _gamejoltcomponent "NewEnumerator2")
        (`|ExecutionSequence`
          (:`then_0`
            (bind (_direction _driver) (`Timeline|Шкала времени` :!via `Reverse` :!label _label_2)
              (:`Update`
                (`SceneComponent.K2_SetRelativeRotation` (`self.Door`) (`KismetMathLibrary.RLerp` (struct) (struct :`Yaw` -100.0) _driver) false false))
              (:`Finished`
                (switch `/Game/Objects/Enum/RotateStateEnum` (`self.Door State`)
                  (:`NewEnumerator0`
                    (set `self.Door State` "NewEnumerator1"))
                  (:`NewEnumerator1`
                    (set `self.Door State` "NewEnumerator0"))))))
          (:`then_1`
            (`KismetSystemLibrary.Delay` 0.2)
            (`AudioComponent.Play` (`self.Door Close`) 0.0))))
      (:`NewEnumerator1`
        (`/Game/Objects/Tutorial/TutorialComponent.Check Use Type` _tutorialcomponent "NewEnumerator1")
        (`/Game/Objects/GameJolt/GameJoltComponent.Check Use Type` _gamejoltcomponent "NewEnumerator1")
        (`|ExecutionSequence`
          (:`then_0`
            (goto _label_2))
          (:`then_1`
            (`AudioComponent.Play` (`self.Door Open`) 0.0)))))))

(fn `Load Data`
  (params (JSON :type String))
  (returns (Object :type "VaRestJsonObject Object Reference"))
  (bind _object (`parent.Load Data` JSON))
  (`|ExecutionSequence`
    (:`then_0`
      (bind (_has_field_ _return_value) (`/Game/Function/BP_JSON_FunctionLibrary.Get Value As Int` _object "Door State"))
      (if (and _has_field_ (!= _return_value (`KismetMathLibrary.Conv_ByteToInt` (`self.Door State`))))
        (`self.Interact` (`self.Door`))))
    (:`then_1`
      (return _object))))

(fn `Save Data`
  (returns (JSON :type "VaRestJsonObject Object Reference"))
  (bind _json (`parent.Save Data`))
  (`VaRestJsonObject.SetIntegerField` _json "Door State" (`KismetMathLibrary.Conv_ByteToInt` (`self.Door State`)))
  (return _json))

(fn `UserConstructionScript`)
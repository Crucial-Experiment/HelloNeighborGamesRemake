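; Garage door object that swings and slides its mesh between two poses when enabled or disabled through its parent class.
; Enable and Disable switch between Open and Close playback, wait a second, then run one timeline forward or in reverse to lerp location and rotation.
; The timeline's finish toggles the On/Off State, which is saved and loaded as a JSON integer; loading does not reposition the mesh.
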(event `self.ReceiveBeginPlay`
  ;[1 1 1] Begin Play
  (`parent.ReceiveBeginPlay`)
  (`self.Set Flat Mode` "NewEnumerator1"))

(event `self.Enable`
  ;[1 1 1] Rotate
  (`parent.Enable`)
  (`AudioComponent.Play` (`self.Open`) 0.0)
  (`AudioComponent.Stop` (`self.Close`))
  (`KismetSystemLibrary.Delay` 1.0)
  (bind (_direction _alpha) (`Timeline|Rotate Timeline` :!label _label)
    (:`Update`
      (`SceneComponent.K2_SetRelativeLocationAndRotation` (`self.Door Mesh`) (`KismetMathLibrary.VLerp` (0.0 0.0 -270.0) (0.0 0.0 0.0) _alpha) (`KismetMathLibrary.RLerp` (struct) (struct :`Roll` 90.0) _alpha) false false))
    (:`Finished`
      (switch `/Game/Objects/Enum/TumblerStateEnum` (`self.State`)
        (:`NewEnumerator0`
          (set `self.State` "NewEnumerator1"))
        (:`NewEnumerator1`
          (set `self.State` "NewEnumerator0"))))))

(event `self.Disable`
  ;[1 1 1] Rotate
  (`parent.Disable`)
  (`AudioComponent.Stop` (`self.Open`))
  (`AudioComponent.Play` (`self.Close`) 0.0)
  (`KismetSystemLibrary.Delay` 1.0)
  (goto _label :!via `Reverse`))

(fn `Load Data`
  (params (JSON :type String))
  (returns (Object :type "VaRestJsonObject Object Reference"))
  (bind _object (`parent.Load Data` JSON))
  (`|ExecutionSequence`
    (:`then_0`
      (bind (_has_field_ _return_value) (`/Game/Function/BP_JSON_FunctionLibrary.Get Value As Int` _object "State"))
      (if (and _has_field_ (!= _return_value (`KismetMathLibrary.Conv_ByteToInt` (`self.State`))))
        (set `self.State` (cast `/Game/Objects/Enum/TumblerStateEnum` (`KismetMathLibrary.Conv_IntToByte` _return_value)))))
    (:`then_1`
      (return _object))))

(fn `Save Data`
  (returns (JSON :type "VaRestJsonObject Object Reference"))
  (bind _json (`parent.Save Data`))
  (`VaRestJsonObject.SetIntegerField` _json "State" (`KismetMathLibrary.Conv_ByteToInt` (`self.State`)))
  (return _json))

(fn `UserConstructionScript`
  (`parent.UserConstructionScript`))
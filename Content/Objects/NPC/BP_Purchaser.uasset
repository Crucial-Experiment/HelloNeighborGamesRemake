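; BP_Purchaser is a cart-pushing shopper NPC that hunts the player and restarts the level on catching them.
; On spawn it attaches a random item from the CashBox's NeedPurchases list.
; PawnSensing spots standing or fast-moving characters, setting the blackboard target and enabling the light, creak audio and catch box.
; A looping timer drops the chase once the player crouches.
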(event `self.ReceiveBeginPlay`
  (bind _asbp_student_anim (cast `/Game/Objects/NPC/AI/BP_Student_Anim` (`SkeletalMeshComponent.GetAnimInstance` (`self.Mesh`))))
  (set `/Game/Objects/NPC/AI/BP_Student_Anim.Cart` 1.0 _asbp_student_anim)
  (bind _returnvalue (`GameplayStatics.GetActorOfClass` "/Game/Objects/BP_Objects/BP_CashBox.BP_CashBox_C"))
  (`/Engine/EditorBlueprintResources/StandardMacros.IsValid` _returnvalue
    (:`Is Valid`
      (bind _returnvalue_2 (`|SpawnActorFromClass` (`KismetArrayLibrary.Array_Random` (`/Game/Objects/BP_Objects/BP_CashBox.Need Purchases` _returnvalue)) (`KismetMathLibrary.MakeTransform` (0.0 0.0 0.0)) "Undefined" "MultiplyWithRoot" null null))
      (`/Game/Objects/Structurs/BP_Object.Set Flat Mode` _returnvalue_2 "NewEnumerator1")
      (`self.SetActorEnableCollision` _returnvalue_2 false)
      (`self.K2_AttachToComponent` _returnvalue_2 (`self.Scene`) "None" "SnapToTarget" "SnapToTarget" "SnapToTarget" true))))

(event `Player is Crouch`
  (if (`Character.bIsCrouched` (`self.Player`))
    (set `self.Player` null)
    (`BlackboardComponent.SetValueAsObject` (`AIBlueprintHelperLibrary.GetBlackboard` null) "Player" null)
    (`SceneComponent.SetVisibility` (`self.PointLight`) false false)
    (set `PrimitiveComponent.bGenerateOverlapEvents` false (`self.Box`))
    (`KismetSystemLibrary.K2_ClearAndInvalidateTimerHandle` (`self.Crouch Timer`))
    (`AudioComponent.Stop` (`self.Creak`))))

(event `self.PawnSensing.OnSeePawn`
  (params (Pawn :type "Pawn Object Reference"))
  (bind _player (`self.Player`))
  (bind _ascharacter (cast `Character` Pawn))
  (bind _output_get (set `self.Player` _ascharacter))
  (if (not (`Character.bIsCrouched` _player))
    (`BlackboardComponent.SetValueAsObject` (`AIBlueprintHelperLibrary.GetBlackboard` null) "Player" _output_get :!label _label)
    (`SceneComponent.SetVisibility` (`self.PointLight`) true false)
    (set `PrimitiveComponent.bGenerateOverlapEvents` true (`self.Box`))
    (bind _returnvalue (`KismetSystemLibrary.K2_SetTimerDelegate` (delegate `Player is Crouch`) 0.8 true true))
    (set `self.Crouch Timer` _returnvalue)
    (`AudioComponent.Play` (`self.Creak`) 0.0)
    (elif (>= (`KismetMathLibrary.VSize` (`self.GetVelocity` _player)) 100.0)
      (goto _label))))

(event `self.Box.OnComponentBeginOverlap`
  (params (OverlappedComponent :type "PrimitiveComponent Object Reference") (OtherActor :type "Actor Object Reference") (OtherComp :type "PrimitiveComponent Object Reference") (OtherBodyIndex :type Integer) (bFromSweep :type Boolean) (SweepResult :type "HitResult Structure (by ref)"))
  (bind _asbp_player (cast `/Game/Player/BP_Player` OtherActor))
  (`AudioComponent.Stop` (`self.Creak`))
  (`AudioComponent.Play` (`self.Catch`) 0.0)
  (`self.DisableInput` _asbp_player (`GameplayStatics.GetPlayerController` 0))
  (`KismetSystemLibrary.Delay` 2.0)
  (bind _returnvalue (`GameplayStatics.GetCurrentLevelName` true))
  (`GameplayStatics.OpenLevel` (`KismetStringLibrary.Conv_StringToName` _returnvalue)))

(fn `UserConstructionScript`)
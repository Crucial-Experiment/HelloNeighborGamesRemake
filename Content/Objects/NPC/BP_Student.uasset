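; BP_Student is an NPC that pursues and catches the player, restarting the level on contact.
; Seeing a pawn while not inactive writes it to the Blackboard as Player and turns on a point light.
; SetState toggles the inactive state, assigning or clearing a random school table in the Blackboard, switching catch overlaps and hiding the light.
; Touching BP_Player plays Catch, disables input and reloads the level after a delay.
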(event `Set State`
  (bind _returnvalue (`AIBlueprintHelperLibrary.GetBlackboard` null))
  (bind _box (`self.Box`))
  (if (not (`self.Inaction`))
    (set `self.Inaction` true)
    (bind _outactors (`GameplayStatics.GetAllActorsOfClass` "/Game/Objects/BP_Objects/BP_School_Table.BP_School_Table_C"))
    (`BlackboardComponent.SetValueAsObject` _returnvalue "School Table" (`KismetArrayLibrary.Array_Random` _outactors))
    (set `PrimitiveComponent.bGenerateOverlapEvents` false _box)
    (else
      (set `self.Inaction` false)
      (`BlackboardComponent.SetValueAsObject` _returnvalue "School Table" null)
      (set `PrimitiveComponent.bGenerateOverlapEvents` true _box)))
  (`SceneComponent.SetVisibility` (`self.PointLight`) false false))

(event `self.PawnSensing.OnSeePawn`
  (params (Pawn :type "Pawn Object Reference"))
  (if (not (`self.Inaction`))
    (`BlackboardComponent.SetValueAsObject` (`AIBlueprintHelperLibrary.GetBlackboard` null) "Player" Pawn)
    (`SceneComponent.SetVisibility` (`self.PointLight`) true false)))

(event `self.Box.OnComponentBeginOverlap`
  (params (OverlappedComponent :type "PrimitiveComponent Object Reference") (OtherActor :type "Actor Object Reference") (OtherComp :type "PrimitiveComponent Object Reference") (OtherBodyIndex :type Integer) (bFromSweep :type Boolean) (SweepResult :type "HitResult Structure (by ref)"))
  (bind _asbp_player (cast `/Game/Player/BP_Player` OtherActor))
  (`AudioComponent.Play` (`self.Catch`) 0.0)
  (`self.DisableInput` _asbp_player (`GameplayStatics.GetPlayerController` 0))
  (`KismetSystemLibrary.Delay` 2.0)
  (bind _returnvalue (`GameplayStatics.GetCurrentLevelName` true))
  (`GameplayStatics.OpenLevel` (`KismetStringLibrary.Conv_StringToName` _returnvalue)))

(fn `UserConstructionScript`)
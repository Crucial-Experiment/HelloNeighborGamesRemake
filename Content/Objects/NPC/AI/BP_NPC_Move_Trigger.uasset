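; Trigger box that sends the FakeSosed NPC to a preset AnimPoint when the player overlaps it or Execute is called.
; After a delay it disables overlap events, signals the NPC's state change, sets walk speed and writes blackboard keys for the target point and non-random movement.
; It also plays an optional sound with an optional timed stop, then fires OnTouch.
; Only the Execute path first switches the NPC's mesh to Animation Blueprint mode.
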(event `Execute`
  (bind _sound (`self.Sound`))
  (bind _audio (`self.Audio`))
  (bind _stop_delay (`self.Stop Delay`))
  (bind _fake_sosed (`/Game/Function/BP_MacroLibrary.Find Fake Sosed`)
    (:`Is Valid`
      (`SkeletalMeshComponent.SetAnimationMode` (`Character.Mesh` _fake_sosed) "AnimationBlueprint" true))
    (:`Is Not Valid`
      _))
  (`KismetSystemLibrary.Delay` (`self.Delay`) :!label _label)
  (`|ExecutionSequence`
    (:`then_0`
      (set `PrimitiveComponent.bGenerateOverlapEvents` false (`self.Box`)))
    (:`then_1`
      (bind _fake_sosed_2 (`/Game/Function/BP_MacroLibrary.Find Fake Sosed`)
        (:`Is Valid`
          (`/Game/Objects/NPC/BP_Fake_Sosed.On State Change` _fake_sosed_2)
          (set `CharacterMovementComponent.MaxWalkSpeed` (`self.Max Walk Speed`) (`Character.CharacterMovement` _fake_sosed_2))
          (bind _returnvalue (`AIBlueprintHelperLibrary.GetBlackboard` _fake_sosed_2))
          (`BlackboardComponent.SetValueAsObject` _returnvalue "Point" (`self.Anim Point`))
          (`BlackboardComponent.SetValueAsBool` _returnvalue "RandomMove" false))))
    (:`then_2`
      (`/Engine/EditorBlueprintResources/StandardMacros.IsValid` _sound
        (:`Is Valid`
          (`AudioComponent.SetSound` _audio _sound)
          (set `AudioComponent.bOverrideAttenuation` (`self.Override Attenuation`) _audio)
          (`AudioComponent.Play` _audio 0.0)
          (if (!= _stop_delay 0.0)
            (`KismetSystemLibrary.Delay` _stop_delay)
            (`AudioComponent.Stop` _audio)))))
    (:`then_3`
      (`self.On Touch`))))

(event `self.Box.OnComponentBeginOverlap`
  (params (OverlappedComponent :type "PrimitiveComponent Object Reference") (OtherActor :type "Actor Object Reference") (OtherComp :type "PrimitiveComponent Object Reference") (OtherBodyIndex :type Integer) (bFromSweep :type Boolean) (SweepResult :type "HitResult Structure (by ref)"))
  (cast `/Game/Player/BP_Player` OtherActor)
  (goto _label))

(fn `UserConstructionScript`)
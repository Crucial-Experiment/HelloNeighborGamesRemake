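; BP_Teacher is an AI NPC that spots pawns and catches the player, restarting the level.
; SetState toggles Inaction, switching its light, blackboard RandomMove flag and catch-box overlaps; BeginPlay starts with movement flag and overlaps off.
; While not inactive, PawnSensing writes any seen pawn to the blackboard's Player key.
; Box overlap with BP_Player plays Catch, disables input, then reloads the current level after a short delay.
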(event `self.ReceiveBeginPlay`
  (`BlackboardComponent.SetValueAsBool` (`AIBlueprintHelperLibrary.GetBlackboard` null) "RandomMove" false :!label _label)
  (set `PrimitiveComponent.bGenerateOverlapEvents` false (`self.Box`)))

(event `Set State`
  (bind _pointlight (`self.PointLight`))
  (if (not (`self.Inaction`))
    (set `self.Inaction` true)
    (`SceneComponent.SetVisibility` _pointlight false false)
    (goto _label)
    (else
      (set `self.Inaction` false)
      (`SceneComponent.SetVisibility` _pointlight true false)
      (`BlackboardComponent.SetValueAsBool` (`AIBlueprintHelperLibrary.GetBlackboard` null) "RandomMove" true)
      (set `PrimitiveComponent.bGenerateOverlapEvents` true (`self.Box`)))))

(event `self.PawnSensing.OnSeePawn`
  (params (Pawn :type "Pawn Object Reference"))
  (if (not (`self.Inaction`))
    (`BlackboardComponent.SetValueAsObject` (`AIBlueprintHelperLibrary.GetBlackboard` null) "Player" Pawn)))

(event `self.Box.OnComponentBeginOverlap`
  (params (OverlappedComponent :type "PrimitiveComponent Object Reference") (OtherActor :type "Actor Object Reference") (OtherComp :type "PrimitiveComponent Object Reference") (OtherBodyIndex :type Integer) (bFromSweep :type Boolean) (SweepResult :type "HitResult Structure (by ref)"))
  (bind _asbp_player (cast `/Game/Player/BP_Player` OtherActor))
  (`AudioComponent.Play` (`self.Catch`) 0.0)
  (`self.DisableInput` _asbp_player (`GameplayStatics.GetPlayerController` 0))
  (`KismetSystemLibrary.Delay` 2.0)
  (bind _returnvalue (`GameplayStatics.GetCurrentLevelName` true))
  (`GameplayStatics.OpenLevel` (`KismetStringLibrary.Conv_StringToName` _returnvalue)))

(fn `UserConstructionScript`)
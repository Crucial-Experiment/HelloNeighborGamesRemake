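; BP_Rotate is an interactive hinged door that can be locked, chair-blocked or rigged with a bucket, saving state as JSON.
; Interact checks the blockers, then makes AI noise and toggles a timeline-driven rotation; RemoteOpen skips the checks.
; Opening and closing play sounds and message linked actors, while interacting triggers any bucket's temporary post-process effect.
; Construction places props and sets the nav link, marking chair, bucket or auto-locked doors as low-height nav areas.
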(event `On Door Open`
  ;[1 1 1] On Door Open / Close
  (for _array_element (`self.On Open`)
    (message `/Game/Function/BP_Interface.Interact` _array_element null (`self.K2_GetActorLocation`))))

(event `On Door Close`
  ;[1 1 1] On Door Open / Close
  (for _array_element (`self.On Close`)
    (message `/Game/Function/BP_Interface.Interact` _array_element null (`self.K2_GetActorLocation`))))

(event `Remove Rotate`
  ;[1 1 1] Begin Play
  (`ActorComponent.K2_DestroyComponent` (`self.Rotate`)))

(event `self.ReceiveBeginPlay`
  ;[1 1 1] Begin Play
  (`|ExecutionSequence`
    (:`then_0`
      (bind _chair (`self.Chair`)
        (:`then`
          (set `/Game/Objects/BP_Objects/BP_Chair.Rotate` self _chair)
          (`self.Connect Chair`))
        (:`else`)))
    (:`then_1`
      (add `self.Door Open` (delegate `On Door Open`))
      (add `self.Door Close` (delegate `On Door Close`))
      (add `self.Spawn Door Part` (delegate `Remove Rotate`)))
    (:`then_2`
      (bind _bucket (`self.Bucket`)
        (:`then`
          (set `/Game/Objects/BP_Objects/BP_Bucket_2.Rotate` self _bucket))
        (:`else`)))))

(event `/Game/Function/BP_Interface.Interact`
  (params (Component :type "PrimitiveComponent Object Reference") (Location :type "Vector Structure"))
  (bind _tutorialcomponent (`self.TutorialComponent`))
  (bind (_rotate_b_roll _rotate_b_pitch _rotate_b_yaw) (`KismetMathLibrary.BreakRotator` (`self.Rotate B`)))
  (bind (_rotate_b_roll_2 _rotate_b_pitch_2 _rotate_b_yaw_2) (`KismetMathLibrary.BreakRotator` (`self.Rotate B`)))
  (bind _open_sound (`self.Open Sound`))
  (bind _close_sound (`self.Close Sound`))
  (bind _bucket_post_process (`self.Bucket Post Process`))
  ;[1 1 1] Event Interact and Remote Open
  (if (== Component (`self.Rotate`))
    (`/Game/Objects/Tutorial/TutorialComponent.Check Use Type` (`self.TutorialComponent`) "NewEnumerator6")
    (`/Game/Objects/GameJolt/GameJoltComponent.Check Use Type` (`self.GameJoltComponent`) "NewEnumerator6")
    (if (and (== (`KismetArrayLibrary.Array_Length` (`self.Locks`)) 0) (not (`KismetSystemLibrary.IsValid` (`self.Chair`))) (not (`self.Auto Lock`)) (not (`self.Start Look`)))
      (`|ExecutionSequence`
        (:`then_0`
          (`self.MakeNoise` 1.0 (`GameplayStatics.GetPlayerPawn` 0) (`self.K2_GetActorLocation`) 45.0))
        (:`then_1`
          (switch `/Game/Objects/Enum/RotateStateEnum` (`self.Rotate State`) :!label _label
            (:`NewEnumerator0`
              (set `self.Rotate State` "NewEnumerator3")
              ;;[1 1 1] Rotate
              (`/Game/Objects/Tutorial/TutorialComponent.Check Use Type` _tutorialcomponent "NewEnumerator2")
              (bind (_direction _alpha) (`Timeline|Rotate Timeline` :!via `Reverse` :!label _label_2)
                (:`Update`
                  (`SceneComponent.K2_SetRelativeRotation` (`self.Rotate`) (`KismetMathLibrary.RLerp` (`self.Rotate A`) (`KismetMathLibrary.MakeRotator` _rotate_b_roll_2 _rotate_b_pitch_2 (select `bool` false :`false` _rotate_b_yaw_2 :`true` (`KismetMathLibrary.SelectFloat` _rotate_b_yaw -100.0 (>= (`KismetMathLibrary.Dot_VectorVector` (`KismetMathLibrary.GetDirectionUnitVector` (`self.K2_GetActorLocation`) Location) (`self.GetActorForwardVector`)) 0.0)) :!type "Float (double-precision)")) _alpha) false false))
                (:`Finished`
                  (switch `/Game/Objects/Enum/RotateStateEnum` (`self.Rotate State`)
                    (:`NewEnumerator2`
                      (set `self.Rotate State` "NewEnumerator0"))
                    (:`NewEnumerator3`
                      (set `self.Rotate State` "NewEnumerator1")
                      (`self.Door Close`)
                      ;;[1 1 1] Close Sound
                      (`/Engine/EditorBlueprintResources/StandardMacros.IsValid` _close_sound
                        (:`Is Valid`
                          (`GameplayStatics.PlaySoundAtLocation` _close_sound (`self.K2_GetActorLocation`) (struct) 1.0 1.0 0.0 (`self.Attenuation Settings`) null null null))))))))
            (:`NewEnumerator1`
              (set `self.Rotate State` "NewEnumerator2")
              (`|ExecutionSequence`
                (:`then_0`
                  (`/Game/Objects/Tutorial/TutorialComponent.Check Use Type` _tutorialcomponent "NewEnumerator1")
                  (goto _label_2))
                (:`then_1`
                  ;;[1 1 1] Open Sound
                  (`/Engine/EditorBlueprintResources/StandardMacros.IsValid` _open_sound
                    (:`Is Valid`
                      (`GameplayStatics.PlaySoundAtLocation` _open_sound (`self.K2_GetActorLocation`) (struct) 1.0 1.0 0.0 (`self.Attenuation Settings`) null null null))))
                (:`then_2`
                  (`self.Door Open`))))))
        (:`then_2`
          (bind _bucket (`self.Bucket`)
            (:`then`
              (`/Game/Objects/Structurs/BP_Object.Set Flat Mode` _bucket "NewEnumerator0")
              (set `PostProcessComponent.bEnabled` true _bucket_post_process)
              (bind _watercomponent (`/Game/Objects/BP_Objects/BP_Bucket_2.WaterComponent` _bucket))
              (set `/Game/Objects/Structurs/WaterComponent.Fill` 0.0 _watercomponent)
              (`/Game/Objects/Structurs/WaterComponent.Update Water Box` _watercomponent)
              (`KismetSystemLibrary.Delay` 4.5)
              (set `PostProcessComponent.bEnabled` false _bucket_post_process))
            (:`else`))))
      (else
        (`GameplayStatics.PlaySoundAtLocation` (`self.Lock Sound`) (`self.K2_GetActorLocation`) (struct) 1.0 1.0 0.0 (`self.Attenuation Settings`) null null null)))))

(event `Remote Open`
  ;[1 1 1] Event Interact and Remote Open
  (goto _label))

(event `Check Bucket`
  (bind (_returnvalue_location _returnvalue_rotation) (`KismetMathLibrary.BreakTransform` (`SceneComponent.K2_GetComponentToWorld` (`self.Bucket Loc`))))
  ;[1 1 1] Check Bucket
  (bind _bucket (`self.Bucket`)
    (:`then`
      (`SceneComponent.K2_SetRelativeRotation` (`self.Rotate`) (struct :`Yaw` 25.0) false false)
      (`/Game/Objects/Structurs/BP_Object.Set Flat Mode` _bucket "NewEnumerator1")
      (`self.K2_SetActorLocationAndRotation` _bucket _returnvalue_location _returnvalue_rotation false true)
      (`NavModifierComponent.SetAreaClass` (`self.NavModifier`) "/Script/NavigationSystem.NavArea_LowHeight")
      (`/Game/Objects/BP_Objects/BP_Bucket_2.Rotate` _bucket
        (:`then`)
        (:`else`
          (set `/Game/Objects/BP_Objects/BP_Bucket_2.Rotate` self _bucket))))
    (:`else`)))

(fn `Connect Chair`
  (bind _chair (`self.Chair`))
  (if (and (`KismetSystemLibrary.IsValid` _chair) (`self.Can Place Chair`))
    (`/Game/Objects/Structurs/BP_Object.Set Flat Mode` _chair "NewEnumerator1")
    (`self.K2_AttachToComponent` _chair (`self.Scene`) "None" "SnapToTarget" "SnapToTarget" "KeepWorld" true)
    (`NavModifierComponent.SetAreaClass` (`self.NavModifier`) "/Script/NavigationSystem.NavArea_LowHeight")
    (elif (not (`self.Auto Lock`))
      (`NavModifierComponent.SetAreaClass` (`self.NavModifier`) "/Script/NavigationSystem.NavArea_Default"))))

(fn `Load Data`
  (params (JSON :type String))
  (returns (Object :type "VaRestJsonObject Object Reference"))
  (locals (`JSON Object` :type "VaRestJsonObject Object Reference"))
  (bind _json_object (`local.JSON Object`))
  (bind (_has_field_ _return_value) (`/Game/Function/BP_JSON_FunctionLibrary.Get Value As Int` _json_object "Material"))
  (bind (_has_field__2 _return_value_2) (`/Game/Function/BP_JSON_FunctionLibrary.Get Value As Int` (`local.JSON Object`) "State"))
  (bind (_has_field__3 _return_value_3) (`/Game/Function/BP_JSON_FunctionLibrary.Get Value As Bool` _json_object "Auto Lock"))
  (bind _returnvalue (`VaRestSubsystem.ConstructVaRestJsonObject` (subsystem `VaRestSubsystem`)))
  (bind _output_get (set `local.JSON Object` _returnvalue))
  (bind _returnvalue_2 (`VaRestJsonObject.DecodeJson` _output_get JSON true))
  (if _returnvalue_2
    (`|ExecutionSequence`
      (:`then_0`
        (if _has_field__3
          (set `self.Auto Lock` _return_value_3)))
      (:`then_1`
        (if _has_field_
          (set `self.Material` (cast `/Game/Objects/Enum/DoorMaterialEnim` (`KismetMathLibrary.Conv_IntToByte` _return_value)))))
      (:`then_2`
        (if (and _has_field__2 (!= _return_value_2 (`KismetMathLibrary.Conv_ByteToInt` (`self.Rotate State`))))
          (`self.Interact` (`self.Rotate`))))
      (:`then_3`
        (return (`local.JSON Object`))))))

(fn `Save Data`
  (returns (JSON :type "VaRestJsonObject Object Reference"))
  (if (`self.Need Save`)
    (return (`|MakeJson` (`KismetMathLibrary.Conv_IntToDouble` (`KismetMathLibrary.Conv_ByteToInt` (`self.Rotate State`))) (`self.Auto Lock`) (`KismetMathLibrary.Conv_IntToDouble` (`KismetMathLibrary.Conv_ByteToInt` (`self.Material`)))))))

(fn `UserConstructionScript`
  (bind _rotate (`self.Rotate`))
  (`|ExecutionSequence`
    (:`then_0`
      (switch `/Game/Objects/Enum/RotateStateEnum` (`self.Rotate State`)
        (:`NewEnumerator0`
          (`SceneComponent.K2_SetRelativeRotation` _rotate (struct :`Yaw` 100.0) false false))
        (:`NewEnumerator1`
          (`SceneComponent.K2_SetRelativeRotation` :`self` _rotate))))
    (:`then_1`
      (`self.Connect Chair`))
    (:`then_2`
      (bind _asbp_nav_link_proxy (cast `/Game/Objects/Structurs/BP_NavLinkProxy` (`ChildActorComponent.ChildActor` (`self.Nav Link Proxy`))))
      (`/Game/Objects/Structurs/BP_NavLinkProxy.Set Nav Link` _asbp_nav_link_proxy (`self.Left`) (`self.Right`) (`self.Direction`)))
    (:`then_3`
      (`self.Check Bucket`))
    (:`then_4`
      (if (`self.Auto Lock`)
        (`NavModifierComponent.SetAreaClass` (`self.NavModifier`) "/Script/NavigationSystem.NavArea_LowHeight")))))
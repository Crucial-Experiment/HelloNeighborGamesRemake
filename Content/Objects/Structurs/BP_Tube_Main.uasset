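; BP_Tube_Main is a switchable tube that passes water through a network of linked tubes.
; SetState toggles it On or Off, then calls StartChild or StopChild, which recursively update HasWater on the Child tubes.
; Water spreads only through On tubes that are Generators or already have water, while stopping clears all downstream tubes.
; WaterMove plays during flow, and WaterEnd plays when a supplied tube is switched off.
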(event `Stop Child`
  (for _array_element (`self.Child`)
    (set `/Game/Objects/Structurs/BP_Tube_Main.Has Water` false _array_element)
    (`AudioComponent.Stop` (`self.water_move`))
    (`self.Stop Child` _array_element)))

(event `Set State`
  (bind _water_end (`self.water_end`))
  (switch `/Game/Objects/Enum/TumblerStateEnum` (`self.State`)
    (:`NewEnumerator0`
      (set `self.State` "NewEnumerator1")
      (if (or (`self.Has Water`) (`self.Generator`))
        (`AudioComponent.Stop` (`self.water_move`))
        (`AudioComponent.Play` _water_end 0.0))
      (`self.Stop Child`))
    (:`NewEnumerator1`
      (set `self.State` "NewEnumerator0")
      (`AudioComponent.Stop` _water_end)
      (`self.Start Child`))))

(event `Start Child`
  (if (and (or (`self.Has Water`) (`self.Generator`)) (`|EnumEquality` (`self.State`) "NewEnumerator0"))
    (for _array_element (`self.Child`)
      (set `/Game/Objects/Structurs/BP_Tube_Main.Has Water` true _array_element)
      (`self.Start Child` _array_element))
    (`AudioComponent.Play` (`self.water_move`) 0.0)))

(fn `UserConstructionScript`
  (`parent.UserConstructionScript`))
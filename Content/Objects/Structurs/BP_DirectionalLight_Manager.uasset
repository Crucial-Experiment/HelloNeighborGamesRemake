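; BP_DirectionalLight_Manager is a placeable actor that supplies a directional light on the Mobile platform.
; On BeginPlay it checks the current platform and, only for Mobile, spawns a DirectionalLight at its own transform.
; It then copies its color, intensity, temperature and shadow-casting settings onto the new light.
; The construction script tints an Arrow component with the light color as a preview.
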(event `self.ReceiveBeginPlay`
  (switch `/Game/UMG/EPlatform` (`/Game/Function/BP_FunctionLibrary.Get Current Platform`)
    (:`NewEnumerator2`
      (bind _returnvalue (`|SpawnActorFromClass` "/Script/Engine.DirectionalLight" (`self.GetTransform`) "Undefined" "MultiplyWithRoot" null null))
      (bind _lightcomponent (`Light.LightComponent` _returnvalue))
      (`LightComponent.SetLightColor` _lightcomponent (`self.Light Color`) true)
      (`LightComponent.SetIntensity` _lightcomponent (`self.Intensity`))
      (`LightComponent.SetUseTemperature` _lightcomponent (`self.Use Temperature`))
      (`LightComponent.SetTemperature` _lightcomponent (`self.Temperature`))
      (`LightComponentBase.SetCastShadows` _lightcomponent (`self.Cast Shadows`)))))

(fn `UserConstructionScript`
  (`ArrowComponent.SetArrowColor` (`self.Arrow`) (`self.Light Color`)))
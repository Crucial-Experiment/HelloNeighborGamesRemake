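; BP_Lock is a lock object that registers itself with a linked Rotate object and becomes a pickup when unlocked.
; On BeginPlay it auto-locks if Rotate is valid, joining its Locks list and disabling pickup.
; Unlocking leaves that list, switches flat mode and grab type, plays a sound, and notifies tutorial and GameJolt components.
; Construction applies color parameters to the material, and save data stores the lock state, replaying Unlock on load.
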(event `self.ReceiveBeginPlay`
  ;[1 1 1] Auto Lock
  (`parent.ReceiveBeginPlay`)
  (`self.Rotate`
    (:`then`
      (`self.Lock`))
    (:`else`)))

(event `Unlock`
  (bind _rotate (`self.Rotate`))
  ;[1 1 1] Unlock
  (`self.Unlock Event`)
  (`|ExecutionSequence`
    (:`then_0`
      (`/Engine/EditorBlueprintResources/StandardMacros.IsValid` _rotate
        (:`Is Valid`
          (`KismetArrayLibrary.Array_RemoveItem` (`/Game/Objects/Structurs/BP_Rotate.Locks` _rotate) self))))
    (:`then_1`
      (`self.Set Flat Mode` "NewEnumerator0")
      (set `self.CanPickUp` true)
      (`GameplayStatics.PlaySoundAtLocation` (`self.Unlock Sound`) (`self.K2_GetActorLocation`) (struct) 1.0 1.0 0.0 null null null null)
      (set `/Game/Objects/Structurs/GrabComponent.GrabType` "NewEnumerator4" (`self.GrabComponent`))
      (`/Game/Objects/Tutorial/TutorialComponent.Check Use Type` (`self.TutorialComponent`) "NewEnumerator6")
      (`/Game/Objects/GameJolt/GameJoltComponent.Check Use Type` (`self.GameJoltComponent`) "NewEnumerator6"))))

(event `Lock`
  (bind _rotate (`self.Rotate`))
  ;[1 1 1] Lock
  (`self.Lock Event`)
  (`|ExecutionSequence`
    (:`then_0`
      (`/Engine/EditorBlueprintResources/StandardMacros.IsValid` _rotate
        (:`Is Valid`
          (`KismetArrayLibrary.Array_Add` (`/Game/Objects/Structurs/BP_Rotate.Locks` _rotate) self))))
    (:`then_1`
      (`self.Set Flat Mode` "NewEnumerator1")
      (set `self.CanPickUp` false)
      (set `/Game/Objects/Structurs/GrabComponent.GrabType` "NewEnumerator0" (`self.GrabComponent`)))))

(fn `Load Data`
  (params (JSON :type String))
  (returns (Object :type "VaRestJsonObject Object Reference"))
  (bind _object (`parent.Load Data` JSON))
  (`|ExecutionSequence`
    (:`then_0`
      (bind (_has_field_ _return_value) (`/Game/Function/BP_JSON_FunctionLibrary.Get Value As Bool` _object "State"))
      (if (and _has_field_ (not _return_value))
        (`self.Unlock`)))
    (:`then_1`
      (return _object))))

(fn `Save Data`
  (returns (JSON :type "VaRestJsonObject Object Reference"))
  (bind _json (`parent.Save Data`))
  (`VaRestJsonObject.SetBoolField` _json "State" (and (`|EnumEquality` (`/Game/Objects/Structurs/FlatComponent.Mode` (`self.FlatComponent`)) "NewEnumerator1") (not (`self.CanPickUp`))))
  (return _json))

(fn `UserConstructionScript`
  (`parent.UserConstructionScript`)
  (`MeshComponent.SetVectorParameterValueOnMaterials` (`self.Root`) "color" (`KismetMathLibrary.Conv_LinearColorToVector` (`self.Color`)))
  (`MeshComponent.SetScalarParameterValueOnMaterials` (`self.Root`) "Contrast" (`self.Contrast`))
  (`MeshComponent.SetScalarParameterValueOnMaterials` (`self.Root`) "Desaturation" (`self.Desaturation`)))
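; Interactable physics object for flat-screen and VR play, with empty use-event hooks, tutorial/GameJolt use checks and impact sounds.
; FlatComponent's mode drives its state: free, fixed, inventory, deleted (moved far away) or attached to Sosed's belt.
; GrabComponent handles VR grabs, adding per-hand trigger input, socket snapping and custom hand poses or visibility.
; Helpers provide hand-or-camera line traces, grip release, hand overlap tests and JSON save/load of mode and position.
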(event `On Item Dropped`
  (bind _flatcomponent (`self.FlatComponent`))
  (`/Game/Objects/Tutorial/TutorialComponent.Check Use Type` (`self.TutorialComponent`) "NewEnumerator5")
  (`/Game/Objects/GameJolt/GameJoltComponent.Check Use Type` (`self.GameJoltComponent`) "NewEnumerator5")
  (remove `/Game/Objects/Structurs/FlatComponent.Slot Change` _flatcomponent (delegate `On Slot Change`))
  (remove `/Game/Objects/Structurs/FlatComponent.Taken` _flatcomponent (delegate `On Item Taken`))
  (remove `/Game/Objects/Structurs/FlatComponent.Dropped` _flatcomponent (delegate `On Item Dropped`))
  (bind _player (`/Game/Function/BP_MacroLibrary.Find Player`)
    (:`Is Valid`
      (remove `/Game/Player/BP_Player.Left Mouse Button` _player (delegate `On Press LMB`))
      (remove `/Game/Player/BP_Player.Right Mouse Button` _player (delegate `On Press RMB`)))))

(event `On Slot Change`)

(event `On Item Taken`)

(event `On Press LMB`)

(event `On Press RMB`)

(event `EnhancedInput|/Game/Player/VR/Input/Actions/IA_Trigger_Left`
  (params (ActionValue :type Boolean) (ElapsedSeconds :type "Float (double-precision)") (TriggeredSeconds :type "Float (double-precision)") (InputAction :type "InputAction Object Reference" :default "/Game/Player/VR/Input/Actions/IA_Trigger_Left.IA_Trigger_Left"))
  ;[1 1 1] VR Triggers
  (:`Started`
    (if (`|EnumEquality` (`/Game/Objects/Structurs/GrabComponent.GetHeldByHand` (`self.GrabComponent`)) "Left")
      (`self.VR Left Trigger` self))))

(event `/Game/Function/BP_Interface.PickUp`
  (bind _flatcomponent (`self.FlatComponent`))
  ;[1 1 1] Pick Up and Begin Play
  (if (`self.CanPickUp`) :!label _label
    (`|ExecutionSequence`
      (:`then_0`
        (`/Game/Objects/Structurs/FlatComponent.Add Item To Inventory` (`self.FlatComponent`) self))
      (:`then_1`
        (add `/Game/Objects/Structurs/FlatComponent.Slot Change` _flatcomponent (delegate `On Slot Change`))
        (add `/Game/Objects/Structurs/FlatComponent.Taken` _flatcomponent (delegate `On Item Taken`))
        (add `/Game/Objects/Structurs/FlatComponent.Dropped` _flatcomponent (delegate `On Item Dropped`))
        (bind _player (`/Game/Function/BP_MacroLibrary.Find Player`)
          (:`Is Valid`
            (add `/Game/Player/BP_Player.Left Mouse Button` _player (delegate `On Press LMB`))
            (add `/Game/Player/BP_Player.Right Mouse Button` _player (delegate `On Press RMB`)))))
      (:`then_2`
        ;[1 1 1] Tutorial
        (`/Game/Objects/Tutorial/TutorialComponent.Check Use Type` (`self.TutorialComponent`) "NewEnumerator0"))
      (:`then_3`
        ;[1 1 1] GameJolt
        (`/Game/Objects/GameJolt/GameJoltComponent.Check Use Type` (`self.GameJoltComponent`) "NewEnumerator0")))))

(event `self.ReceiveBeginPlay`
  (bind _mode (`/Game/Objects/Structurs/FlatComponent.Mode` (`self.FlatComponent`)))
  ;[1 1 1] Pick Up and Begin Play
  (`PrimitiveComponent.SetMassOverrideInKg` (`self.Root`) "None" (`self.Mass Scale`) true)
  (`self.Set Flat Mode` _mode)
  (set `/Game/Objects/Structurs/GrabComponent.GrabType` (select `bool` (`self.CanPickUp`) :`false` "NewEnumerator0" :`true` "NewEnumerator4" :!type "/Game/Objects/Enum/GrabType Enum") (`self.GrabComponent`))
  (set `self.Game Start Transform` (`self.GetTransform`))
  (set `self.Game Start Flat Mode` _mode)
  (switch `/Game/Objects/Enum/FlatModeEnum` _mode
    (:`NewEnumerator4`
      (`KismetSystemLibrary.Delay` 0.2)
      (goto _label))))

(event `EnhancedInput|/Game/Player/VR/Input/Actions/IA_Trigger_Right`
  (params (ActionValue :type Boolean) (ElapsedSeconds :type "Float (double-precision)") (TriggeredSeconds :type "Float (double-precision)") (InputAction :type "InputAction Object Reference" :default "/Game/Player/VR/Input/Actions/IA_Trigger_Right.IA_Trigger_Right"))
  ;[1 1 1] VR Triggers
  (:`Started`
    (if (`|EnumEquality` (`/Game/Objects/Structurs/GrabComponent.GetHeldByHand` (`self.GrabComponent`)) "Right")
      (`self.VR Right Trigger` self))))

(event `self.Root.OnComponentHit`
  (params (HitComponent :type "PrimitiveComponent Object Reference") (OtherActor :type "Actor Object Reference") (OtherComp :type "PrimitiveComponent Object Reference") (NormalImpulse :type "Vector Structure") (Hit :type "HitResult Structure (by ref)"))
  (bind _flatcomponent (`self.FlatComponent`))
  (bind _hit_sound (`/Game/Objects/Structurs/FlatComponent.Hit Sound` (`self.FlatComponent`)))
  ;[1 1 1] Hit
  (`/Engine/EditorBlueprintResources/StandardMacros.CompareFloat` (`KismetMathLibrary.VSize` NormalImpulse) (`/Game/Objects/Structurs/FlatComponent.Hit Compare` (`self.FlatComponent`))
    (:`>`
      (`/Engine/EditorBlueprintResources/StandardMacros.DoOnce` false :!label _label_2
        (:`Completed`
          (`|ExecutionSequence`
            (:`then_0`
              (`/Engine/EditorBlueprintResources/StandardMacros.IsValid` _hit_sound
                (:`Is Valid`
                  (`GameplayStatics.PlaySoundAtLocation` _hit_sound (`.Location` (`GameplayStatics.BreakHitResult` Hit)) (struct) 1.0 1.0 0.0 (select `/Game/Sounds/Attenuation/AttenuationEnum` (`/Game/Objects/Structurs/FlatComponent.Hit Attenuation` _flatcomponent) :`NewEnumerator0` "/Game/Sounds/Attenuation/Silent.Silent" :`NewEnumerator1` "/Game/Sounds/Attenuation/Middle.Middle" :`NewEnumerator2` "/Game/Sounds/Attenuation/Loud.Loud" :`NewEnumerator3` "/Game/Sounds/Attenuation/Epic.Epic" :!type "SoundAttenuation Object Reference") null null null)
                  (`KismetSystemLibrary.Delay` 0.4)
                  (goto _label_2 :!via `Reset`))))
            (:`then_1`
              (switch `/Game/Objects/Enum/FlatModeEnum` (`/Game/Objects/Structurs/FlatComponent.Mode` _flatcomponent)
                (:`NewEnumerator5`
                  (`self.Set Flat Mode` "NewEnumerator0"))))))))))

(event `self.GrabComponent.OnGrabbed`
  (params (`Self Ref` :type "/Game/Objects/Structurs/GrabComponent Object Reference"))
  (bind _flatcomponent (`self.FlatComponent`))
  (bind _flatcomponent_2 (`self.FlatComponent`))
  (bind _flatcomponent_3 (`self.FlatComponent`))
  (bind _flatcomponent_4 (`self.FlatComponent`))
  (bind _returnvalue (`|EnumEquality` (`/Game/Objects/Structurs/GrabComponent.GetHeldByHand` (`self.GrabComponent`)) "Right"))
  (bind _returnvalue_2 (select `bool` _returnvalue :`false` (`/Game/Objects/Structurs/FlatComponent.Left Socket` _flatcomponent) :`true` (`/Game/Objects/Structurs/FlatComponent.Right Socket` _flatcomponent)))
  (bind _returnvalue_3 (select `bool` (`|EnumEquality` (`/Game/Objects/Structurs/GrabComponent.GetHeldByHand` (`self.GrabComponent`)) "Right") :`false` (`/Game/Objects/Structurs/FlatComponent.Left Hand Anim` _flatcomponent_3) :`true` (`/Game/Objects/Structurs/FlatComponent.Right Hand Anim` _flatcomponent_3)))
  ;[1 1 1] Grabbed and Dropped
  (`self.EnableInput` (`GameplayStatics.GetPlayerController` 0))
  (`/Game/Objects/Tutorial/TutorialComponent.Check Use Type` (`self.TutorialComponent`) "NewEnumerator0")
  (`/Game/Objects/GameJolt/GameJoltComponent.Check Use Type` (`self.GameJoltComponent`) "NewEnumerator0")
  (`EnhancedInputSubsystemInterface.AddMappingContext` (pcsubsystem `EnhancedInputLocalPlayerSubsystem` (`GameplayStatics.GetPlayerController` 0)) (select `bool` (`|EnumEquality` (`/Game/Objects/Structurs/GrabComponent.GetHeldByHand` (`self.GrabComponent`)) "Right") :`false` "/Game/Player/VR/Input/IMC_Trigger_Left.IMC_Trigger_Left" :`true` "/Game/Player/VR/Input/IMC_Trigger_Right.IMC_Trigger_Right" :!type "InputMappingContext Object Reference") 1 (struct))
  (add `self.VR Left Trigger` (delegate `On VR Use`))
  (add `self.VR Right Trigger` (delegate `On VR Use`))
  (`|ExecutionSequence`
    (:`then_0`
      (bind _player (`/Game/Function/BP_MacroLibrary.Find Player`)
        (:`Is Valid`
          (`PrimitiveComponent.IgnoreActorWhenMoving` (`Character.CapsuleComponent` _player) self true))))
    (:`then_1`
      (bind _player_2 (`/Game/Function/BP_MacroLibrary.Find Player`)
        (:`Is Valid`
          (bind _returnvalue_4 (select `bool` _returnvalue :`false` (`/Game/Player/BP_Player.HandLeft` _player_2) :`true` (`/Game/Player/BP_Player.HandRight` _player_2) :!type "SkeletalMeshComponent Object Reference"))
          (set `self.VR Hand Skeletal` _returnvalue_4)
          (if (!= _returnvalue_2 "None")
            (`self.K2_AttachToComponent` _returnvalue_4 _returnvalue_2 "SnapToTarget" "SnapToTarget" "SnapToTarget"))
          (`|ExecutionSequence`
            (:`then_0`
              (bind _asabp_mannequins_xr (cast `/Game/Player/VR/MannequinsXR/Meshes/ABP_MannequinsXR` (`SkeletalMeshComponent.GetAnimInstance` _returnvalue_4)))
              (set `self.VR Hand Anim` _asabp_mannequins_xr)
              (`/Engine/EditorBlueprintResources/StandardMacros.IsValid` _returnvalue_3
                (:`Is Valid`
                  (set `/Game/Player/VR/MannequinsXR/Meshes/ABP_MannequinsXR.Custom Anim` _returnvalue_3 _asabp_mannequins_xr)
                  (set `/Game/Player/VR/MannequinsXR/Meshes/ABP_MannequinsXR.Use Custom Anim` true _asabp_mannequins_xr))
                (:`Is Not Valid`
                  (if (`/Game/Objects/Structurs/FlatComponent.Use Pose Alpha?` _flatcomponent_2)
                    (set `/Game/Player/VR/MannequinsXR/Meshes/ABP_MannequinsXR.PoseAlphaGrasp` (`/Game/Objects/Structurs/FlatComponent.Pose Alpha Grap` _flatcomponent_4) _asabp_mannequins_xr)
                    (set `/Game/Player/VR/MannequinsXR/Meshes/ABP_MannequinsXR.PoseAlphaIndexCurl` (`/Game/Objects/Structurs/FlatComponent.Pose Alpha Index Curl` _flatcomponent_4) _asabp_mannequins_xr)
                    (set `/Game/Player/VR/MannequinsXR/Meshes/ABP_MannequinsXR.PoseAlphaPoint` (`/Game/Objects/Structurs/FlatComponent.Pose Alpha Point` _flatcomponent_4) _asabp_mannequins_xr)
                    (set `/Game/Player/VR/MannequinsXR/Meshes/ABP_MannequinsXR.PoseAlphaThumbUp` (`/Game/Objects/Structurs/FlatComponent.Pose Alpha Thumb Up` _flatcomponent_4) _asabp_mannequins_xr)))))
            (:`then_1`
              (`SceneComponent.SetVisibility` _returnvalue_4 (select `EVisibiltyOptionsEnum` (`/Game/Objects/Structurs/FlatComponent.Hand Visibility` _flatcomponent_2) :`Dataflow_VisibilityOptions_Visible` true) false))))))))

(event `self.GrabComponent.OnDropped`
  (params (`Self Ref` :type "/Game/Objects/Structurs/GrabComponent Object Reference"))
  ;[1 1 1] Grabbed and Dropped
  (`self.DisableInput` (`GameplayStatics.GetPlayerController` 0))
  (`/Game/Objects/Tutorial/TutorialComponent.Check Use Type` (`self.TutorialComponent`) "NewEnumerator5")
  (`/Game/Objects/GameJolt/GameJoltComponent.Check Use Type` (`self.GameJoltComponent`) "NewEnumerator5")
  (`EnhancedInputSubsystemInterface.RemoveMappingContext` (pcsubsystem `EnhancedInputLocalPlayerSubsystem` (`GameplayStatics.GetPlayerController` 0)) (select `bool` (`|EnumEquality` (`/Game/Objects/Structurs/GrabComponent.GetHeldByHand` (`self.GrabComponent`)) "Right") :`false` "/Game/Player/VR/Input/IMC_Trigger_Left.IMC_Trigger_Left" :`true` "/Game/Player/VR/Input/IMC_Trigger_Right.IMC_Trigger_Right" :!type "InputMappingContext Object Reference") (struct))
  (remove `self.VR Left Trigger` (delegate `On VR Use`))
  (remove `self.VR Right Trigger` (delegate `On VR Use`))
  (`|ExecutionSequence`
    (:`then_0`
      (bind _player (`/Game/Function/BP_MacroLibrary.Find Player`)
        (:`Is Valid`
          (`PrimitiveComponent.IgnoreActorWhenMoving` (`Character.CapsuleComponent` _player) self false))))
    (:`then_1`
      (if (`self.CanPickUp`)
        (`self.Set Flat Mode` "NewEnumerator0")))
    (:`then_2`
      (`self.K2_DetachFromActor` "KeepRelative")
      (`|ExecutionSequence`
        (:`then_0`
          (bind _vr_hand_anim (`self.VR Hand Anim`)
            (:`then`
              (set `/Game/Player/VR/MannequinsXR/Meshes/ABP_MannequinsXR.Use Custom Anim` false _vr_hand_anim)
              (set `self.VR Hand Anim` null))
            (:`else`)))
        (:`then_1`
          (bind _vr_hand_skeletal (`self.VR Hand Skeletal`)
            (:`then`
              (`SceneComponent.SetVisibility` _vr_hand_skeletal true false))
            (:`else`)))))))

(event `Interact (Owner)`
  (params (Component :type "PrimitiveComponent Object Reference") (Location :type "Vector Structure"))
  (`/Game/Function/BP_Interface.Interact` self Component Location))

(event `On VR Use`
  ;[1 1 1] Grabbed and Dropped
)

(fn `Line Trace`
  (params (Distance :type "Float (double-precision)") (Type :type "/Game/Objects/Enum/LineTraceEnum Enum" :default "NewEnumerator0"))
  (returns (Actor :type "Actor Object Reference") (Component :type "PrimitiveComponent Object Reference") (Location :type "Vector Structure"))
  (bind _asbp_player (cast `/Game/Player/BP_Player` (`GameplayStatics.GetPlayerCharacter` 0))
    (:`then`
      _)
    (:`CastFailed`
      _))
  (bind _handleft_scene (`/Game/Player/BP_Player.HandLeft Scene` _asbp_player))
  (bind _handright_scene (`/Game/Player/BP_Player.HandRight Scene` _asbp_player))
  (bind _start_vr (`/Game/Player/BP_Player.Start VR` _asbp_player))
  (bind _returnvalue (select `bool` _start_vr :`false` (`PlayerCameraManager.TransformComponent` (`GameplayStatics.GetPlayerCameraManager` 0)) :`true` (select `EControllerHand` (`/Game/Objects/Structurs/GrabComponent.GetHeldByHand` (`self.GrabComponent`)) :`Left` _handleft_scene :`Right` _handright_scene :`LeftShoulder` _handleft_scene :`RightShoulder` _handright_scene :`LeftElbow` _handleft_scene :`RightElbow` _handright_scene :`LeftKnee` _handleft_scene :`RightKnee` _handright_scene :`LeftFoot` _handleft_scene :`RightFoot` _handright_scene)))
  (bind _returnvalue_2 (`SceneComponent.K2_GetComponentLocation` _returnvalue))
  (bind (_outhit _returnvalue_3) (`KismetSystemLibrary.LineTraceSingle` _returnvalue_2 (+ _returnvalue_2 (* (`SceneComponent.GetForwardVector` _returnvalue) Distance)) "TraceTypeQuery1" false (`|MakeArray` (`GameplayStatics.GetPlayerCharacter` 0) :!type "Actor Object Reference") (select `/Game/Objects/Enum/LineTraceEnum` Type :`NewEnumerator1` (select `bool` _start_vr :`true` "ForDuration" :!type "EDrawDebugTrace Enum") :`NewEnumerator2` "ForDuration")))
  (if _returnvalue_3
    (bind (_bblockinghit _binitialoverlap _time _distance _location _impactpoint _normal _impactnormal _physmat _hitactor _hitcomponent) (`GameplayStatics.BreakHitResult` _outhit))
    (return _hitactor _hitcomponent _location)))

(fn `Load Data`
  (params (JSON :type String))
  (returns (Object :type "VaRestJsonObject Object Reference"))
  (locals (`JSON Object` :type "VaRestJsonObject Object Reference"))
  (bind (_has_field_ _return_value) (`/Game/Function/BP_JSON_FunctionLibrary.Get Value As Vector` (`local.JSON Object`) "Position" (`|EnumEquality` (`/Game/Objects/Structurs/FlatComponent.Mode` (`self.FlatComponent`)) "NewEnumerator0")))
  (bind _returnvalue (cast `/Game/Objects/Enum/FlatModeEnum` (`KismetMathLibrary.Conv_IntToByte` (`VaRestJsonObject.GetIntegerField` (`local.JSON Object`) "Flat Mode"))))
  (bind _returnvalue_2 (`VaRestSubsystem.ConstructVaRestJsonObject` (subsystem `VaRestSubsystem`)))
  (bind _output_get (set `local.JSON Object` _returnvalue_2))
  (bind _returnvalue_3 (`VaRestJsonObject.DecodeJson` _output_get JSON true))
  (if _returnvalue_3
    (`|ExecutionSequence`
      (:`then_0`
        (`self.Set Flat Mode` _returnvalue)
        (set `self.Game Start Flat Mode` _returnvalue)
        (if _has_field_
          (`self.K2_SetActorLocation` _return_value)))
      (:`then_1`
        (return (`local.JSON Object`))))))

(fn `Overlap VR Hands`
  (params (Actor :type "Actor Object Reference") (Component :type "PrimitiveComponent Object Reference"))
  (returns (Overlap :type Boolean))
  (bind _asbp_player (cast `/Game/Player/BP_Player` Actor)
    (:`then`
      (if (== Component (`/Game/Player/BP_Player.Sphere Left` _asbp_player))
        _
        (elif (== Component (`/Game/Player/BP_Player.Sphere Right` _asbp_player))
          _
          (else
            (return false))))
      (return true))
    (:`CastFailed`
      (return false))))

(fn `Save Data`
  (returns (JSON :type "VaRestJsonObject Object Reference"))
  (locals (`JSON Object` :type "VaRestJsonObject Object Reference"))
  (bind _target (`|MakeJson` (`KismetMathLibrary.Conv_IntToDouble` (`KismetMathLibrary.Conv_ByteToInt` (`/Game/Objects/Structurs/FlatComponent.Mode` (`self.FlatComponent`))))))
  (if (`self.Need Save`)
    (`/Game/Function/BP_JSON_FunctionLibrary.Set Vector Field` _target "Position" (`self.K2_GetActorLocation`))
    (return _target)))

(fn `Set Flat Mode`
  (params (`New Mode` :type "/Game/Objects/Enum/FlatModeEnum Enum" :default "NewEnumerator0"))
  (bind _root (`self.Root`))
  (bind _output_get (set `/Game/Objects/Structurs/FlatComponent.Mode` `New Mode` (`self.FlatComponent`)))
  (switch `/Game/Objects/Enum/FlatModeEnum` _output_get
    (:`NewEnumerator0`
      (`PrimitiveComponent.SetSimulatePhysics` _root true))
    (:`NewEnumerator1`
      (`PrimitiveComponent.SetSimulatePhysics` _root false))
    (:`NewEnumerator3`
      (`PrimitiveComponent.SetSimulatePhysics` (`self.Root`) false)
      (`SceneComponent.K2_SetWorldLocation` (`self.Root`) (-1.0000000200408773e+20 -1.0000000200408773e+20 -1.0000000200408773e+20) true false))
    (:`NewEnumerator4`
      (`self.PickUp`))
    (:`NewEnumerator2`
      (bind _sosed (`/Game/Function/BP_MacroLibrary.Find Sosed`)
        (:`Is Valid`
          (`PrimitiveComponent.SetSimulatePhysics` (`self.Root`) false)
          (`self.SetActorEnableCollision` true)
          (`self.K2_AttachToComponent` (`Character.Mesh` _sosed) "belt" "SnapToTarget" "SnapToTarget" "SnapToTarget")
          (`PrimitiveComponent.IgnoreActorWhenMoving` (`self.Root`) _sosed true)
          (`PrimitiveComponent.IgnoreActorWhenMoving` (`Character.CapsuleComponent` _sosed) self true))))))

(fn `Try Release`
  (returns (Released :type Boolean))
  (bind _player (`/Game/Function/BP_MacroLibrary.Find Player`)
    (:`Is Valid`
      (`|ExecutionSequence`
        (:`then_0`
          (bind _heldcomponentright (`/Game/Player/BP_Player.HeldComponentRight` _player))
          (`/Engine/EditorBlueprintResources/StandardMacros.IsValid` _heldcomponentright
            (:`Is Valid`
              _)))
        (:`then_1`
          (bind _heldcomponentleft (`/Game/Player/BP_Player.HeldComponentLeft` _player))
          (`/Engine/EditorBlueprintResources/StandardMacros.IsValid` _heldcomponentleft
            (:`Is Valid`
              _))))
      (bind _breleased (`/Game/Objects/Structurs/GrabComponent.TryRelease` (select `EControllerHand` (`/Game/Objects/Structurs/GrabComponent.GetHeldByHand` (`self.GrabComponent`)) :`Left` _heldcomponentleft :`Right` _heldcomponentright :`LeftShoulder` _heldcomponentleft :`RightShoulder` _heldcomponentright :`LeftElbow` _heldcomponentleft :`RightElbow` _heldcomponentright :`LeftKnee` _heldcomponentleft :`RightKnee` _heldcomponentright :`LeftFoot` _heldcomponentleft :`RightFoot` _heldcomponentright)))
      (if _breleased
        (if (`|EnumEquality` (`/Game/Objects/Structurs/GrabComponent.GetHeldByHand` (`self.GrabComponent`)) "Left")
          (set `/Game/Player/BP_Player.HeldComponentLeft` null _player)
          (else
            (set `/Game/Player/BP_Player.HeldComponentRight` null _player)))
        (return _breleased)
        (else
          (return _breleased))))))

(fn `UserConstructionScript`)
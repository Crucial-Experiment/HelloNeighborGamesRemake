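; BP_NavLinkProxy is a nav link proxy whose point links are driven by its Left, Right and Direction variables.
; The construction script overwrites every PointLinks entry with a link built from those values.
; SetNavLink stores new endpoints and direction, then repeats the same rebuild.
; Direction uses an Auto/LeftToRight/RightToLeft/Culture enum mapped to nav link directions, with Auto and Culture both becoming two-way.
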(fn `Set Nav Link`
  (params (Left :type "Vector Structure") (Right :type "Vector Structure") (Direction :type "ETextFlowDirection Enum" :default "Auto"))
  (bind _pointlinks (`self.PointLinks`))
  (set `self.Left` Left)
  (set `self.Right` Right)
  (set `self.Direction` Direction)
  (for (_ _array_index) _pointlinks
    (`KismetArrayLibrary.Array_Set` _pointlinks _array_index (make `NavigationLink` (`self.Left`) (`self.Right`) (select `ETextFlowDirection` (`self.Direction`) :`Auto` "BothWays" :`LeftToRight` "LeftToRight" :`RightToLeft` "RightToLeft" :`Culture` "BothWays" :!type "ENavLinkDirection Enum")))))

(fn `UserConstructionScript`
  (bind _pointlinks (`self.PointLinks`))
  (for (_ _array_index) _pointlinks
    (`KismetArrayLibrary.Array_Set` _pointlinks _array_index (make `NavigationLink` (`self.Left`) (`self.Right`) (select `ETextFlowDirection` (`self.Direction`) :`Auto` "BothWays" :`LeftToRight` "LeftToRight" :`RightToLeft` "RightToLeft" :`Culture` "BothWays" :!type "ENavLinkDirection Enum")))))
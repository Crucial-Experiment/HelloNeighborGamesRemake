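; Level transition trigger that opens a named level when BP_Player overlaps its box, or when its OpenLevel event is called.
; It first shows the configured widget, then loads the level after a short delay; without a valid widget class nothing happens.
; With an HMD enabled the widget goes onto the MainMenu component of each BP_Menu actor, otherwise it is added to the viewport.
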(event `Open Level`
  (bind _widget (`self.Widget` :!label _label)
    (:`then`
      (if (`HeadMountedDisplayFunctionLibrary.IsHeadMountedDisplayEnabled`)
        (bind _outactors (`GameplayStatics.GetAllActorsOfClass` "/Game/UMG/BP_Menu.BP_Menu_C"))
        (for _array_element _outactors
          (bind _returnvalue (`|CreateWidget` _widget))
          (`WidgetComponent.SetWidget` (`/Game/UMG/BP_Menu.Main Menu` _array_element) _returnvalue)
          (`KismetSystemLibrary.Delay` 0.5 :!label _label_2)
          (`GameplayStatics.OpenLevel` (`self.Name`)))
        (else
          (bind _returnvalue_2 (`|CreateWidget` _widget))
          (`UserWidget.AddToViewport` _returnvalue_2 0)
          (goto _label_2))))
    (:`else`)))

(event `self.Box.OnComponentBeginOverlap`
  (params (OverlappedComponent :type "PrimitiveComponent Object Reference") (OtherActor :type "Actor Object Reference") (OtherComp :type "PrimitiveComponent Object Reference") (OtherBodyIndex :type Integer) (bFromSweep :type Boolean) (SweepResult :type "HitResult Structure (by ref)"))
  (cast `/Game/Player/BP_Player` OtherActor)
  (goto _label))

(fn `UserConstructionScript`)
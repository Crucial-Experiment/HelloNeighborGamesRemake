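; BP_Key is a holdable key item that unlocks code-matched BP_Lock actors, rifle range locks and neighbor car trunks.
; On desktop, left click line-traces for a target; in VR, lock overlap starts a looping timer that unlocks when key pitch nears level.
; Unlocks route through server events, trunk state is multicast, and single-use keys are then released and destroyed.
; Construction tints its materials, and keys that are too hot sizzle and drop after pickup.
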(event `Wait Key Rotation`
  ;[1 1 1] VR Interact
  (bind _output_get (set `self.VR Rotation` (`self.K2_GetActorRotation`)))
  (if (and (>= (.pitch _output_get) -5.0) (<= (.pitch _output_get) 5.0))
    (`KismetSystemLibrary.K2_ClearAndInvalidateTimerHandle` (`self.VR Key Rotation Timer`))
    (`self.Unlock (Server)` (`self.VR Lock`))
    (set `self.VR Lock` null)
    ;[1 1 1] Key
    (if (`self.Use Once`) :!label _label
      (`self.Try Release`)
      (`self.Destroy Key (Server)`))))

(event `self.VR Interact.OnComponentEndOverlap`
  (params (OverlappedComponent :type "PrimitiveComponent Object Reference") (OtherActor :type "Actor Object Reference") (OtherComp :type "PrimitiveComponent Object Reference") (OtherBodyIndex :type Integer))
  ;[1 1 1] VR Interact
  (cast `/Game/Objects/Structurs/BP_Lock` OtherActor)
  (set `self.VR Lock` null)
  (`KismetSystemLibrary.K2_ClearAndInvalidateTimerHandle` (`self.VR Key Rotation Timer`)))

(event `self.VR Interact.OnComponentBeginOverlap`
  (params (OverlappedComponent :type "PrimitiveComponent Object Reference") (OtherActor :type "Actor Object Reference") (OtherComp :type "PrimitiveComponent Object Reference") (OtherBodyIndex :type Integer) (bFromSweep :type Boolean) (SweepResult :type "HitResult Structure (by ref)"))
  ;[1 1 1] VR Interact
  (bind _asbp_lock (cast `/Game/Objects/Structurs/BP_Lock` OtherActor))
  (for _array_element (`/Game/Objects/Structurs/BP_Lock.Code` _asbp_lock)
    (if (`KismetStringLibrary.EqualEqual_StrStr` _array_element (`self.Code`))
      (set `self.VR Lock` _asbp_lock)
      (bind _returnvalue (`KismetSystemLibrary.K2_SetTimerDelegate` (delegate `Wait Key Rotation`) 0.1 true true))
      (set `self.VR Key Rotation Timer` _returnvalue))))

(event `self.ReceiveBeginPlay`
  ;[1 1 1] Begin Play
  (`parent.ReceiveBeginPlay`)
  (bind _player (`/Game/Function/BP_MacroLibrary.Find Player`)
    (:`Is Valid`
      (set `PrimitiveComponent.bGenerateOverlapEvents` (`/Game/Player/BP_Player.Start VR` _player) (`self.VR Interact`)))))

(event `On Press LMB_1`
  ;[1 1 1] Key
  (bind _player (`/Game/Function/BP_MacroLibrary.Find Player`)
    (:`Is Valid`
      (bind _item (`/Game/Player/BP_Player.Get Item` _player))
      (if (== _item self)
        (bind (_actor _component) (`self.Line Trace` 150.0 "NewEnumerator1" :!label _label_2))
        (bind _asbp_lock (cast `/Game/Objects/Structurs/BP_Lock` _actor)
          (:`then`
            (for _array_element (`/Game/Objects/Structurs/BP_Lock.Code` _asbp_lock)
              (if (`KismetStringLibrary.EqualEqual_StrStr` _array_element (`self.Code`))
                (`self.Unlock (Server)` _asbp_lock)
                (`/Game/Objects/Tutorial/TutorialComponent.Check Use Type` (`self.TutorialComponent`) "NewEnumerator6" :!label _label_3)
                (`/Game/Objects/GameJolt/GameJoltComponent.Check Use Type` (`self.GameJoltComponent`) "NewEnumerator6")
                (goto _label))))
          (:`CastFailed`
            (bind _asbp_rifle_range (cast `/Game/Objects/BP_Objects/BP_Rifle_Range` _actor)
              (:`then`
                (if (and (== _component (`/Game/Objects/BP_Objects/BP_Rifle_Range.Lock RR` _asbp_rifle_range)) (`KismetStringLibrary.EqualEqual_StrStr` (`self.Code`) "RifleRange"))
                  (`/Game/Objects/BP_Objects/BP_Rifle_Range.Unlock (Server)` _asbp_rifle_range)
                  (goto _label_3)))
              (:`CastFailed`
                (bind _asbp_neighbor_car (cast `/Game/Objects/BP_Objects/BP_Neighbor_Car` _actor))
                (if (and (`KismetStringLibrary.EqualEqual_StrStr` (`/Game/Objects/BP_Objects/BP_Neighbor_Car.Key Code` _asbp_neighbor_car) (`self.Code`)) (`/Game/Objects/BP_Objects/BP_Neighbor_Car.Lock Trunk` _asbp_neighbor_car))
                  (`self.Unlock Trunk (Server)` _asbp_neighbor_car)
                  (goto _label_3))))))))))

(event `Unlock (Server)`
  (params (Lock :type "/Game/Objects/Structurs/BP_Lock Object Reference"))
  ;[1 1 1] Key
  (`/Game/Objects/Structurs/BP_Lock.Unlock` Lock))

(event `Destroy Key (Server)`
  ;[1 1 1] Key
  (`self.K2_DestroyActor`))

(event `self.On VR Use`
  ;[1 1 1] Key
  (`parent.On VR Use`)
  (if (`self.Old VR Use`)
    (goto _label_2)))

(event `Unlock Trunk (Server)`
  (params (`Neighbor Car` :type "/Game/Objects/BP_Objects/BP_Neighbor_Car Object Reference"))
  ;[1 1 1] Key
  (`self.Unlock Trunk (All)` `Neighbor Car`))

(event `Unlock Trunk (All)`
  (params (`Neighbor Car` :type "/Game/Objects/BP_Objects/BP_Neighbor_Car Object Reference"))
  ;[1 1 1] Key
  (set `/Game/Objects/BP_Objects/BP_Neighbor_Car.Lock Trunk` false `Neighbor Car`))

(event `/Game/Function/BP_Interface.PickUp`
  ;[1 1 1] Pick Up
  (`parent.PickUp`)
  (`KismetSystemLibrary.Delay` 0.2)
  (if (> (`/Game/Objects/Structurs/TemperatureComponent.Temperature` (`self.TemperatureComponent`)) 0.2)
    (`GameplayStatics.PlaySound2D` "/Game/Sounds/Objects/Noise/sizzle_burn_Cue.sizzle_burn_Cue" 1.0 1.0 0.0 null null)
    (`self.Try Release`)))

(fn `UserConstructionScript`
  (`parent.UserConstructionScript`)
  (set `/Game/Objects/Structurs/TemperatureComponent.Actor` (`self.Root`) (`self.TemperatureComponent`))
  (`MeshComponent.SetVectorParameterValueOnMaterials` (`self.Root`) "color" (`KismetMathLibrary.Conv_LinearColorToVector` (`self.Color`)))
  (`MeshComponent.SetScalarParameterValueOnMaterials` (`self.Root`) "Contrast" (`self.Contrast`))
  (`MeshComponent.SetScalarParameterValueOnMaterials` (`self.Root`) "Desaturation" (`self.Desaturation`)))
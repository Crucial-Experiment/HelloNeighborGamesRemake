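; BP_Electricity is a structure object that tracks whether it has electricity and whether it is a generator.
; Enable and Disable notify the tutorial component and set the power flag, then re-run the BeginPlay generator check, so generators always remain powered.
; Save and load extend the parent's JSON data with both flags, writing them only when saving is needed and reading each only if present.
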(event `self.ReceiveBeginPlay`
  (`parent.ReceiveBeginPlay`)
  (if (`self.Generator`) :!label _label
    (set `self.Has Electricity` true)))

(event `Enable`
  (`/Game/Objects/Tutorial/TutorialComponent.Check Use Type` (`self.TutorialComponent`) "NewEnumerator3")
  (set `self.Has Electricity` true)
  (goto _label))

(event `Disable`
  (`/Game/Objects/Tutorial/TutorialComponent.Check Use Type` (`self.TutorialComponent`) "NewEnumerator4")
  (set `self.Has Electricity` false)
  (goto _label))

(fn `Load Data`
  (params (JSON :type String))
  (returns (Object :type "VaRestJsonObject Object Reference"))
  (bind _object (`parent.Load Data` JSON))
  (`|ExecutionSequence`
    (:`then_0`
      (bind (_has_field_ _return_value) (`/Game/Function/BP_JSON_FunctionLibrary.Get Value As Bool` _object "Generator"))
      (if _has_field_
        (set `self.Generator` _return_value)))
    (:`then_1`
      (bind (_has_field__2 _return_value_2) (`/Game/Function/BP_JSON_FunctionLibrary.Get Value As Bool` _object "Has Electricity"))
      (if _has_field__2
        (set `self.Has Electricity` _return_value_2)))
    (:`then_2`
      (return _object))))

(fn `Save Data`
  (returns (JSON :type "VaRestJsonObject Object Reference"))
  (bind _json (`parent.Save Data`))
  (if (`self.Need Save`)
    (`VaRestJsonObject.SetBoolField` _json "Has Electricity" (`self.Has Electricity`))
    (`VaRestJsonObject.SetBoolField` _json "Generator" (`self.Generator`))
    (return _json)))

(fn `UserConstructionScript`
  (`parent.UserConstructionScript`))
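; BP_Fill is a holdable water container item that pours water when toggled by left click or VR use.
; While pouring, a looping timer drains WaterComponent's Fill and updates the water box, and WaterZone overlaps drive fast cooling through UpdateTemperature.
; Pouring stops when empty, dropped or on slot change, and Fill persists through save/load.
; The VR rotation timer calls an empty event, leaving tilt-to-pour logic unconnected.
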(event `Wait Water Rotation`)

(event `self.GrabComponent.OnGrabbed`
  (params (`Self Ref` :type "/Game/Objects/Structurs/GrabComponent Object Reference"))
  ;[1 1 1] VR
  (bind _returnvalue (`KismetSystemLibrary.K2_SetTimerDelegate` (delegate `Wait Water Rotation`) 0.1 true true))
  (set `self.VR Water Rotation Timer` _returnvalue)
  ;[1 1 1] Begin Play
  (`self.SetActorEnableCollision` true :!label _label)
  (`PrimitiveComponent.SetCollisionEnabled` (`self.Root`) "NoCollision"))

(event `self.ReceiveBeginPlay`
  (bind _watercomponent (`self.WaterComponent`))
  ;[1 1 1] Begin Play
  (`parent.ReceiveBeginPlay`)
  (set `/Game/Objects/Structurs/WaterComponent.Water Box` (`self.Water Box`) _watercomponent)
  (`/Game/Objects/Structurs/WaterComponent.Update Water Box` _watercomponent)
  (`PrimitiveComponent.SetCollisionProfileName` (`self.Water Zone`) "NoCollision" true))

(event `self.GrabComponent.OnDropped`
  (params (`Self Ref` :type "/Game/Objects/Structurs/GrabComponent Object Reference"))
  ;[1 1 1] VR
  (`KismetSystemLibrary.K2_ClearAndInvalidateTimerHandle` (`self.VR Water Rotation Timer`))
  ;[1 1 1] LMB and Drop
  (`PrimitiveComponent.SetCollisionEnabled` (`self.Root`) "QueryAndPhysics" :!label _label_2)
  (switch `/Game/Objects/Enum/TumblerStateEnum` (`self.State`) :!label _label_3
    (:`NewEnumerator0`
      (`ActorComponent.Deactivate` (`self.Water`) :!label _label_4)
      (set `self.State` "NewEnumerator1")
      (`PrimitiveComponent.SetCollisionProfileName` (`self.Water Zone`) "NoCollision" true)
      (`AudioComponent.Stop` (`self.Water Drop Loop`))
      (`KismetSystemLibrary.K2_SetTimerDelegate` (delegate `Water Drop`))
      (clear `/Game/Objects/Structurs/WaterComponent.Water Drop Stop` (`self.WaterComponent`)))))

(event `/Game/Function/BP_Interface.PickUp`
  ;[1 1 1] Begin Play
  (`parent.PickUp`)
  (goto _label))

(event `self.On VR Use`
  ;[1 1 1] LMB and Drop
  (`parent.On VR Use`)
  (if (> (`/Game/Objects/Structurs/WaterComponent.Fill` (`self.WaterComponent`)) 0.0) :!label _label_5
    (switch `/Game/Objects/Enum/TumblerStateEnum` (`self.State`)
      (:`NewEnumerator0`
        (goto _label_4))
      (:`NewEnumerator1`
        (`ActorComponent.Activate` (`self.Water`) false)
        (set `self.State` "NewEnumerator0")
        (`PrimitiveComponent.SetCollisionProfileName` (`self.Water Zone`) "OverlapAllDynamic" true)
        (`AudioComponent.Play` (`self.Water Drop Loop`) 0.0)
        (`KismetSystemLibrary.K2_SetTimerDelegate` (delegate `Water Drop`) 0.5 true)
        (add `/Game/Objects/Structurs/WaterComponent.Water Drop Stop` (`self.WaterComponent`) (delegate `Stop Water Drop`))))
    (else
      (goto _label_4))))

(event `self.On Press LMB`
  ;[1 1 1] LMB and Drop
  (bind _player (`/Game/Function/BP_MacroLibrary.Find Player`)
    (:`Is Valid`
      (bind _item (`/Game/Player/BP_Player.Get Item` _player))
      (if (== _item self)
        (goto _label_5)))))

(event `self.On Item Dropped`
  ;[1 1 1] LMB and Drop
  (goto _label_2))

(event `self.On Slot Change`
  ;[1 1 1] LMB and Drop
  (bind _player (`/Game/Function/BP_MacroLibrary.Find Player`)
    (:`Is Valid`
      (bind _item (`/Game/Player/BP_Player.Get Item` _player))
      (if (== _item self)
        (`self.SetActorEnableCollision` true)
        (`PrimitiveComponent.SetCollisionEnabled` (`self.Root`) "NoCollision")
        (goto _label_3)
        (else
          (`self.SetActorEnableCollision` false)
          (goto _label_3))))))

(event `Stop Water Drop`
  ;[1 1 1] LMB and Drop
  (goto _label_4))

(event `self.Water Zone.OnComponentBeginOverlap`
  (params (OverlappedComponent :type "PrimitiveComponent Object Reference") (OtherActor :type "Actor Object Reference") (OtherComp :type "PrimitiveComponent Object Reference") (OtherBodyIndex :type Integer) (bFromSweep :type Boolean) (SweepResult :type "HitResult Structure (by ref)"))
  ;[1 1 1] LMB and Drop
  (`/Game/Objects/Structurs/WaterComponent.Update Temperature` (`self.WaterComponent`) OtherActor true))

(event `Water Drop`
  (bind _watercomponent (`self.WaterComponent`))
  ;[1 1 1] LMB and Drop
  (bind _output_get (set `/Game/Objects/Structurs/WaterComponent.Fill` (`KismetMathLibrary.NormalizeToRange` (- (`/Game/Objects/Structurs/WaterComponent.Fill` _watercomponent) (`/Game/Objects/Structurs/WaterComponent.Speed Shower` _watercomponent)) 0.0 1.0) _watercomponent))
  (`/Game/Objects/Structurs/WaterComponent.Update Water Box` _watercomponent)
  (if (== _output_get 0.0)
    (goto _label_4)))

(event `self.Water Zone.OnComponentEndOverlap`
  (params (OverlappedComponent :type "PrimitiveComponent Object Reference") (OtherActor :type "Actor Object Reference") (OtherComp :type "PrimitiveComponent Object Reference") (OtherBodyIndex :type Integer))
  ;[1 1 1] LMB and Drop
  (`/Game/Objects/Structurs/WaterComponent.Update Temperature` (`self.WaterComponent`) OtherActor false))

(fn `Load Data`
  (params (JSON :type String))
  (returns (Object :type "VaRestJsonObject Object Reference"))
  (bind _watercomponent (`self.WaterComponent`))
  (bind _object (`parent.Load Data` JSON))
  (`|ExecutionSequence`
    (:`then_0`
      (bind (_has_field_ _return_value) (`/Game/Function/BP_JSON_FunctionLibrary.Get Value As Float` _object "Fill"))
      (if _has_field_
        (set `/Game/Objects/Structurs/WaterComponent.Fill` _return_value _watercomponent)
        (`/Game/Objects/Structurs/WaterComponent.Update Water Box` _watercomponent)))
    (:`then_1`
      (return _object))))

(fn `Save Data`
  (returns (JSON :type "VaRestJsonObject Object Reference"))
  (bind _json (`parent.Save Data`))
  (`VaRestJsonObject.SetNumberField` _json "Fill" (`/Game/Objects/Structurs/WaterComponent.Fill` (`self.WaterComponent`)))
  (return _json))

(fn `UserConstructionScript`
  (bind _watercomponent (`self.WaterComponent`))
  (`parent.UserConstructionScript`)
  (set `/Game/Objects/Structurs/WaterComponent.Water Box` (`self.Water Box`) _watercomponent)
  (`/Game/Objects/Structurs/WaterComponent.Update Water Box` _watercomponent))
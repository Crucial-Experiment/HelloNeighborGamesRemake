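; BP_SmartActor is a structure actor Blueprint that provides JSON save and load functions for game objects.
; SaveData returns the result of MakeJson only when the NeedSave flag is set.
; LoadData creates a VaRest JSON object, stores it, decodes the incoming string into it with the incremental parser and returns it.
; It does not apply the decoded values itself, and its construction script is empty.
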(fn `Load Data`
  (params (JSON :type String))
  (returns (Object :type "VaRestJsonObject Object Reference"))
  (locals (`JSON Object` :type "VaRestJsonObject Object Reference"))
  (bind _returnvalue (`VaRestSubsystem.ConstructVaRestJsonObject` (subsystem `VaRestSubsystem`)))
  (bind _output_get (set `local.JSON Object` _returnvalue))
  (`VaRestJsonObject.DecodeJson` _output_get JSON true)
  (return (`local.JSON Object`)))

(fn `Save Data`
  (returns (JSON :type "VaRestJsonObject Object Reference"))
  (if (`self.Need Save`)
    (return (`|MakeJson`))))

(fn `UserConstructionScript`)
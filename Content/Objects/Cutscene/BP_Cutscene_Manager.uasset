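; Cutscene manager actor that plays, pauses or stops a level sequence and handles what happens when it ends.
; On play it can clear player inventories, disable rain, mute atmosphere audio, hide inventory and cursor, and offer a skip widget on PC and console.
; Finish notifies tutorial and GameJolt components, then either restores player state on non-mobile authority, quits, returns to the VR-aware main menu or opens a level.
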(event `Finish`
  (set `self.State` "NewEnumerator1")
  (`/Game/Objects/Tutorial/TutorialComponent.Check Use Type` (`self.TutorialComponent`) "NewEnumerator6")
  (`/Game/Objects/GameJolt/GameJoltComponent.Check Use Type` (`self.GameJoltComponent`) "NewEnumerator6")
  (`self.On Finished`)
  (switch `/Game/Objects/Enum/CutsceneFinish` (`self.Actions after playback`)
    (:`NewEnumerator0`
      (if (and (`|EnumInequality` (`/Game/Function/BP_FunctionLibrary.Get Current Platform`) "NewEnumerator2") (`self.HasAuthority`))
        (bind _player (`/Game/Function/BP_MacroLibrary.Find Player`)
          (:`Is Valid`
            (`KismetSystemLibrary.Delay` 0.2)
            (`|ExecutionSequence`
              (:`then_0`
                (if (`self.Hide Inventory`)
                  (`/Game/UMG/Inventory/WB_Inventory.Show Inventory` (`/Game/Player/BP_Player.Inventory` _player) "None")))
              (:`then_1`
                (if (`self.Hide Cursor`)
                  (`Widget.SetVisibility` (`/Game/Player/BP_Player.Cursor` _player) "Visible")))
              (:`then_2`
                (set `/Game/Player/BP_Player.Cutscene Skip` null _player)
                (switch `/Game/UMG/EPlatform` (`/Game/Function/BP_FunctionLibrary.Get Current Platform`)
                  (:`NewEnumerator0`
                    _)
                  (:`NewEnumerator1`
                    _))
                (bind _widget (`self.Widget`)
                  (:`then`
                    (`Widget.RemoveFromParent` _widget))
                  (:`else`)))
              (:`then_3`
                (if (`self.Disable Atmosphere Time Sound`)
                  (bind _returnvalue (`GameplayStatics.GetActorOfClass` "/Game/BP_Atmosphere_And_Time_Manager.BP_Atmosphere_And_Time_Manager_C"))
                  (`AudioComponent.Play` (`/Game/BP_Atmosphere_And_Time_Manager.Audio` _returnvalue) 0.0))))))))
    (:`NewEnumerator1`
      (`KismetSystemLibrary.QuitGame` null "Quit"))
    (:`NewEnumerator2`
      (if (`HeadMountedDisplayFunctionLibrary.IsHeadMountedDisplayEnabled`)
        (bind _outactors (`GameplayStatics.GetAllActorsOfClass` "/Game/UMG/BP_Menu.BP_Menu_C"))
        (for _array_element _outactors
          (bind _returnvalue_2 (`|CreateWidget` "/Game/UMG/Menu/WB_Loading.WB_Loading_C"))
          (`WidgetComponent.SetWidget` (`/Game/UMG/BP_Menu.Main Menu` _array_element) _returnvalue_2)
          (`KismetSystemLibrary.Delay` 0.5 :!label _label)
          (`GameplayStatics.OpenLevel` "Map_Menu"))
        (else
          (bind _returnvalue_3 (`|CreateWidget` "/Game/UMG/Menu/WB_Loading.WB_Loading_C"))
          (`UserWidget.AddToViewport` _returnvalue_3 0)
          (goto _label))))
    (:`NewEnumerator3`
      (`GameplayStatics.OpenLevel` (`self.Level Name`)))))

(event `self.ReceiveBeginPlay`
  (bind _state (`self.State`))
  (if (and (`|EnumInequality` _state "NewEnumerator1") (`self.HasAuthority`))
    (`self.Set State` _state))
  (add `MovieSceneSequencePlayer.OnFinished` (`LevelSequenceActor.SequencePlayer` (`self.Level Seq`)) (delegate `Finish`)))

(event `Set State`
  (params (`New State` :type "/Game/Objects/Enum/CutscenePlayer Enum" :default "NewEnumerator0"))
  (bind _sequenceplayer (`LevelSequenceActor.SequencePlayer` (`self.Level Seq`)))
  (bind _output_get (set `self.State` `New State`))
  (switch `/Game/Objects/Enum/CutscenePlayer` _output_get
    (:`NewEnumerator0`
      (`MovieSceneSequencePlayer.Play` _sequenceplayer)
      (`|ExecutionSequence`
        (:`then_0`
          (if (`self.Remove Items From Inventory`)
            (bind _outactors (`GameplayStatics.GetAllActorsOfClass` "/Game/Player/BP_Player.BP_Player_C"))
            (for _array_element _outactors
              (bind _items (`/Game/Player/BP_Player.Get Inventory` _array_element))
              (for _array_element_2 _items
                (`/Game/Objects/Structurs/BP_Object.Try Release` _array_element_2)
                (`self.K2_DestroyActor` _array_element_2)))))
        (:`then_1`
          (if (`self.Stop Rain`)
            (bind _returnvalue (`GameplayStatics.GetActorOfClass` "/Game/Objects/BP_Objects/BP_Weather.BP_Weather_C"))
            (`/Game/Objects/BP_Objects/BP_Weather.Disable` _returnvalue)))
        (:`then_2`
          (if (`|EnumInequality` (`/Game/Function/BP_FunctionLibrary.Get Current Platform`) "NewEnumerator2")
            (bind _player (`/Game/Function/BP_MacroLibrary.Find Player`)
              (:`Is Valid`
                (`KismetSystemLibrary.Delay` 0.2)
                (if (`self.Hide Inventory`)
                  (`/Game/UMG/Inventory/WB_Inventory.Hide Inventory` (`/Game/Player/BP_Player.Inventory` _player)))
                (`Widget.SetVisibility` (`/Game/Player/BP_Player.Cursor` _player) (select `bool` (`self.Hide Cursor`) :`false` "Visible" :`true` "Hidden" :!type "ESlateVisibility Enum"))
                (if (`self.Can Skip`)
                  (set `/Game/Player/BP_Player.Cutscene Skip` self _player))
                (switch `/Game/UMG/EPlatform` (`/Game/Function/BP_FunctionLibrary.Get Current Platform`)
                  (:`NewEnumerator0`
                    _)
                  (:`NewEnumerator1`
                    _))
                (if (`self.Can Skip`)
                  (bind _returnvalue_2 (`|CreateWidget` "/Game/UMG/Menu/BW_SkipCutScene.BW_SkipCutScene_C" (`GameplayStatics.GetPlayerController` 0)))
                  (bind _output_get_2 (set `self.Widget` _returnvalue_2))
                  (`UserWidget.AddToViewport` _output_get_2 0))))))
        (:`then_3`
          (if (`self.Disable Atmosphere Time Sound`)
            (bind _returnvalue_3 (`GameplayStatics.GetActorOfClass` "/Game/BP_Atmosphere_And_Time_Manager.BP_Atmosphere_And_Time_Manager_C"))
            (`AudioComponent.Stop` (`/Game/BP_Atmosphere_And_Time_Manager.Audio` _returnvalue_3))))))
    (:`NewEnumerator1`
      (`MovieSceneSequencePlayer.Stop` _sequenceplayer)
      (`self.Finish`))
    (:`NewEnumerator3`
      (`MovieSceneSequencePlayer.Pause` _sequenceplayer))))

(fn `Get Play Time`
  (returns (Return :type "QualifiedFrameTime Structure"))
  (return (`MovieSceneSequencePlayer.GetCurrentTime` (`LevelSequenceActor.SequencePlayer` (`self.Level Seq`)))))

(fn `UserConstructionScript`)
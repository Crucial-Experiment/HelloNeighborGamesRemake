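; BP_Neighbor_Cutscene is a cutscene Neighbor pawn that walks a point path and reports contact with the player.
; Moving starts an AI move loop through Points, playing a grunt at each success and retrying after failures.
; HitBox overlap with BP_Player, beginning or ending, plays a grunt if none is playing, calls HitPlayer and stops movement.
; Refresh teleports it back to its BeginPlay transform and resets the path.
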(event `self.ReceiveBeginPlay`
  ;[1 1 1] Begin Play
  (`self.Stop Moving`)
  (set `self.StartPos` (`self.GetTransform`)))

(event `OnMoving`
  ;[1 1 1] Moving
  (if (`self.bMoving`) :!label _label
    (if (< (`self.CurPoint`) (`KismetArrayLibrary.Array_Length` (`self.Points`)))
      (`|AIMoveTo` self (0.0 0.0 0.0) (`|GetArrayItem` (`self.Points`) (`self.CurPoint`)) 5.0 true
        (:`OnSuccess`
          (if (not (`AudioComponent.IsPlaying` (`self.Grunt 412`)))
            (`AudioComponent.Play` (`self.Grunt 1211`) 0.0))
          (`/Engine/EditorBlueprintResources/StandardMacros.IncrementInt` (`self.CurPoint`)
            (:`  `
              (goto _label))))
        (:`OnFail`
          (`KismetSystemLibrary.Delay` 1.0)
          (goto _label)))
      (else
        (set `self.bMoving` false)))))

(event `self.Hit Box.OnComponentBeginOverlap`
  (params (OverlappedComponent :type "PrimitiveComponent Object Reference") (OtherActor :type "Actor Object Reference") (OtherComp :type "PrimitiveComponent Object Reference") (OtherBodyIndex :type Integer) (bFromSweep :type Boolean) (SweepResult :type "HitResult Structure (by ref)"))
  ;[1 1 1] Player Hit
  (cast `/Game/Player/BP_Player` OtherActor)
  (if (not (or (`AudioComponent.IsPlaying` (`self.Grunt 1211`)) (`AudioComponent.IsPlaying` (`self.Grunt 412`)))) :!label _label_2
    (`GameplayStatics.PlaySound2D` "/Game/Sounds/Sosed/Animations/sosed_grunt_412_Cue.sosed_grunt_412_Cue" 1.0 1.0 0.0 null null)
    (`KismetSystemLibrary.Delay` 0.1))
  (`self.Hit Player`)
  (`self.Stop Moving`))

(event `self.Hit Box.OnComponentEndOverlap`
  (params (OverlappedComponent :type "PrimitiveComponent Object Reference") (OtherActor :type "Actor Object Reference") (OtherComp :type "PrimitiveComponent Object Reference") (OtherBodyIndex :type Integer))
  ;[1 1 1] Player Hit
  (cast `/Game/Player/BP_Player` OtherActor)
  (goto _label_2))

(fn `Moving`
  (set `self.bMoving` true)
  (`self.OnMoving`))

(fn `Refresh`
  (`self.K2_SetActorTransform` (`self.StartPos`) false true)
  (`self.Stop Moving`))

(fn `Stop Moving`
  (set `self.bMoving` false)
  (set `self.CurPoint` 0))

(fn `UserConstructionScript`)
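; DevGAMM bed interactable whose Type selects what happens on use: hide, sleep, cutscene, level restart or level change.
; Hiding uses the Hide timeline to lerp the player to and from CharacterPoint, toggling movement mode and input.
; Sleeping fades the camera, triggers a random Sosed spawn, updates game time and checks off the tutorial entry.
; Cutscene mode fires at a set sleep count; Open Level waits out the cutscene before loading.
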(event `self.Interact`
  (params (Component :type "PrimitiveComponent Object Reference") (Location :type "Vector Structure"))
  (bind _returnvalue (`GameplayStatics.GetPlayerPawn` 0))
  (`/Game/Objects/Tutorial/TutorialComponent.Check Use Type` (`self.TutorialComponent`) "NewEnumerator6")
  (`/Game/Objects/GameJolt/GameJoltComponent.Check Use Type` (`self.GameJoltComponent`) "NewEnumerator6")
  (switch `/Game/Objects/Enum/BedTypeEnum` (`self.Type`)
    (:`NewEnumerator0`
      (`AudioComponent.Play` (`self.Rustle Clothes`) 0.0)
      (if (`self.Player Is Here?`)
        (set `self.Player Is Here?` false)
        (bind (_direction _alpha) (`Timeline|Hide` :!via `Reverse` :!label _label)
          (:`Update`
            (`self.K2_SetActorLocation` (`GameplayStatics.GetPlayerPawn` 0) (`KismetMathLibrary.VLerp` (`self.Player Location`) (`SceneComponent.K2_GetComponentLocation` (`self.Character Point`)) _alpha) false false))
          (:`Finished`
            (bind _player (`/Game/Function/BP_MacroLibrary.Find Player`)
              (:`Is Valid`
                (if (`self.Player Is Here?`)
                  (bind _charactermovement (`Character.CharacterMovement` _player))
                  (`CharacterMovementComponent.SetMovementMode` _charactermovement "MOVE_None" 0)
                  (else
                    (`CharacterMovementComponent.SetMovementMode` _charactermovement "MOVE_Walking" 0)))
                (`self.EnableInput` (`GameplayStatics.GetPlayerPawn` 0) (`GameplayStatics.GetPlayerController` 0))))))
        (else
          (set `self.Player Is Here?` true)
          (`self.DisableInput` _returnvalue (`GameplayStatics.GetPlayerController` 0))
          (set `self.Player Location` (`self.K2_GetActorLocation` _returnvalue))
          (goto _label))))
    (:`NewEnumerator3`
      (`PlayerCameraManager.StartCameraFade` :`self` (`GameplayStatics.GetPlayerCameraManager` 0) :`ToAlpha` 1.0 :`Duration` 5.0 :`bHoldWhenFinished` true :!label _label_2)
      (`|ExecutionSequence`
        (:`then_0`
          (`/Game/Player/BP_GameMode.Random Spawn Sosed` (`/Game/Function/BP_FunctionLibrary.Get Game Mode`))
          (bind _sosed (`/Game/Function/BP_MacroLibrary.Find Sosed`)
            (:`Is Valid`
              (`/Game/Sosed/BP_Sosed.Set Game Time` _sosed)
              (`/Game/Sosed/BP_Sosed.Check Flashlight` _sosed "NewEnumerator0"))
            (:`Is Not Valid`
              _))
          (`PlayerCameraManager.StartCameraFade` :`self` (`GameplayStatics.GetPlayerCameraManager` 0) :`FromAlpha` 1.0 :`Duration` 5.0)
          (`/Engine/EditorBlueprintResources/StandardMacros.IncrementInt` (`self.Sleep Count Temp`)
            (:`  `
              (`self.K2_TeleportTo` :`self` (`GameplayStatics.GetPlayerPawn` 0) :`DestLocation` (`self.K2_GetActorLocation` (`GameplayStatics.GetPlayerController` 0))))))
        (:`then_1`
          (bind _tutorial_manager (`self.Tutorial Manager`)
            (:`then`
              (`/Game/Objects/Tutorial/BP_Tutorial_Manager.Modify List` _tutorial_manager (`self.Text ID`) true))
            (:`else`)))))
    (:`NewEnumerator4`
      (if (== (`self.Sleep Count`) (`self.Sleep Count Temp`))
        (bind _cutscene_manager (`self.Cutscene Manager`)
          (:`then`
            (`/Game/Objects/Cutscene/BP_Cutscene_Manager.Set State` _cutscene_manager "NewEnumerator0")
            (goto _label_2))
          (:`else`))
        (else
          (goto _label_2))))
    (:`NewEnumerator1`
      (`KismetSystemLibrary.ExecuteConsoleCommand` "RestartLevel" null))
    (:`NewEnumerator2`
      (bind _cutscene_manager_2 (`self.Cutscene Manager`)
        (:`then`
          (`/Game/Objects/Cutscene/BP_Cutscene_Manager.Set State` _cutscene_manager_2 "NewEnumerator0")
          (`self.DisableInput` (`GameplayStatics.GetPlayerCharacter` 0) (`GameplayStatics.GetPlayerController` 0))
          (`KismetSystemLibrary.Delay` (`TimeManagementBlueprintLibrary.Conv_QualifiedFrameTimeToSeconds` (`/Game/Objects/Cutscene/BP_Cutscene_Manager.Get Play Time` _cutscene_manager_2)))
          (`PlayerCameraManager.StartCameraFade` :`self` (`GameplayStatics.GetPlayerCameraManager` 0) :`ToAlpha` 1.0 :`Duration` 2.0)
          (`KismetSystemLibrary.Delay` 2.0)
          (bind _returnvalue_2 (`|CreateWidget` "/Game/UMG/Menu/WB_Loading.WB_Loading_C"))
          (`UserWidget.AddToViewport` _returnvalue_2 0)
          (`GameplayStatics.OpenLevel` (`self.Level Name`)))
        (:`else`)))))

(fn `UserConstructionScript`)
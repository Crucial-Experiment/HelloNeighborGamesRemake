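; Interactable, pick-up-able lawn mower prop that drives itself forward while switched on.
; Interact toggles it with start, loop and end sounds, and picking it up also switches it off.
; While on, Tick nudges the root along the Arrow's forward vector without sweep or delta-time scaling, and timelines spin the blade and wheels.
; Both state changes report a use type to the tutorial and GameJolt components.
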(event `self.PickUp`
  (`parent.PickUp`)
  (set `self.Move` false :!label _label)
  (`AudioComponent.Stop` (`self.lawnmower_loop_Cue`))
  (`GameplayStatics.PlaySoundAtLocation` "/Game/Sounds/Objects/Noise/lawnmower_end_Cue.lawnmower_end_Cue" (`self.K2_GetActorLocation`) (struct) 1.0 1.0 0.0 null null null null)
  (`/Game/Objects/Tutorial/TutorialComponent.Check Use Type` (`self.TutorialComponent`) "NewEnumerator4")
  (`/Game/Objects/GameJolt/GameJoltComponent.Check Use Type` (`self.GameJoltComponent`) "NewEnumerator4"))

(event `self.Interact`
  (params (Component :type "PrimitiveComponent Object Reference") (Location :type "Vector Structure"))
  (`parent.Interact` Component Location)
  (if (`self.Move`)
    (goto _label)
    (else
      (`GameplayStatics.PlaySoundAtLocation` "/Game/Sounds/Objects/Noise/lawnmower_start_Cue.lawnmower_start_Cue" (`self.K2_GetActorLocation`) (struct) 1.0 1.0 0.0 null null null null)
      (`KismetSystemLibrary.Delay` 0.7)
      (`AudioComponent.Play` (`self.lawnmower_loop_Cue`) 0.0)
      (set `self.Move` true)
      (`/Game/Objects/Tutorial/TutorialComponent.Check Use Type` (`self.TutorialComponent`) "NewEnumerator3")
      (`/Game/Objects/GameJolt/GameJoltComponent.Check Use Type` (`self.GameJoltComponent`) "NewEnumerator3"))))

(event `self.ReceiveTick`
  (params (DeltaSeconds :type "Float (single-precision)"))
  (if (`self.Move`)
    (`SceneComponent.K2_AddRelativeLocation` (`self.Root`) (`SceneComponent.GetForwardVector` (`self.Arrow`)) false false)
    (`|ExecutionSequence`
      (:`then_0`
        (bind (_direction _alpha) (`Timeline|Blade Rotation`)
          (:`Update`
            (`SceneComponent.K2_AddRelativeRotation` (`self.Blade`) (`KismetMathLibrary.RLerp` (struct) (struct :`Yaw` 15.0) _alpha) false false))))
      (:`then_1`
        (bind (_direction_2 _alpha_2) (`Timeline|Wheel Rotation`)
          (:`Update`
            (`SceneComponent.K2_AddRelativeRotation` (`self.Wheel 1`) (`KismetMathLibrary.RLerp` (struct) (struct :`Roll` -15.0) _alpha_2) false false)
            (`SceneComponent.K2_AddRelativeRotation` (`self.Wheel 3`) (`KismetMathLibrary.RLerp` (struct) (struct :`Roll` -15.0) _alpha_2) false false)
            (`SceneComponent.K2_AddRelativeRotation` (`self.Wheel 4`) (`KismetMathLibrary.RLerp` (struct) (struct :`Roll` -15.0) _alpha_2) false false)
            (`SceneComponent.K2_AddRelativeRotation` (`self.Wheel 2`) (`KismetMathLibrary.RLerp` (struct) (struct :`Roll` -15.0) _alpha_2) false false)))))))

(fn `UserConstructionScript`)
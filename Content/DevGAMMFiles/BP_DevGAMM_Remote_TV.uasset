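; BP_DevGAMM_Remote_TV is a usable TV remote item that operates a TV the player points it at.
; On VR use, or on left mouse press while the player holds it, it line-traces forward and calls RemoteTV on any hit BP_DevGAMM_TV.
; A successful hit also reports the use type to the tutorial and GameJolt components.
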(event `self.ReceiveBeginPlay`
  (`parent.ReceiveBeginPlay`))

(event `self.On VR Use`
  (`parent.On VR Use`)
  (bind _actor (`self.Line Trace` 1500.0 :!label _label))
  (bind _asbp_dev_gamm_tv (cast `/Game/DevGAMMFiles/BP_DevGAMM_TV` _actor))
  (`/Game/DevGAMMFiles/BP_DevGAMM_TV.RemoteTV` _asbp_dev_gamm_tv false)
  (`/Game/Objects/Tutorial/TutorialComponent.Check Use Type` (`self.TutorialComponent`) "NewEnumerator6")
  (`/Game/Objects/GameJolt/GameJoltComponent.Check Use Type` (`self.GameJoltComponent`) "NewEnumerator6"))

(event `self.On Press LMB`
  (bind _player (`/Game/Function/BP_MacroLibrary.Find Player`)
    (:`Is Valid`
      (bind _item (`/Game/Player/BP_Player.Get Item` _player))
      (if (== _item self)
        (goto _label)))))

(fn `UserConstructionScript`
  (`parent.UserConstructionScript`))
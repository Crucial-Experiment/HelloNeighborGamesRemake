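; Interactive table with three sliding parts, likely drawers, that open and close on interaction or by VR grab.
; Interact matches the component, then a FlipFlop plays or reverses that part's timeline slide and plays a sound, though Part2 reuses its open sound for closing.
; VR grabs run looping timers that move capsules along Y with the controller, clamped by spline endpoints.
; Capsules drive the meshes, with Part1 and Part2 cross-linked.
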(event `/Game/Function/BP_Interface.Interact`
  (params (Component :type "PrimitiveComponent Object Reference") (Location :type "Vector Structure"))
  ;[1 1 1] Interact
  (`|ExecutionSequence`
    (:`then_0`
      (if (or (== Component (`self.Part 1`)) (== Component (`self.Part 1 Capsule`)))
        (`/Engine/EditorBlueprintResources/StandardMacros.FlipFlop`
          (:`A`
            (`|ExecutionSequence`
              (:`then_0`
                (bind (_direction _alpha) (`Timeline|Part 1 Loc` :!label _label)
                  (:`Update`
                    (`SceneComponent.K2_SetRelativeLocation` (`self.Part 1`) (`KismetMathLibrary.VLerp` (0.0 0.0 0.0) (0.0 48.0 0.0) _alpha) false false))))
              (:`then_1`
                (`AudioComponent.Play` (`self.Part 1 Open`) 0.0))))
          (:`B`
            (`|ExecutionSequence`
              (:`then_0`
                (goto _label :!via `Reverse`))
              (:`then_1`
                (`AudioComponent.Play` (`self.Part 1 Close`) 0.0)))))))
    (:`then_1`
      (if (or (== Component (`self.Part 2`)) (== Component (`self.Part 2 Capsule`)))
        (`/Engine/EditorBlueprintResources/StandardMacros.FlipFlop`
          (:`A`
            (`|ExecutionSequence`
              (:`then_0`
                (bind (_direction_2 _alpha_2) (`Timeline|Part 2 Loc` :!label _label_2)
                  (:`Update`
                    (`SceneComponent.K2_SetRelativeLocation` (`self.Part 2`) (`KismetMathLibrary.VLerp` (0.0 0.0 0.0) (0.0 75.0 0.0) _alpha_2) false false))))
              (:`then_1`
                (`AudioComponent.Play` (`self.Part 2 Open`) 0.0))))
          (:`B`
            (`|ExecutionSequence`
              (:`then_0`
                (goto _label_2 :!via `Reverse`))
              (:`then_1`
                (`AudioComponent.Play` (`self.Part 2 Open`) 0.0)))))))
    (:`then_2`
      (if (or (== Component (`self.Part 3`)) (== Component (`self.Part 3 Capsule`)))
        (`/Engine/EditorBlueprintResources/StandardMacros.FlipFlop`
          (:`A`
            (`|ExecutionSequence`
              (:`then_0`
                (bind (_direction_3 _alpha_3) (`Timeline|Part 3 Loc` :!label _label_3)
                  (:`Update`
                    (`SceneComponent.K2_SetRelativeLocation` (`self.Part 3`) (`KismetMathLibrary.VLerp` (0.0 0.0 0.0) (0.0 42.0 0.0) _alpha_3) false false))))
              (:`then_1`
                (`AudioComponent.Play` (`self.Part 3 Open`) 0.0))))
          (:`B`
            (`|ExecutionSequence`
              (:`then_0`
                (goto _label_3 :!via `Reverse`))
              (:`then_1`
                (`AudioComponent.Play` (`self.Part 3 Close`) 0.0)))))))))

(event `self.Part 2 Grab.OnGrabbed`
  (params (`Self Ref` :type "/Game/Objects/Structurs/GrabComponent Object Reference"))
  ;[1 1 1] VR
  (bind _returnvalue (`KismetSystemLibrary.K2_SetTimer` null "Update Location Part 2" 0.01 true))
  (set `self.VR Part Time` _returnvalue))

(event `self.Part 1 Grab.OnGrabbed`
  (params (`Self Ref` :type "/Game/Objects/Structurs/GrabComponent Object Reference"))
  ;[1 1 1] VR
  (bind _returnvalue (`KismetSystemLibrary.K2_SetTimer` null "Update Location Part 1" 0.01 true))
  (set `self.VR Part Time` _returnvalue))

(event `self.Part 3 Grab.OnGrabbed`
  (params (`Self Ref` :type "/Game/Objects/Structurs/GrabComponent Object Reference"))
  ;[1 1 1] VR
  (bind _returnvalue (`KismetSystemLibrary.K2_SetTimer` null "Update Location Part 3" 0.01 true))
  (set `self.VR Part Time` _returnvalue))

(event `self.Part 2 Grab.OnDropped`
  (params (`Self Ref` :type "/Game/Objects/Structurs/GrabComponent Object Reference"))
  ;[1 1 1] VR
  (`KismetSystemLibrary.K2_ClearAndInvalidateTimerHandle` (`self.VR Part Time`)))

(event `self.Part 1 Grab.OnDropped`
  (params (`Self Ref` :type "/Game/Objects/Structurs/GrabComponent Object Reference"))
  ;[1 1 1] VR
  (`KismetSystemLibrary.K2_ClearAndInvalidateTimerHandle` (`self.VR Part Time`)))

(event `self.Part 3 Grab.OnDropped`
  (params (`Self Ref` :type "/Game/Objects/Structurs/GrabComponent Object Reference"))
  ;[1 1 1] VR
  (`KismetSystemLibrary.K2_ClearAndInvalidateTimerHandle` (`self.VR Part Time`)))

(fn `Update Location Part 1`
  (bind _part_1_capsule (`self.Part 1 Capsule`))
  (bind _spline (`self.Spline`))
  (bind _returnvalue_x (`KismetMathLibrary.BreakVector` (`SplineComponent.GetLocationAtSplinePoint` _spline 1 "Local")))
  (bind _returnvalue_x_2 (`KismetMathLibrary.BreakVector` (`SplineComponent.GetLocationAtSplinePoint` _spline 0 "Local")))
  (bind (_relativelocation_x _relativelocation_y _relativelocation_z) (`KismetMathLibrary.BreakVector` (`SceneComponent.RelativeLocation` (`self.Part 1 Capsule`))))
  (bind (_relativelocation_x_2 _relativelocation_y_2) (`KismetMathLibrary.BreakVector` (`SceneComponent.RelativeLocation` (`self.Part 1 Capsule`))))
  (bind (_relativelocation_x_3 _relativelocation_y_3) (`KismetMathLibrary.BreakVector` (`SceneComponent.RelativeLocation` _part_1_capsule)))
  (bind (_relativelocation_x_4 _relativelocation_y_4 _relativelocation_z_2) (`KismetMathLibrary.BreakVector` (`SceneComponent.RelativeLocation` (`self.Part 2`))))
  (`SceneComponent.K2_SetRelativeLocation` (`self.Part 1 Capsule`) (`KismetMathLibrary.MakeVector` _relativelocation_x (`KismetMathLibrary.FClamp` (+ _relativelocation_y_3 (.y (.location (`KismetMathLibrary.MakeRelativeTransform` (`SceneComponent.K2_GetComponentToWorld` (`/Game/Objects/Structurs/GrabComponent.MotionControllerRef` (`self.Part 1 Grab`))) (`SceneComponent.K2_GetComponentToWorld` _part_1_capsule))))) _returnvalue_x_2 _returnvalue_x) _relativelocation_z) false false)
  (`SceneComponent.K2_SetRelativeLocation` (`self.Part 2`) (`KismetMathLibrary.MakeVector` _relativelocation_x_4 (- _relativelocation_y_2 53.0) _relativelocation_z_2) false false))

(fn `Update Location Part 2`
  (bind _part_2_capsule (`self.Part 2 Capsule`))
  (bind _spline (`self.Spline`))
  (bind _returnvalue_x (`KismetMathLibrary.BreakVector` (`SplineComponent.GetLocationAtSplinePoint` _spline 1 "Local")))
  (bind _returnvalue_x_2 (`KismetMathLibrary.BreakVector` (`SplineComponent.GetLocationAtSplinePoint` _spline 0 "Local")))
  (bind (_relativelocation_x _relativelocation_y _relativelocation_z) (`KismetMathLibrary.BreakVector` (`SceneComponent.RelativeLocation` (`self.Part 2 Capsule`))))
  (bind (_relativelocation_x_2 _relativelocation_y_2) (`KismetMathLibrary.BreakVector` (`SceneComponent.RelativeLocation` (`self.Part 2 Capsule`))))
  (bind (_relativelocation_x_3 _relativelocation_y_3) (`KismetMathLibrary.BreakVector` (`SceneComponent.RelativeLocation` _part_2_capsule)))
  (bind (_relativelocation_x_4 _relativelocation_y_4 _relativelocation_z_2) (`KismetMathLibrary.BreakVector` (`SceneComponent.RelativeLocation` (`self.Part 1`))))
  (`SceneComponent.K2_SetRelativeLocation` (`self.Part 2 Capsule`) (`KismetMathLibrary.MakeVector` _relativelocation_x (`KismetMathLibrary.FClamp` (+ _relativelocation_y_3 (.y (.location (`KismetMathLibrary.MakeRelativeTransform` (`SceneComponent.K2_GetComponentToWorld` (`/Game/Objects/Structurs/GrabComponent.MotionControllerRef` (`self.Part 2 Grab`))) (`SceneComponent.K2_GetComponentToWorld` _part_2_capsule))))) _returnvalue_x_2 _returnvalue_x) _relativelocation_z) false false)
  (`SceneComponent.K2_SetRelativeLocation` (`self.Part 1`) (`KismetMathLibrary.MakeVector` _relativelocation_x_4 (- _relativelocation_y_2 53.0) _relativelocation_z_2) false false))

(fn `Update Location Part 3`
  (bind _part_3_capsule (`self.Part 3 Capsule`))
  (bind _spline (`self.Spline`))
  (bind _returnvalue_x (`KismetMathLibrary.BreakVector` (`SplineComponent.GetLocationAtSplinePoint` _spline 1 "Local")))
  (bind _returnvalue_x_2 (`KismetMathLibrary.BreakVector` (`SplineComponent.GetLocationAtSplinePoint` _spline 0 "Local")))
  (bind (_relativelocation_x _relativelocation_y _relativelocation_z) (`KismetMathLibrary.BreakVector` (`SceneComponent.RelativeLocation` (`self.Part 3 Capsule`))))
  (bind (_relativelocation_x_2 _relativelocation_y_2) (`KismetMathLibrary.BreakVector` (`SceneComponent.RelativeLocation` (`self.Part 3 Capsule`))))
  (bind (_relativelocation_x_3 _relativelocation_y_3) (`KismetMathLibrary.BreakVector` (`SceneComponent.RelativeLocation` _part_3_capsule)))
  (bind (_relativelocation_x_4 _relativelocation_y_4 _relativelocation_z_2) (`KismetMathLibrary.BreakVector` (`SceneComponent.RelativeLocation` (`self.Part 3`))))
  (`SceneComponent.K2_SetRelativeLocation` (`self.Part 3 Capsule`) (`KismetMathLibrary.MakeVector` _relativelocation_x (`KismetMathLibrary.FClamp` (+ _relativelocation_y_3 (.y (.location (`KismetMathLibrary.MakeRelativeTransform` (`SceneComponent.K2_GetComponentToWorld` (`/Game/Objects/Structurs/GrabComponent.MotionControllerRef` (`self.Part 3 Grab`))) (`SceneComponent.K2_GetComponentToWorld` _part_3_capsule))))) _returnvalue_x_2 _returnvalue_x) _relativelocation_z) false false)
  (`SceneComponent.K2_SetRelativeLocation` (`self.Part 3`) (`KismetMathLibrary.MakeVector` _relativelocation_x_4 (- _relativelocation_y_2 53.0) _relativelocation_z_2) false false))

(fn `UserConstructionScript`
  (`parent.UserConstructionScript`))
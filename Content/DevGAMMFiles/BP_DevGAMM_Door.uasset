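; BP_DevGAMM_Door is a child door Blueprint for the DevGAMM files that can trigger a cutscene when interacted with.
; Its Interact override sets the CutsceneManeger state, skipping parent behavior, when Locks is empty, AutoLock and StartLook are off, and the manager is valid.
; Otherwise it forwards the interaction to the parent, and its construction script only calls the parent's.
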(event `/Game/Function/BP_Interface.Interact`
  (params (Component :type "PrimitiveComponent Object Reference") (Location :type "Vector Structure"))
  (if (and (== (`KismetArrayLibrary.Array_Length` (`self.Locks`)) 0) (not (`self.Auto Lock`)) (`KismetSystemLibrary.IsValid` (`self.Cutscene Maneger`)) (not (`self.Start Look`)))
    (`/Game/Objects/Cutscene/BP_Cutscene_Manager.Set State` (`self.Cutscene Maneger`) "NewEnumerator0")
    (else
      (`parent.Interact` Component Location))))

(fn `UserConstructionScript`
  (`parent.UserConstructionScript`))
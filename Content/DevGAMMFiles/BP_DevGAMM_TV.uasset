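; Interactive TV prop that toggles on and off, switching its sound, two lights and screen material, with power from electricity or a generator.
; Use, VR use and remote events share the toggle; LMB toggles it when held.
; A player switching it on with electricity sends the Neighbor AI to investigate through blackboard keys; other paths can report tutorial and GameJolt use checks.
; Disable blanks the TV; Enable restores it if on.
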(event `RemoteTV`
  (params (`Neighbor?` :type Boolean))
  (bind _root (`self.Root`))
  (bind _tv_sound (`self.TV Sound`))
  (bind _rectlight (`self.RectLight`))
  (if (not `Neighbor?`)
    (if (`|EnumInequality` (`self.State`) "NewEnumerator0") :!label _label
      (if (`self.Has Electricity`)
        ;[1 1 1] Neighbor coming to check
        (bind _sosed (`/Game/Function/BP_MacroLibrary.Find Sosed`)
          (:`Is Valid`
            (if (`|EnumInequality` (`/Game/Sosed/BP_Sosed.Current State` _sosed) "NewEnumerator2")
              (bind _returnvalue (`AIBlueprintHelperLibrary.GetBlackboard` _sosed))
              (`BlackboardComponent.SetValueAsInt` _returnvalue "CheckTask" 8)
              (`BlackboardComponent.SetValueAsVector` _returnvalue "Check Location" (`SceneComponent.K2_GetComponentLocation` (`self.Arrow`)))
              (`BlackboardComponent.SetValueAsObject` _returnvalue "CheckActor" self)
              (`/Game/Sosed/BP_Sosed.Set State` _sosed "NewEnumerator3")
              (if (or (`self.Has Electricity`) (`self.Generator`)) :!label _label_2
                (switch `/Game/Objects/Enum/TumblerStateEnum` (`self.State`)
                  (:`NewEnumerator0`
                    (`AudioComponent.Stop` _tv_sound :!label _label_3)
                    (`LightComponent.SetIntensity` _rectlight 0.0)
                    (`LightComponent.SetIntensity` (`self.PointLight`) 0.0)
                    (set `self.State` "NewEnumerator1")
                    (`PrimitiveComponent.SetMaterial` _root 0 "/Game/Objects/Materials/tv_display_off.tv_display_off"))
                  (:`NewEnumerator1`
                    (`AudioComponent.Play` _tv_sound 0.0)
                    (`LightComponent.SetIntensity` _rectlight 5000.0)
                    (`LightComponent.SetIntensity` (`self.PointLight`) 5000.0)
                    (set `self.State` "NewEnumerator0")
                    (`PrimitiveComponent.SetMaterial` _root 0 "/Game/Objects/Materials/tv_display_on.tv_display_on")))
                (else
                  (goto _label_3)))))
          (:`Is Not Valid`
            (`/Game/Objects/Tutorial/TutorialComponent.Check Use Type` (`self.TutorialComponent`) "NewEnumerator6" :!label _label_4)
            (`/Game/Objects/GameJolt/GameJoltComponent.Check Use Type` (`self.GameJoltComponent`) "NewEnumerator6")
            (goto _label_2))))
      (else
        (goto _label_4)))
    (else
      (goto _label_4))))

(event `self.On VR Use`
  (`parent.On VR Use`)
  (goto _label))

(event `self.Interact`
  (params (Component :type "PrimitiveComponent Object Reference") (Location :type "Vector Structure"))
  (goto _label))

(event `self.On Press LMB`
  (bind _player (`/Game/Function/BP_MacroLibrary.Find Player`)
    (:`Is Valid`
      (bind _item (`/Game/Player/BP_Player.Get Item` _player))
      (if (== _item self)
        (goto _label_2)))))

(event `self.Disable`
  (`parent.Disable`)
  (`AudioComponent.Stop` (`self.TV Sound`))
  (`LightComponent.SetIntensity` (`self.RectLight`) 0.0)
  (`LightComponent.SetIntensity` (`self.PointLight`) 0.0)
  (`PrimitiveComponent.SetMaterial` (`self.Root`) 0 "/Game/Objects/Materials/tv_display_off.tv_display_off"))

(event `self.Enable`
  (`parent.Enable`)
  (if (`|EnumEquality` (`self.State`) "NewEnumerator0")
    (`AudioComponent.Play` (`self.TV Sound`) 0.0)
    (`LightComponent.SetIntensity` (`self.RectLight`) 5000.0)
    (`LightComponent.SetIntensity` (`self.PointLight`) 5000.0)
    (`PrimitiveComponent.SetMaterial` (`self.Root`) 0 "/Game/Objects/Materials/tv_display_on.tv_display_on")))

(fn `UserConstructionScript`)
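; Interactable mailbox actor with a flag and a hinged part that rotate when used.
; The flag toggles through a FlipFlop timeline, while the part uses an Open/Opening/Close/Closing state, ignoring interaction mid-motion.
; Opening plays its sound as movement starts, and closing plays its sound when movement finishes.
; Part use reports to TutorialComponent and GameJoltComponent, with TutorialComponent also receiving separate open and close use types.
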(event `self.Interact`
  (params (Component :type "PrimitiveComponent Object Reference") (Location :type "Vector Structure"))
  (`|ExecutionSequence`
    (:`then_0`
      (if (== Component (`self.Flag`))
        (`/Engine/EditorBlueprintResources/StandardMacros.FlipFlop`
          (:`A`
            (bind (_direction _alpha) (`Timeline|Flag Rotate Timeline` :!label _label)
              (:`Update`
                (`SceneComponent.K2_SetRelativeRotation` (`self.Flag`) (`KismetMathLibrary.RLerp` (struct) (struct :`Roll` -90.0) _alpha) false false))))
          (:`B`
            (goto _label :!via `Reverse`)))))
    (:`then_1`
      ;[1 1 1] Part Rotate
      (if (== Component (`self.Part`))
        (`/Game/Objects/Tutorial/TutorialComponent.Check Use Type` (`self.TutorialComponent`) "NewEnumerator6")
        (`/Game/Objects/GameJolt/GameJoltComponent.Check Use Type` (`self.GameJoltComponent`) "NewEnumerator6")
        (switch `/Game/Objects/Enum/RotateStateEnum` (`self.Part Rotate`)
          (:`NewEnumerator0`
            (set `self.Part Rotate` "NewEnumerator3")
            (`/Game/Objects/Tutorial/TutorialComponent.Check Use Type` (`self.TutorialComponent`) "NewEnumerator2")
            (bind (_direction_2 _alpha_2) (`Timeline|Part Rotate Timeline` :!via `Reverse` :!label _label_2)
              (:`Update`
                (`SceneComponent.K2_SetRelativeRotation` (`self.Part`) (`KismetMathLibrary.RLerp` (struct) (struct :`Roll` -100.0) _alpha_2) false false))
              (:`Finished`
                (switch `/Game/Objects/Enum/RotateStateEnum` (`self.Part Rotate`)
                  (:`NewEnumerator2`
                    (set `self.Part Rotate` "NewEnumerator0"))
                  (:`NewEnumerator3`
                    (set `self.Part Rotate` "NewEnumerator1")
                    (`GameplayStatics.PlaySoundAtLocation` "/Game/Sounds/Objects/OpenClosed/mailbox_close_Cue.mailbox_close_Cue" (`self.K2_GetActorLocation`) (struct) 1.0 1.0 0.0 null null null null))))))
          (:`NewEnumerator1`
            (set `self.Part Rotate` "NewEnumerator2")
            (`|ExecutionSequence`
              (:`then_0`
                (goto _label_2))
              (:`then_1`
                (`GameplayStatics.PlaySoundAtLocation` "/Game/Sounds/Objects/OpenClosed/mailbox_open_Cue.mailbox_open_Cue" (`self.K2_GetActorLocation`) (struct) 1.0 1.0 0.0 null null null null)
                (`/Game/Objects/Tutorial/TutorialComponent.Check Use Type` (`self.TutorialComponent`) "NewEnumerator1")))))))))

(fn `UserConstructionScript`)
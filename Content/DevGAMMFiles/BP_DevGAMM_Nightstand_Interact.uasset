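; Interactable nightstand that slides between two positions in both desktop and VR play, toggling auto-lock on a linked Rotate object.
; Without an HMD, interacting outside the Part1/Part2 components alternately plays and reverses a transform-lerp timeline, gated until each move finishes.
; In VR, grabbing runs a looping timer that follows the motion controller on Y, clamped between spline points, and sets auto-lock past a spline-distance threshold.
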(event `self.ReceiveBeginPlay`
  (`parent.ReceiveBeginPlay`))

(event `/Game/Function/BP_Interface.Interact`
  (params (Component :type "PrimitiveComponent Object Reference") (Location :type "Vector Structure"))
  (bind _rotate (`self.Rotate`))
  (if (and (not (`HeadMountedDisplayFunctionLibrary.IsHeadMountedDisplayEnabled`)) (!= Component (`self.Part 2`)) (!= Component (`self.Part 1`)) (!= Component (`self.Part 1 Capsule`)) (!= Component (`self.Part 2 Capsule`)))
    (`self.Rotate`
      (:`then`
        (`/Engine/EditorBlueprintResources/StandardMacros.DoOnce` false :!label _label
          (:`Completed`
            (`/Engine/EditorBlueprintResources/StandardMacros.FlipFlop`
              (:`A`
                (set `/Game/Objects/Structurs/BP_Rotate.Auto Lock` true _rotate)
                (bind (_direction _alpha) (`Timeline|Шкала времени` :!label _label_2)
                  (:`Update`
                    (`SceneComponent.K2_SetWorldTransform` (`self.Root`) (`KismetMathLibrary.TLerp` (`self.Start Pos`) (`self.End Pos`) _alpha) false false))
                  (:`Finished`
                    (goto _label :!via `Reset`))))
              (:`B`
                (set `/Game/Objects/Structurs/BP_Rotate.Auto Lock` false _rotate)
                (goto _label_2 :!via `Reverse`))))))
      (:`else`))))

(event `self.Global Grab.OnGrabbed`
  (params (`Self Ref` :type "/Game/Objects/Structurs/GrabComponent Object Reference"))
  (bind _returnvalue (`KismetSystemLibrary.K2_SetTimer` null "Update Location Global" 0.01 true))
  (set `self.VR Global Time` _returnvalue))

(event `self.Global Grab.OnDropped`
  (params (`Self Ref` :type "/Game/Objects/Structurs/GrabComponent Object Reference"))
  (`KismetSystemLibrary.K2_ClearAndInvalidateTimerHandle` (`self.VR Global Time`)))

(fn `Update Location Global`
  (bind _global_box (`self.Global Box`))
  (bind _nightstand (`self.Nightstand`))
  (bind _global_spline (`self.Global Spline`))
  (bind (_returnvalue_x _returnvalue_y) (`KismetMathLibrary.BreakVector` (`SplineComponent.GetLocationAtSplinePoint` _global_spline 1 "Local")))
  (bind (_returnvalue_x_2 _returnvalue_y_2) (`KismetMathLibrary.BreakVector` (`SplineComponent.GetLocationAtSplinePoint` _global_spline 0 "Local")))
  (bind (_relativelocation_x _relativelocation_y _relativelocation_z) (`KismetMathLibrary.BreakVector` (`SceneComponent.RelativeLocation` (`self.Global Box`))))
  (bind (_relativelocation_x_2 _relativelocation_y_2 _relativelocation_z_2) (`KismetMathLibrary.BreakVector` (`SceneComponent.RelativeLocation` _nightstand)))
  (bind (_relativelocation_x_3 _relativelocation_y_3) (`KismetMathLibrary.BreakVector` (`SceneComponent.RelativeLocation` _global_box)))
  (`SceneComponent.K2_SetRelativeLocation` (`self.Global Box`) (`KismetMathLibrary.MakeVector` _relativelocation_x (`KismetMathLibrary.FClamp` (+ (.y (.location (`KismetMathLibrary.MakeRelativeTransform` (`SceneComponent.K2_GetComponentToWorld` (`/Game/Objects/Structurs/GrabComponent.MotionControllerRef` (`self.Global Grab`))) (`SceneComponent.K2_GetComponentToWorld` (`self.Global Box`))))) _relativelocation_y) _returnvalue_y_2 _returnvalue_y) _relativelocation_z) false false)
  (`SceneComponent.K2_SetRelativeLocation` _nightstand (`KismetMathLibrary.MakeVector` _relativelocation_x_2 _relativelocation_y_3 _relativelocation_z_2) false false)
  (if (>= (`SplineComponent.GetDistanceAlongSplineAtLocation` (`self.Global Spline`) (`SceneComponent.RelativeLocation` _global_box) "Local") 0.95)
    (bind _rotate (`self.Rotate`)
      (:`then`
        (set `/Game/Objects/Structurs/BP_Rotate.Auto Lock` true _rotate))
      (:`else`))
    (else
      (bind _rotate_2 (`self.Rotate`)
        (:`then`
          (set `/Game/Objects/Structurs/BP_Rotate.Auto Lock` false _rotate_2))
        (:`else`)))))

(fn `UserConstructionScript`
  (`parent.UserConstructionScript`))
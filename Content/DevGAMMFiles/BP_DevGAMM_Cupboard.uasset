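; BP_DevGAMM_Cupboard is a cupboard with a sliding drawer that opens by interaction or VR grab.
; Interacting with the drawer or its capsule flip-flops the Open timeline, lerping the drawer along local Y with open and close sounds.
; While Part1Grab is held, a looping timer moves the capsule toward the motion controller on Y, clamped by spline endpoints, and the drawer follows at a fixed offset.
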(event `/Game/Function/BP_Interface.Interact`
  (params (Component :type "PrimitiveComponent Object Reference") (Location :type "Vector Structure"))
  (if (or (== Component (`self.Drawer`)) (== Component (`self.Part 1 Capsule`)))
    (`/Engine/EditorBlueprintResources/StandardMacros.FlipFlop`
      (:`A`
        (`|ExecutionSequence`
          (:`then_0`
            (bind (_direction _lerp) (`Timeline|Open` :!label _label)
              (:`Update`
                (`SceneComponent.K2_SetRelativeLocation` (`self.Drawer`) (`KismetMathLibrary.VLerp` (0.0 0.0 0.0) (0.0 40.0 0.0) _lerp) false false))))
          (:`then_1`
            (`AudioComponent.Play` (`self.Open Sound`) 0.0))))
      (:`B`
        (`|ExecutionSequence`
          (:`then_0`
            (goto _label :!via `Reverse`))
          (:`then_1`
            (`AudioComponent.Play` (`self.Close Sound`) 0.0)))))))

(event `self.Part 1 Grab.OnGrabbed`
  (params (`Self Ref` :type "/Game/Objects/Structurs/GrabComponent Object Reference"))
  (bind _returnvalue (`KismetSystemLibrary.K2_SetTimer` null "Update Location Part 1" 0.01 true))
  (set `self.VR Part Time` _returnvalue))

(event `self.Part 1 Grab.OnDropped`
  (params (`Self Ref` :type "/Game/Objects/Structurs/GrabComponent Object Reference"))
  (`KismetSystemLibrary.K2_ClearAndInvalidateTimerHandle` (`self.VR Part Time`)))

(fn `Update Location Part 1`
  (bind _part_1_capsule (`self.Part 1 Capsule`))
  (bind _spline (`self.Spline`))
  (bind _returnvalue_x (`KismetMathLibrary.BreakVector` (`SplineComponent.GetLocationAtSplinePoint` _spline 1 "Local")))
  (bind _returnvalue_x_2 (`KismetMathLibrary.BreakVector` (`SplineComponent.GetLocationAtSplinePoint` _spline 0 "Local")))
  (bind (_relativelocation_x _relativelocation_y _relativelocation_z) (`KismetMathLibrary.BreakVector` (`SceneComponent.RelativeLocation` (`self.Part 1 Capsule`))))
  (bind (_relativelocation_x_2 _relativelocation_y_2) (`KismetMathLibrary.BreakVector` (`SceneComponent.RelativeLocation` (`self.Part 1 Capsule`))))
  (bind (_relativelocation_x_3 _relativelocation_y_3) (`KismetMathLibrary.BreakVector` (`SceneComponent.RelativeLocation` _part_1_capsule)))
  (bind (_relativelocation_x_4 _relativelocation_y_4 _relativelocation_z_2) (`KismetMathLibrary.BreakVector` (`SceneComponent.RelativeLocation` (`self.Drawer`))))
  (`SceneComponent.K2_SetRelativeLocation` (`self.Part 1 Capsule`) (`KismetMathLibrary.MakeVector` _relativelocation_x (`KismetMathLibrary.FClamp` (+ _relativelocation_y_3 (.y (.location (`KismetMathLibrary.MakeRelativeTransform` (`SceneComponent.K2_GetComponentToWorld` (`/Game/Objects/Structurs/GrabComponent.MotionControllerRef` (`self.Part 1 Grab`))) (`SceneComponent.K2_GetComponentToWorld` _part_1_capsule))))) _returnvalue_x_2 _returnvalue_x) _relativelocation_z) false false)
  (`SceneComponent.K2_SetRelativeLocation` (`self.Drawer`) (`KismetMathLibrary.MakeVector` _relativelocation_x_4 (- _relativelocation_y_2 33.0) _relativelocation_z_2) false false))

(fn `UserConstructionScript`
  (`parent.UserConstructionScript`))
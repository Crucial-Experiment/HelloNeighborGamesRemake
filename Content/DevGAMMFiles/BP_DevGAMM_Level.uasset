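; BP_DevGAMM_Level is a push-button switch that turns a linked list of Electricity objects on and off.
; Interact, or a VR hand overlapping the button, alternates disabling and enabling them when powered or a generator, and otherwise disables them.
; A separate FlipFlop plays or reverses a timeline that slides the button, even without power.
; Its own Enable and Disable call the parent and propagate to the linked objects.
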(event `self.Enable`
  (`parent.Enable`)
  (for _array_element (`self.Electricity`) :!label _label
    (`/Engine/EditorBlueprintResources/StandardMacros.IsValid` _array_element
      (:`Is Valid`
        (`self.Enable` _array_element)))))

(event `/Game/Function/BP_Interface.Interact`
  (params (Component :type "PrimitiveComponent Object Reference") (Location :type "Vector Structure"))
  (bind _generator (`self.Generator`))
  (`|ExecutionSequence` :!label _label_2
    (:`then_0`
      (if (or (`self.Has Electricity`) _generator)
        (`/Engine/EditorBlueprintResources/StandardMacros.FlipFlop`
          (:`A`
            (for _array_element (`self.Electricity`) :!label _label_3
              (`/Engine/EditorBlueprintResources/StandardMacros.IsValid` _array_element
                (:`Is Valid`
                  (`self.Disable` _array_element)))))
          (:`B`
            (goto _label)))
        (elif (not _generator)
          (goto _label_3))))
    (:`then_1`
      (if (or (== Component (`self.Button`)) (== (stale `self.Button.OnComponentBeginOverlap` OtherComp) (`self.Button`)))
        (`/Engine/EditorBlueprintResources/StandardMacros.FlipFlop`
          (:`A`
            (`|ExecutionSequence`
              (:`then_0`
                (bind (_direction _alpha) (`Timeline|Button Loc` :!label _label_4)
                  (:`Update`
                    (`SceneComponent.K2_SetRelativeLocation` (`self.Button`) (`KismetMathLibrary.VLerp` (-10.0 0.0 -11.0) (0.0 0.0 -11.0) _alpha) false false))))))
          (:`B`
            (`|ExecutionSequence`
              (:`then_0`
                (goto _label_4 :!via `Reverse`)))))))))

(event `self.Disable`
  (`parent.Disable`)
  (goto _label_3))

(event `self.Button.OnComponentBeginOverlap`
  (params (OverlappedComponent :type "PrimitiveComponent Object Reference") (OtherActor :type "Actor Object Reference") (OtherComp :type "PrimitiveComponent Object Reference") (OtherBodyIndex :type Integer) (bFromSweep :type Boolean) (SweepResult :type "HitResult Structure (by ref)"))
  (if (`self.Overlap VR Hands` OtherActor OtherComp)
    (goto _label_2)))

(fn `UserConstructionScript`
  (`parent.UserConstructionScript`))
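; BP_Holiday_Manager is a placed actor that applies seasonal changes to the level at BeginPlay when its Holiday matches the current holiday.
; It adds optional Niagara and particle effects, then spawns listed actors with configured collision, overriding meshes on StaticMeshActor and BP_Object entries.
; It also makes an optional Landscape movable to relocate it, and swaps the skeletal mesh on referenced actors.
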(event `self.ReceiveBeginPlay`
  (bind _returnvalue (`self.GetTransform`))
  (if (`|EnumEquality` (`self.Holiday`) (`/Game/Function/BP_FunctionLibrary.Get Current Holiday`))
    (`|ExecutionSequence`
      (:`then_0`
        (bind _niagara_system (`self.Niagara System`)
          (:`then`
            (bind _returnvalue_2 (`AddComponent|NODE_AddNiagaraComponent-0` :`RelativeTransform` _returnvalue))
            (`NiagaraComponent.SetAsset` _returnvalue_2 _niagara_system true))
          (:`else`)))
      (:`then_1`
        (bind _particle_system (`self.Particle System`)
          (:`then`
            (bind _returnvalue_3 (`AddComponent|NODE_AddParticleSystemComponent-0` :`RelativeTransform` _returnvalue))
            (`ParticleSystemComponent.SetTemplate` _returnvalue_3 _particle_system))
          (:`else`)))
      (:`then_2`
        (for _array_element (`self.Actors`)
          (bind _returnvalue_4 (`|SpawnActorFromClass` (break `/Game/Function/HolidayActorStruct` _array_element) (`.Transform_9_19DA582B48A17313E0D3789CE1A2A359` (break `/Game/Function/HolidayActorStruct` _array_element)) "Undefined" "MultiplyWithRoot" null null))
          (`self.SetActorEnableCollision` _returnvalue_4 (`.EnableCollision_12_F16AE19046CFB722F2710BAE61C8B943` (break `/Game/Function/HolidayActorStruct` _array_element)))
          (`/Engine/EditorBlueprintResources/StandardMacros.IsValid` (`.Mesh_6_24BDA54C48387527EC74C2BBD84A4E58` (break `/Game/Function/HolidayActorStruct` _array_element))
            (:`Is Valid`
              (`|ExecutionSequence`
                (:`then_0`
                  (if (== (break `/Game/Function/HolidayActorStruct` _array_element) "/Script/Engine.StaticMeshActor")
                    (bind _asstatic_mesh_actor (cast `StaticMeshActor` _returnvalue_4))
                    (`StaticMeshComponent.SetStaticMesh` (`StaticMeshActor.StaticMeshComponent` _asstatic_mesh_actor) (`.Mesh_6_24BDA54C48387527EC74C2BBD84A4E58` (break `/Game/Function/HolidayActorStruct` _array_element)))))
                (:`then_1`
                  (if (== (break `/Game/Function/HolidayActorStruct` _array_element) "/Game/Objects/Structurs/BP_Object.BP_Object_C")
                    (bind _asbp_object (cast `/Game/Objects/Structurs/BP_Object` _returnvalue_4))
                    (`StaticMeshComponent.SetStaticMesh` (`/Game/Objects/Structurs/BP_Object.Root` _asbp_object) (`.Mesh_6_24BDA54C48387527EC74C2BBD84A4E58` (break `/Game/Function/HolidayActorStruct` _array_element))))))))))
      (:`then_3`
        (bind _landscape (`self.Landscape`)
          (:`then`
            (`SceneComponent.SetMobility` (`Actor.RootComponent` _landscape) "Movable")
            (`self.K2_SetActorLocation` _landscape (`self.New Location`) false false))
          (:`else`)))
      (:`then_4`
        (for _array_element_2 (`self.Meshes`)
          (`SkeletalMeshComponent.SetSkeletalMeshAsset` (`SkeletalMeshActor.SkeletalMeshComponent` _array_element_2) (`self.New Mesh`)))))))

(fn `UserConstructionScript`)
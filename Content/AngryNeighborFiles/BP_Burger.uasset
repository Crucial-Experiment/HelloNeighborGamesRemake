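; BP_Burger is a burger actor that can be eaten in the game, apparently in VR given its VROnly event.
; On EventEat, it checks that the passed actor is itself and that its Eat flag is false, then plays a 2D eating sound and destroys itself.
; BeginPlay is disabled and the construction script only calls its parent.
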(event `/Game/Function/BP_Interface.Eat (VR Only)`
  (params (Actor :type "/Game/Objects/Structurs/BP_Object Object Reference"))
  (if (and (== Actor self) (not (`self.Eat?`)))
    (`GameplayStatics.PlaySound2D` "/Game/AngryNeighborFiles/Audio/burger_eat.burger_eat" 1.0 1.0 0.0 null null)
    (`self.K2_DestroyActor`)))

(fn `UserConstructionScript`
  (`parent.UserConstructionScript`))
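; Basement victim actor that idles with looping animation and screams when the player enters its trigger box, alerting the Neighbor.
; A randomly timed repeating timer plays random idle animations before returning to the base idle.
; On overlap it stops that timer, swaps to scream animation and sound, and, unless the Neighbor's state forbids it, sends them to investigate through blackboard keys and a state change.
; Leaving restores idle and restarts the timer.
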(event `Random Anim`
  (bind _outitem (`KismetArrayLibrary.Array_Random` (`self.Random Idle`)))
  (`SkeletalMeshComponent.PlayAnimation` (`self.SkeletalMesh`) _outitem false)
  (`KismetSystemLibrary.Delay` (+ (`AnimationAsset.GetPlayLength` _outitem) (`self.To Idle Anim Delay`)))
  (`SkeletalMeshComponent.PlayAnimation` (`self.SkeletalMesh`) (`self.Idle Anim`) true))

(event `self.ReceiveBeginPlay`
  (`SkeletalMeshComponent.PlayAnimation` (`self.SkeletalMesh`) (`self.Idle Anim`) true)
  (bind _sosed (`/Game/Function/BP_MacroLibrary.Find Sosed`)
    (:`Is Valid`
      (set `self.Neighbor` _sosed))
    (:`Is Not Valid`
      _))
  (bind _returnvalue (`KismetSystemLibrary.K2_SetTimerDelegate` (delegate `Random Anim`) (`KismetMathLibrary.RandomFloatInRange` (`self.Time Min`) (`self.Time Max`)) true true :!label _label))
  (set `self.Random Anim Timer` _returnvalue))

(event `self.Box.OnComponentBeginOverlap`
  (params (OverlappedComponent :type "PrimitiveComponent Object Reference") (OtherActor :type "Actor Object Reference") (OtherComp :type "PrimitiveComponent Object Reference") (OtherBodyIndex :type Integer) (bFromSweep :type Boolean) (SweepResult :type "HitResult Structure (by ref)"))
  (cast `/Game/Player/BP_Player` OtherActor)
  (`SkeletalMeshComponent.PlayAnimation` (`self.SkeletalMesh`) (`self.Scream Anim`) true)
  (`AudioComponent.Play` (`self.Scream`) 0.0)
  (`AudioComponent.Stop` (`self.Idle`))
  (`KismetSystemLibrary.K2_ClearAndInvalidateTimerHandle` (`self.Random Anim Timer`))
  ;[1 1 1] Neighbor coming to check
  (bind _neighbor (`self.Neighbor`)
    (:`then`
      (if (`|EnumInequality` (`/Game/Sosed/BP_Sosed.Current State` _neighbor) "NewEnumerator2")
        (bind _returnvalue (`AIBlueprintHelperLibrary.GetBlackboard` _neighbor))
        (`BlackboardComponent.SetValueAsInt` _returnvalue "CheckTask" 3)
        (`BlackboardComponent.SetValueAsVector` _returnvalue "Check Location" (`self.K2_GetActorLocation`))
        (`/Game/Sosed/BP_Sosed.Set State` _neighbor "NewEnumerator3")))
    (:`else`)))

(event `self.Box.OnComponentEndOverlap`
  (params (OverlappedComponent :type "PrimitiveComponent Object Reference") (OtherActor :type "Actor Object Reference") (OtherComp :type "PrimitiveComponent Object Reference") (OtherBodyIndex :type Integer))
  (cast `/Game/Player/BP_Player` OtherActor)
  (`SkeletalMeshComponent.PlayAnimation` (`self.SkeletalMesh`) (`self.Idle Anim`) true)
  (`AudioComponent.Stop` (`self.Scream`))
  (`AudioComponent.Play` (`self.Idle`) 0.0)
  (goto _label))

(fn `UserConstructionScript`)
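; BP_Sofa_Interact is an interactable sofa that slides and rotates between its start pose and an end pose.
; Interact calls InteractServer, and the Server.Interact event uses a FlipFlop to alternately play and reverse the SofaMove timeline.
; Each timeline update lerps the Sofa component's world transform from the actor's own location and rotation to EndPos and RotateEnd.
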(event `Interact (Server)`
  (`/Engine/EditorBlueprintResources/StandardMacros.FlipFlop`
    (:`A`
      (bind (_direction _alpha) (`Timeline|Sofa Move` :!label _label)
        (:`Update`
          (`SceneComponent.K2_SetWorldLocationAndRotation` (`self.Sofa`) (`KismetMathLibrary.VLerp` (`self.K2_GetActorLocation`) (`self.End Pos`) _alpha) (`KismetMathLibrary.RLerp` (`self.K2_GetActorRotation`) (`self.Rotate End`) _alpha) false false))))
    (:`B`
      (goto _label :!via `Reverse`))))

(event `/Game/Function/BP_Interface.Interact`
  (params (Component :type "PrimitiveComponent Object Reference") (Location :type "Vector Structure"))
  (`self.Interact (Server)`))

(fn `UserConstructionScript`
  (`parent.UserConstructionScript`))
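; Commode prop with three drawers that open and close, by interaction or by VR grab.
; Interact matches the hit drawer mesh or capsule, then a FlipFlop plays or reverses a timeline sliding it and plays open/close audio or effect.
; In VR, grabbing starts a looping timer that moves the capsule along Y with the motion controller, clamped between spline points, with the drawer following at an offset.
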(event `self.Interact`
  (params (Component :type "PrimitiveComponent Object Reference") (Location :type "Vector Structure"))
  ;[1 1 1] Interact
  (`|ExecutionSequence`
    (:`then_0`
      (if (or (== (`self.Part Big 1`) Component) (== (`self.Part Big 1 Capsule`) Component))
        (`/Engine/EditorBlueprintResources/StandardMacros.FlipFlop`
          (:`A`
            (`|ExecutionSequence`
              (:`then_0`
                (bind (_direction _alpha) (`Timeline|Шкала времени` :!label _label)
                  (:`Update`
                    (`SceneComponent.K2_SetRelativeLocation` (`self.Part Big 1`) (`KismetMathLibrary.VLerp` (0.3 3.4 27.5) (0.3 49.0 27.5) _alpha) false false))))
              (:`then_1`
                (`AudioComponent.Play` (`self.Part Big 1 Open`) 0.0))))
          (:`B`
            (`|ExecutionSequence`
              (:`then_0`
                (goto _label :!via `Reverse`))
              (:`then_1`
                (`AudioComponent.Play` (`self.Part Big 1 Close`) 0.0)))))))
    (:`then_1`
      (if (or (== (`self.Part Big 2`) Component) (== (`self.Part Big 2 Capsule`) Component))
        (`/Engine/EditorBlueprintResources/StandardMacros.FlipFlop`
          (:`A`
            (`|ExecutionSequence`
              (:`then_0`
                (bind (_direction_2 _alpha_2) (`Timeline|Шкала времени_0` :!label _label_2)
                  (:`Update`
                    (`SceneComponent.K2_SetRelativeLocation` (`self.Part Big 2`) (`KismetMathLibrary.VLerp` (0.8 3.0 54.3) (0.8 49.4 54.3) _alpha_2) false false))))
              (:`then_1`
                (`AudioComponent.Play` (`self.Part Big 2 Open`) 0.0))))
          (:`B`
            (`|ExecutionSequence`
              (:`then_0`
                (goto _label_2 :!via `Reverse`))
              (:`then_1`
                (`AudioComponent.Play` (`self.Part Big 2 Close`) 0.0)))))))
    (:`then_3`
      (if (or (== (`self.Part 1`) Component) (== (`self.Part 1 Capsule`) Component))
        (`/Engine/EditorBlueprintResources/StandardMacros.FlipFlop`
          (:`A`
            (`|ExecutionSequence`
              (:`then_0`
                (bind (_direction_3 _alpha_3) (`Timeline|Шкала времени_1` :!label _label_3)
                  (:`Update`
                    (`SceneComponent.K2_SetRelativeLocation` (`self.Part 1`) (`KismetMathLibrary.VLerp` (0.7 3.0 83.0) (0.7 49.4 83.0) _alpha_3) false false))))
              (:`then_1`
                (`AudioComponent.Play` (`self.Part 1 Open`) 0.0))))
          (:`B`
            (`|ExecutionSequence`
              (:`then_0`
                (goto _label_3 :!via `Reverse`))
              (:`then_1`
                (`AudioComponent.Play` (`self.Part 1 Close`) 0.0)))))))))

(event `self.Part 1 Big Grab.OnGrabbed`
  (params (`Self Ref` :type "/Game/Objects/Structurs/GrabComponent Object Reference"))
  ;[1 1 1] VR
  (bind _returnvalue (`KismetSystemLibrary.K2_SetTimer` null "Update Location Part 1 Big" 0.01 true))
  (set `self.VR Part Time` _returnvalue))

(event `self.Part 2 Big Grab.OnGrabbed`
  (params (`Self Ref` :type "/Game/Objects/Structurs/GrabComponent Object Reference"))
  ;[1 1 1] VR
  (bind _returnvalue (`KismetSystemLibrary.K2_SetTimer` null "Update Location Part 2 Big" 0.01 true))
  (set `self.VR Part Time` _returnvalue))

(event `self.Part 1 Grab.OnGrabbed`
  (params (`Self Ref` :type "/Game/Objects/Structurs/GrabComponent Object Reference"))
  ;[1 1 1] VR
  (bind _returnvalue (`KismetSystemLibrary.K2_SetTimer` null "Update Location Part 1" 0.01 true))
  (set `self.VR Part Time` _returnvalue))

(event `self.Part 1 Big Grab.OnDropped`
  (params (`Self Ref` :type "/Game/Objects/Structurs/GrabComponent Object Reference"))
  ;[1 1 1] VR
  (`KismetSystemLibrary.K2_ClearAndInvalidateTimerHandle` (`self.VR Part Time`)))

(event `self.Part 2 Big Grab.OnDropped`
  (params (`Self Ref` :type "/Game/Objects/Structurs/GrabComponent Object Reference"))
  ;[1 1 1] VR
  (`KismetSystemLibrary.K2_ClearAndInvalidateTimerHandle` (`self.VR Part Time`)))

(event `self.Part 1 Grab.OnDropped`
  (params (`Self Ref` :type "/Game/Objects/Structurs/GrabComponent Object Reference"))
  ;[1 1 1] VR
  (`KismetSystemLibrary.K2_ClearAndInvalidateTimerHandle` (`self.VR Part Time`)))

(fn `Update Location Part 1`
  (bind _part_1_capsule (`self.Part 1 Capsule`))
  (bind _spline (`self.Spline`))
  (bind _returnvalue_x (`KismetMathLibrary.BreakVector` (`SplineComponent.GetLocationAtSplinePoint` _spline 1 "Local")))
  (bind _returnvalue_x_2 (`KismetMathLibrary.BreakVector` (`SplineComponent.GetLocationAtSplinePoint` _spline 0 "Local")))
  (bind (_relativelocation_x _relativelocation_y _relativelocation_z) (`KismetMathLibrary.BreakVector` (`SceneComponent.RelativeLocation` (`self.Part 1 Capsule`))))
  (bind (_relativelocation_x_2 _relativelocation_y_2) (`KismetMathLibrary.BreakVector` (`SceneComponent.RelativeLocation` (`self.Part 1 Capsule`))))
  (bind (_relativelocation_x_3 _relativelocation_y_3) (`KismetMathLibrary.BreakVector` (`SceneComponent.RelativeLocation` _part_1_capsule)))
  (bind (_relativelocation_x_4 _relativelocation_y_4 _relativelocation_z_2) (`KismetMathLibrary.BreakVector` (`SceneComponent.RelativeLocation` (`self.Part 1`))))
  (`SceneComponent.K2_SetRelativeLocation` (`self.Part 1 Capsule`) (`KismetMathLibrary.MakeVector` _relativelocation_x (`KismetMathLibrary.FClamp` (+ _relativelocation_y_3 (.y (.location (`KismetMathLibrary.MakeRelativeTransform` (`SceneComponent.K2_GetComponentToWorld` (`/Game/Objects/Structurs/GrabComponent.MotionControllerRef` (`self.Part 1 Grab`))) (`SceneComponent.K2_GetComponentToWorld` _part_1_capsule))))) _returnvalue_x_2 _returnvalue_x) _relativelocation_z) false false)
  (`SceneComponent.K2_SetRelativeLocation` (`self.Part 1`) (`KismetMathLibrary.MakeVector` _relativelocation_x_4 (- _relativelocation_y_2 33.0) _relativelocation_z_2) false false))

(fn `Update Location Part 1 Big`
  (bind _part_big_1_capsule (`self.Part Big 1 Capsule`))
  (bind _spline (`self.Spline`))
  (bind _returnvalue_x (`KismetMathLibrary.BreakVector` (`SplineComponent.GetLocationAtSplinePoint` _spline 1 "Local")))
  (bind _returnvalue_x_2 (`KismetMathLibrary.BreakVector` (`SplineComponent.GetLocationAtSplinePoint` _spline 0 "Local")))
  (bind (_relativelocation_x _relativelocation_y _relativelocation_z) (`KismetMathLibrary.BreakVector` (`SceneComponent.RelativeLocation` (`self.Part Big 1 Capsule`))))
  (bind (_relativelocation_x_2 _relativelocation_y_2) (`KismetMathLibrary.BreakVector` (`SceneComponent.RelativeLocation` (`self.Part Big 1 Capsule`))))
  (bind (_relativelocation_x_3 _relativelocation_y_3) (`KismetMathLibrary.BreakVector` (`SceneComponent.RelativeLocation` _part_big_1_capsule)))
  (bind (_relativelocation_x_4 _relativelocation_y_4 _relativelocation_z_2) (`KismetMathLibrary.BreakVector` (`SceneComponent.RelativeLocation` (`self.Part Big 1`))))
  (`SceneComponent.K2_SetRelativeLocation` (`self.Part Big 1 Capsule`) (`KismetMathLibrary.MakeVector` _relativelocation_x (`KismetMathLibrary.FClamp` (+ _relativelocation_y_3 (.y (.location (`KismetMathLibrary.MakeRelativeTransform` (`SceneComponent.K2_GetComponentToWorld` (`/Game/Objects/Structurs/GrabComponent.MotionControllerRef` (`self.Part 1 Big Grab`))) (`SceneComponent.K2_GetComponentToWorld` _part_big_1_capsule))))) _returnvalue_x_2 _returnvalue_x) _relativelocation_z) false false)
  (`SceneComponent.K2_SetRelativeLocation` (`self.Part Big 1`) (`KismetMathLibrary.MakeVector` _relativelocation_x_4 (- _relativelocation_y_2 33.0) _relativelocation_z_2) false false))

(fn `Update Location Part 2 Big`
  (bind _part_big_2_capsule (`self.Part Big 2 Capsule`))
  (bind _spline (`self.Spline`))
  (bind _returnvalue_x (`KismetMathLibrary.BreakVector` (`SplineComponent.GetLocationAtSplinePoint` _spline 1 "Local")))
  (bind _returnvalue_x_2 (`KismetMathLibrary.BreakVector` (`SplineComponent.GetLocationAtSplinePoint` _spline 0 "Local")))
  (bind (_relativelocation_x _relativelocation_y _relativelocation_z) (`KismetMathLibrary.BreakVector` (`SceneComponent.RelativeLocation` (`self.Part Big 2 Capsule`))))
  (bind (_relativelocation_x_2 _relativelocation_y_2) (`KismetMathLibrary.BreakVector` (`SceneComponent.RelativeLocation` (`self.Part Big 2 Capsule`))))
  (bind (_relativelocation_x_3 _relativelocation_y_3) (`KismetMathLibrary.BreakVector` (`SceneComponent.RelativeLocation` _part_big_2_capsule)))
  (bind (_relativelocation_x_4 _relativelocation_y_4 _relativelocation_z_2) (`KismetMathLibrary.BreakVector` (`SceneComponent.RelativeLocation` (`self.Part Big 2`))))
  (`SceneComponent.K2_SetRelativeLocation` (`self.Part Big 2 Capsule`) (`KismetMathLibrary.MakeVector` _relativelocation_x (`KismetMathLibrary.FClamp` (+ _relativelocation_y_3 (.y (.location (`KismetMathLibrary.MakeRelativeTransform` (`SceneComponent.K2_GetComponentToWorld` (`/Game/Objects/Structurs/GrabComponent.MotionControllerRef` (`self.Part 2 Big Grab`))) (`SceneComponent.K2_GetComponentToWorld` _part_big_2_capsule))))) _returnvalue_x_2 _returnvalue_x) _relativelocation_z) false false)
  (`SceneComponent.K2_SetRelativeLocation` (`self.Part Big 2`) (`KismetMathLibrary.MakeVector` _relativelocation_x_4 (- _relativelocation_y_2 33.0) _relativelocation_z_2) false false))

(fn `UserConstructionScript`)
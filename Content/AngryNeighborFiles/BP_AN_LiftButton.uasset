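; Lift button panel that extends its parent's floor buttons with a fifth-floor button.
; UpdateFloors unhides Button5 and strips its "interactive" tag when the linked Lift has a fifth floor.
; Interacting with the visible button changes the Lift's state, pauses if the current floor has a door, then sets the target floor and changes state again.
; The construction script applies the shared button material to the first three buttons.
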(event `self.Update Floors`
  (bind _lift (`self.Lift`))
  (bind _button_5 (`self.Button_5`))
  (`parent.Update Floors`)
  (`/Engine/EditorBlueprintResources/StandardMacros.IsValid` _lift
    (:`Is Valid`
      (if (`KismetArrayLibrary.Array_IsValidIndex` (`/Game/Objects/BP_Objects/BP_Lift.Floors` _lift) 4)
        (`SceneComponent.SetHiddenInGame` _button_5 false false)
        (`KismetArrayLibrary.Array_RemoveItem` (`ActorComponent.ComponentTags` _button_5) "interactive")))))

(event `self.Interact (All)`
  (params (Component :type "PrimitiveComponent Object Reference"))
  (bind _button_5 (`self.Button_5`))
  (bind _lift (`self.Lift`))
  (`parent.Interact (All)` Component)
  (if (and (== Component _button_5) (not (`SceneComponent.bHiddenInGame` _button_5)))
    (`/Engine/EditorBlueprintResources/StandardMacros.IsValid` (`/Game/Objects/BP_Objects/BP_LiftFloor.Lift Door` (`|GetArrayItem` (`/Game/Objects/BP_Objects/BP_Lift.Floors` _lift) (`/Game/Objects/BP_Objects/BP_Lift.Flour` _lift)))
      (:`Is Valid`
        (`/Game/Objects/BP_Objects/BP_Lift.Set State` (`self.Lift`) "NewEnumerator3")
        (`KismetSystemLibrary.Delay` 1.6))
      (:`Is Not Valid`
        (`/Game/Objects/BP_Objects/BP_Lift.Set State` (`self.Lift`) "NewEnumerator3")))
    (set `/Game/Objects/BP_Objects/BP_Lift.Flour` 4 _lift)
    (`/Game/Objects/BP_Objects/BP_Lift.Set State` _lift "NewEnumerator1")))

(fn `UserConstructionScript`
  (`PrimitiveComponent.SetMaterial` (`self.Button_2`) 0 "/Game/AngryNeighborFiles/Materials/Lift_Buttons_mat.Lift_Buttons_mat")
  (`PrimitiveComponent.SetMaterial` (`self.Button_3`) 0 "/Game/AngryNeighborFiles/Materials/Lift_Buttons_mat.Lift_Buttons_mat")
  (`PrimitiveComponent.SetMaterial` (`self.Button_1`) 0 "/Game/AngryNeighborFiles/Materials/Lift_Buttons_mat.Lift_Buttons_mat"))
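; BP_Lever2 is an interactable power switch that enables or disables the actors in its Electricity array.
; Interaction runs through a server event, playing a sound and a timeline that slides the Level component between its on and off positions.
; When the slide finishes, it sets State, notifies tutorial and GameJolt components, and calls Tumbler.
; Tumbler passes power on only when the lever is On and has electricity or is a Generator.
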(event `self.ReceiveBeginPlay`
  ;[1 1 1] Begin Play
  (`parent.ReceiveBeginPlay`)
  (`PrimitiveComponent.SetSimulatePhysics` (`self.Root`) false)
  (`self.Tumbler` (`self.State`)))

(event `self.Enable`
  ;[1 1 1] Tumbler
  (`parent.Enable`)
  (switch `/Game/Objects/Enum/TumblerStateEnum` (`self.State`) :!label _label
    (:`NewEnumerator0`
      (for _array_element (`self.Electricity`)
        (`/Engine/EditorBlueprintResources/StandardMacros.IsValid` _array_element
          (:`Is Valid`
            (`self.Enable` _array_element)))))))

(event `Tumbler`
  (params (State :type "/Game/Objects/Enum/TumblerStateEnum Enum" :default "NewEnumerator0"))
  (bind _generator (`self.Generator`))
  ;[1 1 1] Tumbler
  (if (or (`self.Has Electricity`) _generator)
    (switch `/Game/Objects/Enum/TumblerStateEnum` State
      (:`NewEnumerator0`
        (goto _label))
      (:`NewEnumerator1`
        (for _array_element (`self.Electricity`) :!label _label_2
          (`/Engine/EditorBlueprintResources/StandardMacros.IsValid` _array_element
            (:`Is Valid`
              (`self.Disable` _array_element))))))
    (elif (not _generator)
      (goto _label_2))))

(event `self.Disable`
  ;[1 1 1] Tumbler
  (`parent.Disable`)
  (goto _label_2))

(event `Interact (Server)`
  (params (Component :type "PrimitiveComponent Object Reference"))
  (bind _tutorialcomponent (`self.TutorialComponent`))
  (bind _gamejoltcomponent (`self.GameJoltComponent`))
  (bind _state (`self.State`))
  ;[1 1 1] Rotation
  (if (== Component (`self.Level`))
    (switch `/Game/Objects/Enum/RotateStateEnum` (`self.Rotate State`)
      (:`NewEnumerator0`
        (set `self.Rotate State` "NewEnumerator3")
        (`|ExecutionSequence`
          (:`then_0`
            (bind (_direction _alpha) (`Timeline|Rotate Timeline` :!via `PlayFromStart` :!label _label_3)
              (:`Update`
                (`SceneComponent.K2_SetRelativeLocation` (`self.Level`) (`KismetMathLibrary.VLerp` (select `/Game/Objects/Enum/TumblerStateEnum` _state :`NewEnumerator0` (0.0 0.0 -4.0) :`NewEnumerator1` (0.0 0.0 3.3) :!type "Vector Structure") (select `/Game/Objects/Enum/TumblerStateEnum` _state :`NewEnumerator0` (0.0 0.0 3.3) :`NewEnumerator1` (0.0 0.0 -4.0) :!type "Vector Structure") _alpha) false false))
              (:`Finished`
                (switch `/Game/Objects/Enum/RotateStateEnum` (`self.Rotate State`)
                  (:`NewEnumerator2`
                    (set `self.Rotate State` "NewEnumerator0")
                    (set `self.State` "NewEnumerator0")
                    (`/Game/Objects/Tutorial/TutorialComponent.Check Use Type` _tutorialcomponent "NewEnumerator3")
                    (`/Game/Objects/GameJolt/GameJoltComponent.Check Use Type` _gamejoltcomponent "NewEnumerator3"))
                  (:`NewEnumerator3`
                    (set `self.Rotate State` "NewEnumerator1")
                    (set `self.State` "NewEnumerator1")
                    (`/Game/Objects/Tutorial/TutorialComponent.Check Use Type` _tutorialcomponent "NewEnumerator4")
                    (`/Game/Objects/GameJolt/GameJoltComponent.Check Use Type` _gamejoltcomponent "NewEnumerator4")))
                (`self.Tumbler` (`self.State`)))))
          (:`then_1`
            (`GameplayStatics.PlaySoundAtLocation` (`self.On / Off Sound`) (`self.K2_GetActorLocation`) (struct) 1.0 1.0 0.0 null null null null))))
      (:`NewEnumerator1`
        (set `self.Rotate State` "NewEnumerator2")
        (`|ExecutionSequence`
          (:`then_0`
            (goto _label_3 :!via `PlayFromStart`))
          (:`then_1`
            (`GameplayStatics.PlaySoundAtLocation` (`self.On / Off Sound`) (`self.K2_GetActorLocation`) (struct) 1.0 1.0 0.0 null null null null)))))))

(event `self.Interact`
  (params (Component :type "PrimitiveComponent Object Reference") (Location :type "Vector Structure"))
  ;[1 1 1] Rotation
  (`self.Interact (Server)` Component))

(fn `UserConstructionScript`
  (bind _level (`self.Level`))
  (`parent.UserConstructionScript`)
  (switch `/Game/Objects/Enum/TumblerStateEnum` (`self.State`)
    (:`NewEnumerator0`
      (`SceneComponent.K2_SetRelativeLocation` _level (0.0 0.0 -4.0) false false)
      (set `self.Rotate State` "NewEnumerator0"))
    (:`NewEnumerator1`
      (`SceneComponent.K2_SetRelativeLocation` _level (0.0 0.0 3.0) false false)
      (set `self.Rotate State` "NewEnumerator1"))))
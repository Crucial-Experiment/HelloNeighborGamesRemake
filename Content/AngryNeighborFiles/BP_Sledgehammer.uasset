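; Sledgehammer item that smashes brick obstacles and breaks window glass.
; Left click while held plays the swing animation and a timeline before the hit; VR use hits immediately.
; The hit plays a sound and line-traces, destroying bricks or breaking AN_GC bricks through server events, while windows break via a direct call.
; Successful hits report the use type to the tutorial and GameJolt components.
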(event `Crush (Server)`
  (params (Brick :type "/Game/Objects/BP_Objects/BP_Brick Object Reference"))
  (`self.Set Flat Mode` Brick "NewEnumerator0")
  (`/Game/Objects/Tutorial/TutorialComponent.Check Use Type` (`self.TutorialComponent`) "NewEnumerator6")
  (`/Game/Objects/GameJolt/GameJoltComponent.Check Use Type` (`self.GameJoltComponent`) "NewEnumerator6")
  (`/Game/Objects/BP_Objects/BP_Brick.Destroy` Brick))

(event `self.On VR Use`
  (`parent.On VR Use`)
  (bind _actor (`self.Line Trace` 300.0 "NewEnumerator1" :!label _label))
  (`GameplayStatics.PlaySound2D` "/Game/AngryNeighborFiles/Audio/damage_hammer.damage_hammer" 1.0 1.0 0.0 null null)
  (bind _asbp_brick (cast `/Game/Objects/BP_Objects/BP_Brick` _actor)
    (:`then`
      (`self.Crush (Server)` _asbp_brick)
      (`/Game/Objects/Tutorial/TutorialComponent.Check Use Type` (`self.TutorialComponent`) "NewEnumerator6" :!label _label_2)
      (`/Game/Objects/GameJolt/GameJoltComponent.Check Use Type` (`self.GameJoltComponent`) "NewEnumerator6"))
    (:`CastFailed`
      (bind _asbp_window_1 (cast `/Game/Objects/BP_Objects/BP_Window1` _actor)
        (:`then`
          (`/Game/Objects/BP_Objects/BP_Window1.Broke Glass` _asbp_window_1)
          (goto _label_2))
        (:`CastFailed`
          (bind _asbp_an_gc_bricks (cast `/Game/AngryNeighborFiles/BP_AN_GC_Bricks` _actor))
          (`self.AN Crush (Server)` _asbp_an_gc_bricks))))))

(event `self.ReceiveBeginPlay`
  (`parent.ReceiveBeginPlay`))

(event `self.On Press LMB`
  (bind _player (`/Game/Function/BP_MacroLibrary.Find Player`)
    (:`Is Valid`
      (bind _item (`/Game/Player/BP_Player.Get Item` _player))
      (if (== _item self)
        (`/Engine/EditorBlueprintResources/StandardMacros.DoOnce` false :!label _label_3
          (:`Completed`
            (`SkeletalMeshComponent.PlayAnimation` (`self.SkeletalMesh`) "/Game/AngryNeighborFiles/Animations/nailpuller_hit.nailpuller_hit" false)
            (`|ExecutionSequence`
              (:`then_0`
                (goto _label_3 :!via `Reset`))
              (:`then_1`
                (`Timeline|Шкала времени` :!via `PlayFromStart`
                  (:`Finished`
                    (goto _label)))))))))))

(event `AN Crush (Server)`
  (params (Bricks :type "/Game/AngryNeighborFiles/BP_AN_GC_Bricks Object Reference"))
  (`/Game/Objects/Tutorial/TutorialComponent.Check Use Type` (`self.TutorialComponent`) "NewEnumerator6")
  (`/Game/Objects/GameJolt/GameJoltComponent.Check Use Type` (`self.GameJoltComponent`) "NewEnumerator6")
  (`/Game/AngryNeighborFiles/BP_AN_GC_Bricks.Break` Bricks))

(fn `UserConstructionScript`
  (`parent.UserConstructionScript`))
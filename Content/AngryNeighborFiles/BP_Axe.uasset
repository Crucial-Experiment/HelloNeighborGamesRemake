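; BP_Axe is a usable held item that breaks or releases objects in the world.
; A left click while held plays a swing animation and AxeAnim timeline, then runs a short line trace with a hit sound; VR use traces immediately.
; Casts on the hit actor unlock big door blocks, break window glass, drop pictures into physics or break cameras.
; Door and window hits also notify the tutorial and GameJolt components.
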(event `self.On VR Use`
  (`parent.On VR Use`)
  (bind _actor (`self.Line Trace` 150.0 "NewEnumerator1" :!label _label))
  (`GameplayStatics.PlaySound2D` "/Game/AngryNeighborFiles/Audio/damage_axe.damage_axe" 1.0 1.0 0.0 null null)
  (bind _asbp_door_block_big (cast `/Game/AngryNeighborFiles/BP_Door_Block_Big` _actor)
    (:`then`
      (if (not (`/Game/Objects/Structurs/BP_Object.CanPickUp` _asbp_door_block_big))
        (`/Engine/EditorBlueprintResources/StandardMacros.DoOnce` false :!label _label_2
          (:`Completed`
            (`self.Unlock (Server)` _asbp_door_block_big)
            (`/Game/Objects/Tutorial/TutorialComponent.Check Use Type` (`self.TutorialComponent`) "NewEnumerator6" :!label _label_3)
            (`/Game/Objects/GameJolt/GameJoltComponent.Check Use Type` (`self.GameJoltComponent`) "NewEnumerator6")
            (goto _label_2 :!via `Reset`)))))
    (:`CastFailed`
      (bind _asbp_window_1 (cast `/Game/Objects/BP_Objects/BP_Window1` _actor)
        (:`then`
          (`/Game/Objects/BP_Objects/BP_Window1.Broke Glass` _asbp_window_1)
          (goto _label_3))
        (:`CastFailed`
          (bind _asbp_an_picture (cast `/Game/AngryNeighborFiles/BP_AN_Picture` _actor)
            (:`then`
              (`PrimitiveComponent.SetSimulatePhysics` (`/Game/AngryNeighborFiles/BP_AN_Picture.Picture` _asbp_an_picture) true))
            (:`CastFailed`
              (bind _asbp_camera (cast `/Game/Objects/BP_Objects/BP_Camera` _actor))
              (`/Game/Objects/BP_Objects/BP_Camera.Camera Broke` _asbp_camera))))))))

(event `self.On Press LMB`
  (`parent.On Press LMB`)
  (bind _player (`/Game/Function/BP_MacroLibrary.Find Player`)
    (:`Is Valid`
      (bind _item (`/Game/Player/BP_Player.Get Item` _player))
      (if (== _item self)
        (`SkeletalMeshComponent.PlayAnimation` (`self.SkeletalMesh`) "/Game/AngryNeighborFiles/Animations/nailpuller_hit.nailpuller_hit" false)
        (`Timeline|Axe Anim` :!via `PlayFromStart`
          (:`Finished`
            (goto _label)))))))

(fn `UserConstructionScript`
  (`parent.UserConstructionScript`))
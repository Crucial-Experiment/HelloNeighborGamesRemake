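; Interactive fridge for the Angry Neighbor game whose Door2 swings open and closed when interacted with.
; Interact extends the parent's logic, then plays or reverses a timeline that lerps the door's rotation, flipping Door2State when it finishes.
; Each use reports an open or close use type to the tutorial and GameJolt components.
; The open sound plays immediately, while the close sound follows a short delay.
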(event `/Game/Function/BP_Interface.Interact`
  (params (Component :type "PrimitiveComponent Object Reference") (Location :type "Vector Structure"))
  (bind _tutorialcomponent (`self.TutorialComponent`))
  (bind _gamejoltcomponent (`self.GameJoltComponent`))
  (`parent.Interact` Component Location)
  (if (== Component (`self.Door 2`))
    (switch `/Game/Objects/Enum/RotateStateEnum` (`self.Door 2 State`)
      (:`NewEnumerator0`
        (`/Game/Objects/Tutorial/TutorialComponent.Check Use Type` _tutorialcomponent "NewEnumerator2")
        (`/Game/Objects/GameJolt/GameJoltComponent.Check Use Type` _gamejoltcomponent "NewEnumerator2")
        (`|ExecutionSequence`
          (:`then_0`
            (bind (_direction _driver) (`Timeline|Шкала времени_0` :!via `Reverse` :!label _label)
              (:`Update`
                (`SceneComponent.K2_SetRelativeRotation` (`self.Door 2`) (`KismetMathLibrary.RLerp` (struct) (struct :`Yaw` -100.0) _driver) false false))
              (:`Finished`
                (switch `/Game/Objects/Enum/RotateStateEnum` (`self.Door 2 State`)
                  (:`NewEnumerator0`
                    (set `self.Door 2 State` "NewEnumerator1"))
                  (:`NewEnumerator1`
                    (set `self.Door 2 State` "NewEnumerator0"))))))
          (:`then_1`
            (`KismetSystemLibrary.Delay` 0.2)
            (`AudioComponent.Play` (`self.Door Close`) 0.0))))
      (:`NewEnumerator1`
        (`/Game/Objects/Tutorial/TutorialComponent.Check Use Type` _tutorialcomponent "NewEnumerator1")
        (`/Game/Objects/GameJolt/GameJoltComponent.Check Use Type` _gamejoltcomponent "NewEnumerator1")
        (`|ExecutionSequence`
          (:`then_0`
            (goto _label))
          (:`then_1`
            (`AudioComponent.Play` (`self.Door Open`) 0.0)))))))

(fn `UserConstructionScript`
  (`parent.UserConstructionScript`))
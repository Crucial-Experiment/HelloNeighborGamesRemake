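; Crowbar item for Angry Neighbor that pries door blocks loose and breaks windows.
; A left click while the player holds it plays the hit animation, then a timeline delays the strike; VR use strikes immediately.
; The strike runs a short line trace with a hit sound, calling UnlockServer on door blocks not yet pickable or BrokeGlass on windows.
; Either result reports the use type to the tutorial and GameJolt components.
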(event `self.On VR Use`
  (`parent.On VR Use`)
  (bind _actor (`self.Line Trace` 150.0 "NewEnumerator1" :!label _label))
  (`GameplayStatics.PlaySound2D` "/Game/AngryNeighborFiles/Audio/damage_hammer.damage_hammer" 1.0 1.0 0.0 null null)
  (bind _asbp_door_block_anim (cast `/Game/Objects/BP_Objects/BP_Door_Block_Anim` _actor)
    (:`then`
      (if (not (`/Game/Objects/Structurs/BP_Object.CanPickUp` _asbp_door_block_anim))
        (`/Engine/EditorBlueprintResources/StandardMacros.DoOnce` false :!label _label_2
          (:`Completed`
            (`self.Unlock (Server)` _asbp_door_block_anim)
            (`/Game/Objects/Tutorial/TutorialComponent.Check Use Type` (`self.TutorialComponent`) "NewEnumerator6" :!label _label_3)
            (`/Game/Objects/GameJolt/GameJoltComponent.Check Use Type` (`self.GameJoltComponent`) "NewEnumerator6")
            (goto _label_2 :!via `Reset`)))))
    (:`CastFailed`
      (bind _asbp_window_1 (cast `/Game/Objects/BP_Objects/BP_Window1` _actor))
      (`/Game/Objects/BP_Objects/BP_Window1.Broke Glass` _asbp_window_1)
      (goto _label_3))))

(event `self.On Press LMB`
  (bind _player (`/Game/Function/BP_MacroLibrary.Find Player`)
    (:`Is Valid`
      (bind _item (`/Game/Player/BP_Player.Get Item` _player))
      (if (== _item self)
        (`/Engine/EditorBlueprintResources/StandardMacros.DoOnce` false :!label _label_4
          (:`Completed`
            (`SkeletalMeshComponent.PlayAnimation` (`self.SkeletalMesh`) "/Game/AngryNeighborFiles/Animations/nailpuller_hit.nailpuller_hit" false)
            (`|ExecutionSequence`
              (:`then_0`
                (goto _label_4 :!via `Reset`))
              (:`then_1`
                (`Timeline|Шкала времени_0` :!via `PlayFromStart`
                  (:`Finished`
                    (goto _label)))))))))))

(fn `UserConstructionScript`
  (`parent.UserConstructionScript`))
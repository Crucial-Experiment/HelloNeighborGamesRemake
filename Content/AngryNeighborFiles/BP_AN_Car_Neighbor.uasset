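; Neighbor's car actor with two doors that open and close through an Interact event on the hit component.
; Each door has its own state and timeline, which plays or reverses to lerp the door's yaw in mirrored directions and flips the state on finish.
; Each use reports its type to the tutorial and GameJolt components and plays a door sound, slightly delayed when closing.
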(event `/Game/Function/BP_Interface.Interact`
  (params (Component :type "PrimitiveComponent Object Reference") (Location :type "Vector Structure"))
  (bind _tutorialcomponent (`self.TutorialComponent`))
  (bind _gamejoltcomponent (`self.GameJoltComponent`))
  (bind _gamejoltcomponent_2 (`self.GameJoltComponent`))
  (bind _tutorialcomponent_2 (`self.TutorialComponent`))
  (`|ExecutionSequence`
    (:`then_0`
      (if (== Component (`self.Door`))
        (switch `/Game/Objects/Enum/RotateStateEnum` (`self.Door State`)
          (:`NewEnumerator0`
            (`/Game/Objects/Tutorial/TutorialComponent.Check Use Type` _tutorialcomponent_2 "NewEnumerator2")
            (`/Game/Objects/GameJolt/GameJoltComponent.Check Use Type` _gamejoltcomponent_2 "NewEnumerator2")
            (`|ExecutionSequence`
              (:`then_0`
                (bind (_direction _driver) (`Timeline|Door Rotation` :!via `Reverse` :!label _label)
                  (:`Update`
                    (`SceneComponent.K2_SetRelativeRotation` (`self.Door`) (`KismetMathLibrary.RLerp` (struct) (struct :`Yaw` 150.0) _driver) false false))
                  (:`Finished`
                    (switch `/Game/Objects/Enum/RotateStateEnum` (`self.Door State`)
                      (:`NewEnumerator0`
                        (set `self.Door State` "NewEnumerator1"))
                      (:`NewEnumerator1`
                        (set `self.Door State` "NewEnumerator0"))))))
              (:`then_1`
                (`KismetSystemLibrary.Delay` 0.3)
                (`AudioComponent.Play` (`self.Door Close`) 0.0))))
          (:`NewEnumerator1`
            (`/Game/Objects/Tutorial/TutorialComponent.Check Use Type` _tutorialcomponent_2 "NewEnumerator1")
            (`/Game/Objects/GameJolt/GameJoltComponent.Check Use Type` _gamejoltcomponent_2 "NewEnumerator1")
            (`|ExecutionSequence`
              (:`then_0`
                (goto _label))
              (:`then_1`
                (`AudioComponent.Play` (`self.Door Open`) 0.0)))))))
    (:`then_1`
      (if (== Component (`self.Door 2`))
        (switch `/Game/Objects/Enum/RotateStateEnum` (`self.Door 2 State`)
          (:`NewEnumerator0`
            (`/Game/Objects/Tutorial/TutorialComponent.Check Use Type` _tutorialcomponent "NewEnumerator2")
            (`/Game/Objects/GameJolt/GameJoltComponent.Check Use Type` _gamejoltcomponent "NewEnumerator2")
            (`|ExecutionSequence`
              (:`then_0`
                (bind (_direction_2 _driver_2) (`Timeline|Шкала времени` :!via `Reverse` :!label _label_2)
                  (:`Update`
                    (`SceneComponent.K2_SetRelativeRotation` (`self.Door 2`) (`KismetMathLibrary.RLerp` (struct) (struct :`Yaw` -150.0) _driver_2) false false))
                  (:`Finished`
                    (switch `/Game/Objects/Enum/RotateStateEnum` (`self.Door 2 State`)
                      (:`NewEnumerator0`
                        (set `self.Door 2 State` "NewEnumerator1"))
                      (:`NewEnumerator1`
                        (set `self.Door 2 State` "NewEnumerator0"))))))
              (:`then_1`
                (`KismetSystemLibrary.Delay` 0.3)
                (`AudioComponent.Play` (`self.Door Close`) 0.0))))
          (:`NewEnumerator1`
            (`/Game/Objects/Tutorial/TutorialComponent.Check Use Type` _tutorialcomponent "NewEnumerator1")
            (`/Game/Objects/GameJolt/GameJoltComponent.Check Use Type` _gamejoltcomponent "NewEnumerator1")
            (`|ExecutionSequence`
              (:`then_0`
                (goto _label_2))
              (:`then_1`
                (`AudioComponent.Play` (`self.Door Open`) 0.0)))))))))

(fn `UserConstructionScript`)
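; BP_Cube_Place is a puzzle socket that unlocks when a matching color cube or a red cube enters its Box.
; Color cubes must match ColorCubeType, while red cubes unlock it unconditionally.
; Unlock calls the parent logic, snaps the cube to Place, disables its pickup and turns on the green material and light.
; The construction script shows red if the Rotate reference is valid, otherwise green.
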(event `self.Unlock`
  (`parent.Unlock`)
  (`self.Set Flat Mode` "NewEnumerator1")
  (set `self.CanPickUp` false)
  (`self.K2_AttachToComponent` (`self.Other Actor`) (`self.Place`) "None" "SnapToTarget" "SnapToTarget" "SnapToTarget" true)
  (`PrimitiveComponent.SetMaterial` (`self.CubePlace`) 0 "/Game/AngryNeighborFiles/Materials/electro_button_green_mat.electro_button_green_mat")
  (`SceneComponent.SetVisibility` (`self.GreenLight`) true false))

(event `self.Box.OnComponentBeginOverlap`
  (params (OverlappedComponent :type "PrimitiveComponent Object Reference") (OtherActor :type "Actor Object Reference") (OtherComp :type "PrimitiveComponent Object Reference") (OtherBodyIndex :type Integer) (bFromSweep :type Boolean) (SweepResult :type "HitResult Structure (by ref)"))
  (bind _returnvalue (`GameplayStatics.GetObjectClass` OtherActor))
  (if (or (== _returnvalue (`self.Color Cubes`)) (== _returnvalue (`self.Red Cube`)))
    (set `self.Other Actor` OtherActor)
    (`|ExecutionSequence`
      (:`then_0`
        (bind _asbp_color_cubes (cast `/Game/AngryNeighborFiles/BP_Color_Cubes` OtherActor))
        (if (== (`/Game/AngryNeighborFiles/BP_Color_Cubes.State` _asbp_color_cubes) (`self.Color Cube Type`))
          (`self.Unlock`)
          (set `/Game/Objects/Structurs/BP_Object.CanPickUp` false _asbp_color_cubes)
          (`self.Set Flat Mode` _asbp_color_cubes "NewEnumerator1")))
      (:`then_1`
        (bind _asbp_red_cube (cast `/Game/DevGAMMFiles/BP_RedCube` OtherActor))
        (`self.Unlock`)
        (set `/Game/Objects/Structurs/BP_Object.CanPickUp` false _asbp_red_cube)
        (`self.Set Flat Mode` _asbp_red_cube "NewEnumerator1")))))

(fn `UserConstructionScript`
  (bind _redlight (`self.RedLight`))
  (bind _cubeplace (`self.CubePlace`))
  (`parent.UserConstructionScript`)
  (`self.Rotate`
    (:`then`
      (`PrimitiveComponent.SetMaterial` _cubeplace 0 "/Game/AngryNeighborFiles/Materials/electro_button_red_mat.electro_button_red_mat")
      (`SceneComponent.SetVisibility` (`self.GreenLight`) false false)
      (`SceneComponent.SetVisibility` _redlight true false))
    (:`else`
      (`PrimitiveComponent.SetMaterial` _cubeplace 0 "/Game/AngryNeighborFiles/Materials/electro_button_green_mat.electro_button_green_mat")
      (`SceneComponent.SetVisibility` (`self.GreenLight`) true false)
      (`SceneComponent.SetVisibility` _redlight false false))))
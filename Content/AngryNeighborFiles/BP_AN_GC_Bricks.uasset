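; BP_AN_GC_Bricks is a breakable brick actor that shatters when its Break event is called.
; Break destroys the Box component, spawns an FS_MasterField field actor at the actor's transform and plays a breaking sound at its location.
; The actor destroys itself after a short delay, and its construction script only calls the parent's.
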(event `Break`
  (`ActorComponent.K2_DestroyComponent` (`self.Box`))
  (`|SpawnActorFromClass` "/Engine/EditorResources/FieldNodes/FS_MasterField.FS_MasterField_C" (`self.GetTransform`) "Undefined" "MultiplyWithRoot" null null)
  (`GameplayStatics.PlaySoundAtLocation` (`self.Bricks Breake`) (`self.K2_GetActorLocation`) (struct) 1.0 1.0 0.0 null null null null)
  (`KismetSystemLibrary.Delay` 3.5)
  (`self.K2_DestroyActor`))

(fn `UserConstructionScript`
  (`parent.UserConstructionScript`))
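; BP_Kitchen_Set is a kitchen set prop with a door that opens and closes when interacted with.
; The Interact event checks for the Door1 component, then a FlipFlop alternates between opening and closing.
; The DoorOpen timeline plays or reverses to lerp the door's relative yaw through 90 degrees, while Door1Open or Door1Close plays alongside each swing.
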(event `/Game/Function/BP_Interface.Interact`
  (params (Component :type "PrimitiveComponent Object Reference") (Location :type "Vector Structure"))
  (if (== (`self.Door1`) Component)
    (`/Engine/EditorBlueprintResources/StandardMacros.FlipFlop`
      (:`A`
        (`|ExecutionSequence`
          (:`then_0`
            (bind (_direction _alpha) (`Timeline|Door Open` :!label _label)
              (:`Update`
                (`SceneComponent.K2_SetRelativeRotation` (`self.Door1`) (`KismetMathLibrary.RLerp` (struct) (struct :`Pitch` -90.0) _alpha) false false))))
          (:`then_1`
            (`AudioComponent.Play` (`self.Door1_Open`) 0.0))))
      (:`B`
        (`|ExecutionSequence`
          (:`then_0`
            (goto _label :!via `Reverse`))
          (:`then_1`
            (`AudioComponent.Play` (`self.Door1_Close`) 0.0)))))))

(fn `UserConstructionScript`)
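; Floor indicator display for a lift, with a rotating arrow and up to five level markers.
; On BeginPlay it unhides one marker for each valid floor in the linked Lift.
; FloorChanged lerps the arrow to the current floor's preset rotation using a fixed-step Delay loop instead of Tick or a Timeline.
; When the arrow arrives, the current floor's marker gets the bulb material and the others get the button material.
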(event `self.ReceiveBeginPlay`
  (bind _lift (`self.Lift`))
  (`/Engine/EditorBlueprintResources/StandardMacros.IsValid` _lift
    (:`Is Valid`
      (for (_array_element _array_index) (`/Game/Objects/BP_Objects/BP_Lift.Floors` _lift)
        (`/Engine/EditorBlueprintResources/StandardMacros.IsValid` _array_element
          (:`Is Valid`
            (`SceneComponent.SetHiddenInGame` (`|GetArrayItem` (`|MakeArray` (`self.Level 1`) (`self.Level 2`) (`self.Level 3`) (`self.Level 4`) (`self.Level 5`)) _array_index) false false)))))))

(event `self.Floor Changed`
  (set `self.Prev Rotation` (`SceneComponent.K2_GetComponentRotation` (`self.Arrow`)))
  (set `self.Alpha` 0.0)
  (`SceneComponent.K2_SetRelativeRotation` (`self.Arrow`) (`KismetMathLibrary.RLerp` (`self.Prev Rotation`) (`|GetArrayItem` (`self.Arrow Rotations`) (`self.Current Floar`)) (`self.Alpha`)) false false :!label _label)
  (set `self.Alpha` (+ (`self.Alpha`) (* (`self.Speed`) 0.0166)))
  (`KismetSystemLibrary.Delay` 0.0166)
  (if (>= (`self.Alpha`) 1.0)
    (for (_array_element _array_index) (`|MakeArray` (`self.Level 1`) (`self.Level 2`) (`self.Level 3`) (`self.Level 4`) (`self.Level 5`))
      (if (== _array_index (`self.Current Floar`))
        (`PrimitiveComponent.SetMaterial` _array_element 0 "/Game/Objects/Materials/dl_bulb_m.dl_bulb_m")
        (else
          (`PrimitiveComponent.SetMaterial` _array_element 0 "/Game/AngryNeighborFiles/Materials/Lift_Buttons_mat.Lift_Buttons_mat"))))
    (else
      (goto _label))))

(fn `UserConstructionScript`
  (`parent.UserConstructionScript`))
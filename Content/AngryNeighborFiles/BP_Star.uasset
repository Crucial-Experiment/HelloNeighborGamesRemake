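; BP_Star is a carryable puzzle item that players place into one of five slots on a BP_Star_Place.
; On a left click while it is held, a short line trace identifies the targeted slot box, then the star is released and placed through a server-to-all event pair.
; Placement snaps it to the slot, disables that box's collision, locks pickup, registers the star with the holder and triggers its star check.
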(event `self.ReceiveBeginPlay`
  (`parent.ReceiveBeginPlay`))

(event `self.On Press LMB`
  (bind _player (`/Game/Function/BP_MacroLibrary.Find Player`)
    (:`Is Valid`
      (bind _item (`/Game/Player/BP_Player.Get Item` _player))
      (if (== _item self)
        (bind (_actor _component) (`self.Line Trace` 150.0))
        (bind _asbp_star_place (cast `/Game/AngryNeighborFiles/BP_Star_Place` _actor))
        (`|ExecutionSequence`
          (:`then_0`
            (bind _box1 (`/Game/AngryNeighborFiles/BP_Star_Place.Box1` _asbp_star_place))
            (if (== _component _box1)
              (`self.Try Release`)
              (`self.Place (Server)` _box1 _asbp_star_place)))
          (:`then_1`
            (bind _box2 (`/Game/AngryNeighborFiles/BP_Star_Place.Box2` _asbp_star_place))
            (if (== _component _box2)
              (`self.Try Release`)
              (`self.Place (Server)` _box2 _asbp_star_place)))
          (:`then_2`
            (bind _box3 (`/Game/AngryNeighborFiles/BP_Star_Place.Box3` _asbp_star_place))
            (if (== _component _box3)
              (`self.Try Release`)
              (`self.Place (Server)` _box3 _asbp_star_place)))
          (:`then_3`
            (bind _box4 (`/Game/AngryNeighborFiles/BP_Star_Place.Box4` _asbp_star_place))
            (if (== _component _box4)
              (`self.Try Release`)
              (`self.Place (Server)` _box4 _asbp_star_place)))
          (:`then_4`
            (bind _box5 (`/Game/AngryNeighborFiles/BP_Star_Place.Box5` _asbp_star_place))
            (if (== _component _box5)
              (`self.Try Release`)
              (`self.Place (Server)` _box5 _asbp_star_place))))))))

(event `Place (All)`
  (params (Component :type "PrimitiveComponent Object Reference") (`Star Place` :type "/Game/AngryNeighborFiles/BP_Star_Place Object Reference"))
  (`self.K2_SetActorLocationAndRotation` (`SceneComponent.K2_GetComponentLocation` Component) (`SceneComponent.K2_GetComponentRotation` Component))
  (`PrimitiveComponent.SetCollisionEnabled` Component "NoCollision")
  (`self.Set Flat Mode` "NewEnumerator1")
  (`KismetArrayLibrary.Array_Add` (`/Game/AngryNeighborFiles/BP_Star_Place.Star Count` `Star Place`) self)
  (set `self.CanPickUp` false)
  (`/Game/AngryNeighborFiles/BP_Star_Place.Check Stars` `Star Place`))

(event `Place (Server)`
  (params (Component :type "PrimitiveComponent Object Reference") (`Star Place` :type "/Game/AngryNeighborFiles/BP_Star_Place Object Reference"))
  (`self.Place (All)` Component `Star Place`))

(fn `UserConstructionScript`
  (`parent.UserConstructionScript`))
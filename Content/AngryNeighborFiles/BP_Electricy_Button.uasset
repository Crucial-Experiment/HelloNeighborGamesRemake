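; A wall button blueprint that switches on a linked set of Electricity actors when used, by interaction or VR hand overlap.
; Interaction routes through a server event to a multicast that, if it has electricity or is a generator, calls the parent Enable and each valid Electricity entry's Enable.
; The multicast always recolors the button material and point light blue, while hand overlap runs the same logic locally.
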(event `self.Interact`
  (params (Component :type "PrimitiveComponent Object Reference") (Location :type "Vector Structure"))
  (`self.Interact (Server)`))

(event `self.Enable`
  (`parent.Enable`)
  (for _array_element (`self.Electricity`) :!label _label
    (`/Engine/EditorBlueprintResources/StandardMacros.IsValid` _array_element
      (:`Is Valid`
        (`self.Enable` _array_element)))))

(event `Interact (Server)`
  (`self.Interact (All)`))

(event `Interact (All)`
  (`|ExecutionSequence` :!label _label_2
    (:`then_0`
      (if (or (`self.Has Electricity`) (`self.Generator`))
        (goto _label)))
    (:`then_1`
      (`PrimitiveComponent.SetMaterial` (`self.Button`) 0 "/Game/Objects/Materials/plastic_blue_Inst.plastic_blue_Inst")
      (`LightComponent.SetLightColor` (`self.PointLight`) (struct :`G` 0.08411 :`B` 1.0 :`A` 1.0) true))))

(event `self.Button.OnComponentBeginOverlap`
  (params (OverlappedComponent :type "PrimitiveComponent Object Reference") (OtherActor :type "Actor Object Reference") (OtherComp :type "PrimitiveComponent Object Reference") (OtherBodyIndex :type Integer) (bFromSweep :type Boolean) (SweepResult :type "HitResult Structure (by ref)"))
  (if (`self.Overlap VR Hands` OtherActor OtherComp)
    (goto _label_2)))

(fn `UserConstructionScript`)
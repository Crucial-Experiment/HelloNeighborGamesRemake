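; Secret wall that slides to an end position when enabled through its parent class's Enable event.
; BeginPlay sets that end position to a hardcoded world location unless Custom is set.
; The DoorMove timeline lerps Root from the actor's current location, re-read each update, toward the end position.
; Disable reverses the timeline, but no start position is stored for the wall to return to.
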(event `self.ReceiveBeginPlay`
  (`parent.ReceiveBeginPlay`)
  (if (not (`self.Custom`))
    (set `self.Pos End` (370.5 -3250.0 143.0))))

(event `self.Enable`
  (`parent.Enable`)
  (bind (_direction _lerp) (`Timeline|Door Move` :!label _label)
    (:`Update`
      (`SceneComponent.K2_SetWorldLocation` (`self.Root`) (`KismetMathLibrary.VLerp` (`self.K2_GetActorLocation`) (`self.Pos End`) _lerp) false false))))

(event `self.Disable`
  (`parent.Disable`)
  (goto _label :!via `Reverse`))

(fn `UserConstructionScript`
  (`parent.UserConstructionScript`))
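; Lift actor for the Angry Neighbor content that opens and closes its cabin doors to suit the current floor.
; OpenDoor and CloseDoor look up the current BP_AN_LiftFloor in the Floors array through the Flour index and read its LiftDoorDirection.
; That direction picks one of two BP_LiftDoor child actors, Door2 for Left or Door for Right, to open or close.
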(event `self.Open Door`
  (bind _asbp_an_lift_floor (cast `/Game/AngryNeighborFiles/BP_AN_LiftFloor` (`|GetArrayItem` (`self.Floors`) (`self.Flour`))))
  (switch `ETouchSwipeDirection` (`/Game/AngryNeighborFiles/BP_AN_LiftFloor.Lift Door Direction` _asbp_an_lift_floor)
    (:`Left`
      (bind _asbp_lift_door (cast `/Game/Objects/BP_Objects/BP_LiftDoor` (`ChildActorComponent.ChildActor` (`self.Door 2`))))
      (`/Game/Objects/BP_Objects/BP_LiftDoor.Open` _asbp_lift_door))
    (:`Right`
      (bind _asbp_lift_door_2 (cast `/Game/Objects/BP_Objects/BP_LiftDoor` (`ChildActorComponent.ChildActor` (`self.Door`))))
      (`/Game/Objects/BP_Objects/BP_LiftDoor.Open` _asbp_lift_door_2))))

(event `self.Close Door`
  (bind _asbp_an_lift_floor (cast `/Game/AngryNeighborFiles/BP_AN_LiftFloor` (`|GetArrayItem` (`self.Floors`) (`self.Flour`))))
  (switch `ETouchSwipeDirection` (`/Game/AngryNeighborFiles/BP_AN_LiftFloor.Lift Door Direction` _asbp_an_lift_floor)
    (:`Left`
      (bind _asbp_lift_door (cast `/Game/Objects/BP_Objects/BP_LiftDoor` (`ChildActorComponent.ChildActor` (`self.Door 2`))))
      (`/Game/Objects/BP_Objects/BP_LiftDoor.Close` _asbp_lift_door))
    (:`Right`
      (bind _asbp_lift_door_2 (cast `/Game/Objects/BP_Objects/BP_LiftDoor` (`ChildActorComponent.ChildActor` (`self.Door`))))
      (`/Game/Objects/BP_Objects/BP_LiftDoor.Close` _asbp_lift_door_2))))

(fn `UserConstructionScript`
  (`parent.UserConstructionScript`))
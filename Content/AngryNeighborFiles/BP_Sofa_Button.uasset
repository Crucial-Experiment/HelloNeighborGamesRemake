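; BP_Sofa_Button is an interactable button that toggles a stack of BP_AN_Blocker actors in the level.
; Interact routes through a server RPC to a multicast, which plays the Activate sound or animation and runs a FlipFlop.
; The FlipFlop alternates between destroying all blockers with blue material and spawning three at hardcoded locations with red material.
; VR hand overlap jumps straight into that logic, bypassing the RPCs.
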(event `/Game/Function/BP_Interface.Interact`
  (params (Component :type "PrimitiveComponent Object Reference") (Location :type "Vector Structure"))
  (`self.Interact (Server)`))

(event `Interact (Server)`
  (`self.Interact (All)`))

(event `Interact (All)`
  (`AudioComponent.Play` (`self.Activate`) 0.0 :!label _label)
  (`/Engine/EditorBlueprintResources/StandardMacros.FlipFlop`
    (:`A`
      (`|ExecutionSequence`
        (:`then_0`
          (bind _outactors (`GameplayStatics.GetAllActorsOfClass` "/Game/AngryNeighborFiles/BP_AN_Blocker.BP_AN_Blocker_C"))
          (for _array_element _outactors
            (`self.K2_DestroyActor` _array_element)))
        (:`then_1`
          (`PrimitiveComponent.SetMaterial` (`self.Button`) 0 "/Game/Objects/Materials/plastic_blue_Inst.plastic_blue_Inst"))))
    (:`B`
      (`|ExecutionSequence`
        (:`then_0`
          (`|SpawnActorFromClass` "/Game/AngryNeighborFiles/BP_AN_Blocker.BP_AN_Blocker_C" (`KismetMathLibrary.MakeTransform` (333.0 -3248.0 -62.0)) "Undefined" "MultiplyWithRoot" null null))
        (:`then_1`
          (`|SpawnActorFromClass` "/Game/AngryNeighborFiles/BP_AN_Blocker.BP_AN_Blocker_C" (`KismetMathLibrary.MakeTransform` (333.0 -3248.0 -124.0)) "Undefined" "MultiplyWithRoot" null null))
        (:`then_2`
          (`|SpawnActorFromClass` "/Game/AngryNeighborFiles/BP_AN_Blocker.BP_AN_Blocker_C" (`KismetMathLibrary.MakeTransform` (333.0 -3248.0 -192.0)) "Undefined" "MultiplyWithRoot" null null))
        (:`then_3`
          (`PrimitiveComponent.SetMaterial` (`self.Button`) 0 "/Game/Objects/Materials/plastic_red_Inst.plastic_red_Inst"))))))

(event `self.Button.OnComponentBeginOverlap`
  (params (OverlappedComponent :type "PrimitiveComponent Object Reference") (OtherActor :type "Actor Object Reference") (OtherComp :type "PrimitiveComponent Object Reference") (OtherBodyIndex :type Integer) (bFromSweep :type Boolean) (SweepResult :type "HitResult Structure (by ref)"))
  (if (`self.Overlap VR Hands` OtherActor OtherComp)
    (goto _label)))

(fn `UserConstructionScript`)
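; Interactable wall picture actor for the Angry Neighbor game that moves to an end pose when used.
; Interact plays the PictureMove timeline, which lerps the Picture component's world location and rotation from the actor's transform to PosEnd and RotateEnd.
; When NonInteractable is set, BeginPlay sets both end values to the actor's current transform, so the lerp leaves the picture at that pose.
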(event `self.ReceiveBeginPlay`
  (if (`self.Non Interactable`)
    (set `self.Rotate End` (`self.K2_GetActorRotation`))
    (set `self.Pos End` (`self.K2_GetActorLocation`))))

(event `/Game/Function/BP_Interface.Interact`
  (params (Component :type "PrimitiveComponent Object Reference") (Location :type "Vector Structure"))
  (bind (_direction _lerp) (`Timeline|Picture Move`)
    (:`Update`
      (`SceneComponent.K2_SetWorldLocationAndRotation` (`self.Picture`) (`KismetMathLibrary.VLerp` (`self.K2_GetActorLocation`) (`self.Pos End`) _lerp) (`KismetMathLibrary.RLerp` (`self.K2_GetActorRotation`) (`self.Rotate End`) _lerp) false false))))

(fn `UserConstructionScript`)
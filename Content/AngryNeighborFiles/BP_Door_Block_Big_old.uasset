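; Big door block actor, marked old by its name, that breaks into two separate pieces when unlocked.
; Unlock runs the parent logic, then spawns the Part1 and Part2 block actors at the world transforms of two Scene components that serve as placement markers.
; The original actor destroys itself after a very short delay, leaving the spawned parts in its place.
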(event `self.Unlock`
  (`parent.Unlock`)
  (`|ExecutionSequence`
    (:`then_1`
      (`|ExecutionSequence`
        (:`then_0`
          (`KismetSystemLibrary.Delay` 0.01)
          (`self.K2_DestroyActor`))
        (:`then_1`
          (`|SpawnActorFromClass` "/Game/Objects/BP_Objects/BP_Door_Block_Part1.BP_Door_Block_Part1_C" (`KismetMathLibrary.MakeTransform` (`SceneComponent.K2_GetComponentLocation` (`self.Scene`)) (`SceneComponent.K2_GetComponentRotation` (`self.Scene`)) (`SceneComponent.K2_GetComponentScale` (`self.Scene`))) "Undefined" "MultiplyWithRoot" null null))
        (:`then_2`
          (`|SpawnActorFromClass` "/Game/Objects/BP_Objects/BP_Door_Block_Part2.BP_Door_Block_Part2_C" (`KismetMathLibrary.MakeTransform` (`SceneComponent.K2_GetComponentLocation` (`self.Scene1`)) (`SceneComponent.K2_GetComponentRotation` (`self.Scene1`)) (`SceneComponent.K2_GetComponentScale` (`self.Scene1`))) "Undefined" "MultiplyWithRoot" null null))))))

(fn `UserConstructionScript`
  (`parent.UserConstructionScript`))
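; Interactive bookcase with twelve individually sliding parts, likely drawers, that open and close on interaction.
; The Interact event compares the passed component against each part in turn, and each match runs its own FlipFlop to alternate open and close.
; Each part has a timeline that lerps its relative location outward along local Y or reverses it back, alongside separate open and close sounds or effects played from the start.
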(event `/Game/Function/BP_Interface.Interact`
  (params (Component :type "PrimitiveComponent Object Reference") (Location :type "Vector Structure"))
  (`|ExecutionSequence`
    (:`then_0`
      (if (== (`self.Part1`) Component)
        (`/Engine/EditorBlueprintResources/StandardMacros.FlipFlop`
          (:`A`
            (`|ExecutionSequence`
              (:`then_0`
                (bind (_direction _lerp) (`Timeline|Part 1 Loc` :!label _label)
                  (:`Update`
                    (`SceneComponent.K2_SetRelativeLocation` (`self.Part1`) (`KismetMathLibrary.VLerp` (-135.5 0.0 66.0) (-135.5 40.0 66.0) _lerp) false false))))
              (:`then_1`
                (`AudioComponent.Play` (`self.Part 1 Open`) 0.0))))
          (:`B`
            (`|ExecutionSequence`
              (:`then_0`
                (goto _label :!via `Reverse`))
              (:`then_1`
                (`AudioComponent.Play` (`self.Part 1 Close`) 0.0)))))))
    (:`then_1`
      (if (== (`self.Part2`) Component)
        (`/Engine/EditorBlueprintResources/StandardMacros.FlipFlop`
          (:`A`
            (`|ExecutionSequence`
              (:`then_0`
                (bind (_direction_2 _lerp_2) (`Timeline|Part 2 Loc` :!label _label_2)
                  (:`Update`
                    (`SceneComponent.K2_SetRelativeLocation` (`self.Part2`) (`KismetMathLibrary.VLerp` (-52.0 0.0 65.8) (-52.0 40.0 65.8) _lerp_2) false false))))
              (:`then_1`
                (`AudioComponent.Play` (`self.Part 2 Open`) 0.0))))
          (:`B`
            (`|ExecutionSequence`
              (:`then_0`
                (goto _label_2 :!via `Reverse`))
              (:`then_1`
                (`AudioComponent.Play` (`self.Part 2 Close`) 0.0)))))))
    (:`then_2`
      (if (== (`self.Part3`) Component)
        (`/Engine/EditorBlueprintResources/StandardMacros.FlipFlop`
          (:`A`
            (`|ExecutionSequence`
              (:`then_0`
                (bind (_direction_3 _lerp_3) (`Timeline|Part 3 Loc` :!label _label_3)
                  (:`Update`
                    (`SceneComponent.K2_SetRelativeLocation` (`self.Part3`) (`KismetMathLibrary.VLerp` (-52.0 0.0 43.1) (-52.0 40.0 43.1) _lerp_3) false false))))
              (:`then_1`
                (`AudioComponent.Play` (`self.Part 3 Open`) 0.0))))
          (:`B`
            (`|ExecutionSequence`
              (:`then_0`
                (goto _label_3 :!via `Reverse`))
              (:`then_1`
                (`AudioComponent.Play` (`self.Part 3 Close`) 0.0)))))))
    (:`then_3`
      (if (== (`self.Part4`) Component)
        (`/Engine/EditorBlueprintResources/StandardMacros.FlipFlop`
          (:`A`
            (`|ExecutionSequence`
              (:`then_0`
                (bind (_direction_4 _lerp_4) (`Timeline|Part 4 Loc` :!label _label_4)
                  (:`Update`
                    (`SceneComponent.K2_SetRelativeLocation` (`self.Part4`) (`KismetMathLibrary.VLerp` (-135.5 0.0 43.1) (-135.5 40.0 43.1) _lerp_4) false false))))
              (:`then_1`
                (`AudioComponent.Play` (`self.Part 4 Open`) 0.0))))
          (:`B`
            (`|ExecutionSequence`
              (:`then_0`
                (goto _label_4 :!via `Reverse`))
              (:`then_1`
                (`AudioComponent.Play` (`self.Part 4 Close`) 0.0)))))))
    (:`then_4`
      (if (== (`self.Part5`) Component)
        (`/Engine/EditorBlueprintResources/StandardMacros.FlipFlop`
          (:`A`
            (`|ExecutionSequence`
              (:`then_0`
                (bind (_direction_5 _lerp_5) (`Timeline|Part 5 Loc` :!label _label_5)
                  (:`Update`
                    (`SceneComponent.K2_SetRelativeLocation` (`self.Part5`) (`KismetMathLibrary.VLerp` (-135.5 0.0 20.5) (-135.5 40.0 20.5) _lerp_5) false false))))
              (:`then_1`
                (`AudioComponent.Play` (`self.Part 5 Open`) 0.0))))
          (:`B`
            (`|ExecutionSequence`
              (:`then_0`
                (goto _label_5 :!via `Reverse`))
              (:`then_1`
                (`AudioComponent.Play` (`self.Part 5 Close`) 0.0)))))))
    (:`then_5`
      (if (== (`self.Part6`) Component)
        (`/Engine/EditorBlueprintResources/StandardMacros.FlipFlop`
          (:`A`
            (`|ExecutionSequence`
              (:`then_0`
                (bind (_direction_6 _lerp_6) (`Timeline|Part 6 Loc` :!label _label_6)
                  (:`Update`
                    (`SceneComponent.K2_SetRelativeLocation` (`self.Part6`) (`KismetMathLibrary.VLerp` (-52.0 0.0 20.5) (-52.0 40.0 20.5) _lerp_6) false false))))
              (:`then_1`
                (`AudioComponent.Play` (`self.Part 6 Open`) 0.0))))
          (:`B`
            (`|ExecutionSequence`
              (:`then_0`
                (goto _label_6 :!via `Reverse`))
              (:`then_1`
                (`AudioComponent.Play` (`self.Part 6 Close`) 0.0)))))))
    (:`then_6`
      (if (== (`self.Part7`) Component)
        (`/Engine/EditorBlueprintResources/StandardMacros.FlipFlop`
          (:`A`
            (`|ExecutionSequence`
              (:`then_0`
                (bind (_direction_7 _lerp_7) (`Timeline|Part 7 Loc` :!label _label_7)
                  (:`Update`
                    (`SceneComponent.K2_SetRelativeLocation` (`self.Part7`) (`KismetMathLibrary.VLerp` (52.1 0.0 65.8) (52.1 40.0 65.8) _lerp_7) false false))))
              (:`then_1`
                (`AudioComponent.Play` (`self.Part 7 Open`) 0.0))))
          (:`B`
            (`|ExecutionSequence`
              (:`then_0`
                (goto _label_7 :!via `Reverse`))
              (:`then_1`
                (`AudioComponent.Play` (`self.Part 7 Close`) 0.0)))))))
    (:`then_7`
      (if (== (`self.Part8`) Component)
        (`/Engine/EditorBlueprintResources/StandardMacros.FlipFlop`
          (:`A`
            (`|ExecutionSequence`
              (:`then_0`
                (bind (_direction_8 _lerp_8) (`Timeline|Part 8 Loc` :!label _label_8)
                  (:`Update`
                    (`SceneComponent.K2_SetRelativeLocation` (`self.Part8`) (`KismetMathLibrary.VLerp` (135.8 0.0 65.8) (135.8 40.0 65.8) _lerp_8) false false))))
              (:`then_1`
                (`AudioComponent.Play` (`self.Part 8 Open`) 0.0))))
          (:`B`
            (`|ExecutionSequence`
              (:`then_0`
                (goto _label_8 :!via `Reverse`))
              (:`then_1`
                (`AudioComponent.Play` (`self.Part 8 Close`) 0.0)))))))
    (:`then_8`
      (if (== (`self.Part9`) Component)
        (`/Engine/EditorBlueprintResources/StandardMacros.FlipFlop`
          (:`A`
            (`|ExecutionSequence`
              (:`then_0`
                (bind (_direction_9 _lerp_9) (`Timeline|Part 9 Loc` :!label _label_9)
                  (:`Update`
                    (`SceneComponent.K2_SetRelativeLocation` (`self.Part9`) (`KismetMathLibrary.VLerp` (52.1 0.0 43.1) (52.1 40.0 43.1) _lerp_9) false false))))
              (:`then_1`
                (`AudioComponent.Play` (`self.Part 9 Open`) 0.0))))
          (:`B`
            (`|ExecutionSequence`
              (:`then_0`
                (goto _label_9 :!via `Reverse`))
              (:`then_1`
                (`AudioComponent.Play` (`self.Part 9 Close`) 0.0)))))))
    (:`then_9`
      (if (== (`self.Part10`) Component)
        (`/Engine/EditorBlueprintResources/StandardMacros.FlipFlop`
          (:`A`
            (`|ExecutionSequence`
              (:`then_0`
                (bind (_direction_10 _lerp_10) (`Timeline|Part 10 Loc` :!label _label_10)
                  (:`Update`
                    (`SceneComponent.K2_SetRelativeLocation` (`self.Part10`) (`KismetMathLibrary.VLerp` (135.8 0.0 43.1) (135.8 40.0 43.1) _lerp_10) false false))))
              (:`then_1`
                (`AudioComponent.Play` (`self.Part 10 Open`) 0.0))))
          (:`B`
            (`|ExecutionSequence`
              (:`then_0`
                (goto _label_10 :!via `Reverse`))
              (:`then_1`
                (`AudioComponent.Play` (`self.Part 10 Close`) 0.0)))))))
    (:`then_10`
      (if (== (`self.Part11`) Component)
        (`/Engine/EditorBlueprintResources/StandardMacros.FlipFlop`
          (:`A`
            (`|ExecutionSequence`
              (:`then_0`
                (bind (_direction_11 _lerp_11) (`Timeline|Part 11 Loc` :!label _label_11)
                  (:`Update`
                    (`SceneComponent.K2_SetRelativeLocation` (`self.Part11`) (`KismetMathLibrary.VLerp` (52.1 0.0 20.6) (52.1 40.0 20.6) _lerp_11) false false))))
              (:`then_1`
                (`AudioComponent.Play` (`self.Part 11 Open`) 0.0))))
          (:`B`
            (`|ExecutionSequence`
              (:`then_0`
                (goto _label_11 :!via `Reverse`))
              (:`then_1`
                (`AudioComponent.Play` (`self.Part 11 Close`) 0.0)))))))
    (:`then_11`
      (if (== (`self.Part12`) Component)
        (`/Engine/EditorBlueprintResources/StandardMacros.FlipFlop`
          (:`A`
            (`|ExecutionSequence`
              (:`then_0`
                (bind (_direction_12 _lerp_12) (`Timeline|Part 12 Loc` :!label _label_12)
                  (:`Update`
                    (`SceneComponent.K2_SetRelativeLocation` (`self.Part12`) (`KismetMathLibrary.VLerp` (135.8 0.0 20.6) (135.8 40.0 20.6) _lerp_12) false false))))
              (:`then_1`
                (`AudioComponent.Play` (`self.Part 12 Open`) 0.0))))
          (:`B`
            (`|ExecutionSequence`
              (:`then_0`
                (goto _label_12 :!via `Reverse`))
              (:`then_1`
                (`AudioComponent.Play` (`self.Part 12 Close`) 0.0)))))))))

(fn `UserConstructionScript`)
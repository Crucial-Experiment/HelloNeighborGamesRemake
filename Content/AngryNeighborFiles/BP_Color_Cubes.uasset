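; BP_Color_Cubes is a pickable inventory item that spawns copies of itself, with a State selecting red, blue or green material and icon.
; The construction script applies that look, and pickup destroys the cube if the inventory already holds one of the same State.
; Left-click while held, or VR use, triggers a server spawn: red and blue copies launch along camera forward at different strengths, while green ones get a flat mode instead.
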(event `/Game/Function/BP_Interface.PickUp`
  (bind _player (`/Game/Function/BP_MacroLibrary.Find Player`)
    (:`Is Valid`
      (bind _items (`/Game/Player/BP_Player.Get Inventory` _player))
      (bind _filteredarray (`KismetArrayLibrary.FilterArray` _items "BP_Color_Cubes_C"))
      (if (`KismetArrayLibrary.Array_IsNotEmpty` _filteredarray)
        (for _array_element _filteredarray
          (if (== (`/Game/AngryNeighborFiles/BP_Color_Cubes.State` _array_element) (`self.State`))
            (`self.K2_DestroyActor`)))
        (`/Engine/EditorBlueprintResources/StandardMacros.IsValid` (`self.FlatComponent`)
          (:`Is Valid`
            (`parent.PickUp`)))
        (else
          (`parent.PickUp`))))))

(event `self.On Press LMB`
  (bind _player (`/Game/Function/BP_MacroLibrary.Find Player`)
    (:`Is Valid`
      (bind _item (`/Game/Player/BP_Player.Get Item` _player))
      (if (== _item self)
        (`self.Spawn (Server)` :!label _label)))))

(event `self.On VR Use`
  (`parent.On VR Use`)
  (goto _label))

(event `Spawn (Server)`
  (bind _returnvalue (`self.GetActorForwardVector` (`GameplayStatics.GetPlayerCameraManager` 0)))
  (bind _returnvalue_2 (`SceneComponent.K2_GetComponentLocation` (`self.Spawn Point`)))
  (switch `int` (`self.State`)
    (:`0`
      (bind _returnvalue_3 (`|SpawnActorFromClass` "BP_Color_Cubes_C" (`KismetMathLibrary.MakeTransform` _returnvalue_2) "Undefined" "MultiplyWithRoot" null null))
      (bind _root (`/Game/Objects/Structurs/BP_Object.Root` _returnvalue_3))
      (`PrimitiveComponent.AddImpulse` _root (* _returnvalue 50000.0) "None" false)
      (set `/Game/AngryNeighborFiles/BP_Color_Cubes.State` (`self.State`) _returnvalue_3)
      (`PrimitiveComponent.SetMaterial` _root 0 "/Game/AngryNeighborFiles/Materials/ColorCubeRed.ColorCubeRed")
      (set `/Game/Objects/Structurs/FlatComponent.Icon` "/Game/AngryNeighborFiles/Texture/InvIcons/RGBICO.RGBICO" (`/Game/Objects/Structurs/BP_Object.FlatComponent` _returnvalue_3)))
    (:`1`
      (bind _returnvalue_4 (`|SpawnActorFromClass` "BP_Color_Cubes_C" (`KismetMathLibrary.MakeTransform` _returnvalue_2) "Undefined" "MultiplyWithRoot" null null))
      (bind _root_2 (`/Game/Objects/Structurs/BP_Object.Root` _returnvalue_4))
      (`PrimitiveComponent.AddImpulse` _root_2 (* _returnvalue 250000.0) "None" false)
      (set `/Game/AngryNeighborFiles/BP_Color_Cubes.State` (`self.State`) _returnvalue_4)
      (`PrimitiveComponent.SetMaterial` _root_2 0 "/Game/AngryNeighborFiles/Materials/ColorCubeBlue.ColorCubeBlue")
      (set `/Game/Objects/Structurs/FlatComponent.Icon` "/Game/AngryNeighborFiles/Texture/InvIcons/BLUEICO.BLUEICO" (`/Game/Objects/Structurs/BP_Object.FlatComponent` _returnvalue_4)))
    (:`2`
      (bind _returnvalue_5 (`|SpawnActorFromClass` "BP_Color_Cubes_C" (`KismetMathLibrary.MakeTransform` _returnvalue_2) "Undefined" "MultiplyWithRoot" null null))
      (`self.Set Flat Mode` _returnvalue_5 "NewEnumerator1")
      (set `/Game/AngryNeighborFiles/BP_Color_Cubes.State` (`self.State`) _returnvalue_5)
      (`PrimitiveComponent.SetMaterial` (`/Game/Objects/Structurs/BP_Object.Root` _returnvalue_5) 0 "/Game/AngryNeighborFiles/Materials/ColorCubeGreen.ColorCubeGreen")
      (set `/Game/Objects/Structurs/FlatComponent.Icon` "/Game/AngryNeighborFiles/Texture/InvIcons/GREENICO.GREENICO" (`/Game/Objects/Structurs/BP_Object.FlatComponent` _returnvalue_5)))))

(fn `UserConstructionScript`
  (bind _root (`self.Root`))
  (`parent.UserConstructionScript`)
  (switch `int` (`self.State`)
    (:`0`
      (`PrimitiveComponent.SetMaterial` _root 0 "/Game/AngryNeighborFiles/Materials/ColorCubeRed.ColorCubeRed")
      (set `/Game/Objects/Structurs/FlatComponent.Icon` "/Game/AngryNeighborFiles/Texture/InvIcons/RGBICO.RGBICO" (`self.FlatComponent`)))
    (:`1`
      (`PrimitiveComponent.SetMaterial` _root 0 "/Game/AngryNeighborFiles/Materials/ColorCubeBlue.ColorCubeBlue")
      (set `/Game/Objects/Structurs/FlatComponent.Icon` "/Game/AngryNeighborFiles/Texture/InvIcons/BLUEICO.BLUEICO" (`self.FlatComponent`)))
    (:`2`
      (`PrimitiveComponent.SetMaterial` _root 0 "/Game/AngryNeighborFiles/Materials/ColorCubeGreen.ColorCubeGreen")
      (set `/Game/Objects/Structurs/FlatComponent.Icon` "/Game/AngryNeighborFiles/Texture/InvIcons/GREENICO.GREENICO" (`self.FlatComponent`)))))
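; Interactable kitchen stove with a hinged door (Part1) and a sliding drawer (Part2) that open and close on Interact.
; Each part's state picks forward or reverse timeline playback to lerp its rotation or location, flipping state when finished.
; Each toggle plays a sound, slightly delayed for door closing, and reports the use type to the Tutorial and GameJolt components.
; Interactions with other components pass to the parent.
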(event `/Game/Function/BP_Interface.Interact`
  (params (Component :type "PrimitiveComponent Object Reference") (Location :type "Vector Structure"))
  (bind _part_1 (`self.Part 1`))
  (bind _tutorialcomponent (`self.TutorialComponent`))
  (bind _gamejoltcomponent (`self.GameJoltComponent`))
  (bind _tutorialcomponent_2 (`self.TutorialComponent`))
  (bind _gamejoltcomponent_2 (`self.GameJoltComponent`))
  (`|ExecutionSequence`
    (:`then_0`
      (if (== Component _part_1)
        (switch `/Game/Objects/Enum/RotateStateEnum` (`self.Part 1 State`)
          (:`NewEnumerator0`
            (`/Game/Objects/Tutorial/TutorialComponent.Check Use Type` _tutorialcomponent_2 "NewEnumerator2")
            (`/Game/Objects/GameJolt/GameJoltComponent.Check Use Type` _gamejoltcomponent_2 "NewEnumerator2")
            (`|ExecutionSequence`
              (:`then_0`
                (bind (_direction _driver) (`Timeline|Part 1 Rotation` :!via `Reverse` :!label _label)
                  (:`Update`
                    (`SceneComponent.K2_SetRelativeRotation` (`self.Part 1`) (`KismetMathLibrary.RLerp` (struct) (struct :`Roll` 50.0) _driver) false false))
                  (:`Finished`
                    (switch `/Game/Objects/Enum/RotateStateEnum` (`self.Part 1 State`)
                      (:`NewEnumerator0`
                        (set `self.Part 1 State` "NewEnumerator1"))
                      (:`NewEnumerator1`
                        (set `self.Part 1 State` "NewEnumerator0"))))))
              (:`then_1`
                (`KismetSystemLibrary.Delay` 0.2)
                (`AudioComponent.Play` (`self.Cabinet Close`) 0.0))))
          (:`NewEnumerator1`
            (`/Game/Objects/Tutorial/TutorialComponent.Check Use Type` _tutorialcomponent_2 "NewEnumerator1")
            (`/Game/Objects/GameJolt/GameJoltComponent.Check Use Type` _gamejoltcomponent_2 "NewEnumerator1")
            (`|ExecutionSequence`
              (:`then_0`
                (goto _label))
              (:`then_1`
                (`AudioComponent.Play` (`self.Cabinet Open`) 0.0)))))))
    (:`then_1`
      (if (== Component (`self.Part 2`))
        (switch `/Game/Objects/Enum/RotateStateEnum` (`self.Part 2 State`)
          (:`NewEnumerator0`
            (`/Game/Objects/Tutorial/TutorialComponent.Check Use Type` _tutorialcomponent "NewEnumerator2")
            (`/Game/Objects/GameJolt/GameJoltComponent.Check Use Type` _gamejoltcomponent "NewEnumerator2")
            (`|ExecutionSequence`
              (:`then_0`
                (bind (_direction_2 _driver_2) (`Timeline|Part 2 Location` :!via `Reverse` :!label _label_2)
                  (:`Update`
                    (`SceneComponent.K2_SetRelativeLocation` (`self.Part 2`) (`KismetMathLibrary.VLerp` (0.0 16.0 18.0) (0.0 60.0 18.0) _driver_2) false false))
                  (:`Finished`
                    (switch `/Game/Objects/Enum/RotateStateEnum` (`self.Part 2 State`)
                      (:`NewEnumerator0`
                        (set `self.Part 2 State` "NewEnumerator1"))
                      (:`NewEnumerator1`
                        (set `self.Part 2 State` "NewEnumerator0"))))))
              (:`then_1`
                (`AudioComponent.Play` (`self.Cabinet Slide Close`) 0.0))))
          (:`NewEnumerator1`
            (`/Game/Objects/Tutorial/TutorialComponent.Check Use Type` _tutorialcomponent "NewEnumerator1")
            (`/Game/Objects/GameJolt/GameJoltComponent.Check Use Type` _gamejoltcomponent "NewEnumerator1")
            (`|ExecutionSequence`
              (:`then_0`
                (goto _label_2))
              (:`then_1`
                (`AudioComponent.Play` (`self.Cabinet Slide Open`) 0.0)))))))
    (:`then_2`
      (if (and (!= Component _part_1) (!= Component (`self.Part 2`)))
        (`parent.Interact` Component Location)))))

(fn `UserConstructionScript`
  (`parent.UserConstructionScript`))
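; BP_Siren is a siren prop that can be switched on and off through SirenOn and SirenOff events.
; When on, it plays its sound, lights a spotlight and runs a timeline that spins the Pusher component through a full roll rotation.
; When off, it zeroes the light and stops the sound and timeline.
; BeginPlay applies whichever state the Activate flag holds.
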(event `Event Siren On`
  (set `self.Activate` true)
  (`|ExecutionSequence` :!label _label
    (:`then_0`
      (`AudioComponent.Play` (`self.Siren Sound`) 0.0))
    (:`then_1`
      (bind (_direction _lerp) (`Timeline|Pusher Rotate` :!label _label_2)
        (:`Update`
          (`SceneComponent.K2_SetRelativeRotation` (`self.Pusher`) (`KismetMathLibrary.RLerp` (struct) (struct :`Yaw` 360.0) _lerp) false false))))
    (:`then_2`
      (`LightComponent.SetIntensity` (`self.SpotLight`) 15000.0))))

(event `self.ReceiveBeginPlay`
  (`parent.ReceiveBeginPlay`)
  (if (`self.Activate`)
    (goto _label)
    (else
      (`|ExecutionSequence` :!label _label_3
        (:`then_0`
          (`LightComponent.SetIntensity` (`self.SpotLight`) 0.0))
        (:`then_1`
          (`AudioComponent.Stop` (`self.Siren Sound`)))
        (:`then_2`
          (goto _label_2 :!via `Stop`))))))

(event `Event Siren Off`
  (set `self.Activate` false)
  (goto _label_3))

(fn `UserConstructionScript`
  (`parent.UserConstructionScript`))
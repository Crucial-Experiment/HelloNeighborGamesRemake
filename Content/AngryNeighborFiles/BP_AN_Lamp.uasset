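; Interactable lamp Blueprint that toggles its point light on and off.
; Each Interact event alternates through a FlipFlop, starting by hiding PointLight and then showing it on the next use.
; Each toggle plays a sound, with LampOn paired with hiding the light and LampOff with showing it, opposite to their names.
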(event `/Game/Function/BP_Interface.Interact`
  (params (Component :type "PrimitiveComponent Object Reference") (Location :type "Vector Structure"))
  (bind _pointlight (`self.PointLight`))
  (if true
    (`/Engine/EditorBlueprintResources/StandardMacros.FlipFlop`
      (:`A`
        (`|ExecutionSequence`
          (:`then_0`
            (`AudioComponent.Play` (`self.Lamp_On`) 0.0))
          (:`then_1`
            (`SceneComponent.SetVisibility` _pointlight false false))))
      (:`B`
        (`|ExecutionSequence`
          (:`then_0`
            (`SceneComponent.SetVisibility` _pointlight true false))
          (:`then_1`
            (`AudioComponent.Play` (`self.Lamp_Off`) 0.0)))))))

(fn `UserConstructionScript`)
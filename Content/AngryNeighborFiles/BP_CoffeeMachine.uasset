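; Coffee machine electrical device that switches on when an actor of a configured class enters its box trigger.
; The actor snaps to the placement component, and if it is a BP_Object its flat mode changes.
; Tumbler and the Enable/Disable overrides propagate power to the linked Electricity actors according to switch state, available electricity and whether the machine is a generator.
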(event `self.Box.OnComponentBeginOverlap`
  (params (OverlappedComponent :type "PrimitiveComponent Object Reference") (OtherActor :type "Actor Object Reference") (OtherComp :type "PrimitiveComponent Object Reference") (OtherBodyIndex :type Integer) (bFromSweep :type Boolean) (SweepResult :type "HitResult Structure (by ref)"))
  ;[1 1 1] Attach
  (if (== (`GameplayStatics.GetObjectClass` OtherActor) (`self.Actor Class`))
    (`self.K2_AttachToComponent` OtherActor (`self.Place To`) "None" "SnapToTarget" "SnapToTarget" "SnapToTarget" true)
    (set `self.State` "NewEnumerator0")
    (`self.Tumbler` "NewEnumerator0")
    (bind _asbp_object (cast `/Game/Objects/Structurs/BP_Object` OtherActor))
    (`self.Set Flat Mode` _asbp_object "NewEnumerator1")))

(event `self.Enable`
  ;[1 1 1] Tumbler
  (`parent.Enable`)
  (switch `/Game/Objects/Enum/TumblerStateEnum` (`self.State`) :!label _label
    (:`NewEnumerator0`
      (for _array_element (`self.Electricity`)
        (`/Engine/EditorBlueprintResources/StandardMacros.IsValid` _array_element
          (:`Is Valid`
            (`self.Enable` _array_element)))))))

(event `Tumbler`
  (params (State :type "/Game/Objects/Enum/TumblerStateEnum Enum" :default "NewEnumerator0"))
  (bind _generator (`self.Generator`))
  ;[1 1 1] Tumbler
  (if (or (`self.Has Electricity`) _generator)
    (switch `/Game/Objects/Enum/TumblerStateEnum` State
      (:`NewEnumerator0`
        (goto _label))
      (:`NewEnumerator1`
        (for _array_element (`self.Electricity`) :!label _label_2
          (`/Engine/EditorBlueprintResources/StandardMacros.IsValid` _array_element
            (:`Is Valid`
              (`self.Disable` _array_element))))))
    (elif (not _generator)
      (goto _label_2))))

(event `self.Disable`
  ;[1 1 1] Tumbler
  (`parent.Disable`)
  (goto _label_2))

(fn `UserConstructionScript`)
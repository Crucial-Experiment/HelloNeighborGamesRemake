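; Interactive electrical switch box with an optional door and lever arm that powers linked devices on or off.
; Timelines animate door and lever; a finished lever throw updates State, notifies tutorial and GameJolt components, and calls Tumbler.
; Tumbler enables or disables the Electricity array and BPRotate's AutoLock, respecting supply or generator status.
; With SosedMove set, using the lever sends the Neighbor AI to investigate via blackboard; SosedRemote switches it back on.
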(event `self.Interact`
  (params (Component :type "PrimitiveComponent Object Reference") (Location :type "Vector Structure"))
  (bind _tutorialcomponent (`self.TutorialComponent`))
  (bind _gamejoltcomponent (`self.GameJoltComponent`))
  (bind _state (`self.State`))
  (bind _door_rotate (`self.Door Rotate`))
  (`|ExecutionSequence`
    (:`then_0`
      ;[1 1 1] Door
      (if (== Component (`self.Door`))
        (switch `/Game/Objects/Enum/RotateStateEnum` (`self.Door Rotate`)
          (:`NewEnumerator0`
            (set `self.Door Rotate` "NewEnumerator3")
            (`|ExecutionSequence`
              (:`then_0`
                (bind (_direction _alpha) (`Timeline|Door Timeline` :!via `PlayFromStart` :!label _label)
                  (:`Update`
                    (`SceneComponent.K2_SetRelativeRotation` (`self.Door`) (`KismetMathLibrary.RLerp` (select `/Game/Objects/Enum/RotateStateEnum` _door_rotate :`NewEnumerator1` (struct :`Yaw` 100.0) :`NewEnumerator3` (struct :`Yaw` 100.0) :!type "Rotator Structure") (select `/Game/Objects/Enum/RotateStateEnum` _door_rotate :`NewEnumerator0` (struct :`Yaw` 100.0) :`NewEnumerator2` (struct :`Yaw` 100.0) :!type "Rotator Structure") _alpha) false false))
                  (:`Finished`
                    (switch `/Game/Objects/Enum/RotateStateEnum` (`self.Door Rotate`)
                      (:`NewEnumerator2`
                        (set `self.Door Rotate` "NewEnumerator0"))
                      (:`NewEnumerator3`
                        (set `self.Door Rotate` "NewEnumerator1"))))))
              (:`then_1`
                (`GameplayStatics.PlaySoundAtLocation` (`self.Gate Close Sound`) (`self.K2_GetActorLocation`) (struct) 1.0 1.0 0.0 null null null null))))
          (:`NewEnumerator1`
            (set `self.Door Rotate` "NewEnumerator2")
            (`|ExecutionSequence`
              (:`then_0`
                (goto _label :!via `PlayFromStart`))
              (:`then_1`
                (`GameplayStatics.PlaySoundAtLocation` (`self.Gate Open Sound`) (`self.K2_GetActorLocation`) (struct) 1.0 1.0 0.0 null null null null)))))))
    (:`then_1`
      ;[1 1 1] Arm
      (if (and (== Component (`self.Arm`)) (`self.Show Arm`))
        (`|ExecutionSequence`
          (:`then_0`
            (switch `/Game/Objects/Enum/RotateStateEnum` (`self.Arm Rotate Status`) :!label _label_2
              (:`NewEnumerator0`
                (set `self.Arm Rotate Status` "NewEnumerator3")
                (`|ExecutionSequence`
                  (:`then_0`
                    (bind (_direction_2 _alpha_2) (`Timeline|Arm Timeline` :!via `PlayFromStart` :!label _label_3)
                      (:`Update`
                        (`SceneComponent.K2_SetRelativeRotation` (`self.Arm`) (`KismetMathLibrary.RLerp` (select `/Game/Objects/Enum/TumblerStateEnum` _state :`NewEnumerator1` (struct :`Roll` 170.0) :!type "Rotator Structure") (select `/Game/Objects/Enum/TumblerStateEnum` _state :`NewEnumerator0` (struct :`Roll` 170.0) :!type "Rotator Structure") _alpha_2) false false))
                      (:`Finished`
                        (switch `/Game/Objects/Enum/RotateStateEnum` (`self.Arm Rotate Status`)
                          (:`NewEnumerator2`
                            (set `self.Arm Rotate Status` "NewEnumerator0")
                            (set `self.State` "NewEnumerator0")
                            (`/Game/Objects/Tutorial/TutorialComponent.Check Use Type` _tutorialcomponent "NewEnumerator3")
                            (`/Game/Objects/GameJolt/GameJoltComponent.Check Use Type` _gamejoltcomponent "NewEnumerator3"))
                          (:`NewEnumerator3`
                            (set `self.Arm Rotate Status` "NewEnumerator1")
                            (set `self.State` "NewEnumerator1")
                            (`/Game/Objects/Tutorial/TutorialComponent.Check Use Type` _tutorialcomponent "NewEnumerator4")
                            (`/Game/Objects/GameJolt/GameJoltComponent.Check Use Type` _gamejoltcomponent "NewEnumerator4")))
                        (`self.Tumbler` (`self.State`)))))
                  (:`then_1`
                    (`GameplayStatics.PlaySoundAtLocation` (`self.Switch Off Sound`) (`self.K2_GetActorLocation`) (struct) 1.0 1.0 0.0 null null null null))))
              (:`NewEnumerator1`
                (set `self.Arm Rotate Status` "NewEnumerator2")
                (`|ExecutionSequence`
                  (:`then_0`
                    (goto _label_3 :!via `PlayFromStart`))
                  (:`then_1`
                    (`GameplayStatics.PlaySoundAtLocation` (`self.Switch On Sound`) (`self.K2_GetActorLocation`) (struct) 1.0 1.0 0.0 null null null null))))))
          (:`then_1`
            (if (`self.Sosed Move`)
              ;[1 1 1] Sosed
              (bind _sosed (`/Game/Function/BP_MacroLibrary.Find Sosed`)
                (:`Is Valid`
                  (if (`|EnumInequality` (`/Game/Sosed/BP_Sosed.Current State` _sosed) "NewEnumerator2")
                    (bind _returnvalue (`AIBlueprintHelperLibrary.GetBlackboard` _sosed))
                    (`BlackboardComponent.SetValueAsInt` _returnvalue "CheckTask" 4)
                    (`BlackboardComponent.SetValueAsVector` _returnvalue "Check Location" (`SceneComponent.K2_GetComponentLocation` (`self.Arrow`)))
                    (`BlackboardComponent.SetValueAsObject` _returnvalue "Electricity" self)
                    (`/Game/Sosed/BP_Sosed.Set State` _sosed "NewEnumerator3")))))))))))

(event `self.ReceiveBeginPlay`
  ;[1 1 1] Begin Play
  (`parent.ReceiveBeginPlay`)
  (`PrimitiveComponent.SetSimulatePhysics` (`self.Root`) false)
  (`self.Tumbler` (`self.State`))
  (if (not (`self.Has Door?`))
    (`ActorComponent.K2_DestroyComponent` (`self.Door`))))

(event `Sosed Remote`
  ;[1 1 1] Arm
  (if (`|EnumEquality` (`self.State`) "NewEnumerator1")
    (goto _label_2)))

(event `self.Enable`
  ;[1 1 1] Tumbler
  (`parent.Enable`)
  (switch `/Game/Objects/Enum/TumblerStateEnum` (`self.State`) :!label _label_4
    (:`NewEnumerator0`
      (for _array_element (`self.Electricity`)
        (`/Engine/EditorBlueprintResources/StandardMacros.IsValid` _array_element
          (:`Is Valid`
            (`self.Enable` _array_element))))
      (bind _bp_rotate (`self.BP_Rotate`)
        (:`then`
          (set `/Game/Objects/Structurs/BP_Rotate.Auto Lock` false _bp_rotate))
        (:`else`)))))

(event `Tumbler`
  (params (State :type "/Game/Objects/Enum/TumblerStateEnum Enum" :default "NewEnumerator0"))
  (bind _generator (`self.Generator`))
  ;[1 1 1] Tumbler
  (if (or (`self.Has Electricity`) _generator)
    (switch `/Game/Objects/Enum/TumblerStateEnum` State
      (:`NewEnumerator0`
        (goto _label_4))
      (:`NewEnumerator1`
        (for _array_element (`self.Electricity`) :!label _label_5
          (`/Engine/EditorBlueprintResources/StandardMacros.IsValid` _array_element
            (:`Is Valid`
              (`self.Disable` _array_element))))
        (bind _bp_rotate (`self.BP_Rotate`)
          (:`then`
            (set `/Game/Objects/Structurs/BP_Rotate.Auto Lock` true _bp_rotate))
          (:`else`))))
    (elif (not _generator)
      (goto _label_5))))

(event `self.Disable`
  ;[1 1 1] Tumbler
  (`parent.Disable`)
  (goto _label_5))

(fn `UserConstructionScript`
  (bind _arm (`self.Arm`))
  (bind _door (`self.Door`))
  (bind _show_arm (`self.Show Arm`))
  (bind _componenttags (`ActorComponent.ComponentTags` (`self.Arm`)))
  (`|ExecutionSequence`
    (:`then_0`
      (`SceneComponent.SetHiddenInGame` (`self.Arm`) (not _show_arm) false))
    (:`then_1`
      (if _show_arm
        (`KismetArrayLibrary.Array_Add` _componenttags "interactive")
        (else
          (`KismetArrayLibrary.Array_RemoveItem` _componenttags "interactive"))))
    (:`then_2`
      (switch `/Game/Objects/Enum/TumblerStateEnum` (`self.State`)
        (:`NewEnumerator0`
          (`SceneComponent.K2_SetRelativeRotation` :`self` _arm)
          (set `self.Arm Rotate Status` "NewEnumerator0"))
        (:`NewEnumerator1`
          (`SceneComponent.K2_SetRelativeRotation` _arm (struct :`Roll` 170.0) false false)
          (set `self.Arm Rotate Status` "NewEnumerator1"))))
    (:`then_3`
      (switch `/Game/Objects/Enum/RotateStateEnum` (`self.Door Rotate`)
        (:`NewEnumerator0`
          (`SceneComponent.K2_SetRelativeRotation` _door (struct :`Yaw` 100.0) false false :!label _label))
        (:`NewEnumerator2`
          (goto _label))
        (:`NewEnumerator1`
          (`SceneComponent.K2_SetRelativeRotation` :`self` _door :!label _label_2))
        (:`NewEnumerator3`
          (goto _label_2))))
    (:`then_4`
      (`SceneComponent.SetHiddenInGame` (`self.Door`) (not (`self.Has Door?`)) false))))
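; BP_Saucepan is a pickupable saucepan prop that burns the player when picked up hot.
; On pickup it runs the parent logic, waits briefly, then checks its TemperatureComponent and, above a threshold, plays a sizzle burn sound and calls TryRelease.
; The construction script points the TemperatureComponent at the saucepan's root.
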(event `/Game/Function/BP_Interface.PickUp`
  (`parent.PickUp`)
  (`KismetSystemLibrary.Delay` 0.2)
  (if (> (`/Game/Objects/Structurs/TemperatureComponent.Temperature` (`self.TemperatureComponent`)) 0.2)
    (`GameplayStatics.PlaySound2D` "/Game/Sounds/Objects/Noise/sizzle_burn_Cue.sizzle_burn_Cue" 1.0 1.0 0.0 null null)
    (`self.Try Release`)))

(fn `UserConstructionScript`
  (`parent.UserConstructionScript`)
  (set `/Game/Objects/Structurs/TemperatureComponent.Actor` (`self.Root`) (`self.TemperatureComponent`)))
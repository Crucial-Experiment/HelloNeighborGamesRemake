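; BP_Safe is an interactable safe whose door swings open and closed.
; Interact forwards to a server-side event, which acts only when the targeted component is the Door.
; A FlipFlop alternates between playing and reversing a timeline that lerps the door's relative rotation, with an open or close sound at the actor's location.
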(event `Interact (Server)`
  (params (Component :type "PrimitiveComponent Object Reference"))
  (if (== (`self.Door`) Component)
    (`/Engine/EditorBlueprintResources/StandardMacros.FlipFlop`
      (:`A`
        (`GameplayStatics.PlaySoundAtLocation` (`self.Safe Door Open Sound`) (`self.K2_GetActorLocation`) (struct) 1.0 1.0 0.0 null null null null)
        (bind (_direction _alpha) (`Timeline|Rotate Timeline` :!label _label)
          (:`Update`
            (`SceneComponent.K2_SetRelativeRotation` (`self.Door`) (`KismetMathLibrary.RLerp` (struct) (struct :`Yaw` -155.0) _alpha) false false))))
      (:`B`
        (`GameplayStatics.PlaySoundAtLocation` (`self.Safe Door Close Sound`) (`self.K2_GetActorLocation`) (struct) 1.0 1.0 0.0 null null null null)
        (goto _label :!via `Reverse`)))))

(event `/Game/Function/BP_Interface.Interact`
  (params (Component :type "PrimitiveComponent Object Reference") (Location :type "Vector Structure"))
  (`self.Interact (Server)` Component))

(fn `UserConstructionScript`)
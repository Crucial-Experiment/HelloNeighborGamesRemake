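; BP_HammerTrigger is a level trigger that picks one of two endings, End1T or End2F, once a one-second looping timer reaches RestartTime.
; Unlock replicates through server to all: if BP_Electrical has electricity in a given state, the game restarts.
; Otherwise it sets the End1T outcome, rotates PowerPole and notifies tutorial and GameJolt components.
; End1T finishing teleports DoorSpawn to a new transform; End2F finishing restarts the game.
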(event `self.ReceiveBeginPlay`
  (`PlayerCameraManager.StartCameraFade` (`GameplayStatics.GetPlayerCameraManager` 0) 1.0 0.0 2.0 (struct :`R` 1.0 :`G` 1.0 :`B` 1.0 :`A` 1.0) false true)
  (`KismetSystemLibrary.K2_SetTimerDelegate` (delegate `CustomEvent_1`) 1.0 true true))

(event `End 1T Finish`
  (`self.K2_SetActorTransform` (`self.Door Spawn`) (`self.New Door Transform`) false true))

(event `CustomEvent_1`
  (bind _end1t (`self.End1T`))
  (bind _end2f (`self.End2F`))
  (bind _output_get (set `self.Timer` (+ (`self.Timer`) 1.0)))
  (`KismetSystemLibrary.PrintString` (`KismetStringLibrary.Conv_DoubleToString` _output_get) true false)
  (if (>= (`self.Timer`) (`self.Restart Time`))
    (`KismetSystemLibrary.K2_SetTimerDelegate` (delegate `CustomEvent_1`))
    (if (`self.MoreOrEqually`)
      (`/Game/Objects/Cutscene/BP_Cutscene_Manager.Set State` _end1t "NewEnumerator0")
      (add `/Game/Objects/Cutscene/BP_Cutscene_Manager.On Finished` _end1t (delegate `End 1T Finish`))
      (else
        (`/Game/Objects/Cutscene/BP_Cutscene_Manager.Set State` _end2f "NewEnumerator0")
        (add `/Game/Objects/Cutscene/BP_Cutscene_Manager.On Finished` _end2f (delegate `End 2F Finish`))))))

(event `Unlock (Server)`
  (`self.Unlock (All)`))

(event `End 2F Finish`
  (`GameMode.RestartGame` (`/Game/Function/BP_FunctionLibrary.Get Game Mode`) :!label _label))

(event `self.Unlock`
  (`self.Unlock (Server)`))

(event `Unlock (All)`
  (bind _returnvalue (`GameplayStatics.GetActorOfClass` "/Game/Objects/BP_Objects/BP_Electrical.BP_Electrical_C"))
  (if (and (`/Game/Objects/Structurs/BP_Electricity.Has Electricity` _returnvalue) (`|EnumEquality` (`/Game/Objects/BP_Objects/BP_Electrical.State` _returnvalue) "NewEnumerator0"))
    (goto _label)
    (else
      (set `self.MoreOrEqually` true)
      (`self.K2_SetActorRelativeRotation` (`self.Power Pole`) (struct :`Yaw` 90.0) false false)
      (`/Game/Objects/Tutorial/TutorialComponent.Check Use Type` (`self.TutorialComponent`) "NewEnumerator6")
      (`/Game/Objects/GameJolt/GameJoltComponent.Check Use Type` (`self.GameJoltComponent`) "NewEnumerator6"))))

(fn `UserConstructionScript`
  (`parent.UserConstructionScript`))
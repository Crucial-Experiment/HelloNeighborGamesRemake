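; BP_Lattice_Long is a lattice gate that moves vertically in response to electrical power.
; Enable and Disable call their parent versions, then CheckState plays the location timeline if HasElectricity or Generator is true, otherwise reverses it, with an open or close sound.
; Each timeline update lerps the root from its current, uncached world location toward a Z offset by UpDown, signed by power state, and applies it as relative location.
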(event `self.Enable`
  ;[1 1 1] Begin Play and Electricity
  (`parent.Enable`)
  (`self.Check State` :!label _label))

(event `self.Disable`
  ;[1 1 1] Begin Play and Electricity
  (`parent.Disable`)
  (goto _label))

(event `self.ReceiveBeginPlay`
  ;[1 1 1] Begin Play and Electricity
  (`parent.ReceiveBeginPlay`))

(event `Check State`
  (bind _up___down (`self.Up / Down`))
  (bind _root (`self.Root`))
  (bind (_returnvalue_x _returnvalue_y _returnvalue_z) (`KismetMathLibrary.BreakVector` (`SceneComponent.K2_GetComponentLocation` _root)))
  (bind (_returnvalue_x_2 _returnvalue_y_2 _returnvalue_z_2) (`KismetMathLibrary.BreakVector` (`SceneComponent.K2_GetComponentLocation` _root)))
  (bind _returnvalue (or (`self.Has Electricity`) (`self.Generator`)))
  ;[1 1 1] Check State
  (if _returnvalue
    (`|ExecutionSequence`
      (:`then_0`
        (bind (_direction _alpha) (`Timeline|Location Timeline` :!label _label_2)
          (:`Update`
            (`SceneComponent.K2_SetRelativeLocation` (`self.Root`) (`KismetMathLibrary.VLerp` (`SceneComponent.K2_GetComponentLocation` (`self.Root`)) (select `bool` _returnvalue :`false` (`KismetMathLibrary.MakeVector` _returnvalue_x _returnvalue_y (- _returnvalue_z _up___down)) :`true` (`KismetMathLibrary.MakeVector` _returnvalue_x_2 _returnvalue_y_2 (+ _returnvalue_z_2 _up___down))) _alpha) false false))))
      (:`then_1`
        (`GameplayStatics.PlaySoundAtLocation` "/Game/Sounds/Objects/OpenClosed/gate_open_Cue.gate_open_Cue" (`self.K2_GetActorLocation`) (struct) 1.0 1.0 0.0 null null null null)))
    (else
      (`|ExecutionSequence`
        (:`then_0`
          (goto _label_2 :!via `Reverse`))
        (:`then_1`
          (`GameplayStatics.PlaySoundAtLocation` "/Game/Sounds/Objects/OpenClosed/gate_close_metal_Cue.gate_close_metal_Cue" (`self.K2_GetActorLocation`) (struct) 1.0 1.0 0.0 null null null null))))))

(fn `UserConstructionScript`)
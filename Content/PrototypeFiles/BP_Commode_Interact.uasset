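; Interactable commode prop that toggles its Root component toward or back from an end position when the player interacts.
; Alternate interactions play or reverse the NightstandLoc timeline and switch AutoLock on Rotate on or off.
; The timeline lerps Root's world transform from the current actor transform to EndPos.
; A DoOnce blocks repeat interaction until the timeline finishes.
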(event `/Game/Function/BP_Interface.Interact`
  (params (Component :type "PrimitiveComponent Object Reference") (Location :type "Vector Structure"))
  (bind _rotate (`self.Rotate`))
  (`/Engine/EditorBlueprintResources/StandardMacros.DoOnce` false :!label _label
    (:`Completed`
      (`/Engine/EditorBlueprintResources/StandardMacros.FlipFlop`
        (:`A`
          (set `/Game/Objects/Structurs/BP_Rotate.Auto Lock` true _rotate)
          (bind (_direction _alpha) (`Timeline|Nightstand Loc` :!label _label_2)
            (:`Update`
              (`SceneComponent.K2_SetWorldTransform` (`self.Root`) (`KismetMathLibrary.TLerp` (`self.GetTransform`) (`self.End Pos`) _alpha) false false))
            (:`Finished`
              (goto _label :!via `Reset`))))
        (:`B`
          (set `/Game/Objects/Structurs/BP_Rotate.Auto Lock` false _rotate)
          (goto _label_2 :!via `Reverse`))))))

(fn `UserConstructionScript`
  (`parent.UserConstructionScript`))
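; VR inventory slot that holds one BP_Object at a time.
; Overlapping actors' GrabComponents are tracked and their grab/drop events bound, with AddItem and RemoveItem as direct entry points.
; Dropping an eligible object disables its physics, attaches it and scales it to the slot; grabbing or leaving detaches it and restores its scale.
; The slot mesh resizes as feedback, and capture and release fire callbacks.
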(event `Add Item`
  (params (`Grab Component` :type "/Game/Objects/Structurs/GrabComponent Object Reference"))
  (`KismetArrayLibrary.Array_Add` (`self.Tracked Grab Comp`) `Grab Component`)
  (add `/Game/Objects/Structurs/GrabComponent.OnGrabbed` `Grab Component` (delegate `On Grabbed`))
  (add `/Game/Objects/Structurs/GrabComponent.OnDropped` `Grab Component` (delegate `On Dropped`))
  (`self.Try Capture` `Grab Component`))

(event `self.ReceiveBeginPlay`
  (set `self.Init Self Scale` (`SceneComponent.K2_GetComponentScale` (`self.Mesh`))))

(event `self.Slot.OnComponentBeginOverlap`
  (params (OverlappedComponent :type "PrimitiveComponent Object Reference") (OtherActor :type "Actor Object Reference") (OtherComp :type "PrimitiveComponent Object Reference") (OtherBodyIndex :type Integer) (bFromSweep :type Boolean) (SweepResult :type "HitResult Structure (by ref)"))
  (if (not (`self.Deactivate`))
    (for _array_element (`self.K2_GetComponentsByClass` OtherActor "/Game/Objects/Structurs/GrabComponent.GrabComponent_C")
      (`KismetArrayLibrary.Array_Add` (`self.Tracked Grab Comp`) _array_element)
      (add `/Game/Objects/Structurs/GrabComponent.OnGrabbed` _array_element (delegate `On Grabbed`))
      (add `/Game/Objects/Structurs/GrabComponent.OnDropped` _array_element (delegate `On Dropped`)))
    (`self.Increase Cell Size`)))

(event `On Dropped`
  (params (`Self Ref` :type "/Game/Objects/Structurs/GrabComponent Object Reference"))
  (`self.Try Capture` `Self Ref`)
  (`self.Increase Cell Size`))

(event `On Grabbed`
  (params (`Self Ref` :type "/Game/Objects/Structurs/GrabComponent Object Reference"))
  (`self.Try Drop` (`ActorComponent.GetOwner` `Self Ref`))
  (`self.Decrease Cell Size`))

(event `self.Slot.OnComponentEndOverlap`
  (params (OverlappedComponent :type "PrimitiveComponent Object Reference") (OtherActor :type "Actor Object Reference") (OtherComp :type "PrimitiveComponent Object Reference") (OtherBodyIndex :type Integer))
  (if (not (`self.Deactivate`))
    (`self.Try Drop` OtherActor)
    (for _array_element (`self.K2_GetComponentsByClass` OtherActor "/Game/Objects/Structurs/GrabComponent.GrabComponent_C")
      (`KismetArrayLibrary.Array_RemoveItem` (`self.Tracked Grab Comp`) _array_element)
      (remove `/Game/Objects/Structurs/GrabComponent.OnGrabbed` _array_element (delegate `On Grabbed`))
      (remove `/Game/Objects/Structurs/GrabComponent.OnDropped` _array_element (delegate `On Dropped`)))
    (`self.Decrease Cell Size`)))

(event `Remove Item`
  (params (`Grab Component` :type "/Game/Objects/Structurs/GrabComponent Object Reference"))
  (`KismetArrayLibrary.Array_RemoveItem` (`self.Tracked Grab Comp`) `Grab Component`)
  (remove `/Game/Objects/Structurs/GrabComponent.OnGrabbed` `Grab Component` (delegate `On Grabbed`))
  (remove `/Game/Objects/Structurs/GrabComponent.OnDropped` `Grab Component` (delegate `On Dropped`))
  (`self.Try Drop` (`ActorComponent.GetOwner` `Grab Component`)))

(fn `Decrease Cell Size`
  (`SceneComponent.SetWorldScale3D` (`self.Mesh`) (`self.Init Self Scale`)))

(fn `Increase Cell Size`
  (`SceneComponent.SetWorldScale3D` (`self.Mesh`) (* (`self.Init Self Scale`) 1.2)))

(fn `Try Capture`
  (params (`Grab Comp` :type "/Game/Objects/Structurs/GrabComponent Object Reference"))
  (bind _hold_actor (`self.Hold Actor`))
  (`/Engine/EditorBlueprintResources/StandardMacros.IsValid` (`self.Hold Actor`)
    (:`Is Not Valid`
      (bind _asbp_object (cast `/Game/Objects/Structurs/BP_Object` (`ActorComponent.GetOwner` `Grab Comp`)))
      (bind _flatcomponent (`/Game/Objects/Structurs/BP_Object.FlatComponent` _asbp_object))
      (if (and (`/Game/Objects/Structurs/FlatComponent.Can Put In Slot` _flatcomponent) (`|EnumInequality` (`/Game/Objects/Structurs/FlatComponent.Mode` _flatcomponent) "NewEnumerator1"))
        (bind _output_get (set `self.Hold Actor` _asbp_object))
        (set `self.Init Actor Scale` (`self.GetActorScale3D` _output_get))
        (`/Game/Objects/Structurs/GrabComponent.SetPrimitiveCompPhysics` `Grab Comp` false)
        (`self.K2_AttachToComponent` (`self.Hold Actor`) (`self.DefaultSceneRoot`) "None" "SnapToTarget" "KeepWorld" "KeepWorld" true)
        (`self.SetActorScale3D` _hold_actor (* (`self.Init Self Scale`) 0.65))
        (`self.On Capture` _hold_actor)))))

(fn `Try Drop`
  (params (Actor :type "Actor Object Reference"))
  (bind _hold_actor (`self.Hold Actor`))
  (bind _hold_actor_2 (`self.Hold Actor`))
  (`/Engine/EditorBlueprintResources/StandardMacros.IsValid` _hold_actor_2
    (:`Is Valid`
      (if (and (== Actor _hold_actor_2) (`/Game/Objects/Structurs/FlatComponent.Can Put In Slot` (`/Game/Objects/Structurs/BP_Object.FlatComponent` _hold_actor_2)))
        (if (== (`self.GetAttachParentActor` (`self.Hold Actor`)) self)
          (`self.K2_DetachFromActor` _hold_actor "KeepWorld" "KeepWorld" "KeepWorld"))
        (`self.SetActorScale3D` _hold_actor (`self.Init Actor Scale`))
        (`self.On Drop` _hold_actor)
        (set `self.Hold Actor` null)))))

(fn `UserConstructionScript`)
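; VR inventory actor that holds four item slots as child actors and switches them on and off as a group.
; Activate and Deactivate loop over the slots, setting each slot's Deactivate flag and showing or hiding both the slot and its held actor.
; They also switch the held actor's GrabComponent grab type to match the state.
; The event graph is empty, so both functions rely on external callers.
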(fn `Activate`
  (for _array_element (`self.Get Slots`)
    (bind _asbp_inventory_slot (cast `/Game/Player/VR/BP_Inventory_Slot` _array_element))
    (set `/Game/Player/VR/BP_Inventory_Slot.Deactivate` false _asbp_inventory_slot)
    (`self.SetActorHiddenInGame` _array_element false)
    (`self.SetActorHiddenInGame` (`/Game/Player/VR/BP_Inventory_Slot.Hold Actor` _asbp_inventory_slot) false)
    (set `/Game/Objects/Structurs/GrabComponent.GrabType` "NewEnumerator4" (`/Game/Objects/Structurs/BP_Object.GrabComponent` (`/Game/Player/VR/BP_Inventory_Slot.Hold Actor` _asbp_inventory_slot)))))

(fn `Deactivate`
  (for _array_element (`self.Get Slots`)
    (bind _asbp_inventory_slot (cast `/Game/Player/VR/BP_Inventory_Slot` _array_element))
    (set `/Game/Player/VR/BP_Inventory_Slot.Deactivate` true _asbp_inventory_slot)
    (`self.SetActorHiddenInGame` _array_element true)
    (`self.SetActorHiddenInGame` (`/Game/Player/VR/BP_Inventory_Slot.Hold Actor` _asbp_inventory_slot) true)
    (set `/Game/Objects/Structurs/GrabComponent.GrabType` "NewEnumerator0" (`/Game/Objects/Structurs/BP_Object.GrabComponent` (`/Game/Player/VR/BP_Inventory_Slot.Hold Actor` _asbp_inventory_slot)))))

(fn `Get Slots`
  (returns (Array :type "Array of Actor Object Reference"))
  (return (`|MakeArray` (`ChildActorComponent.ChildActor` (`self.Slot 1`)) (`ChildActorComponent.ChildActor` (`self.Slot 2`)) (`ChildActorComponent.ChildActor` (`self.Slot 3`)) (`ChildActorComponent.ChildActor` (`self.Slot 4`)))))

(fn `UserConstructionScript`)
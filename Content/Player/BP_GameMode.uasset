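; Game mode that bootstraps a level: applies saved volume, nickname and Game Jolt auto-login, or benchmarks hardware and creates a first save.
; After a short delay it restores the GameInstance's pending save into objects, player, inventory, time and cutscenes, matched by object name, then clears it.
; On authority it spawns or relocates the Sosed at a random spawn point.
; It also tracks players by net ID and shows log messages.
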(event `self.ReceiveBeginPlay`
  ;[1 1 1] Begin Play
  (`|ExecutionSequence`
    (:`then_0`
      (`GameJolt.Initialize` 918070 "a019aaa30567337a8c3aee30fd469652")
      (`GameplayStatics.SetBaseSoundMix` "/Game/Sounds/Attenuation/SM_Volume.SM_Volume")
      (`KismetSystemLibrary.Delay` 0.2)
      (`self.Load Save Game`))
    (:`then_1`
      (bind _returnvalue (`GameplayStatics.DoesSaveGameExist` "GameSave"))
      (if _returnvalue
        (bind _returnvalue_2 (`GameplayStatics.LoadGameFromSlot` "GameSave"))
        (bind _asbp_save_game (cast `/Game/Function/BP_SaveGame` _returnvalue_2))
        (`GameplayStatics.SetSoundMixClassOverride` "/Game/Sounds/Attenuation/SM_Volume.SM_Volume" "/Engine/EngineSounds/Music.Music" (`/Game/Function/BP_SaveGame.Volume_Music` _asbp_save_game))
        (`GameplayStatics.SetSoundMixClassOverride` "/Game/Sounds/Attenuation/SM_Volume.SM_Volume" "/Engine/EngineSounds/SFX.SFX" (`/Game/Function/BP_SaveGame.Volume_Sound` _asbp_save_game))
        (`GameplayStatics.SetSoundMixClassOverride` "/Game/Sounds/Attenuation/SM_Volume.SM_Volume" "/Engine/EngineSounds/Master.Master" (`/Game/Function/BP_SaveGame.Volume_Master` _asbp_save_game))
        (bind _player_nick_name (`/Game/Function/BP_SaveGame.Player Nick Name` _asbp_save_game))
        (if (`KismetTextLibrary.NotEqual_TextText` _player_nick_name (`KismetTextLibrary.MakeInvariantText` ""))
          (set `/Game/Function/BP_GameInstance.Player Nick Name` _player_nick_name (`/Game/Function/BP_FunctionLibrary.Get Game Instance`)))
        (bind _gj_username (`/Game/Function/BP_SaveGame.GJ_UserName` _asbp_save_game))
        (bind _gj_usertoken (`/Game/Function/BP_SaveGame.GJ_UserToken` _asbp_save_game))
        (if (and (not (`KismetStringLibrary.IsEmpty` _gj_username)) (not (`KismetStringLibrary.IsEmpty` _gj_usertoken)))
          (bind _error (`Login.Login` _gj_username _gj_usertoken)
            (:`Failure`
              (`KismetSystemLibrary.PrintString` (`KismetStringLibrary.Concat_StrStr` "Auto Login Error: " (`|GetEnumeratorNameAsString` _error)) true false (struct :`R` 1.0 :`G` 0.045605 :`A` 1.0)))))
        (else
          (bind _returnvalue_3 (`GameUserSettings.GetGameUserSettings`))
          (`GameUserSettings.RunHardwareBenchmark` _returnvalue_3 10 1.0 1.0)
          (`GameUserSettings.ApplyHardwareBenchmarkResults` _returnvalue_3)
          (bind _returnvalue_4 (`GameplayStatics.CreateSaveGameObject` "/Game/Function/BP_SaveGame.BP_SaveGame_C"))
          (set `/Game/Function/BP_SaveGame.VRMode` false _returnvalue_4)
          (`GameplayStatics.SaveGameToSlot` _returnvalue_4 "GameSave"))))
    (:`then_2`
      (`self.Random Spawn Sosed`))
    (:`then_3`
      (`KismetSystemLibrary.ExecuteConsoleCommand` "DisableAllScreenMessages" null))
    (:`then_4`
      (add `/Game/Function/BP_GameInstance.Log Message` (`/Game/Function/BP_FunctionLibrary.Get Game Instance`) (delegate `Log Message`)))))

(event `Log Message`
  (params (Message :type String) (`Print To Player` :type Boolean))
  (bind _returnvalue (`KismetTextLibrary.Conv_StringToText` Message))
  ;[1 1 1] Begin Play
  (if `Print To Player`
    (bind _log_message_widget (`self.Log Message Widget`)
      (:`then`
        (`/Game/UMG/Online/WB_LogMessage.Print Message` _log_message_widget _returnvalue))
      (:`else`
        (bind _returnvalue_2 (`|CreateWidget` "/Game/UMG/Online/WB_LogMessage.WB_LogMessage_C" (`GameplayStatics.GetPlayerController` 0)))
        (bind _output_get (set `self.Log Message Widget` _returnvalue_2))
        (`UserWidget.AddToViewport` _output_get 0)
        (`/Game/UMG/Online/WB_LogMessage.Print Message` _output_get _returnvalue)))))

(event `Random Spawn Sosed`
  ;[1 1 1] Sosed
  (if (`self.HasAuthority`)
    (bind _outactors (`GameplayStatics.GetAllActorsOfClass` "/Game/Sosed/BP_Sosed.BP_Sosed_C"))
    (if (== (`KismetArrayLibrary.Array_Length` _outactors) 0)
      (bind _outactors_2 (`GameplayStatics.GetAllActorsOfClass` "/Game/Sosed/BP_Sosed_Spawn_Point.BP_Sosed_Spawn_Point_C"))
      (bind _outitem (`KismetArrayLibrary.Array_Random` _outactors_2))
      (`/Engine/EditorBlueprintResources/StandardMacros.IsValid` _outitem
        (:`Is Valid`
          (`|SpawnActorFromClass` "/Game/Sosed/BP_Sosed.BP_Sosed_C" (`self.GetTransform` _outitem) "Undefined" "MultiplyWithRoot" null null)))
      (else
        (bind _outactors_3 (`GameplayStatics.GetAllActorsOfClass` "/Game/Sosed/BP_Sosed_Spawn_Point.BP_Sosed_Spawn_Point_C"))
        (if (!= (`KismetArrayLibrary.Array_Length` _outactors_3) 0)
          (bind _outitem_2 (`KismetArrayLibrary.Array_Random` _outactors_3))
          (`self.K2_SetActorLocationAndRotation` (`|GetArrayItem` _outactors) (`self.K2_GetActorLocation` _outitem_2) (`self.K2_GetActorRotation` _outitem_2) false true))))))

(event `self.K2_PostLogin`
  (params (NewPlayer :type "PlayerController Object Reference"))
  (bind _num_players (`self.Num Players`))
  ;[1 1 1] Player State
  (`BlueprintMapLibrary.Map_Add` (`self.Unique Net Id Rep`) (`PlayerState.BP_GetUniqueId` (`Controller.PlayerState` NewPlayer)) _num_players)
  (set `self.Num Players` (+ _num_players 1)))

(event `self.K2_OnLogout`
  (params (ExitingController :type "Controller Object Reference"))
  ;[1 1 1] Player State
  (`BlueprintMapLibrary.Map_Remove` (`self.Unique Net Id Rep`) (`PlayerState.BP_GetUniqueId` (`Controller.PlayerState` ExitingController)))
  (set `self.Num Players` (- (`self.Num Players`) 1)))

(fn `Get Unique Net Id`
  (params (`New Unique Net Id Rep` :type "UniqueNetIdRepl Structure (by ref)"))
  (returns (`Player Index` :type Integer))
  (return (`BlueprintMapLibrary.Map_Find` (`self.Unique Net Id Rep`) `New Unique Net Id Rep`)))

(fn `Load Save Game`
  (bind _saved_game (`/Game/Function/BP_GameInstance.Saved Game` (`/Game/Function/BP_FunctionLibrary.Get Game Instance`)))
  (bind _player_inventory (`/Game/Function/BP_MapSave.Player Inventory` _saved_game))
  (`/Engine/EditorBlueprintResources/StandardMacros.IsValid` (`/Game/Function/BP_GameInstance.Saved Game` (`/Game/Function/BP_FunctionLibrary.Get Game Instance`))
    (:`Is Valid`
      (`|ExecutionSequence`
        (:`then_0`
          (`|ExecutionSequence`
            (:`then_0`
              ;[1 1 1] Objects
              (bind _outactors (`GameplayStatics.GetAllActorsOfClass` "/Game/Objects/Structurs/BP_Object.BP_Object_C"))
              (for _array_element _outactors
                (bind (_value _returnvalue) (`BlueprintMapLibrary.Map_Find` (`/Game/Function/BP_MapSave.Object Json` (`/Game/Function/BP_GameInstance.Saved Game` (`/Game/Function/BP_FunctionLibrary.Get Game Instance`))) (`KismetSystemLibrary.GetObjectName` _array_element)))
                (if _returnvalue
                  (`/Game/Objects/Structurs/BP_Object.Load Data` _array_element _value))))
            (:`then_1`
              ;[1 1 1] Player
              (`self.K2_SetActorLocation` (`GameplayStatics.GetPlayerCharacter` 0) (`/Game/Function/BP_MapSave.Player Location` _saved_game) false false)
              (`Controller.SetControlRotation` (`GameplayStatics.GetPlayerController` 0) (`/Game/Function/BP_MapSave.Player Control Rotation` _saved_game))
              (bind _outactors_2 (`GameplayStatics.GetAllActorsOfClass` "/Game/Objects/Structurs/BP_Object.BP_Object_C"))
              (for _array_element_2 _outactors_2
                (if (`KismetArrayLibrary.Array_IsValidIndex` _player_inventory (`KismetArrayLibrary.Array_Find` _player_inventory (`KismetSystemLibrary.GetObjectName` _array_element_2)))
                  (`/Game/Objects/Structurs/BP_Object.PickUp` _array_element_2))))
            (:`then_2`
              ;[1 1 1] Game Time
              (bind _returnvalue_2 (`GameplayStatics.GetActorOfClass` "/Game/BP_Atmosphere_And_Time_Manager.BP_Atmosphere_And_Time_Manager_C"))
              (`/Engine/EditorBlueprintResources/StandardMacros.IsValid` _returnvalue_2
                (:`Is Valid`
                  (set `/Game/BP_Atmosphere_And_Time_Manager.Current Time` (`/Game/Function/BP_MapSave.Game Time` (`/Game/Function/BP_GameInstance.Saved Game` (`/Game/Function/BP_FunctionLibrary.Get Game Instance`))) _returnvalue_2)
                  (`/Game/BP_Atmosphere_And_Time_Manager.Refresh` _returnvalue_2))))
            (:`then_3`
              ;[1 1 1] Rotate Objects
              (bind _outactors_3 (`GameplayStatics.GetAllActorsOfClass` "/Game/Objects/Structurs/BP_Rotate.BP_Rotate_C"))
              (for _array_element_3 _outactors_3
                (bind (_value_2 _returnvalue_3) (`BlueprintMapLibrary.Map_Find` (`/Game/Function/BP_MapSave.Rotate Json` (`/Game/Function/BP_GameInstance.Saved Game` (`/Game/Function/BP_FunctionLibrary.Get Game Instance`))) (`KismetSystemLibrary.GetObjectName` _array_element_3)))
                (if _returnvalue_3
                  (`/Game/Objects/Structurs/BP_Rotate.Load Data` _array_element_3 _value_2))))
            (:`then_4`
              ;[1 1 1] Simple Objects
              (bind _outactors_4 (`GameplayStatics.GetAllActorsOfClass` "/Game/Objects/Structurs/BP_SmartActor.BP_SmartActor_C"))
              (for _array_element_4 _outactors_4
                (bind (_value_3 _returnvalue_4) (`BlueprintMapLibrary.Map_Find` (`/Game/Function/BP_MapSave.Simple Json` (`/Game/Function/BP_GameInstance.Saved Game` (`/Game/Function/BP_FunctionLibrary.Get Game Instance`))) (`KismetSystemLibrary.GetObjectName` _array_element_4)))
                (if _returnvalue_4
                  (`/Game/Objects/Structurs/BP_SmartActor.Load Data` _array_element_4 _value_3))))
            (:`then_5`
              ;[1 1 1] Cutscene Manager
              (bind _outactors_5 (`GameplayStatics.GetAllActorsOfClass` "/Game/Objects/Cutscene/BP_Cutscene_Manager.BP_Cutscene_Manager_C"))
              (for _array_element_5 _outactors_5
                (bind (_value_4 _returnvalue_5) (`BlueprintMapLibrary.Map_Find` (`/Game/Function/BP_MapSave.Cutscene Manager State` (`/Game/Function/BP_GameInstance.Saved Game` (`/Game/Function/BP_FunctionLibrary.Get Game Instance`))) (`KismetSystemLibrary.GetObjectName` _array_element_5)))
                (if _returnvalue_5
                  (if (`|EnumInequality` (`/Game/Objects/Cutscene/BP_Cutscene_Manager.State` _array_element_5) _value_4)
                    (`/Game/Objects/Cutscene/BP_Cutscene_Manager.Set State` _array_element_5 _value_4)))))))
        (:`then_1`
          (bind _sosed (`/Game/Function/BP_MacroLibrary.Find Sosed`)
            (:`Is Valid`
              (`/Game/Sosed/BP_Sosed.Set State` _sosed "NewEnumerator0"))))
        (:`then_2`
          (set `/Game/Function/BP_GameInstance.Saved Game` null (`/Game/Function/BP_FunctionLibrary.Get Game Instance`)))))))

(fn `UserConstructionScript`)
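; Blueprint function library of shared game helpers: typed game mode, game instance and manager getters, platform and holiday detection, map and accessory lookups, object checks and window restoring.
; CalculateTravelTime divides navmesh path length by character max speed, and RandomSplinePoints builds a centered random-walk spline.
; SaveGame fills BP_MapSave with player, level, time and cutscene state, plus per-actor JSON keyed by object name.
; An empty slot name selects the next free numbered slot.
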(fn `Calculate Travel Time`
  (params (`Path Start` :type "Vector Structure") (`Path End` :type "Vector Structure") (`Character Ref` :type "Character Object Reference"))
  (returns (`Travel Time` :type "Float (double-precision)"))
  (locals (`Previous Point` :type "Vector Structure") (`Path Length` :type "Float (double-precision)"))
  (bind _returnvalue (`NavigationSystemV1.FindPathToLocationSynchronously` null `Path Start` `Path End` null "/Script/NavigationSystem.RecastFilter_UseDefaultArea"))
  (for (_array_element _array_index) (`NavigationPath.PathPoints` _returnvalue)
    (if (> _array_index 0)
      (set `local.Path Length` (+ (`local.Path Length`) (`KismetMathLibrary.VSize` (- (`local.Previous Point`) _array_element))))
      (set `local.Previous Point` _array_element)))
  (return (/ (`local.Path Length`) (`MovementComponent.GetMaxSpeed` (`Character.CharacterMovement` `Character Ref`)))))

(fn `Checking Class`
  (params (Class :type "Actor Class Reference") (`Class Array` :type "Array of Actor Class Reference"))
  (returns (Status :type Boolean))
  (locals (`Checking Status` :type Boolean))
  (for _array_element `Class Array`
    (set `local.Checking Status` (== _array_element Class)))
  (return (`local.Checking Status`)))

(fn `Checking Object`
  (params (Component :type "ActorComponent Object Reference") (`Mesh Component` :type "StaticMeshComponent Object Reference"))
  (returns (Bool :type Boolean))
  (return (== Component `Mesh Component`)))

(fn `Checking Objects`
  (params (Actors :type "Array of Actor Object Reference") (Component :type "ActorComponent Object Reference"))
  (returns (Actor :type "Actor Object Reference") (Bool :type Boolean))
  (for _array_element Actors
    (return _array_element (== Component _array_element))))

(fn `Find Next Free Slot`
  (returns (`Slot Name` :type String) (`Slot Index` :type Integer))
  (locals (`Save Slot Index` :type Integer))
  (bind _save_slot_index (`local.Save Slot Index`))
  (for _index (range 101)
    (set `local.Save Slot Index` _index)
    (bind _returnvalue (`GameplayStatics.DoesSaveGameExist` (`KismetStringLibrary.Concat_StrStr` "SaveSlot_" (`KismetStringLibrary.Conv_IntToString` _index))))
    (if (not _returnvalue)
      (break)))
  (return (`KismetStringLibrary.Concat_StrStr` "SaveSlot_" (`KismetStringLibrary.Conv_IntToString` _save_slot_index)) _save_slot_index))

(fn `Get Accessories`
  (params (Type :type Integer))
  (returns (Accessories :type "Array of /Game/Player/Functions/Accessories_Struct Structure"))
  (locals (`Head Accessories` :type "Array of /Game/Player/Functions/Accessories_Struct Structure") (`Face Accessories` :type "Array of /Game/Player/Functions/Accessories_Struct Structure") (`Backpack Accessories` :type "Array of /Game/Player/Functions/Accessories_Struct Structure"))
  (return (select `int` Type :`0` (`local.Head Accessories`) :`1` (`local.Face Accessories`) :`2` (`local.Backpack Accessories`))))

(fn `Get Atmosphere And Time Manager`
  (returns (Manager :type "/Game/BP_Atmosphere_And_Time_Manager Object Reference"))
  (bind _returnvalue (`GameplayStatics.GetActorOfClass` null "/Game/BP_Atmosphere_And_Time_Manager.BP_Atmosphere_And_Time_Manager_C"))
  (return _returnvalue))

(fn `Get Current Holiday`
  (returns (Holiday :type "/Game/UMG/EHoliday Enum"))
  (locals (`Not Suitable` :type Boolean))
  (bind _returnvalue (`KismetMathLibrary.Today`))
  (bind _returnvalue_2 (`KismetMathLibrary.Today`))
  (`|ExecutionSequence`
    (:`then_0`
      (if (or (and (== (`KismetMathLibrary.GetMonth` _returnvalue) 12) (>= (`KismetMathLibrary.GetDay` _returnvalue) 24)) (and (== (`KismetMathLibrary.GetMonth` _returnvalue) 1) (<= (`KismetMathLibrary.GetDay` _returnvalue) 6)))
        (return "NewEnumerator1")
        (else
          (set `local.Not Suitable` true))))
    (:`then_1`
      (if (and (== (`KismetMathLibrary.GetMonth` _returnvalue_2) 10) (== (`KismetMathLibrary.GetDay` _returnvalue_2) 31))
        (return "NewEnumerator2")
        (else
          (set `local.Not Suitable` true))))
    (:`then_2`
      (if (`local.Not Suitable`)
        (return "NewEnumerator0")))))

(fn `Get Current Platform`
  (returns (Platform :type "/Game/UMG/EPlatform Enum"))
  (switch `string` (`GameplayStatics.GetPlatformName`)
    (:`Default`
      _)
    (:`Windows`
      _)
    (:`Linux`
      _)
    (:`Mac`
      _)
    (:`PS4`
      (return "NewEnumerator1"))
    (:`XboxOne`
      (return "NewEnumerator1"))
    (:`Android`
      (return "NewEnumerator2"))
    (:`IOS`
      (return "NewEnumerator2"))
    (:`MagicLeap`
      (return "NewEnumerator3"))
    (:`AppleARKit`
      (return "NewEnumerator3"))
    (:`FGoogleARCoreXRTrackingSystem`
      (return "NewEnumerator3"))
    (:`FGoogleVRHMD`
      (return "NewEnumerator3"))
    (:`PSVR`
      (return "NewEnumerator3"))
    (:`OSVR`
      (return "NewEnumerator3"))
    (:`SimpleHMD`
      (return "NewEnumerator3"))
    (:`SteamVR`
      (return "NewEnumerator3"))
    (:`OculusHMD`
      (return "NewEnumerator3"))
    (:`WindowsMixedRealityHMD`
      (return "NewEnumerator3")))
  (return "NewEnumerator0"))

(fn `Get Game Instance`
  (returns (`Game Instance` :type "/Game/Function/BP_GameInstance Object Reference"))
  (bind _asbp_game_instance (cast `/Game/Function/BP_GameInstance` (`GameplayStatics.GetGameInstance` null))
    (:`then`
      (return _asbp_game_instance))
    (:`CastFailed`
      (return null))))

(fn `Get Game Mode`
  (returns (`Game Mode` :type "/Game/Player/BP_GameMode Object Reference"))
  (bind _asbp_game_mode (cast `/Game/Player/BP_GameMode` (`GameplayStatics.GetGameMode` null))
    (:`then`
      (return _asbp_game_mode))
    (:`CastFailed`
      (return null))))

(fn `Get Maps Info`
  (returns (`Maps Info` :type "Array of /Game/UMG/Menu/Map_Info_Struct Structure") (`Levels Without Saving` :type "Array of Name"))
  (locals (Maps :type "Array of /Game/UMG/Menu/Map_Info_Struct Structure") (Levels :type "Array of Name"))
  (return (`local.Maps`) (`local.Levels`)))

(fn `Random Spline Points`
  (params (Spline :type "SplineComponent Object Reference") (Count :type Integer) (`Half Angle` :type "Float (double-precision)") (Distance :type "Float (double-precision)"))
  (locals (`Last Point` :type "Vector Structure") (`Generated Points` :type "Array of Vector Structure"))
  (bind _generated_points (`local.Generated Points`))
  (for _ (range (+ Count 1))
    (bind _output_get (set `local.Last Point` (+ (`local.Last Point`) (* (`KismetMathLibrary.RandomUnitVectorInConeInDegrees` (`KismetMathLibrary.RandomUnitVector`) `Half Angle`) Distance))))
    (`KismetArrayLibrary.Array_Add` (`local.Generated Points`) _output_get))
  (for (_array_element _array_index) _generated_points
    (`KismetArrayLibrary.Array_Set` (`local.Generated Points`) _array_index (- _array_element (`KismetMathLibrary.GetVectorArrayAverage` _generated_points))))
  (`SplineComponent.SetSplinePoints` Spline _generated_points "Local" true))

(fn `Restoring Windows`
  (bind _outactors (`GameplayStatics.GetAllActorsOfClass` null "/Game/Objects/BP_Objects/BP_Window1.BP_Window1_C"))
  (for _array_element _outactors
    (if (`/Game/Objects/BP_Objects/BP_Window1.Can be Restored` _array_element)
      (`/Game/Objects/BP_Objects/BP_Window1.Restoring Windows` _array_element))))

(fn `Save Game`
  (params (`Slot Name` :type String))
  (returns (ReturnValue :type Boolean))
  (locals (`Save Game` :type "/Game/Function/BP_MapSave Object Reference"))
  (bind _returnvalue (`KismetStringLibrary.IsEmpty` `Slot Name`))
  (bind _returnvalue_2 (`KismetMathLibrary.Now`))
  (bind _save_game (`local.Save Game`))
  (bind _save_game_2 (`local.Save Game`))
  (if _returnvalue
    (bind _slot_name (`self.Find Next Free Slot` null)))
  (bind _returnvalue_3 (`GameplayStatics.CreateSaveGameObject` "/Game/Function/BP_MapSave.BP_MapSave_C"))
  (bind _output_get (set `local.Save Game` _returnvalue_3))
  (set `/Game/Function/BP_MapSave.Save Time` (`KismetStringLibrary.Concat_StrStr` (`KismetStringLibrary.Conv_IntToString` (`KismetMathLibrary.GetDay` _returnvalue_2)) "." (`KismetStringLibrary.Conv_IntToString` (`KismetMathLibrary.GetMonth` _returnvalue_2)) "." (`KismetStringLibrary.Conv_IntToString` (`KismetMathLibrary.GetYear` _returnvalue_2)) " " (`KismetTextLibrary.Conv_TextToString` (`KismetTextLibrary.AsTimespan_Timespan` (`KismetMathLibrary.GetTimeOfDay` _returnvalue_2)))) _output_get)
  (`|ExecutionSequence`
    (:`then_0`
      (`|ExecutionSequence`
        (:`then_0`
          ;[1 1 1] Player
          (bind _asbp_player (cast `/Game/Player/BP_Player` (`GameplayStatics.GetPlayerCharacter` null)))
          (set `/Game/Function/BP_MapSave.Player Location` (`Actor.K2_GetActorLocation` _asbp_player) _save_game)
          (set `/Game/Function/BP_MapSave.Player Control Rotation` (`Pawn.GetControlRotation` _asbp_player) _save_game)
          (bind _items (`/Game/Player/BP_Player.Get Inventory` _asbp_player))
          (for _array_element _items
            (`KismetArrayLibrary.Array_Add` (`/Game/Function/BP_MapSave.Player Inventory` _save_game) (`KismetSystemLibrary.GetObjectName` _array_element))))
        (:`then_1`
          ;[1 1 1] Map Info
          (bind _returnvalue_4 (`GameplayStatics.GetCurrentLevelName` null))
          (for (_array_element_2 _array_index) (`self.Get Maps Info` null)
            (bind ((`Levels_14_6D5FBA4C4ED3E761930751A6B557FAF0` _levels)) (break `/Game/UMG/Menu/Map_Info_Struct` _array_element_2))
            (bind _returnvalue_5 (`KismetStringLibrary.Conv_StringToName` _returnvalue_4))
            (if (`KismetArrayLibrary.Array_Contains` _levels _returnvalue_5)
              (set `/Game/Function/BP_MapSave.Level Info Index` _array_index _save_game_2)
              (set `/Game/Function/BP_MapSave.Level Custom Param Id` (`KismetArrayLibrary.Array_Find` _levels _returnvalue_5) _save_game_2))))
        (:`then_2`
          ;[1 1 1] Save Objects Data
          (bind _outactors (`GameplayStatics.GetAllActorsOfClass` null "/Game/Objects/Structurs/BP_Object.BP_Object_C"))
          (for _array_element_3 _outactors
            (bind _json (`/Game/Objects/Structurs/BP_Object.Save Data` _array_element_3))
            (`BlueprintMapLibrary.Map_Add` (`/Game/Function/BP_MapSave.Object Json` (`local.Save Game`)) (`KismetSystemLibrary.GetObjectName` _array_element_3) (`VaRestJsonObject.EncodeJson` _json))))
        (:`then_3`
          ;[1 1 1] Game Time
          (bind _returnvalue_6 (`GameplayStatics.GetActorOfClass` null "/Game/BP_Atmosphere_And_Time_Manager.BP_Atmosphere_And_Time_Manager_C"))
          (`/Engine/EditorBlueprintResources/StandardMacros.IsValid` _returnvalue_6
            (:`Is Valid`
              (set `/Game/Function/BP_MapSave.Game Time` (`/Game/BP_Atmosphere_And_Time_Manager.Current Time` _returnvalue_6) (`local.Save Game`)))))
        (:`then_4`
          ;[1 1 1] Save Rotate Objects Data
          (bind _outactors_2 (`GameplayStatics.GetAllActorsOfClass` null "/Game/Objects/Structurs/BP_Rotate.BP_Rotate_C"))
          (for _array_element_4 _outactors_2
            (bind _json_2 (`/Game/Objects/Structurs/BP_Rotate.Save Data` _array_element_4))
            (`BlueprintMapLibrary.Map_Add` (`/Game/Function/BP_MapSave.Rotate Json` (`local.Save Game`)) (`KismetSystemLibrary.GetObjectName` _array_element_4) (`VaRestJsonObject.EncodeJson` _json_2))))
        (:`then_5`
          ;[1 1 1] Save Rotate Objects Data
          (bind _outactors_3 (`GameplayStatics.GetAllActorsOfClass` null "/Game/Objects/Structurs/BP_SmartActor.BP_SmartActor_C"))
          (for _array_element_5 _outactors_3
            (bind _json_3 (`/Game/Objects/Structurs/BP_SmartActor.Save Data` _array_element_5))
            (`BlueprintMapLibrary.Map_Add` (`/Game/Function/BP_MapSave.Simple Json` (`local.Save Game`)) (`KismetSystemLibrary.GetObjectName` _array_element_5) (`VaRestJsonObject.EncodeJson` _json_3))))
        (:`then_6`
          ;[1 1 1] Cutscene Manager
          (bind _outactors_4 (`GameplayStatics.GetAllActorsOfClass` null "/Game/Objects/Cutscene/BP_Cutscene_Manager.BP_Cutscene_Manager_C"))
          (for _array_element_6 _outactors_4
            (`BlueprintMapLibrary.Map_Add` (`/Game/Function/BP_MapSave.Cutscene Manager State` (`local.Save Game`)) (`KismetSystemLibrary.GetObjectName` _array_element_6) (`/Game/Objects/Cutscene/BP_Cutscene_Manager.State` _array_element_6))))))
    (:`then_1`
      (bind _returnvalue_7 (`GameplayStatics.SaveGameToSlot` (`local.Save Game`) (select `bool` _returnvalue :`false` `Slot Name` :`true` _slot_name)))
      (return _returnvalue_7))))
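; Blueprint function library of null-safe helpers for reading and writing typed fields on JSON objects.
; Getters return a HasField flag with the value, falling back to defaults when the object is invalid.
; Vectors and rotators are stored as three number fields suffixed X, Y and Z, and bytes as integers.
; The vector getter can optionally raise Z by a fixed offset, while setters skip the validity check.
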(fn `Get Value As Bool`
  (params (JSON :type "VaRestJsonObject Object Reference") (`Field Name` :type String))
  (returns (`Has Field ` :type Boolean) (`Return Value` :type Boolean))
  (`/Engine/EditorBlueprintResources/StandardMacros.IsValid` JSON
    (:`Is Valid`
      (return (`VaRestJsonObject.HasField` JSON `Field Name`) (`VaRestJsonObject.GetBoolField` JSON `Field Name`)))
    (:`Is Not Valid`
      (return false false))))

(fn `Get Value As Byte`
  (params (JSON :type "VaRestJsonObject Object Reference") (`Field Name` :type String))
  (returns (`Has Field ` :type Boolean) (`Return Value` :type Byte))
  (bind (_has_field_ _return_value) (`self.Get Value As Int` JSON `Field Name`))
  (`/Engine/EditorBlueprintResources/StandardMacros.IsValid` JSON
    (:`Is Valid`
      (return _has_field_ (`KismetMathLibrary.Conv_IntToByte` _return_value)))
    (:`Is Not Valid`
      (return false 0))))

(fn `Get Value As Float`
  (params (JSON :type "VaRestJsonObject Object Reference") (`Field Name` :type String))
  (returns (`Has Field ` :type Boolean) (`Return Value` :type "Float (double-precision)"))
  (`/Engine/EditorBlueprintResources/StandardMacros.IsValid` JSON
    (:`Is Valid`
      (return (`VaRestJsonObject.HasField` JSON `Field Name`) (`VaRestJsonObject.GetNumberField` JSON `Field Name`)))
    (:`Is Not Valid`
      (return false 0.0))))

(fn `Get Value As Int`
  (params (JSON :type "VaRestJsonObject Object Reference") (`Field Name` :type String))
  (returns (`Has Field ` :type Boolean) (`Return Value` :type Integer))
  (`/Engine/EditorBlueprintResources/StandardMacros.IsValid` JSON
    (:`Is Valid`
      (return (`VaRestJsonObject.HasField` JSON `Field Name`) (`VaRestJsonObject.GetIntegerField` JSON `Field Name`)))
    (:`Is Not Valid`
      (return false 0))))

(fn `Get Value As Rotator`
  (params (JSON :type "VaRestJsonObject Object Reference") (`Field Name` :type String))
  (returns (`Has Field ` :type Boolean) (`Return Value` :type "Rotator Structure"))
  (bind (_has_field_ _return_value) (`self.Get Value As Float` JSON (`KismetStringLibrary.Concat_StrStr` `Field Name` " Z")))
  (bind (_has_field__2 _return_value_2) (`self.Get Value As Float` JSON (`KismetStringLibrary.Concat_StrStr` `Field Name` " X")))
  (bind (_has_field__3 _return_value_3) (`self.Get Value As Float` JSON (`KismetStringLibrary.Concat_StrStr` `Field Name` " Y")))
  (`/Engine/EditorBlueprintResources/StandardMacros.IsValid` JSON
    (:`Is Valid`
      (if (and _has_field__2 _has_field__3 _has_field_)
        (return true (`KismetMathLibrary.MakeRotator` _return_value_2 _return_value_3 _return_value))
        (else
          _)))
    (:`Is Not Valid`
      _))
  (return false))

(fn `Get Value As String`
  (params (JSON :type "VaRestJsonObject Object Reference") (`Field Name` :type String))
  (returns (`Has Field ` :type Boolean) (`Return Value` :type String))
  (`/Engine/EditorBlueprintResources/StandardMacros.IsValid` JSON
    (:`Is Valid`
      (return (`VaRestJsonObject.HasField` JSON `Field Name`) (`VaRestJsonObject.GetStringField` JSON `Field Name`)))
    (:`Is Not Valid`
      (return false ""))))

(fn `Get Value As Vector`
  (params (JSON :type "VaRestJsonObject Object Reference") (`Field Name` :type String) (`Z Offset` :type Boolean))
  (returns (`Has Field ` :type Boolean) (`Return Value` :type "Vector Structure"))
  (bind (_has_field_ _return_value) (`self.Get Value As Float` JSON (`KismetStringLibrary.Concat_StrStr` `Field Name` " Z")))
  (bind (_has_field__2 _return_value_2) (`self.Get Value As Float` JSON (`KismetStringLibrary.Concat_StrStr` `Field Name` " X")))
  (bind (_has_field__3 _return_value_3) (`self.Get Value As Float` JSON (`KismetStringLibrary.Concat_StrStr` `Field Name` " Y")))
  (`/Engine/EditorBlueprintResources/StandardMacros.IsValid` JSON
    (:`Is Valid`
      (if (and _has_field__2 _has_field__3 _has_field_)
        (return true (`KismetMathLibrary.MakeVector` _return_value_2 _return_value_3 (select `bool` `Z Offset` :`false` _return_value :`true` (+ _return_value 20.0))))
        (else
          _)))
    (:`Is Not Valid`
      _))
  (return false (0.0 0.0 0.0)))

(fn `Set Byte Field`
  (params (JSON :type "VaRestJsonObject Object Reference") (`Field Name` :type String) (Byte :type Byte))
  (`VaRestJsonObject.SetIntegerField` JSON `Field Name` (`KismetMathLibrary.Conv_ByteToInt` Byte)))

(fn `Set Rotator Field`
  (params (JSON :type "VaRestJsonObject Object Reference") (`Field Name` :type String) (Vector :type "Rotator Structure"))
  (`VaRestJsonObject.SetNumberField` JSON (`KismetStringLibrary.Concat_StrStr` `Field Name` " X") (.roll Vector))
  (`VaRestJsonObject.SetNumberField` JSON (`KismetStringLibrary.Concat_StrStr` `Field Name` " Y") (.pitch Vector))
  (`VaRestJsonObject.SetNumberField` JSON (`KismetStringLibrary.Concat_StrStr` `Field Name` " Z") (.yaw Vector)))

(fn `Set Vector Field`
  (params (JSON :type "VaRestJsonObject Object Reference") (`Field Name` :type String) (Vector :type "Vector Structure"))
  (`VaRestJsonObject.SetNumberField` JSON (`KismetStringLibrary.Concat_StrStr` `Field Name` " X") (.x Vector))
  (`VaRestJsonObject.SetNumberField` JSON (`KismetStringLibrary.Concat_StrStr` `Field Name` " Y") (.y Vector))
  (`VaRestJsonObject.SetNumberField` JSON (`KismetStringLibrary.Concat_StrStr` `Field Name` " Z") (.z Vector)))